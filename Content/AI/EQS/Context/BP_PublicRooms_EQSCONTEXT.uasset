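; EQS context that supplies the public rooms an NPC is not already inside, for use in AI environment queries.
; It gathers every RoomVolume actor in the world and keeps those flagged as Public.
; It then removes any room volumes overlapping the querier actor and returns the remaining set.
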(fn ProvideActorsSet
  (params (QuerierObject :type Object%20Object%20Reference) (QuerierActor :type Actor%20Object%20Reference))
  (bind _outactors (Actor|GetAllActorsOfClass "/Script/DoubleAgent.RoomVolume"))
  ;[1 1 1] Get all public rooms
  (for _array_element _outactors
    (if (Variables|/Script/DoubleAgent.RoomVolume|GetbPublic _array_element)
      (Utilities|Array|Add (Variables|Default|GetTempArray) _array_element)))
  ;[1 1 1] Remove rooms that NPC is already inside
  (for _array_element_2 (Collision|GetOverlappingActors QuerierActor "/Script/DoubleAgent.RoomVolume" :!class /Script/Engine.Actor)
    (Utilities|Array|RemoveItem (Variables|Default|GetTempArray) _array_element_2))
  (return (Variables|Default|GetTempArray)))