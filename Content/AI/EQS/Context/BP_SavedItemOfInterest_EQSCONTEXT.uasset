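; An EQS context that supplies saved item-of-interest locations to AI environment queries.
; It overrides ProvideLocationsSet to read two vector keys, the primary and secondary saved items of interest, from the querier's blackboard.
; Both vectors are returned as the location set, with no check on whether either key is set.
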(fn ProvideLocationsSet
  (params (QuerierObject :type Object%20Object%20Reference) (QuerierActor :type Actor%20Object%20Reference))
  (bind _returnvalue (AI|GetBlackboard QuerierActor))
  (Utilities|Array|Add (LocalVariables|GetArray) (AI|Components|Blackboard|GetValueasVector _returnvalue (Utilities|Name|MakeLiteralName "SavedItemOfInterest")))
  (Utilities|Array|Add (LocalVariables|GetArray) (AI|Components|Blackboard|GetValueasVector _returnvalue (Utilities|Name|MakeLiteralName "2ndSavedItemOfInterest")))
  (return (LocalVariables|GetArray)))