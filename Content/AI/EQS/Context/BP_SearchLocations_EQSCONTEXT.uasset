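; EQS context that supplies BP_SearchLocation actors to AI environment queries.
; It loops over all search locations in the world, accepting those not visible to camera, or visible ones when the querier's CamerasActive blackboard key is true.
; The return sits inside the loop, so it outputs upon the first accepted location rather than collecting every match.
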(fn ProvideActorsSet
  (params (QuerierObject :type Object%20Object%20Reference) (QuerierActor :type Actor%20Object%20Reference))
  (bind _outactors (Actor|GetAllActorsOfClass "/Game/AI/SearchSystem/BP_SearchLocation.BP_SearchLocation_C"))
  (for _array_element _outactors
    (if (or (not (Variables|/Game/AI/SearchSystem/BP_SearchLocation.BP_SearchLocation_C|GetbVisibleToCamera _array_element)) (and (Variables|/Game/AI/SearchSystem/BP_SearchLocation.BP_SearchLocation_C|GetbVisibleToCamera _array_element) (ScalableFloat|GetValueasBool (AI|GetBlackboard QuerierActor) (Utilities|Name|MakeLiteralName "CamerasActive"))))
      (Utilities|Array|Add (Variables|Default|GetActors) _array_element)
      (return (Variables|Default|GetActors)))))