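; EQS context that supplies nearby stationary AI characters as a crowd reference for environment queries.
; It sphere-overlaps Pawns of the AI character base class within a fixed radius of the querier, keeping those with near-zero velocity.
; The ignore list casts the querier actor to AIController to get its pawn, so it excludes the querier only if that actor is a controller.
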(fn ProvideActorsSet
  (params (QuerierObject :type Object%20Object%20Reference) (QuerierActor :type Actor%20Object%20Reference))
  (bind _outactors (Collision|SphereOverlapActors (Transformation|GetActorLocation QuerierActor) 1.5e+03 (Utilities|Array|MakeArray "ObjectTypeQuery3") "/Game/AI/NPC/BP_AICharacterBase_CHARACTER.BP_AICharacterBase_CHARACTER_C" (Utilities|Array|MakeArray (Pawn|GetControlledPawn (.AsAIController (Utilities|Casting|CastToAIController QuerierActor))))))
  (for _array_element _outactors
    (if (< (Math|Vector|VectorLength (Transformation|GetVelocity _array_element)) 1.0)
      (Utilities|Array|Add (Variables|Default|GetOut%20Actors) _array_element)))
  (return (Variables|Default|GetOut%20Actors)))