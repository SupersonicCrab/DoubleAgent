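; EQS context that supplies the search locations the querying AI has not yet searched.
; It gathers every BP_SearchLocation in the world and drops those already in the AI controller's SearchedLocations list.
; When the querier's CamerasActive blackboard flag is set, it also excludes locations marked VisibleToCamera.
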(fn ProvideActorsSet
  (params (QuerierObject :type Object%20Object%20Reference) (QuerierActor :type Actor%20Object%20Reference))
  (LocalVariables|SetCamerasActive (ScalableFloat|GetValueasBool (AI|GetBlackboard QuerierActor) (Utilities|Name|MakeLiteralName "CamerasActive")))
  (Utilities|Array|Clear (Variables|Default|GetActors))
  (bind _outactors (Actor|GetAllActorsOfClass "/Game/AI/SearchSystem/BP_SearchLocation.BP_SearchLocation_C"))
  (for _array_element _outactors
    (if (== (Utilities|Array|FindItem (Variables|/Game/AI/NPC/BP_AIControllerBase_AICONTROLLER.BP_AIControllerBase_AICONTROLLER_C|GetsearchedLocations (.AsBP%20AIController%20Base%20AICONTROLLER (Utilities|Casting|CastToBP_AIControllerBase_AICONTROLLER (AI|GetAIController QuerierActor)))) (.AsSearch%20Location (Utilities|Casting|CastToSearchLocation _array_element))) -1)
      (if (not (and (Variables|/Game/AI/SearchSystem/BP_SearchLocation.BP_SearchLocation_C|GetbVisibleToCamera (.AsBP%20Search%20Location (Utilities|Casting|CastToBP_SearchLocation _array_element))) (LocalVariables|GetCamerasActive)))
        (Utilities|Array|Add (Variables|Default|GetActors) (.AsBP%20Search%20Location (Utilities|Casting|CastToBP_SearchLocation _array_element))))))
  (return (Variables|Default|GetActors)))