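; EQS context that provides every enabled BP_Landline actor in the level as a set for AI environment queries.
; It gathers all landlines and keeps only those with LandlineEnabled set.
; When none are enabled, it also sets the querier's BackupAvailable blackboard key to false, so the query has a side effect on AI state.
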(fn ProvideActorsSet
  (params (QuerierObject :type Object%20Object%20Reference) (QuerierActor :type Actor%20Object%20Reference))
  (bind _temparray (LocalVariables|GetTempArray))
  (Utilities|Array|Clear (LocalVariables|GetTempArray))
  ;[1 1 1] Get all landlines
  (bind _outactors (Actor|GetAllActorsOfClass "/Game/SecuritySystem/Landlines/BP_Landline.BP_Landline_C"))
  (for _array_element _outactors
    ;[1 1 1] Add all enabled landlines to array
    (if (Variables|/Game/SecuritySystem/Landlines/BP_Landline.BP_Landline_C|GetbLandlineEnabled _array_element)
      (Utilities|Array|Add (LocalVariables|GetTempArray) _array_element)))
  (if (!= (Utilities|Array|Length _temparray) 0)
    _
    (else
      ;[1 1 1] Update BackupAvailable if no landlines are enabled
      (AI|Components|Blackboard|SetValueasBool (AI|GetBlackboard QuerierActor) (Utilities|Name|MakeLiteralName "BackupAvailable") false)))
  (return _temparray))