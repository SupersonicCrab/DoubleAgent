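; EQS context that supplies the civilians in the querier's designated room who have no visible wine.
; It reads the DesignatedRoom RoomVolume from the querier's blackboard and gathers the BP_Civilian_CHARACTER actors overlapping it.
; Civilians whose Wine component is hidden form the returned actor set, which is empty if the blackboard value is not a RoomVolume.
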(fn ProvideActorsSet
  (params (QuerierObject :type Object%20Object%20Reference) (QuerierActor :type Actor%20Object%20Reference))
  (bind _asroom_volume (Utilities|Casting|CastToRoomVolume (AI|Components|Blackboard|GetValueasObject (AI|GetBlackboard QuerierActor) (Utilities|Name|MakeLiteralName "DesignatedRoom")))
    (:then
      (for _array_element (Collision|GetOverlappingActors _asroom_volume "/Game/AI/NPC/Civilian/BP_Civilian_CHARACTER.BP_Civilian_CHARACTER_C" :!class /Script/Engine.Actor)
        (if (not (Rendering|IsVisible (Variables|/Game/AI/NPC/Civilian/BP_Civilian_CHARACTER.BP_Civilian_CHARACTER_C|GetWine (.AsBP%20Civilian%20CHARACTER (Utilities|Casting|CastToBP_Civilian_CHARACTER _array_element)))))
          (Utilities|Array|Add (Variables|Default|GetTempArray) (.AsBP%20Civilian%20CHARACTER (Utilities|Casting|CastToBP_Civilian_CHARACTER _array_element)))))
      (return (Variables|Default|GetTempArray)))
    (:CastFailed
      (return 0))))