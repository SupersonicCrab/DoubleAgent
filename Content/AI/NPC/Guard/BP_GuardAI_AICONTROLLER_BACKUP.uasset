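; Guard AI controller (named as a backup) that extends parent sight handling to coordinate guards who see each other.
; Sight ticks compare both guards' blackboards, dropping this guard's duplicate tasks, or marking search locations the other is taking, using path cost when both share one.
; Sight updates maintain the observed-civilian count, record seen search locations and copy another guard's latest searched location.
; Sighted actors are routed by class display name.
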(fn ConstructionScript)

(fn GuardVisionTick
  (params (AsGuard :type Actor%20Object%20Reference))
  (bind _returnvalue (Utilities|Name|MakeLiteralName "TempObject"))
  (bind _lightswitch (LocalVariables|GetlightSwitch))
  (bind _actionstatus (LocalVariables|GetactionStatus))
  (bind _unconsciousnpc (LocalVariables|GetunconsciousNPC))
  (bind _noiselocation (LocalVariables|GetnoiseLocation))
  ;[1 1 1] Setting values for easy retrival
  (bind _output_get (LocalVariables|SetOtherGuard AsGuard))
  (LocalVariables|SetotherGuardBlackboard (AI|GetBlackboard _output_get))
  (LocalVariables|SetselfBlackboard (AI|GetBlackboard 0))
  ;[1 1 1] ActionStatus handling
  (if (and (!= (LocalVariables|Getidle) (Class|BlackboardComponent|GetValueasEnum (LocalVariables|GetselfBlackboard) _actionstatus)) (== (Class|BlackboardComponent|GetValueasEnum (LocalVariables|GetselfBlackboard) _actionstatus) (Class|BlackboardComponent|GetValueasEnum (LocalVariables|GetotherGuardBlackboard) _actionstatus))) ; if performing action and if performing same action
    (switch string (Utilities|String|EnumtoString (Utilities|Enum|ByteToEnumBP_EActionStatus (Class|BlackboardComponent|GetValueasEnum (LocalVariables|GetselfBlackboard) _actionstatus)))
      (:Default
        ;[1 1 1] Default response
        (AI|Components|Blackboard|SetValueasEnum (LocalVariables|GetselfBlackboard) (LocalVariables|GetactionStatus) (LocalVariables|Getidle)))
      (:LightSwitch
        ;[1 1 1] If going to the same lightswitch
        (if (== (AI|Components|Blackboard|GetValueasObject (LocalVariables|GetselfBlackboard) _lightswitch) (AI|Components|Blackboard|GetValueasObject (LocalVariables|GetotherGuardBlackboard) _lightswitch))
          (AI|Components|Blackboard|ClearValue (LocalVariables|GetselfBlackboard) (LocalVariables|GetlightSwitch))
          (AI|Components|Blackboard|SetValueasEnum (LocalVariables|GetselfBlackboard) (LocalVariables|GetactionStatus) (LocalVariables|Getidle))))
      (:Revive
        ;[1 1 1] If reviving the same NPC
        (if (== (AI|Components|Blackboard|GetValueasObject (LocalVariables|GetselfBlackboard) _unconsciousnpc) (AI|Components|Blackboard|GetValueasObject (LocalVariables|GetotherGuardBlackboard) _unconsciousnpc))
          (AI|Components|Blackboard|ClearValue (LocalVariables|GetselfBlackboard) (LocalVariables|GetunconsciousNPC))
          (AI|Components|Blackboard|SetValueasEnum (LocalVariables|GetselfBlackboard) (LocalVariables|GetunconsciousNPC) (LocalVariables|Getidle))))
      (:CameraStation
        ;[1 1 1] If both going to camera hub
        (AI|Components|Blackboard|SetValueasBool (LocalVariables|GetselfBlackboard) (LocalVariables|GetcamerasActive) true)
        (AI|Components|Blackboard|SetValueasEnum (LocalVariables|GetselfBlackboard) (LocalVariables|GetactionStatus) (LocalVariables|Getidle)))
      (:NoiseInvestigation
        ;[1 1 1] If going to the same noise location
        (if (Math|Vector|Equal(Vector) (AI|Components|Blackboard|GetValueasVector (LocalVariables|GetselfBlackboard) _noiselocation) (AI|Components|Blackboard|GetValueasVector (LocalVariables|GetotherGuardBlackboard) _noiselocation) 1.0)
          (AI|Components|Blackboard|ClearValue (LocalVariables|GetselfBlackboard) (LocalVariables|GetnoiseLocation))
          (AI|Components|Blackboard|SetValueasEnum (LocalVariables|GetselfBlackboard) (LocalVariables|GetactionStatus) (LocalVariables|Getidle))))
      (:Searching
        ;[1 1 1] If both guards going to the same search location
        (bind _asbp_search_location (Utilities|Casting|CastToBP_SearchLocation (AI|Components|Blackboard|GetValueasObject (LocalVariables|GetotherGuardBlackboard) _returnvalue) :!label _label))
        (if (== (Utilities|Array|FindItem (Variables|Default|GetSearchedLocations) _asbp_search_location) -1) ; If other guard is going to search location that is unsearched
          (if (== _asbp_search_location (.AsBP%20Search%20Location (Utilities|Casting|CastToBP_SearchLocation (AI|Components|Blackboard|GetValueasObject (LocalVariables|GetselfBlackboard) _returnvalue)))) ; If both going to the same location
            (if (< (.PathCost (Class|NavigationSystemV1|GetPathCost (Transformation|GetActorLocation (LocalVariables|GetOtherGuard)) (Transformation|GetActorLocation _asbp_search_location) 0 0)) (.PathCost (Class|NavigationSystemV1|GetPathCost (Transformation|GetActorLocation (Pawn|GetControlledPawn)) (Transformation|GetActorLocation _asbp_search_location) 0 0))) ; If other guard is closer to search location
              (CallFunction|AddSearchLocation _asbp_search_location :!label _label_2))
            (else
              (goto _label_2)))))
      (:Backup
        (AI|Components|Blackboard|SetValueasEnum (LocalVariables|GetselfBlackboard) (LocalVariables|GetactionStatus) (LocalVariables|Getidle)))
      (:Investigation
        (goto _label)))))

(fn HandleSightTick
  (params (OtherActor :type Actor%20Object%20Reference) (Sensed :type Boolean) (Camera :type BP%20Camera%20Object%20Reference))
  (|CallParentFunction OtherActor Sensed Camera)
  (switch string (Utilities|String|LeftChop (Utilities|GetClassDisplayName (Utilities|GetClass OtherActor)) 2)
    (:BP_Guard_CHARACTER
      (CallFunction|GuardVisionTick OtherActor))))

(fn HandleSightUpdate
  (params (OtherActor :type Actor%20Object%20Reference) (Sensed :type Boolean))
  (|CallParentFunction OtherActor Sensed)
  (switch string (Utilities|String|LeftChop (Utilities|GetClassDisplayName (Utilities|GetClass OtherActor)) 2)
    (:BP_Civilian_CHARACTER
      (CallFunction|CivilianVisionUpdate Sensed))
    (:BP_SearchLocation
      (CallFunction|SearchLocationUpdate OtherActor))
    (:BP_Guard_CHARACTER
      (CallFunction|GuardVisionUpdate OtherActor))))

(fn CivilianVisionUpdate
  (params (CanSee :type Boolean))
  (bind _returnvalue (AI|GetBlackboard 0))
  (bind _returnvalue_2 (Utilities|Name|MakeLiteralName "ObservedCivilians"))
  (bind _returnvalue_3 (Class|BlackboardComponent|GetValueasInt _returnvalue _returnvalue_2))
  (if CanSee
    (LocalVariables|Setresult (+ _returnvalue_3 1))
    (else
      (LocalVariables|Setresult (- _returnvalue_3 1))))
  (Class|BlackboardComponent|SetValueasInt _returnvalue _returnvalue_2 (LocalVariables|Getresult)))

(fn SearchLocationUpdate
  (params (AsSearchLocation :type Actor%20Object%20Reference))
  (bind _assearch_location (Utilities|Casting|CastToSearchLocation AsSearchLocation))
  (bind _searchedlocations (Variables|Default|GetSearchedLocations))
  (if (== (Utilities|Array|FindItem _searchedlocations _assearch_location) -1) ; If search location is not already marked as searched
    (Utilities|Array|Add _searchedlocations _assearch_location)))

(fn GuardVisionUpdate
  (params (AsGuard :type Actor%20Object%20Reference))
  (bind _asbp_guard_character (Utilities|Casting|CastToBP_Guard_CHARACTER AsGuard))
  (bind _asbp_guard_ai_aicontroller (Utilities|Casting|CastToBP_GuardAI_AICONTROLLER_BACKUP (AI|GetAIController _asbp_guard_character)))
  (if (!= (Utilities|Array|Length (Variables|/Game/AI/NPC/BP_AIControllerBase_AICONTROLLER.BP_AIControllerBase_AICONTROLLER_C|GetSearchedLocations _asbp_guard_ai_aicontroller)) 0)
    (if (== (Utilities|Array|FindItem (Variables|Default|GetSearchedLocations) (Utilities|Array|Get(acopy) (Variables|/Game/AI/NPC/BP_AIControllerBase_AICONTROLLER.BP_AIControllerBase_AICONTROLLER_C|GetSearchedLocations _asbp_guard_ai_aicontroller) (Utilities|Array|LastIndex (Variables|/Game/AI/NPC/BP_AIControllerBase_AICONTROLLER.BP_AIControllerBase_AICONTROLLER_C|GetSearchedLocations _asbp_guard_ai_aicontroller)))) -1) ; If other guard has a search location that guard does not have
      (CallFunction|AddSearchLocation (Utilities|Array|Get(acopy) (Variables|/Game/AI/NPC/BP_AIControllerBase_AICONTROLLER.BP_AIControllerBase_AICONTROLLER_C|GetSearchedLocations _asbp_guard_ai_aicontroller) (Utilities|Array|LastIndex (Variables|/Game/AI/NPC/BP_AIControllerBase_AICONTROLLER.BP_AIControllerBase_AICONTROLLER_C|GetSearchedLocations _asbp_guard_ai_aicontroller)))))))