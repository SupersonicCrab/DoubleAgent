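; Guard NPC character Blueprint that extends a parent character with patrol route, ammo and flashlight behavior.
; On BeginPlay the server writes the designated route and a starting ammo count to the AI blackboard and takes ownership of the moving light child actor.
; A flashlight network event override toggles the hand and holster flashlight meshes and sets the SelfLit flag to match.
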(event EventNetSetFlashlightOut
  (params (FlashlightOut :type Boolean))
  (|CallParentFunction FlashlightOut)
  (Rendering|SetVisibility (Variables|Default|GetFlashlightHand) FlashlightOut true)
  (bind _output_get (Variables|Default|SetbSelfLit FlashlightOut))
  (Rendering|SetVisibility (Variables|Default|GetFlashlightHolster) (not _output_get) false))

(event EventBeginPlay
  (bind _returnvalue (AI|GetBlackboard 0))
  ;[1 1 1] Setup
  (|CallParentFunction)
  (if (Networking|IsServer)
    (AI|Components|Blackboard|SetValueasObject _returnvalue (Utilities|Name|MakeLiteralName "DesignatedRoute") (Variables|Default|GetDesignatedRoute))
    (Class|BlackboardComponent|SetValueasInt _returnvalue (Utilities|Name|MakeLiteralName "Ammo") 5)
    (Actor|SetOwner (Variables|/Script/Engine.ChildActorComponent|GetChildActor (Variables|Default|GetMovingLight)) self)))

(fn ConstructionScript)