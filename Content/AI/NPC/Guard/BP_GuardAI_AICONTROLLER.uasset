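; Guard NPC AI controller that extends parent sight handling to coordinate guards and track what they observe.
; Sight handlers branch on class name, counting visible civilians on the blackboard and recording seen search locations as searched.
; On seeing another guard, it compares both blackboards and drops duplicate actions such as light switch, revive or noise investigation.
; Search conflicts favor the shorter path cost, and other guards' targets and their rooms' locations get marked searched.
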(fn ConstructionScript)

(fn GuardVisionTick
  (params (AsGuard :type Actor%20Object%20Reference))
  (bind _returnvalue (Utilities|Name|MakeLiteralName "TempObject"))
  (bind _lightswitch (LocalVariables|GetlightSwitch))
  (bind _actionstatus (LocalVariables|GetactionStatus))
  (bind _unconsciousnpc (LocalVariables|GetunconsciousNPC))
  (bind _noiselocation (LocalVariables|GetnoiseLocation))
  (bind _searchedlocations (Variables|Default|GetsearchedLocations))
  (bind _searchedlocations_2 (Variables|Default|GetsearchedLocations))
  ;[1 1 1] Setting values for easy retrival
  (bind _output_get (LocalVariables|SetOtherGuard AsGuard))
  (LocalVariables|SetotherGuardBlackboard (AI|GetBlackboard _output_get))
  (LocalVariables|SetselfBlackboard (AI|GetBlackboard 0))
  ;[1 1 1] ActionStatus handling
  (if (and (!= (LocalVariables|Getidle) (Class|BlackboardComponent|GetValueasEnum (LocalVariables|GetselfBlackboard) _actionstatus)) (== (Class|BlackboardComponent|GetValueasEnum (LocalVariables|GetselfBlackboard) _actionstatus) (Class|BlackboardComponent|GetValueasEnum (LocalVariables|GetotherGuardBlackboard) _actionstatus))) ; if performing action and if performing same action
    (switch string (Utilities|String|EnumtoString (Utilities|Enum|ByteToEnumEActionStatus (Class|BlackboardComponent|GetValueasEnum (LocalVariables|GetselfBlackboard) _actionstatus)))
      (:Default
        ;[1 1 1] Default response
        (AI|Components|Blackboard|SetValueasEnum (LocalVariables|GetselfBlackboard) (LocalVariables|GetactionStatus) (LocalVariables|Getidle)))
      (:LightSwitch
        ;[1 1 1] If going to the same lightswitch
        (if (== (AI|Components|Blackboard|GetValueasObject (LocalVariables|GetselfBlackboard) _lightswitch) (AI|Components|Blackboard|GetValueasObject (LocalVariables|GetotherGuardBlackboard) _lightswitch))
          (AI|Components|Blackboard|ClearValue (LocalVariables|GetselfBlackboard) (LocalVariables|GetlightSwitch))
          (AI|Components|Blackboard|SetValueasEnum (LocalVariables|GetselfBlackboard) (LocalVariables|GetactionStatus) (LocalVariables|Getidle))))
      (:Revive
        ;[1 1 1] If reviving the same NPC
        (if (== (AI|Components|Blackboard|GetValueasObject (LocalVariables|GetselfBlackboard) _unconsciousnpc) (AI|Components|Blackboard|GetValueasObject (LocalVariables|GetotherGuardBlackboard) _unconsciousnpc))
          (AI|Components|Blackboard|ClearValue (LocalVariables|GetselfBlackboard) (LocalVariables|GetunconsciousNPC))
          (AI|Components|Blackboard|SetValueasEnum (LocalVariables|GetselfBlackboard) (LocalVariables|GetunconsciousNPC) (LocalVariables|Getidle))))
      (:CameraStation
        ;[1 1 1] If both going to camera hub
        (AI|Components|Blackboard|SetValueasBool (LocalVariables|GetselfBlackboard) (LocalVariables|GetcamerasActive) true)
        (AI|Components|Blackboard|SetValueasEnum (LocalVariables|GetselfBlackboard) (LocalVariables|GetactionStatus) (LocalVariables|Getidle)))
      (:NoiseInvestigation
        ;[1 1 1] If going to the same noise location
        (if (Math|Vector|Equal(Vector) (AI|Components|Blackboard|GetValueasVector (LocalVariables|GetselfBlackboard) _noiselocation) (AI|Components|Blackboard|GetValueasVector (LocalVariables|GetotherGuardBlackboard) _noiselocation) 1.0)
          (AI|Components|Blackboard|ClearValue (LocalVariables|GetselfBlackboard) (LocalVariables|GetnoiseLocation))
          (AI|Components|Blackboard|SetValueasEnum (LocalVariables|GetselfBlackboard) (LocalVariables|GetactionStatus) (LocalVariables|Getidle))))
      (:Searching
        ;[1 1 1] If both guards going to the same search location
        (if (== (Utilities|Array|FindItem _searchedlocations_2 (.AsSearch%20Location%20BP%20CPP (Utilities|Casting|CastToSearchLocation_BP_CPP (AI|Components|Blackboard|GetValueasObject (LocalVariables|GetotherGuardBlackboard) _returnvalue)))) -1) ; If other guard is going to search location that is unsearched
          (if (== (.AsBP%20Search%20Location (Utilities|Casting|CastToBP_SearchLocation (AI|Components|Blackboard|GetValueasObject (LocalVariables|GetotherGuardBlackboard) _returnvalue))) (.AsBP%20Search%20Location (Utilities|Casting|CastToBP_SearchLocation (AI|Components|Blackboard|GetValueasObject (LocalVariables|GetselfBlackboard) _returnvalue)))) ; If both going to the same location
            (if (< (.PathCost (Class|NavigationSystemV1|GetPathCost (Transformation|GetActorLocation (LocalVariables|GetOtherGuard)) (Transformation|GetActorLocation (.AsBP%20Search%20Location (Utilities|Casting|CastToBP_SearchLocation (AI|Components|Blackboard|GetValueasObject (LocalVariables|GetotherGuardBlackboard) _returnvalue)))) 0 0)) (.PathCost (Class|NavigationSystemV1|GetPathCost (Transformation|GetActorLocation (Pawn|GetControlledPawn)) (Transformation|GetActorLocation (.AsBP%20Search%20Location (Utilities|Casting|CastToBP_SearchLocation (AI|Components|Blackboard|GetValueasObject (LocalVariables|GetotherGuardBlackboard) _returnvalue)))) 0 0))) ; If other guard is closer to search location
              (Utilities|Array|Add _searchedlocations_2 (.AsSearch%20Location%20BP%20CPP (Utilities|Casting|CastToSearchLocation_BP_CPP (AI|Components|Blackboard|GetValueasObject (LocalVariables|GetotherGuardBlackboard) _returnvalue))) :!label _label)
              (if (!= (Utilities|Array|Length (Variables|/Game/AI/SearchSystem/BP_SearchLocation.BP_SearchLocation_C|GetRoom (.AsBP%20Search%20Location (Utilities|Casting|CastToBP_SearchLocation (AI|Components|Blackboard|GetValueasObject (LocalVariables|GetotherGuardBlackboard) _returnvalue))))) 0) ; If searchlocation has a room(s)
                (for _array_element (Variables|/Game/AI/SearchSystem/BP_SearchLocation.BP_SearchLocation_C|GetRoom (.AsBP%20Search%20Location (Utilities|Casting|CastToBP_SearchLocation (AI|Components|Blackboard|GetValueasObject (LocalVariables|GetotherGuardBlackboard) _returnvalue))))
                  (for _array_element_2 (Variables|/Script/ProjectSpy.RoomVolume_BP_CPP|GetsearchLocations _array_element)
                    (if (== (Utilities|Array|FindItem _searchedlocations _array_element_2) -1) ; If search location is not already marked as searched
                      (Utilities|Array|Add _searchedlocations _array_element_2)))))
              (AI|Components|Blackboard|ClearValue (LocalVariables|GetselfBlackboard) (LocalVariables|GetactionStatus)))
            (else
              (goto _label))))))))

(fn HandleSightTick
  (params (OtherActor :type Actor%20Object%20Reference) (Sensed :type Boolean) (Camera :type Camera%20BP%20Object%20Reference))
  (|CallParentFunction OtherActor Sensed Camera)
  (switch string (Utilities|String|LeftChop (Utilities|GetClassDisplayName (Utilities|GetClass OtherActor)) 2)
    (:Guard_CHARACTER
      (CallFunction|GuardVisionTick OtherActor))))

(fn HandleSightUpdate
  (params (OtherActor :type Actor%20Object%20Reference) (Sensed :type Boolean))
  (|CallParentFunction OtherActor Sensed)
  (switch string (Utilities|String|LeftChop (Utilities|GetClassDisplayName (Utilities|GetClass OtherActor)) 2)
    (:Civilian_CHARACTER
      (CallFunction|CivilianVisionUpdate Sensed))
    (:SearchLocation_BP
      (CallFunction|SearchLocationUpdate OtherActor))))

(fn CivilianVisionUpdate
  (params (CanSee :type Boolean))
  (bind _returnvalue (AI|GetBlackboard 0))
  (bind _returnvalue_2 (Utilities|Name|MakeLiteralName "ObservedCivilians"))
  (bind _returnvalue_3 (Class|BlackboardComponent|GetValueasInt _returnvalue _returnvalue_2))
  (if CanSee
    (LocalVariables|Setresult (+ _returnvalue_3 1))
    (else
      (LocalVariables|Setresult (- _returnvalue_3 1))))
  (Class|BlackboardComponent|SetValueasInt _returnvalue _returnvalue_2 (LocalVariables|Getresult)))

(fn SearchLocationUpdate
  (params (AsSearchLocation :type Actor%20Object%20Reference))
  (bind _assearch_location_bp_cpp (Utilities|Casting|CastToSearchLocation_BP_CPP AsSearchLocation))
  (bind _searchedlocations (Variables|Default|GetsearchedLocations))
  (if (== (Utilities|Array|FindItem _searchedlocations _assearch_location_bp_cpp) -1) ; If search location is not already marked as searched
    (Utilities|Array|Add _searchedlocations _assearch_location_bp_cpp)))