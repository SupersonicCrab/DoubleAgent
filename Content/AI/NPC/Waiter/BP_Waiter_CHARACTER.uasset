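; BP_Waiter_CHARACTER is a waiter NPC character that carries a platter of wine.
; On BeginPlay it runs parent setup, then writes its DrinkStation reference to the AI blackboard.
; The UpdateWineAmount event displays the current wine count by toggling visibility on the platter and three wine components, hiding the platter when the count drops below one.
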(event Custom|UpdateWineAmount
  (params (WineAmount :type Integer))
  (bind _returnvalue (>= WineAmount 1))
  (Rendering|SetVisibility (Variables|Default|GetPlatter) _returnvalue false)
  (Rendering|SetVisibility (Variables|Default|GetWine1) _returnvalue false)
  (Rendering|SetVisibility (Variables|Default|GetWine2) (>= WineAmount 2) false)
  (Rendering|SetVisibility (Variables|Default|GetWine3) (== WineAmount 3) false))

(event EventBeginPlay
  (|CallParentFunction)
  (AI|Components|Blackboard|SetValueasObject (AI|GetBlackboard 0) (Utilities|Name|MakeLiteralName "DrinkStation") (Variables|Default|GetDrinkStation)))

(fn ConstructionScript
  (|CallParentFunction))