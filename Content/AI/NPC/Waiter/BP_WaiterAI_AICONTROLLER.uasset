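; AI controller for the waiter NPC that seeds its blackboard at startup.
; On BeginPlay, the server searches all RoomVolume actors for the first one typed as a kitchen and stores it under the Kitchen key.
; It also sets the HoldingItem key to true, so the waiter starts out flagged as holding an item.
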(event EventBeginPlay
  (bind _returnvalue (AI|GetBlackboard 0))
  ;[1 1 1] Setup
  (|CallParentFunction)
  (if (Networking|IsServer)
    (bind _kitchen (CallFunction|FindKitchen))
    (AI|Components|Blackboard|SetValueasObject _returnvalue (Utilities|Name|MakeLiteralName "Kitchen") _kitchen)
    (AI|Components|Blackboard|SetValueasBool _returnvalue (Utilities|Name|MakeLiteralName "HoldingItem") true)))

(fn ConstructionScript
  (|CallParentFunction))

(fn FindKitchen
  (bind _outactors (Actor|GetAllActorsOfClass "/Script/DoubleAgent.RoomVolume"))
  (for _array_element _outactors
    (if (Utilities|Enum|Equal(Enum) (Variables|/Script/DoubleAgent.RoomVolume|GetERoomType _array_element) "Room_Kitchen")
      (return _array_element))))