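; BP_DrinkStation is a drink station prop, filed with the waiter NPC AI, that varies its dressing at runtime.
; On BeginPlay it independently rolls a random bool for the visibility of two bottle and two glass components, without propagating to children.
; The construction script only calls the parent, so the variation is not set up in the editor.
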(event EventBeginPlay
  (Rendering|SetVisibility (Variables|Default|GetBottle1) (Math|Random|RandomBool) false)
  (Rendering|SetVisibility (Variables|Default|GetBottle2) (Math|Random|RandomBool) false)
  (Rendering|SetVisibility (Variables|Default|GetGlass6) (Math|Random|RandomBool) false)
  (Rendering|SetVisibility (Variables|Default|GetGlass3) (Math|Random|RandomBool) false))

(fn ConstructionScript
  (|CallParentFunction))