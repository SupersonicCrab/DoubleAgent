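; Civilian NPC character that can hold a wine glass, drink, speak and cower, extending parent Net events.
; Server construction randomizes gender and a matching voice actor; BeginPlay later applies the female mesh and randomly grants wine on the server.
; Wine toggles child-actor glass visibility and is hidden when hiding held items or cowering, returning when cowering ends.
; Drinking is forwarded to the anim instance, and speaking clears after the remaining speech time.
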(event Custom|NetDrink
  (params (Drink :type Boolean))
  (Class|AnimationControllerINTERFACE|SetDrink(Message) (Components|SkeletalMesh|GetAnimInstance (Variables|Character|GetMesh)) Drink))

(event EventNetSpeaking
  (params (Speaking :type Boolean))
  (|CallParentFunction Speaking)
  (bind _returnvalue (Class|BaseCharacterCHARACTER|GetSpeechTimeRemaining))
  (Utilities|FlowControl|Delay _returnvalue)
  (|CallParentFunction false))

(event EventNetWine
  (params (Wine :type Boolean))
  (bind _bp_winedrink (Variables|Default|GetBP_WineDrink))
  (|CallParentFunction Wine)
  (bind _asbp_wine_drink (Utilities|Casting|CastToBP_WineDrink (Variables|/Script/Engine.ChildActorComponent|GetChildActor _bp_winedrink)))
  (Rendering|SetVisibility _bp_winedrink Wine true))

(event EventHideHeldItem
  (CallFunction|NetWine false))

(event EventBeginPlay
  (|CallParentFunction)
  (Utilities|FlowControl|Delay 1.0)
  (if (Networking|IsServer)
    (CallFunction|NetWine (== (Math|Random|RandomIntegerinRange 1 5) 1)))
  (if (Utilities|Enum|Equal(Enum) (Variables|Default|GetGender) "Gender_Feminine")
    (Class|SkinnedMeshComponent|SetSkeletalMesh (Variables|Character|GetMesh) "/Game/Art/Meshes/Mannequin/SK_Mannequin_Female.SK_Mannequin_Female" true)))

(event EventNetCower
  (params (Cower :type Boolean))
  (|CallParentFunction Cower)
  (CallFunction|NetWine (not Cower)))

(fn ConstructionScript
  (if (Networking|IsServer)
    (bind _output_get (Variables|Default|SetGender (Utilities|Enum|ByteToEnumEGender (Math|Conversions|ToByte(Integer) (Math|Random|RandomIntegerinRange 0 1)))))
    (switch Utilities|FlowControl|Switch|SwitchonEGender _output_get
      (:Gender_Masculine
        (Variables|Default|SetVoiceActor (Utilities|Enum|ByteToEnumEVoiceActor (Math|Conversions|ToByte(Integer) (Math|Random|RandomIntegerinRange 0 1)))))
      (:Gender_Feminine
        (Variables|Default|SetVoiceActor (Utilities|Enum|ByteToEnumEVoiceActor (Math|Conversions|ToByte(Integer) (Math|Random|RandomIntegerinRange 2 3))))))))