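; Civilian NPC AI controller that tracks, on each guard's blackboard, how many civilians are observing that guard.
; It extends the parent sight handler, identifying guards by matching the sensed actor's class display name with its last two characters trimmed.
; Gaining sight of a guard increments that guard's ObservingCivilians blackboard integer, and losing sight decrements it.
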(fn ConstructionScript)

(fn HandleSightUpdate
  (params (OtherActor :type Actor%20Object%20Reference) (Sensed :type Boolean))
  (|CallParentFunction OtherActor Sensed)
  (switch string (Utilities|String|LeftChop (Utilities|GetClassDisplayName (Utilities|GetClass OtherActor)) 2)
    (:BP_Guard_CHARACTER
      (CallFunction|GuardVisionUpdate OtherActor Sensed))))

(fn GuardVisionUpdate
  (params (AsGuard :type Actor%20Object%20Reference) (CanSee :type Boolean))
  (bind _returnvalue (AI|GetBlackboard AsGuard))
  (bind _returnvalue_2 (Utilities|Name|MakeLiteralName "ObservingCivilians"))
  (bind _returnvalue_3 (Class|BlackboardComponent|GetValueasInt _returnvalue _returnvalue_2))
  (if CanSee
    (LocalVariables|Setresult (+ _returnvalue_3 1))
    (else
      (LocalVariables|Setresult (- _returnvalue_3 1))))
  (Class|BlackboardComponent|SetValueasInt _returnvalue _returnvalue_2 (LocalVariables|Getresult)))