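; Base AI controller for stealth-game NPCs that runs a behavior tree and feeds its blackboard from sight, hearing and radio events.
; A timed sight tick scores player detection by distance and angle (or camera view), applies decay, and copies alert state from seen NPCs.
; A second timer keeps door and NPC memory, flagging opened doors.
; Path-reachable noises and delayed radio calls also update blackboard state.
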(event OnPerceptionUpdated(HearingPerception)
  (params (UpdatedActors :type Array%20of%20Actor%20Object%20References))
  ;[1 1 1] Hearing perception update
  (for _array_element UpdatedActors
    (bind _info (Class|AIPerceptionComponent|GetActorsPerception (Variables|Default|GetHearingPerception) _array_element))
    (if (.bSuccessfullySensed (Utilities|Struct|BreakAIStimulus (Utilities|Array|Get(acopy) (.lastsensedstimuli _info) 1)))
      (PerceptionHandling|HandleHearingUpdate (.target _info) (.StimulusLocation (Utilities|Struct|BreakAIStimulus (Utilities|Array|Get(acopy) (.lastsensedstimuli _info) 1))) (.Tag (Utilities|Struct|BreakAIStimulus (Utilities|Array|Get(acopy) (.lastsensedstimuli _info) 1)))))))

(event OnPerceptionUpdated(SightPerception)
  (params (UpdatedActors :type Array%20of%20Actor%20Object%20References))
  ;[1 1 1] Sight perception update
  (for _array_element UpdatedActors
    (bind _info (Class|AIPerceptionComponent|GetActorsPerception (Variables|Default|GetSightPerception) _array_element))
    (PerceptionHandling|HandleSightUpdate (.target _info) (Utilities|Struct|BreakAIStimulus (Utilities|Array|Get(acopy) (.lastsensedstimuli _info))))))

(event Custom|RadioEventDelay
  (params (RadioEvent :type F%20Radio%20Event%20Structure))
  ;[1 1 1] Handle radio events
  (Utilities|Time|SetTimerbyEvent (delegate Custom|RadioEventStart) (Utilities|Struct|BreakFRadioEvent RadioEvent)))

(event Custom|RadioEventStart
  ;[1 1 1] Handle radio events
  (RadioHandling|HandleRadioEvent (stale Custom|RadioEventDelay RadioEvent)))

(event EventBeginPlay
  (bind _returnvalue (AI|GetBlackboard 0))
  ;[1 1 1] Setup
  (AI|RunBehaviorTree (Variables|Default|GetBehaviorTree))
  (AI|Components|Blackboard|SetValueasBool _returnvalue (Utilities|Name|MakeLiteralName "CamerasActive") true)
  (AI|Components|Blackboard|SetValueasBool _returnvalue (Utilities|Name|MakeLiteralName "Power") true)
  (AI|Components|Blackboard|SetValueasBool _returnvalue (Utilities|Name|MakeLiteralName "BackupAvailable") true)
  (AI|Components|Blackboard|SetValueasObject _returnvalue (Utilities|Name|MakeLiteralName "SelfActor") (Pawn|GetControlledPawn))
  (Variables|Default|SetPerceptionFPS (Variables|Default|GetDefaultPerceptionFPS))
  (PerceptionHandling|SightTick)
  (Variables|Default|SetPerceptionMemoryFPS (Variables|Default|GetDefaultMemoryPerceptionFPS))
  (Memory|SightMemoryTick))

(fn ConstructionScript)

(fn SightTick
  (Utilities|FlowControl|Sequence
    (:then_0
      (bind _array_element (Utilities|Array|ForEachLoopwithBreak (Class|AIPerceptionComponent|GetCurrentlyPerceivedActors (Variables|Default|GetSightPerception) "/Script/AIModule.AISense_Sight"))
        (:LoopBody
          (bind _info (Class|AIPerceptionComponent|GetActorsPerception (Variables|Default|GetSightPerception) _array_element))
          (if (Utilities|Struct|BreakAIStimulus (Utilities|Array|Get(acopy) (.lastsensedstimuli _info)))
            (PerceptionHandling|HandleSightTick (.target _info) (Utilities|Struct|BreakAIStimulus (Utilities|Array|Get(acopy) (.lastsensedstimuli _info))))))))
    (:then_1
      (PerceptionTick|DetectionFalloff))
    (:then_2
      (if (!= (Variables|Default|GetPerceptionFPS) 0.0)
        (Utilities|Time|SetTimerbyFunctionName 0 "SightTick" (/ 1.0 (Variables|Default|GetPerceptionFPS)))))))

(fn HandleSightTick
  (params (OtherActor :type Actor%20Object%20Reference) (Sensed :type Boolean) (Camera :type BP%20Camera%20Object%20Reference))
  (bind _returnvalue (Utilities|GetClass OtherActor))
  (if (Utilities|ClassIsChildOf _returnvalue "/Game/AI/NPC/BP_AICharacterBase_CHARACTER.BP_AICharacterBase_CHARACTER_C")
    (PerceptionTick|NPCBaseVisionTick OtherActor Sensed) ; Base AiBaseController response
    (else
      (switch string (Utilities|String|LeftChop (Utilities|GetClassDisplayName _returnvalue) 2)
        (:BP_Player_CHARACTER
          (Utilities|IsValid Camera
            (:Is%20Valid
              (PerceptionTick|PlayerVisionCameraTick OtherActor Camera))
            (:Is%20Not%20Valid
              (PerceptionTick|PlayerVisionTick OtherActor))))
        (:BP_CameraHub
          (PerceptionTick|CameraHubTick OtherActor))))))

(fn HandleSightUpdate
  (params (OtherActor :type Actor%20Object%20Reference) (Sensed :type Boolean))
  (bind _returnvalue (Utilities|GetClass OtherActor))
  (switch string (Utilities|String|LeftChop (Utilities|GetClassDisplayName _returnvalue) 2)
    (:Default
      (if (Utilities|ClassIsChildOf _returnvalue "/Game/Interactable/Door/BP_Door.BP_Door_C")
        (Memory|DoorMemoryUpdate OtherActor)
        (elif (Utilities|ClassIsChildOf _returnvalue "/Game/AI/NPC/BP_AICharacterBase_CHARACTER.BP_AICharacterBase_CHARACTER_C")
          (Memory|NPCMemoryUpdate OtherActor))))
    (:BP_Player_CHARACTER
      (PerceptionUpdate|PlayerVisionUpdate OtherActor Sensed))))

(fn HandleHearingUpdate
  (params (OtherActor :type Actor%20Object%20Reference) (Location :type Vector) (Tag :type Name))
  (bind _returnvalue (AI|GetBlackboard 0))
  (bind _self self)
  ;[1 1 1] Check if NPC can get to sound
  (if (Utilities|Enum|Equal(Enum) (.ReturnValue (Class|NavigationSystemV1|GetPathCost (Transformation|GetActorLocation self) Location 0 "/Script/AIModule.NavFilter_AIControllerDefault")) "Success")
    ;[1 1 1] Ensuring sound isn't coming from the NPC itself
    (if (and (!= (Pawn|GetControlledPawn _self) OtherActor) (!= _self OtherActor))
      (switch name Tag
        (:Local
          ;[1 1 1] Set speaker
          (AI|Components|Blackboard|SetValueasObject _returnvalue (Utilities|Name|MakeLiteralName "Speaker") OtherActor))
        (:Noise
          ;[1 1 1] Set noiseLocation
          (AI|Components|Blackboard|SetValueasVector _returnvalue (Utilities|Name|MakeLiteralName "NoiseLocation") Location))
        (:LoudNoise
          ;[1 1 1] Set loudNoiseLocation
          (AI|Components|Blackboard|SetValueasVector _returnvalue (Utilities|Name|MakeLiteralName "LoudNoiseLocation") Location))))))

(fn HandleRadioEvent
  (params (RadioEvent :type F%20Radio%20Event%20Structure))
  (bind (_radioevent _location _delay _npc) (Utilities|Struct|BreakFRadioEvent RadioEvent))
  (switch Utilities|FlowControl|Switch|SwitchonERadioEvent _radioevent
    (:NewEnumerator1
      (RadioHandling|RadioCheckinCall))
    (:NewEnumerator2
      (RadioHandling|RadioCheckinResponse _npc))
    (:NewEnumerator3
      (RadioHandling|RadioAlert _location))
    (:NewEnumerator4
      (RadioHandling|RadioEngage _location))))

(fn NPCBaseVisionTick
  (params (AsNPC :type Actor%20Object%20Reference) (CanSee :type Boolean))
  (bind _returnvalue (AI|GetBlackboard 0))
  (bind _returnvalue_2 (AI|GetBlackboard 0))
  (bind _returnvalue_3 (Utilities|Name|MakeLiteralName "Detection"))
  (bind _returnvalue_4 (AI|GetBlackboard AsNPC))
  (bind _returnvalue_5 (Utilities|Name|MakeLiteralName "CanSeePlayer"))
  (bind _returnvalue_6 (AI|GetBlackboard 0))
  (bind _returnvalue_7 (Utilities|Name|MakeLiteralName "PlayerLastSeen"))
  (bind _returnvalue_8 (Utilities|Name|MakeLiteralName "UnconsciousNPC"))
  (bind _returnvalue_9 (AI|GetBlackboard 0))
  (bind _returnvalue_10 (AI|GetBlackboard 0))
  (bind _returnvalue_11 (Utilities|Name|MakeLiteralName "BackupAvailable"))
  (bind _returnvalue_12 (AI|GetBlackboard AsNPC))
  (bind _returnvalue_13 (AI|GetBlackboard AsNPC))
  (bind _returnvalue_14 (Utilities|Name|MakeLiteralName "VocalStatus"))
  (bind _returnvalue_15 (AI|GetBlackboard 0))
  (bind _returnvalue_16 (AI|Components|Blackboard|GetValueasObject _returnvalue _returnvalue_8))
  (bind _returnvalue_17 (Class|BlackboardComponent|GetValueasFloat _returnvalue_13 _returnvalue_3))
  (bind _returnvalue_18 (Class|BlackboardComponent|GetValueasFloat _returnvalue_2 _returnvalue_3))
  (bind _returnvalue_19 (Class|BlackboardComponent|GetValueasEnum _returnvalue_12 _returnvalue_14))
  (bind _returnvalue_20 (Utilities|IsValid _returnvalue_16))
  (bind _returnvalue_21 (Utilities|Enum|ByteToEnumEVocalStatus _returnvalue_19))
  (Utilities|FlowControl|Sequence
    (:then_0
      ;[1 1 1] Check for unconscious NPC
      (if (Class|BrainComponent|IsRunning (Variables|/Script/AIModule.AIController|GetBrainComponent (AI|GetAIController AsNPC))) ; is NPC awake
        (if _returnvalue_20 ; if UnconciousNPC is set
          (if (== _returnvalue_16 AsNPC) ; If UnconciousNPC is now awake
            (AI|Components|Blackboard|ClearValue _returnvalue _returnvalue_8) ; Clear UnconciousNPC
          ))
        (elif (not _returnvalue_20) ; if UnconsciousNPC is not set
          (AI|Components|Blackboard|SetValueasObject _returnvalue _returnvalue_8 AsNPC) ; Set UnconsciousNPC
        )))
    (:then_1
      ;[1 1 1] Speaker evaluation
      (AI|Components|Blackboard|SetValueasBool _returnvalue_15 (Utilities|Name|MakeLiteralName "CanSeeSpeaker") (Utilities|Enum|Equal(Enum) (Utilities|GetObjectName (AI|GetAIController AsNPC)) (Utilities|GetObjectName (AI|Components|Blackboard|GetValueasObject _returnvalue_15 (Utilities|Name|MakeLiteralName "Speaker"))))))
    (:then_2
      ;[1 1 1] Copy detection
      (if (and (> _returnvalue_17 _returnvalue_18) (< _returnvalue_18 9e+01)) ; if othernpc has higher detection and if self is not above 90
        (AI|Components|Blackboard|SetValueasFloat _returnvalue_2 _returnvalue_3 _returnvalue_17) ; Copy detection perception
      ))
    (:then_3
      ;[1 1 1] ActionStatus handling
      (switch string (Utilities|String|EnumtoString (Utilities|Enum|ByteToEnumEActionStatus (Class|BlackboardComponent|GetValueasEnum (AI|GetBlackboard AsNPC) (Utilities|Name|MakeLiteralName "ActionStatus"))))
        (:CameraStation
          (AI|Components|Blackboard|SetValueasBool (AI|GetBlackboard 0) (Utilities|Name|MakeLiteralName "CamerasActive") true))))
    (:then_4
      ;[1 1 1] Copy PlayerLastSeen
      (if (and (not (ScalableFloat|GetValueasBool _returnvalue_6 _returnvalue_5)) (ScalableFloat|GetValueasBool _returnvalue_4 _returnvalue_5)) ; If other npc has a playerlastseen vector and self does not
        (AI|Components|Blackboard|SetValueasVector _returnvalue_6 _returnvalue_7 (AI|Components|Blackboard|GetValueasVector _returnvalue_4 _returnvalue_7))))
    (:then_5
      ;[1 1 1] Update BackupAvailable
      (if (and (ScalableFloat|GetValueasBool _returnvalue_9 _returnvalue_11) (not (ScalableFloat|GetValueasBool (AI|GetBlackboard AsNPC) _returnvalue_11))) ; If other npc believes backup is not available
        (AI|Components|Blackboard|SetValueasBool _returnvalue_9 _returnvalue_11 false)))
    (:then_6
      ;[1 1 1] Update vocalStatus
      (if (< (Utilities|Enum|ByteToEnumEVocalStatus (Class|BlackboardComponent|GetValueasEnum _returnvalue_10 _returnvalue_14)) _returnvalue_21) ; if other npc has a higher vocal status
        (AI|Components|Blackboard|SetValueasEnum _returnvalue_10 _returnvalue_14 _returnvalue_21)))))

(fn PlayerVisionTick
  (params (AsPlayer :type Actor%20Object%20Reference))
  (bind _returnvalue (Utilities|Name|MakeLiteralName "Detection"))
  (bind _returnvalue_2 (Pawn|GetControlledPawn))
  (bind _returnvalue_3 (Utilities|Name|MakeLiteralName "Detection"))
  (bind _returnvalue_4 (AI|GetBlackboard 0))
  (bind _returnvalue_5 (Transformation|GetActorLocation AsPlayer))
  (bind _asbp_player_character (Utilities|Casting|CastToBP_Player_CHARACTER AsPlayer))
  (bind _detectionrate (Variables|Default|GetDetectionRate))
  (bind _sightrange (Variables|Default|GetSightRange))
  (bind _returnvalue_6 (Class|BlackboardComponent|GetValueasFloat _returnvalue_4 _returnvalue))
  (bind _returnvalue_7 (Transformation|GetActorLocation _returnvalue_2))
  (bind _returnvalue_8 (Transformation|GetActorForwardVector _returnvalue_2))
  (bind _detectionrating (Variables|/Game/Player/BP_Player_CHARACTER.BP_Player_CHARACTER_C|GetDetectionRating _asbp_player_character))
  (bind _returnvalue_9 (Math|Vector|Distance(Vector) _returnvalue_5 _returnvalue_7))
  (bind _returnvalue_10 (Math|Rotator|FindLookatRotation _returnvalue_7 _returnvalue_5))
  (bind _returnvalue_11 (/ _returnvalue_9 _sightrange))
  (bind _returnvalue_12 (Math|Vector|GetForwardVector _returnvalue_10))
  (bind _returnvalue_13 (- _returnvalue_11 1.0))
  (bind _returnvalue_14 (Math|Vector|DotProduct _returnvalue_8 _returnvalue_12))
  (bind _returnvalue_15 (Math|Float|Absolute(Float) _returnvalue_13))
  (bind _returnvalue_16 (+ _returnvalue_15 _returnvalue_14))
  (bind _returnvalue_17 (/ _returnvalue_16 2.0))
  (bind _returnvalue_18 (* _detectionrate _returnvalue_17))
  (bind _returnvalue_19 (+ _returnvalue_18 _returnvalue_6))
  (bind _returnvalue_20 (> _returnvalue_19 4e+01))
  ;[1 1 1] Threat perception calculations
  (if (and (< _returnvalue_6 1e+02) (or (or (not (Variables|/Script/ProjectSpy.Player_Character|GetroomSafe _asbp_player_character)) (>= _returnvalue_6 9e+01)) (and (< (Transformation|GetDistanceTo _asbp_player_character self) (Variables|Default|GetSearchDistance)) (or (and (< _returnvalue_6 8e+01) (> _detectionrating (Variables|Default|GetSearchThreshold))) (>= _detectionrating 1e+02)))))
    ;[1 1 1] Detection rate calculations
    (if (> _returnvalue_19 1e+02)
      (AI|Components|Blackboard|SetValueasFloat _returnvalue_4 _returnvalue_3 1e+02)
      (else
        (AI|Components|Blackboard|SetValueasFloat _returnvalue_4 _returnvalue_3 _returnvalue_19)))
    ;[1 1 1] Set suspicious
    (if _returnvalue_20
      (AI|Components|Blackboard|SetValueasBool _returnvalue_4 (Utilities|Name|MakeLiteralName "Suspicious") true)
      ;[1 1 1] Update player last seen
      (AI|Components|Blackboard|SetValueasVector _returnvalue_4 (Utilities|Name|MakeLiteralName "PlayerLastSeen") (Transformation|GetActorLocation AsPlayer) :!label _label))
    (elif _returnvalue_20
      (goto _label))))

(fn PlayerVisionUpdate
  (params (AsPlayer :type Actor%20Object%20Reference) (CanSee :type Boolean))
  (bind _returnvalue (AI|GetBlackboard 0))
  (bind _returnvalue_2 (Utilities|Name|MakeLiteralName "LastPlayer"))
  (bind _returnvalue_3 (AI|Components|Blackboard|GetValueasObject _returnvalue _returnvalue_2))
  (AI|Components|Blackboard|SetValueasBool _returnvalue (Utilities|Name|MakeLiteralName "CanSeePlayer") CanSee) ; Updating NPCs perception of canSeePlayer
  ;[1 1 1] Updating lastPlayer
  (if CanSee
    (AI|Components|Blackboard|SetValueasObject _returnvalue _returnvalue_2 AsPlayer) ; Updating lastPlayer for animation tracking
    (else
      (Utilities|IsValid _returnvalue_3
        (:Is%20Valid
          (if (== (.AsActor (Utilities|Casting|CastToActor _returnvalue_3)) AsPlayer)
            (AI|Components|Blackboard|ClearValue _returnvalue _returnvalue_2) ; Clearing lastPlayer on player lost
          ))))))

(fn DetectionFalloff
  (bind _returnvalue (AI|GetBlackboard 0))
  (bind _returnvalue_2 (Utilities|Name|MakeLiteralName "Detection"))
  (bind _returnvalue_3 (Class|BlackboardComponent|GetValueasFloat _returnvalue _returnvalue_2))
  (if (Math|Boolean|ANDBoolean (> _returnvalue_3 0.0) (!= _returnvalue_3 4e+01) (!= _returnvalue_3 9e+01) (not (ScalableFloat|GetValueasBool _returnvalue (Utilities|Name|MakeLiteralName "CanSeePlayer"))))
    (AI|Components|Blackboard|SetValueasFloat _returnvalue (Utilities|Name|MakeLiteralName "Detection") (- (Math|Conversions|ToFloat(Integer) (Math|Float|Round _returnvalue_3)) 1.0))
    (AI|Components|Blackboard|SetValueasBool _returnvalue (Utilities|Name|MakeLiteralName "Suspicious") false)))

(fn RadioAlert
  (params (Location :type Vector))
  (bind _returnvalue (AI|GetBlackboard 0))
  (if (> (Utilities|Enum|ByteToEnumEVocalStatus (Class|BlackboardComponent|GetValueasEnum _returnvalue (Utilities|Name|MakeLiteralName "VocalStatus"))) (LocalVariables|GetVocalStatusAlert))
    ;[1 1 1] If NPC is already alert
    (AI|Components|Blackboard|SetValueasVector _returnvalue (Utilities|Name|MakeLiteralName "PlayerLastSeen") Location)
    (else
      ;[1 1 1] If NPCs vocal status is less than alert
      (AI|Components|Blackboard|SetValueasVector _returnvalue (Utilities|Name|MakeLiteralName "PlayerLastSeen") Location)
      (AI|Components|Blackboard|SetValueasFloat _returnvalue (Utilities|Name|MakeLiteralName "Detection") 9e+01)
      (AI|Components|Blackboard|SetValueasEnum _returnvalue (Utilities|Name|MakeLiteralName "VocalStatus") (LocalVariables|GetVocalStatusAlert)))))

(fn RadioEngage
  (params (Location :type Vector))
  (bind _returnvalue (AI|GetBlackboard 0))
  (if (> (Utilities|Enum|ByteToEnumEVocalStatus (Class|BlackboardComponent|GetValueasEnum _returnvalue (Utilities|Name|MakeLiteralName "VocalStatus"))) (LocalVariables|GetVocalStatusEngaging))
    ;[1 1 1] If NPC is already engaging
    (AI|Components|Blackboard|SetValueasVector _returnvalue (Utilities|Name|MakeLiteralName "PlayerLastSeen") Location)
    (AI|Components|Blackboard|ClearValue _returnvalue (Utilities|Name|MakeLiteralName "InitialLastSeen"))
    (else
      ;[1 1 1] If NPCs vocal status is less than engaging
      (AI|Components|Blackboard|SetValueasVector _returnvalue (Utilities|Name|MakeLiteralName "PlayerLastSeen") Location)
      (AI|Components|Blackboard|SetValueasFloat _returnvalue (Utilities|Name|MakeLiteralName "Detection") 9e+01)
      (AI|Components|Blackboard|SetValueasEnum _returnvalue (Utilities|Name|MakeLiteralName "VocalStatus") (LocalVariables|GetVocalStatusEngaging)))))

(fn RadioCheckinCall
  (AI|Components|Blackboard|SetValueasBool (AI|GetBlackboard 0) (Utilities|Name|MakeLiteralName "CheckIn") true))

(fn RadioCheckinResponse
  (params (NPC :type BP%20AI%20Character%20Base%20CHARACTER%20Object%20Reference))
  (if (ScalableFloat|GetValueasBool (AI|GetBlackboard 0) (Utilities|Name|MakeLiteralName "RadioOperator"))
    (bind _returnvalue (Actor|GetActorOfClass "/Game/SecuritySystem/Radio/BP_RadioHub.BP_RadioHub_C"))
    (Utilities|Array|Add (Variables|/Game/SecuritySystem/Radio/BP_RadioHub.BP_RadioHub_C|GetTempRadioNPCs _returnvalue) NPC)))

(fn CameraHubTick
  (params (AsCameraHub :type Actor%20Object%20Reference))
  (bind _asbp_camera_hub (Utilities|Casting|CastToBP_CameraHub AsCameraHub))
  (bind _operatornpc (Variables|/Game/SecuritySystem/BP_CameraHub.BP_CameraHub_C|GetOperatorNPC _asbp_camera_hub))
  (bind _output_get (LocalVariables|SetselfBlackboard (AI|GetBlackboard 0)))
  (AI|Components|Blackboard|SetValueasBool _output_get (Utilities|Name|MakeLiteralName "CamerasActive") (Utilities|IsValid _operatornpc))
  (AI|Components|Blackboard|SetValueasBool (LocalVariables|GetselfBlackboard) (Utilities|Name|MakeLiteralName "Power") (Variables|/Game/SecuritySystem/BP_CameraHub.BP_CameraHub_C|GetbPowerOn _asbp_camera_hub))
  (Utilities|IsValid _operatornpc
    (:Is%20Not%20Valid
      ;[1 1 1] Set cautious if display is on and no operator
      (if (and (Variables|/Game/SecuritySystem/BP_CameraHub.BP_CameraHub_C|GetbDisplayOn _asbp_camera_hub) (< (Class|BlackboardComponent|GetValueasFloat (LocalVariables|GetselfBlackboard) (LocalVariables|Getdetection)) 4e+01))
        (AI|Components|Blackboard|SetValueasFloat (LocalVariables|GetselfBlackboard) (LocalVariables|Getdetection) 4e+01)
        (AI|Components|Blackboard|SetValueasEnum (LocalVariables|GetselfBlackboard) (Utilities|Name|MakeLiteralName "VocalStatus") (Utilities|Enum|LiteralenumEVocalStatus "NewEnumerator0"))))))

(fn PlayerVisionCameraTick
  (params (AsPlayer :type Actor%20Object%20Reference) (AsCamera :type BP%20Camera%20Object%20Reference))
  (bind _returnvalue (Utilities|Name|MakeLiteralName "Detection"))
  (bind _returnvalue_2 (Utilities|Name|MakeLiteralName "Detection"))
  (bind _returnvalue_3 (AI|GetBlackboard 0))
  (bind _returnvalue_4 (Transformation|GetActorLocation AsPlayer))
  (bind _cameradetectionrate (Variables|Default|GetCameraDetectionRate))
  (bind _scenecapturecomponent2d (Variables|/Game/SecuritySystem/BP_Camera.BP_Camera_C|GetSceneCaptureComponent2D AsCamera))
  (bind _sightrange (Variables|Default|GetSightRange))
  (bind _returnvalue_5 (Transformation|GetWorldLocation _scenecapturecomponent2d))
  (bind _returnvalue_6 (Class|BlackboardComponent|GetValueasFloat _returnvalue_3 _returnvalue))
  (bind _returnvalue_7 (Math|Vector|GetForwardVector _scenecapturecomponent2d))
  (bind _returnvalue_8 (Math|Vector|Distance(Vector) _returnvalue_4 _returnvalue_5))
  (bind _returnvalue_9 (Math|Rotator|FindLookatRotation _returnvalue_5 _returnvalue_4))
  (bind _returnvalue_10 (/ _returnvalue_8 _sightrange))
  (bind _returnvalue_11 (Math|Vector|GetForwardVector _returnvalue_9))
  (bind _returnvalue_12 (- _returnvalue_10 1.0))
  (bind _returnvalue_13 (Math|Vector|DotProduct _returnvalue_7 _returnvalue_11))
  (bind _returnvalue_14 (Math|Float|Absolute(Float) _returnvalue_12))
  (bind _returnvalue_15 (+ _returnvalue_14 _returnvalue_13))
  (bind _returnvalue_16 (/ _returnvalue_15 2.0))
  (bind _returnvalue_17 (* _cameradetectionrate _returnvalue_16))
  (bind _returnvalue_18 (+ _returnvalue_17 _returnvalue_6))
  ;[1 1 1] Threat perception calculations
  (if (and (< _returnvalue_6 1e+02) (or (not (Variables|/Script/ProjectSpy.Player_Character|GetroomSafe (.AsBP%20Player%20CHARACTER (Utilities|Casting|CastToBP_Player_CHARACTER AsPlayer)))) (>= _returnvalue_6 9e+01)))
    ;[1 1 1] Detection rate calculations
    (if (> _returnvalue_18 1e+02)
      (AI|Components|Blackboard|SetValueasFloat _returnvalue_3 _returnvalue_2 1e+02)
      (else
        (AI|Components|Blackboard|SetValueasFloat _returnvalue_3 _returnvalue_2 _returnvalue_18)))
    ;[1 1 1] Update player last seen
    (AI|Components|Blackboard|SetValueasVector _returnvalue_3 (Utilities|Name|MakeLiteralName "PlayerLastSeen") (Transformation|GetActorLocation AsPlayer) :!label _label)
    (elif (> _returnvalue_18 4e+01)
      (goto _label))))

(fn AddSearchLocation
  (params (SearchLocation :type Search%20Location%20Object%20Reference))
  (bind _returnvalue (AI|GetBlackboard 0))
  (bind _returnvalue_2 (Utilities|Name|MakeLiteralName "ActionStatus"))
  (bind _searchedlocations (Variables|Default|GetSearchedLocations))
  (Utilities|Array|Add _searchedlocations SearchLocation)
  (Utilities|Array|Add (LocalVariables|GetAddedLocations) SearchLocation)
  ;[1 1 1] Loop through search location rooms and mark the search locations inside those rooms if missing
  (for _array_element (Variables|/Game/AI/SearchSystem/BP_SearchLocation.BP_SearchLocation_C|GetRoom (.AsBP%20Search%20Location (Utilities|Casting|CastToBP_SearchLocation SearchLocation)))
    (for _array_element_2 (Variables|/Script/ProjectSpy.RoomVolume|GetsearchLocations _array_element)
      (if (== (Utilities|Array|FindItem _searchedlocations _array_element_2) -1)
        (Utilities|Array|Add _searchedlocations _array_element_2)
        (Utilities|Array|Add (LocalVariables|GetAddedLocations) _array_element_2))))
  (bind _asbp_search_location (Utilities|Casting|CastToBP_SearchLocation (AI|Components|Blackboard|GetValueasObject _returnvalue (Utilities|Name|MakeLiteralName "TempObject"))))
  ;[1 1 1] If any of the added locations was being searched
  (if (!= (Utilities|Array|FindItem (LocalVariables|GetAddedLocations) _asbp_search_location) -1)
    (if (Utilities|Enum|Equal(Enum) (Utilities|Enum|ByteToEnumEActionStatus (Class|BlackboardComponent|GetValueasEnum _returnvalue _returnvalue_2)) "NewEnumerator8")
      (AI|Components|Blackboard|SetValueasEnum _returnvalue _returnvalue_2 (Utilities|Enum|LiteralenumEActionStatus "NewEnumerator3")) ; Reset action status
    )))

(fn DoorMemoryUpdate
  (params (AsDoor :type Actor%20Object%20Reference))
  (bind _asbp_door (Utilities|Casting|CastToBP_Door AsDoor))
  (bind _memory (Variables|Default|GetMemory))
  (bind _doormemory (Utilities|Struct|BreakFMemory _memory))
  (bind _dooropen (Variables|/Game/Interactable/Door/BP_Door.BP_Door_C|GetDoorOpen _asbp_door))
  (LocalVariables|SetSavedIndex -1)
  (if (!= (Utilities|Array|Length _doormemory) 0) ; If array length is greater than 0
    ;[1 1 1] Search memory for door
    (bind (_array_element _array_index) (Utilities|Array|ForEachLoopwithBreak _doormemory :!label _label)
      (:LoopBody
        (if (== (.DoorReference (Utilities|Struct|BreakFDoorMemory _array_element)) _asbp_door)
          (LocalVariables|SetSavedIndex _array_index)
          (goto _label Break)))
      (:Completed
        (if (!= (LocalVariables|GetSavedIndex) -1) ; If memory exists
          (if (Math|Boolean|NotEqual(Boolean) (.DoorOpen (Utilities|Struct|BreakFDoorMemory (Utilities|Array|Get(acopy) _doormemory (LocalVariables|GetSavedIndex)))) _dooropen) ; If closed memory is not the same
            (Utilities|Array|SetArrayElem _doormemory (LocalVariables|GetSavedIndex) (Utilities|Struct|MakeFDoorMemory (.DoorReference (Utilities|Struct|BreakFDoorMemory (Utilities|Array|Get(acopy) _doormemory (LocalVariables|GetSavedIndex)))) _dooropen))
            (if _dooropen ; If door is now open
              (AI|Components|Blackboard|SetValueasObject (AI|GetBlackboard 0) (Utilities|Name|MakeLiteralName "OpenedDoor") (.DoorReference (Utilities|Struct|BreakFDoorMemory (Utilities|Array|Get(acopy) _doormemory (LocalVariables|GetSavedIndex)))))))
          (else
            (Utilities|Array|Add _doormemory (Utilities|Struct|MakeFDoorMemory _asbp_door _dooropen)) ; Add door to memory
          ))))
    (else
      (Utilities|Array|Add _doormemory (Utilities|Struct|MakeFDoorMemory _asbp_door _dooropen)) ; Add door to memory
    )))

(fn SightMemoryTick
  (Utilities|FlowControl|Sequence
    (:then_0
      (bind _array_element (Utilities|Array|ForEachLoopwithBreak (Class|AIPerceptionComponent|GetCurrentlyPerceivedActors (Variables|Default|GetSightPerception) "/Script/AIModule.AISense_Sight"))
        (:LoopBody
          (bind _info (Class|AIPerceptionComponent|GetActorsPerception (Variables|Default|GetSightPerception) _array_element))
          (if (Utilities|Struct|BreakAIStimulus (Utilities|Array|Get(acopy) (.lastsensedstimuli _info)))
            (Memory|HandleMemoryTick (.target _info))))))
    (:then_1
      (if (!= (Variables|Default|GetPerceptionMemoryFPS) 0.0)
        (Utilities|Time|SetTimerbyFunctionName 0 "SightMemoryTick" (/ (Variables|Default|GetPerceptionMemoryFPS) 1.0))))))

(fn HandleMemoryTick
  (params (OtherActor :type Actor%20Object%20Reference))
  (bind _returnvalue (Utilities|GetClass OtherActor))
  (if (Utilities|ClassIsChildOf _returnvalue "/Game/Interactable/Door/BP_Door.BP_Door_C")
    (Memory|DoorMemoryUpdate OtherActor)
    (elif (Utilities|ClassIsChildOf _returnvalue "/Game/AI/NPC/BP_AICharacterBase_CHARACTER.BP_AICharacterBase_CHARACTER_C")
      (Memory|NPCMemoryUpdate OtherActor))))

(fn NPCMemoryUpdate
  (params (NPC :type Actor%20Object%20Reference))
  (bind _asbp_aicharacter_base_character (Utilities|Casting|CastToBP_AICharacterBase_CHARACTER NPC))
  (bind _memory (Variables|Default|GetMemory))
  (bind _returnvalue (Transformation|GetActorLocation _asbp_aicharacter_base_character))
  (LocalVariables|SetSavedIndex -1)
  (if (!= (Utilities|Array|Length (.npcmemory _memory)) 0) ; If array length is greater than 0
    ;[1 1 1] Search memory for NPC
    (bind (_array_element _array_index) (Utilities|Array|ForEachLoopwithBreak (.npcmemory _memory) :!label _label)
      (:LoopBody
        (if (== (.NPCReference (Utilities|Struct|BreakFNPCMemory _array_element)) _asbp_aicharacter_base_character)
          (LocalVariables|SetSavedIndex _array_index)
          (goto _label Break)))
      (:Completed
        (if (!= (LocalVariables|GetSavedIndex) -1) ; If memory exists
          (if (Math|Vector|NotEqual(Vector) (.LastSeen (Utilities|Struct|BreakFNPCMemory (Utilities|Array|Get(acopy) (.npcmemory _memory) (LocalVariables|GetSavedIndex)))) _returnvalue 0.0001) ; If last seen does not equal current location
            (Utilities|Array|SetArrayElem (.npcmemory _memory) (LocalVariables|GetSavedIndex) (Utilities|Struct|MakeFNPCMemory (.NPCReference (Utilities|Struct|BreakFNPCMemory (Utilities|Array|Get(acopy) (.npcmemory _memory) (LocalVariables|GetSavedIndex)))) _returnvalue)) ; Update last seen
          )
          (else
            (Utilities|Array|Add (.npcmemory _memory) (Utilities|Struct|MakeFNPCMemory _asbp_aicharacter_base_character _returnvalue)) ; Add NPC to memory
          ))))
    (else
      (Utilities|Array|Add (.npcmemory _memory) (Utilities|Struct|MakeFNPCMemory _asbp_aicharacter_base_character _returnvalue)) ; Add NPC to memory
    )))