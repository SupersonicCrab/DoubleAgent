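; Mob boss NPC character that fixes its voice actor and masculine gender in the construction script.
; On BeginPlay the server passes its designated route to the AI blackboard after running the parent setup.
; An EnableOutline event turns on custom depth with a set stencil value so the mesh can be outlined.
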(event EventBeginPlay
  ;[1 1 1] Setup
  (|CallParentFunction)
  (if (Networking|IsServer)
    (AI|Components|Blackboard|SetValueasObject (AI|GetBlackboard 0) (Utilities|Name|MakeLiteralName "DesignatedRoute") (Variables|Default|GetDesignatedRoute))))

(event EventEnableOutline
  (bind _mesh (Variables|Character|GetMesh))
  (Rendering|SetRenderCustomDepth _mesh true)
  (Rendering|SetCustomDepthStencilValue _mesh 254))

(fn ConstructionScript
  (Variables|Default|SetVoiceActor "MobBoss")
  (Variables|Default|SetGender "Gender_Masculine"))