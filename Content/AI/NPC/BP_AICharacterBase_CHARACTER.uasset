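; Base character for AI NPCs in a networked spy game, supporting pickpocketing, rear takedowns, alerting and a downed state.
; A rear collision volume offers the takedown prompt and closes an open inventory when players leave.
; Delayed inventory checks after pickpocketing update the blackboard and switch navigation filters based on keycard possession.
; Net events relay animation and hitbox changes, while server detection replicates to a debug display.
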(event OnComponentBeginOverlap(BehindCollision)
  (params (OverlappedComponent :type Primitive%20Component%20Object%20Reference) (OtherActor :type Actor%20Object%20Reference) (OtherComp :type Primitive%20Component%20Object%20Reference) (OtherBodyIndex :type Integer) (bFromSweep :type Boolean) (SweepResult :type Hit%20Result%20Structure%20%28by%20ref%29))
  ;[1 1 1] Log UI - And removing the inventory from players if they leave the hitbox
  (bind _asbp_player_character (Utilities|Casting|CastToBP_Player_CHARACTER OtherActor))
  (bind _asbp_spy_player_playercontroller (Utilities|Casting|CastToBP_SpyPlayer_PLAYERCONTROLLER (Pawn|GetController _asbp_player_character)))
  (Utilities|IsValid (Variables|/Game/Player/BP_SpyPlayer_PLAYERCONTROLLER.BP_SpyPlayer_PLAYERCONTROLLER_C|GetContexMenu _asbp_spy_player_playercontroller)
    (:Is%20Valid
      (if (not (Variables|Default|GetbDowned))
        (bind _slotref (Default|OverlapBegin (Variables|/Game/Player/BP_SpyPlayer_PLAYERCONTROLLER.BP_SpyPlayer_PLAYERCONTROLLER_C|GetContexMenu _asbp_spy_player_playercontroller) "Takedown" _asbp_spy_player_playercontroller "Takedown"))
        (Variables|Default|SetTakedownSlotRef _slotref)))))

(event OnComponentEndOverlap(BehindCollision)
  (params (OverlappedComponent :type Primitive%20Component%20Object%20Reference) (OtherActor :type Actor%20Object%20Reference) (OtherComp :type Primitive%20Component%20Object%20Reference) (OtherBodyIndex :type Integer))
  ;[1 1 1] Log UI - And removing the inventory from players if they leave the hitbox
  (bind _asbp_player_character (Utilities|Casting|CastToBP_Player_CHARACTER OtherActor))
  (bind _asbp_spy_player_playercontroller (Utilities|Casting|CastToBP_SpyPlayer_PLAYERCONTROLLER (Pawn|GetController _asbp_player_character)))
  (Utilities|IsValid (Variables|/Game/Player/BP_SpyPlayer_PLAYERCONTROLLER.BP_SpyPlayer_PLAYERCONTROLLER_C|GetContexMenu _asbp_spy_player_playercontroller)
    (:Is%20Valid
      (if (Variables|Default|GetInventoryOpen)
        (Default|ToggleInventory (Variables|Default|GetInventoryComponent) OtherActor)
        (Variables|Default|SetInventoryOpen false))
      (if (!= (Variables|Default|GetTakedownSlotRef) 0)
        (Default|OverlapEnd (Variables|/Game/Player/BP_SpyPlayer_PLAYERCONTROLLER.BP_SpyPlayer_PLAYERCONTROLLER_C|GetContexMenu _asbp_spy_player_playercontroller) (Variables|Default|GetTakedownSlotRef))
        (Variables|Default|SetTakedownSlotRef 0)))))

(event Custom|NetSetTurnTo
  (params (TurnTarget :type Vector))
  ;[1 1 1] Network animation setters
  (Class|AnimationControllerINTERFACE|SetTurnto(Message) (Components|SkeletalMesh|GetAnimInstance (Variables|Character|GetMesh)) TurnTarget))

(event Custom|NetSetLookAt
  (params (LookAt :type Boolean))
  ;[1 1 1] Network animation setters
  (Class|AnimationControllerINTERFACE|SetLookat(Message) (Components|SkeletalMesh|GetAnimInstance (Variables|Character|GetMesh)) LookAt))

(event Custom|NetSetWeaponAim
  (params (WeaponAim :type Boolean))
  ;[1 1 1] Network animation setters
  (Class|AnimationControllerINTERFACE|SetWeaponAim(Message) (Components|SkeletalMesh|GetAnimInstance (Variables|Character|GetMesh)) WeaponAim))

(event Custom|NetSetWeaponOut
  (params (WeaponOut :type Boolean))
  ;[1 1 1] Network animation setters
  (Class|AnimationControllerINTERFACE|SetWeaponOut(Message) (Components|SkeletalMesh|GetAnimInstance (Variables|Character|GetMesh)) WeaponOut))

(event Custom|NetSetEarPiece
  (params (EarPiece :type Boolean))
  ;[1 1 1] Network animation setters
  (Class|AnimationControllerINTERFACE|SetEarPiece(Message) (Components|SkeletalMesh|GetAnimInstance (Variables|Character|GetMesh)) EarPiece))

(event Custom|NetSetFlashlightOut
  (params (FlashlightOut :type Boolean))
  ;[1 1 1] Network animation setters
  (Class|AnimationControllerINTERFACE|SetFlashlightOut(Message) (Components|SkeletalMesh|GetAnimInstance (Variables|Character|GetMesh)) FlashlightOut))

(event Custom|NetSetMelee
  (params (Melee :type Boolean))
  ;[1 1 1] Network animation setters
  (Class|AnimationControllerINTERFACE|SetMelee(Message) (Components|SkeletalMesh|GetAnimInstance (Variables|Character|GetMesh)) Melee))

(event Custom|NetSetCrouch
  (params (Crouch :type Boolean))
  ;[1 1 1] Network animation setters
  (Class|AnimationControllerINTERFACE|SetCrouch(Message) (Components|SkeletalMesh|GetAnimInstance (Variables|Character|GetMesh)) Crouch))

(event Custom|NetShoot
  (params (Shoot :type Boolean))
  ;[1 1 1] Network animation setters
  (Class|AnimationControllerINTERFACE|Shoot(Message) (Components|SkeletalMesh|GetAnimInstance (Variables|Character|GetMesh)) Shoot))

(event Custom|NetInteract
  ;[1 1 1] Network animation setters
  (Class|AnimationControllerINTERFACE|Interact(Message) (Components|SkeletalMesh|GetAnimInstance (Variables|Character|GetMesh))))

(event Custom|NetDownedHitbox
  ;[1 1 1] Update hitboxs over the network
  (Collision|SetCollisionEnabled (Variables|Default|GetCapsuleComponent) "NoCollision")
  (Transformation|SetRelativeTransform (Variables|Default|GetBehindCollision) (Math|Transform|MakeTransform "0, 0, 0" "90.000000, 0, 0" "3.000000,3.000000,3.000000") false true))

(event Custom|NetStandingHitbox
  ;[1 1 1] Update hitboxs over the network
  (Collision|SetCollisionEnabled (Variables|Default|GetCapsuleComponent) "QueryAndPhysics")
  (Transformation|SetRelativeTransform (Variables|Default|GetBehindCollision) (Math|Transform|MakeTransform "-80.000000, 0,10.000000" "0, 0, 0" "2.000000,3.000000,3.000000") false true))

(event Custom|NetSetVectorFocus
  (params (VectorFocus :type Vector))
  ;[1 1 1] Network animation setters
  (Class|AnimationControllerINTERFACE|SetVectorFocus(Message) (Components|SkeletalMesh|GetAnimInstance (Variables|Character|GetMesh)) VectorFocus))

(event Custom|NetSetActorFocus
  (params (Actor :type Actor%20Object%20Reference))
  ;[1 1 1] Network animation setters
  (Class|AnimationControllerINTERFACE|SetActorFocus(Message) (Components|SkeletalMesh|GetAnimInstance (Variables|Character|GetMesh)) Actor))

(event EventBeginPlay
  (bind _inventorycomponent (Variables|Default|GetInventoryComponent))
  (bind _inventory (Variables|/Game/Inventory/BP_InventoryComponent.BP_InventoryComponent_C|GetInventory _inventorycomponent))
  ;[1 1 1] Setup
  (for (_array_element _array_index) (Variables|Default|GetItems)
    (Utilities|Array|SetArrayElem _inventory _array_index _array_element))
  (Variables|/Game/Inventory/BP_InventoryComponent.BP_InventoryComponent_C|SetOriginalInventory _inventorycomponent _inventory)
  (if (Networking|IsServer)
    (CallFunction|CheckInventory)
    (Default|PrepareInventory _inventorycomponent) ; Used to process initial pickup handling
  ))

(event EventTick
  (params (DeltaSeconds :type Float%20%28single-precision%29))
  ;[1 1 1] Debug update
  (CallFunction|DebugDisplayUpdate)
  (CallFunction|UpdateDetection))

(event EventDisableOutline
  (Rendering|SetCustomDepthStencilValue (Variables|Character|GetMesh) 0))

(event EventEnableOutline
  (bind _mesh (Variables|Character|GetMesh))
  (Rendering|SetRenderCustomDepth _mesh true)
  (Rendering|SetCustomDepthStencilValue _mesh 253))

(event EventInteract
  (params (Interactor :type Actor%20Object%20Reference))
  ;[1 1 1] Interact
  (Default|ToggleInventory (Variables|Default|GetInventoryComponent) Interactor)
  (Variables|Default|SetInventoryOpen true)
  (Class|PlayerCharacter|PerformIllegalAction (.AsBP%20Player%20CHARACTER (Utilities|Casting|CastToBP_Player_CHARACTER Interactor)) 1.0)
  (if (not (Class|KismetSystemLibrary|IsTimerActive 0 "CheckInventory"))
    (Utilities|Time|SetTimerbyFunctionName 0 "CheckInventory" (Variables|Default|GetInventoryCheck)) ; Call inventory check after delay
  ))

(fn ConstructionScript)

(fn CheckInventory
  (bind _self self)
  (bind _inventorycomponent (Variables|Default|GetInventoryComponent))
  (bind _inventorycomponent_2 (Variables|Default|GetInventoryComponent))
  (bind _returnvalue (AI|GetAIController _self))
  (Utilities|FlowControl|Sequence
    (:then_0
      ;[1 1 1] Updating blackboards inventoryStatus
      (bind _missingitempriority (Default|CheckInventory _inventorycomponent_2))
      (AI|Components|Blackboard|SetValueasEnum (AI|GetBlackboard 0) (Utilities|Name|MakeLiteralName "InventoryStatus") _missingitempriority)
      (Variables|/Game/Inventory/BP_InventoryComponent.BP_InventoryComponent_C|SetOriginalInventory _inventorycomponent (Variables|/Game/Inventory/BP_InventoryComponent.BP_InventoryComponent_C|GetInventory _inventorycomponent)) ; Update original inventory to new remembered inventory
    )
    (:then_1
      ;[1 1 1] Updating navmesh perception
      (bind _itemfound (Default|CheckItemClass _inventorycomponent_2 "/Game/Inventory/Item/BP_Keycard_Item.BP_Keycard_Item_C"))
      (if _itemfound
        (Variables|/Script/AIModule.AIController|SetDefaultNavigationFilterClass _returnvalue "/Game/AI/Nagivation/QueryFilter/BP_Default_NAVFILTER.BP_Default_NAVFILTER_C")
        (else
          (Variables|/Script/AIModule.AIController|SetDefaultNavigationFilterClass _returnvalue "/Game/AI/Nagivation/QueryFilter/BP_AvoidLockedDoors_NAVFILTER.BP_AvoidLockedDoors_NAVFILTER_C"))))))

(fn EngageNPC
  (bind _returnvalue (AI|GetBlackboard 0))
  (AI|Components|Blackboard|SetValueasFloat _returnvalue (Utilities|Name|MakeLiteralName "Detection") 9e+01)
  (AI|Components|Blackboard|SetValueasEnum _returnvalue (Utilities|Name|MakeLiteralName "VocalStatus") (Utilities|Enum|LiteralenumBP_EVocalStatus "NewEnumerator6")))

(fn AlertNPC
  (bind _returnvalue (AI|GetBlackboard 0))
  (AI|Components|Blackboard|SetValueasFloat _returnvalue (Utilities|Name|MakeLiteralName "Detection") 9e+01)
  (AI|Components|Blackboard|SetValueasEnum _returnvalue (Utilities|Name|MakeLiteralName "VocalStatus") (Utilities|Enum|LiteralenumBP_EVocalStatus "NewEnumerator1")))

(fn TakedownNPC
  (Variables|Default|SetbDowned true)
  (Class|AICharacterBaseCHARACTER|DisableNPC) ; Disabling NPC perception and behaviours
  (CallFunction|NetDownedHitbox))

(fn OnDestroy
  ;[1 1 1] Destroy item traces that will no longer be in use after the owning ai is destroyed
  (for _array_element (.itemmemory (Variables|/Game/AI/NPC/BP_AIControllerBase_AICONTROLLER.BP_AIControllerBase_AICONTROLLER_C|GetMemory (.AsBP%20AIController%20Base%20AICONTROLLER (Utilities|Casting|CastToBP_AIControllerBase_AICONTROLLER (AI|GetAIController 0)))))
    (Actor|DestroyActor (.tracereference _array_element))))

(fn DebugDisplayUpdate
  (bind _returnvalue (Game|GetPlayerCharacter 0))
  (Utilities|IsValid _returnvalue
    (:Is%20Valid
      (Transformation|SetWorldRotation (Variables|Default|GetDebugName) (Math|Rotator|FindLookatRotation (Transformation|GetWorldLocation (Variables|Default|GetDebugName)) (Transformation|GetWorldLocation (Variables|/Game/Player/BP_Player_CHARACTER.BP_Player_CHARACTER_C|GetCamera (.AsBP%20Player%20CHARACTER (Utilities|Casting|CastToBP_Player_CHARACTER _returnvalue))))) false false) ; Look at player camera
    )))

(fn UpdateDetection
  (bind _returnvalue (AI|GetBlackboard 0))
  (if (Networking|IsServer)
    (Utilities|IsValid _returnvalue
      (:Is%20Valid
        (Variables|Default|SetNetDetection (Math|Float|Round (Class|BlackboardComponent|GetValueasFloat _returnvalue (Utilities|Name|MakeLiteralName "Detection"))))))))

(fn OnRepNetDetection
  (Rendering|Components|TextRender|SetText (Variables|Default|GetDebugDetection) (Utilities|Text|ToText(Integer) (Variables|Default|GetNetDetection))))

(fn GetCenter
  (return (Transformation|GetWorldLocation (Variables|Default|GetBehindCollision))))

(fn GetInteractText
  (return "Pickpocket"))