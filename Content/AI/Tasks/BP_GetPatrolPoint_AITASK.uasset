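; Behavior tree task that gives an AI pawn its current patrol destination along its assigned patrol route.
; It reads the DesignatedRoute actor and LastPatrolPoint index from the blackboard, then writes that path point to PatrolLocation.
; Points are converted from relative to world space by adding the route actor's location, ignoring rotation.
; The task fails once the index reaches the path's end and does not advance the index itself.
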(event EventReceiveExecuteAI
  (params (OwnerController :type AI%20Controller%20Object%20Reference) (ControlledPawn :type Pawn%20Object%20Reference))
  (bind _returnvalue (AI|GetBlackboard ControlledPawn))
  (bind _returnvalue_2 (Utilities|Name|MakeLiteralName "DesignatedRoute"))
  (bind _returnvalue_3 (Utilities|Name|MakeLiteralName "LastPatrolPoint"))
  (bind _returnvalue_4 (AI|Components|Blackboard|GetValueasObject _returnvalue _returnvalue_2))
  (bind _returnvalue_5 (Class|BlackboardComponent|GetValueasInt _returnvalue _returnvalue_3))
  (bind _asbp_patrol_route (Utilities|Casting|CastToBP_PatrolRoute _returnvalue_4))
  (bind _path (Variables|/Game/AI/NPC/Guard/BP_PatrolRoute.BP_PatrolRoute_C|GetPath _asbp_patrol_route))
  (if (> (Utilities|Array|Length _path) _returnvalue_5) ; Checking if we are at the end of the path
    (AI|BehaviorTree|SetBlackboardValueasVector (Variables|Default|GetPatrolLocation) (+ (Transformation|GetActorLocation _asbp_patrol_route) (Utilities|Array|Get(acopy) _path _returnvalue_5)))
    (AI|BehaviorTree|FinishExecute true)
    (else
      (AI|BehaviorTree|FinishExecute false))))