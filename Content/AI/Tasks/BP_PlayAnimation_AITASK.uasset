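; Behavior tree task that plays an animation on an AI character as a dynamic montage in the default slot.
; It mirrors playback through the character's NetPlayAnimation and finishes successfully when that specific montage ends, whether interrupted or not.
; On abort it blends the montage out, calls NetStopAnimation and reports success through FinishExecute rather than FinishAbort.
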(event Custom|MontageFinished
  (params (Montage :type Anim%20Montage%20Object%20Reference) (bInterrupted :type Boolean))
  (if (== Montage (stale EventReceiveExecuteAI _returnvalue_2)) ; Finish if correct montage is done
    (AI|BehaviorTree|FinishExecute true)))

(event EventReceiveExecuteAI
  (params (OwnerController :type AI%20Controller%20Object%20Reference) (ControlledPawn :type Pawn%20Object%20Reference))
  (bind _asbp_aicharacter_base_character (Utilities|Casting|CastToBP_AICharacterBase_CHARACTER ControlledPawn))
  (bind _mesh (Variables|/Script/Engine.Character|GetMesh _asbp_aicharacter_base_character))
  (bind _returnvalue (Components|SkeletalMesh|GetAnimInstance _mesh))
  (bind _returnvalue_2 (Class|AnimInstance|PlaySlotAnimationasDynamicMontage _returnvalue (Variables|Default|GetAnimation) "DefaultSlot" 0.25 0.25 1.0 1 -1.0 0.0)) ; Play animation as dynamic montage
  (EventDispatchers|BindEventtoOnMontageEnded _returnvalue (delegate Custom|MontageFinished))
  (Default|NetPlayAnimation _asbp_aicharacter_base_character (Variables|Default|GetAnimation)))

(event EventReceiveAbortAI
  (params (OwnerController :type AI%20Controller%20Object%20Reference) (ControlledPawn :type Pawn%20Object%20Reference))
  (Animation|Montage|MontageStop (Components|SkeletalMesh|GetAnimInstance (Variables|/Script/Engine.Character|GetMesh (.AsBP%20AICharacter%20Base%20CHARACTER (Utilities|Casting|CastToBP_AICharacterBase_CHARACTER (stale EventReceiveExecuteAI ControlledPawn))))) 0.25 (stale EventReceiveExecuteAI _returnvalue_2))
  (Default|NetStopAnimation (.AsBP%20AICharacter%20Base%20CHARACTER (Utilities|Casting|CastToBP_AICharacterBase_CHARACTER (stale EventReceiveExecuteAI ControlledPawn))))
  (AI|BehaviorTree|FinishExecute true))