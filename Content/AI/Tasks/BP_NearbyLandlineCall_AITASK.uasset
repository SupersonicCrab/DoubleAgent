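; BP_NearbyLandlineCall_AITASK is an AI behavior tree task that makes the controlled pawn call for backup through a nearby landline.
; It box-overlaps WorldDynamic objects around the pawn, filtered to Landline_BP, and calls CallBackup on the first result without ranking by distance.
; The task finishes as failed whether or not a landline is found, so it never reports success to the tree.
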(event EventReceiveExecuteAI
  (params (OwnerController :type AI%20Controller%20Object%20Reference) (ControlledPawn :type Pawn%20Object%20Reference))
  ;[1 1 1] Get overlapping landlines
  (bind _outactors (Collision|BoxOverlapActors (Transformation|GetActorLocation ControlledPawn) "1000.000000,1000.000000,1000.000000" (Utilities|Array|MakeArray "ObjectTypeQuery2") "/Game/SecuritySystem/Landlines/Landline_BP.Landline_BP_C" :!class /Script/Engine.KismetSystemLibrary))
  ;[1 1 1] Ensure a landline was found
  (if (!= (Utilities|Array|Length _outactors) 0)
    ;[1 1 1] Call for backup
    (Default|CallBackup (.AsLandline%20BP (Utilities|Casting|CastToLandline_BP (Utilities|Array|Get(acopy) _outactors))))
    (AI|BehaviorTree|FinishExecute false)
    (else
      ;[1 1 1] Fail if no landlines found
      (AI|BehaviorTree|FinishExecute false))))