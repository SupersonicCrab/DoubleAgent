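; Behaviour tree task that revives the unconscious NPC stored in the executing AI's blackboard.
; It resumes that NPC's montages and plays a getting-up animation as a dynamic slot montage, failing if the blackboard target is not an AI character.
; When that montage ends, it clears the downed state, restores the standing hitbox, re-enables the NPC and resets its detection, vocal and suspicion blackboard keys before finishing successfully.
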(event Custom|MontageFinished
  (params (Montage :type Anim%20Montage%20Object%20Reference) (bInterrupted :type Boolean))
  (if (== Montage (stale EventReceiveExecuteAI _returnvalue))
    (Variables|/Game/AI/NPC/BP_AICharacterBase_CHARACTER.BP_AICharacterBase_CHARACTER_C|SetbDowned (stale EventReceiveExecuteAI _asbp_aicharacter_base_character) false)
    (Default|StandingHitbox (stale EventReceiveExecuteAI _asbp_aicharacter_base_character))
    (Default|EnableNPC (stale EventReceiveExecuteAI _asbp_aicharacter_base_character)) ; Turning on perception and behaviour
    ;[1 1 1] Updating blackboard
    (AI|Components|Blackboard|SetValueasFloat (AI|GetBlackboard (stale EventReceiveExecuteAI _asbp_aicharacter_base_character)) (Utilities|Name|MakeLiteralName "Detection") 9e+01)
    (AI|Components|Blackboard|SetValueasEnum (AI|GetBlackboard (stale EventReceiveExecuteAI _asbp_aicharacter_base_character)) (Utilities|Name|MakeLiteralName "VocalStatus") (Utilities|Enum|LiteralenumEVocalStatus "NewEnumerator6"))
    (AI|Components|Blackboard|SetValueasBool (AI|GetBlackboard (stale EventReceiveExecuteAI _asbp_aicharacter_base_character)) (Utilities|Name|MakeLiteralName "CanSeePlayer") false)
    (AI|Components|Blackboard|SetValueasBool (AI|GetBlackboard (stale EventReceiveExecuteAI _asbp_aicharacter_base_character)) (Utilities|Name|MakeLiteralName "Suspicious") false)
    (AI|BehaviorTree|FinishExecute true)))

(event EventReceiveExecuteAI
  (params (OwnerController :type AI%20Controller%20Object%20Reference) (ControlledPawn :type Pawn%20Object%20Reference))
  (bind _asbp_aicharacter_base_character (Utilities|Casting|CastToBP_AICharacterBase_CHARACTER (AI|Components|Blackboard|GetValueasObject (AI|GetBlackboard OwnerController) (Utilities|Name|MakeLiteralName "UnconsciousNPC")))
    (:then
      (Class|AnimInstance|MontageResume (Components|SkeletalMesh|GetAnimInstance (Variables|/Script/Engine.Character|GetMesh _asbp_aicharacter_base_character))) ; Resuming montages to resume animations
      (bind _returnvalue (Class|AnimInstance|PlaySlotAnimationasDynamicMontage (Components|SkeletalMesh|GetAnimInstance (Variables|/Script/Engine.Character|GetMesh _asbp_aicharacter_base_character)) "/Game/Animations/Sequences/Standing/A_GettingUp.A_GettingUp" "DefaultSlot" 0.25 0.25 1.0 1 -1.0 0.0)) ; Getting up animation
      (EventDispatchers|BindEventtoOnMontageEnded (Components|SkeletalMesh|GetAnimInstance (Variables|/Script/Engine.Character|GetMesh _asbp_aicharacter_base_character)) (delegate Custom|MontageFinished)))
    (:CastFailed
      (AI|BehaviorTree|FinishExecute false))))