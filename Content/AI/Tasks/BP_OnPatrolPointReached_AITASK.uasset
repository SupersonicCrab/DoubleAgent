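; Behavior tree task that advances an AI pawn to the next point on its designated patrol route once it reaches one.
; It reads the route, point index and reverse flag from the Blackboard, then steps the index forward or backward.
; At the last point, the route's end behaviour either restarts at the first point or reverses direction.
; Reaching the start in reverse clears the flag, leaves the index at zero, and the task always succeeds.
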(event EventReceiveExecuteAI
  (params (OwnerController :type AI%20Controller%20Object%20Reference) (ControlledPawn :type Pawn%20Object%20Reference))
  (bind _returnvalue (AI|GetBlackboard ControlledPawn))
  (Variables|Default|SetSavedBlackboard _returnvalue)
  (Variables|Default|SetPatrolRoute (.AsBP%20Patrol%20Route (Utilities|Casting|CastToBP_PatrolRoute (AI|Components|Blackboard|GetValueasObject _returnvalue (Utilities|Name|MakeLiteralName "DesignatedRoute")))))
  (Variables|Default|SetCurrentPatrolPoint (Class|BlackboardComponent|GetValueasInt _returnvalue (Utilities|Name|MakeLiteralName "LastPatrolPoint")))
  (if (ScalableFloat|GetValueasBool _returnvalue (Utilities|Name|MakeLiteralName "PatrolReverse"))
    (CallFunction|ReverseBehaviour)
    (else
      (CallFunction|ForwardBehaviour)))
  (AI|BehaviorTree|FinishExecute true))

(fn ReverseBehaviour
  (bind _savedblackboard (Variables|Default|GetSavedBlackboard))
  (if (== (Variables|Default|GetCurrentPatrolPoint) 0) ; If reached start of patrol
    (AI|Components|Blackboard|SetValueasBool _savedblackboard (Utilities|Name|MakeLiteralName "PatrolReverse") false)
    (Class|BlackboardComponent|SetValueasInt _savedblackboard (Utilities|Name|MakeLiteralName "LastPatrolPoint"))
    (else
      (Class|BlackboardComponent|SetValueasInt _savedblackboard (Utilities|Name|MakeLiteralName "LastPatrolPoint") (- (Variables|Default|GetCurrentPatrolPoint) 1)))))

(fn ForwardBehaviour
  (bind _returnvalue (Utilities|Name|MakeLiteralName "LastPatrolPoint"))
  (bind _patrolroute (Variables|Default|GetPatrolRoute))
  (bind _savedblackboard (Variables|Default|GetSavedBlackboard))
  (if (== (Utilities|Array|LastIndex (Variables|/Game/AI/Patrol/BP_PatrolRoute.BP_PatrolRoute_C|GetPath _patrolroute)) (Variables|Default|GetCurrentPatrolPoint)) ; If reached end of patrol
    (switch Utilities|FlowControl|Switch|SwitchonEEndBehaviour (Variables|/Game/AI/Patrol/BP_PatrolRoute.BP_PatrolRoute_C|GetEndBehaviour _patrolroute)
      (:NewEnumerator0
        (Class|BlackboardComponent|SetValueasInt _savedblackboard _returnvalue))
      (:NewEnumerator1
        (AI|Components|Blackboard|SetValueasBool _savedblackboard (Utilities|Name|MakeLiteralName "PatrolReverse") true)
        (Class|BlackboardComponent|SetValueasInt _savedblackboard _returnvalue (- (Variables|Default|GetCurrentPatrolPoint) 1))))
    (else
      (Class|BlackboardComponent|SetValueasInt _savedblackboard _returnvalue (+ (Variables|Default|GetCurrentPatrolPoint) 1)))))