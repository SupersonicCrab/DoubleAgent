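; Behavior tree task that finds the closest search location for an AI and stores it in the blackboard.
; On execute it runs an EQS query for a single best point, with the owner controller as querier.
; When the query finishes, a small sphere overlap at that point resolves the BP_SearchLocation actor and writes it to the SearchLocation key.
; The task fails if the query or the overlap finds nothing.
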(event Custom|OnQueryFinished
  (params (QueryInstance :type Env%20Query%20Instance%20Blueprint%20Wrapper%20Object%20Reference) (QueryStatus :type EEnvQueryStatus%20Enum :default "Processing"))
  (bind (_resultlocations _returnvalue) (AI|EQS|GetQueryResultsasLocations QueryInstance))
  (if _returnvalue
    (bind (_outactors _returnvalue_2) (Collision|SphereOverlapActors (Utilities|Array|Get(acopy) _resultlocations) 1e+01 (Utilities|Array|MakeArray "ObjectTypeQuery1") "/Game/AI/SearchSystem/BP_SearchLocation.BP_SearchLocation_C"))
    (if _returnvalue_2
      (bind _asbp_search_location (Utilities|Casting|CastToBP_SearchLocation (Utilities|Array|Get(acopy) _outactors)))
      (Class|BTFunctionLibrary|SetBlackboardValueasObject (Variables|Default|GetSearchLocation) _asbp_search_location)
      (AI|BehaviorTree|FinishExecute true)
      (else
        (AI|BehaviorTree|FinishExecute false :!label _label)))
    (else
      (goto _label))))

(event EventReceiveExecuteAI
  (params (OwnerController :type AI%20Controller%20Object%20Reference) (ControlledPawn :type Pawn%20Object%20Reference))
  (bind _returnvalue (AI|EQS|RunEQSQuery (Variables|Default|GetEQSBehaviour) OwnerController "SingleResult"))
  (EventDispatchers|BindEventtoOnQueryFinishedEvent _returnvalue (delegate Custom|OnQueryFinished)))