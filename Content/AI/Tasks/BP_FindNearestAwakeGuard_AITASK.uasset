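; Behavior tree task that looks for the nearest awake guard and stores it in the Guard blackboard key.
; It runs the FindNearestGuard EQS query from the controlled pawn, then walks all results until one has a running AI brain component, which counts as awake.
; The loop's final element is written even if none is awake, and the task finishes with the success flag from fetching the query results.
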(event Custom|OnQueryFinished
  (params (QueryInstance :type Env%20Query%20Instance%20Blueprint%20Wrapper%20Object%20Reference) (QueryStatus :type EEnvQueryStatus%20Enum :default "Processing"))
  (bind (_resultactors _returnvalue) (AI|EQS|GetQueryResultsasActors QueryInstance))
  (bind _array_element (Utilities|Array|ForEachLoopwithBreak _resultactors :!label _label)
    (:LoopBody
      (bind _asbp_guard_ai_aicontroller (Utilities|Casting|CastToBP_GuardAI_AICONTROLLER _array_element))
      (if (Class|BrainComponent|IsRunning (Variables|/Script/AIModule.AIController|GetBrainComponent (AI|GetAIController _asbp_guard_ai_aicontroller)))
        (goto _label Break)))
    (:Completed
      (Class|BTFunctionLibrary|SetBlackboardValueasObject (Variables|Default|GetGuard) _array_element)
      (AI|BehaviorTree|FinishExecute _returnvalue))))

(event EventReceiveExecuteAI
  (params (OwnerController :type AI%20Controller%20Object%20Reference) (ControlledPawn :type Pawn%20Object%20Reference))
  (bind _returnvalue (AI|EQS|RunEQSQuery "/Game/AI/EQS/Queries/FindNearestGuard_EQSQUERY.FindNearestGuard_EQSQUERY" ControlledPawn "AllMatching"))
  (EventDispatchers|BindEventtoOnQueryFinishedEvent _returnvalue (delegate Custom|OnQueryFinished)))