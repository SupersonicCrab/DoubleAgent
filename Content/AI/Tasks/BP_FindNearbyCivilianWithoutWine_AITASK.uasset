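; Behavior tree task that finds a nearby civilian who is not holding visible wine, for use by an AI-controlled pawn.
; It runs a sphere overlap around the pawn for civilian characters and picks the first whose Wine component is hidden.
; That civilian is written to a blackboard key, and the task finishes with success only if one was found.
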(event EventReceiveExecuteAI
  (params (OwnerController :type AI%20Controller%20Object%20Reference) (ControlledPawn :type Pawn%20Object%20Reference))
  (Variables|Default|SetbFound false)
  (bind _outactors (Collision|SphereOverlapActors (Transformation|GetActorLocation ControlledPawn) (Variables|Default|GetSphere%20Radius) (Utilities|Array|MakeArray "ObjectTypeQuery3") "/Game/AI/NPC/Civilian/BP_Civilian_CHARACTER.BP_Civilian_CHARACTER_C"))
  (bind _array_element (Utilities|Array|ForEachLoopwithBreak _outactors :!label _label)
    (:LoopBody
      (if (not (Rendering|IsVisible (Variables|/Game/AI/NPC/Civilian/BP_Civilian_CHARACTER.BP_Civilian_CHARACTER_C|GetWine (.AsBP%20Civilian%20CHARACTER (Utilities|Casting|CastToBP_Civilian_CHARACTER _array_element)))))
        (Class|BTFunctionLibrary|SetBlackboardValueasObject (Variables|Default|GetCivilian) (.AsBP%20Civilian%20CHARACTER (Utilities|Casting|CastToBP_Civilian_CHARACTER _array_element)))
        (Variables|Default|SetbFound true)
        (goto _label Break)))
    (:Completed
      (AI|BehaviorTree|FinishExecute (Variables|Default|GetbFound)))))