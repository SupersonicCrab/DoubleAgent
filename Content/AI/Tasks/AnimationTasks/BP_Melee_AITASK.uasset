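; Behavior tree task that makes an AI character perform a melee attack, failing if any montage is already playing on its mesh.
; It registers itself with the anim instance as the animation task message target, sets the networked melee flag and reports a normal-range noise event.
; The Finished override clears the melee flag and calls the parent, or fails if the saved character is no longer valid.
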(event EventReceiveExecuteAI
  (params (OwnerController :type AI%20Controller%20Object%20Reference) (ControlledPawn :type Pawn%20Object%20Reference))
  (bind _asbp_aicharacter_base_character (Utilities|Casting|CastToBP_AICharacterBase_CHARACTER ControlledPawn))
  (Variables|Default|SetSavedCharacter _asbp_aicharacter_base_character)
  (if (not (Class|AnimInstance|IsAnyMontagePlaying (Components|SkeletalMesh|GetAnimInstance (Variables|/Script/Engine.Character|GetMesh _asbp_aicharacter_base_character)))) ; Ensure NPC is not playing any montages
    (Class|AnimationControllerINTERFACE|SetAnimationTask(Message) (Components|SkeletalMesh|GetAnimInstance (Variables|/Script/Engine.Character|GetMesh _asbp_aicharacter_base_character)) self)
    (Default|NetSetMelee _asbp_aicharacter_base_character true)
    (Class|AISenseHearing|ReportNoiseEvent (Transformation|GetActorLocation ControlledPawn) 1.0 ControlledPawn (.normal (Utilities|Struct|MakeFSoundType 5e+02 1.5e+03 3.5e+03)) "Noise")
    (else
      (AI|BehaviorTree|FinishExecute false))))

(fn Finished
  (bind _savedcharacter (Variables|Default|GetSavedCharacter))
  (Utilities|IsValid _savedcharacter
    (:Is%20Valid
      (Default|NetSetMelee _savedcharacter false)
      (|CallParentFunction))
    (:Is%20Not%20Valid
      (AI|BehaviorTree|FinishExecute false))))