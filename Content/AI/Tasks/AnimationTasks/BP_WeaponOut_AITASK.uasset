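; Behavior tree task that triggers a weapon-out animation change on an AI character.
; It casts the controlled pawn to BP_AICharacterBase_CHARACTER and fails if a montage is already playing on its mesh.
; Otherwise it messages the anim instance with a reference to itself and the WeaponOut value, leaving the task running without finishing it here.
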(event EventReceiveExecuteAI
  (params (OwnerController :type AI%20Controller%20Object%20Reference) (ControlledPawn :type Pawn%20Object%20Reference))
  (bind _asbp_aicharacter_base_character (Utilities|Casting|CastToBP_AICharacterBase_CHARACTER ControlledPawn))
  (if (not (Class|AnimInstance|IsAnyMontagePlaying (Components|SkeletalMesh|GetAnimInstance (Variables|/Script/Engine.Character|GetMesh _asbp_aicharacter_base_character)))) ; Ensure NPC is not playing any montages
    (Class|AnimationControllerINTERFACE|SetAnimationTask(Message) (Components|SkeletalMesh|GetAnimInstance (Variables|/Script/Engine.Character|GetMesh _asbp_aicharacter_base_character)) self)
    (Class|AnimationControllerINTERFACE|SetWeaponOut(Message) (Components|SkeletalMesh|GetAnimInstance (Variables|/Script/Engine.Character|GetMesh _asbp_aicharacter_base_character)) (Variables|Default|GetbWeaponOut))
    (else
      (AI|BehaviorTree|FinishExecute false))))