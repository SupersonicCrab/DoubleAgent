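; Behavior tree task that has an AI character close the door stored in its Door blackboard key.
; It runs only when no montage is playing, first registering itself with the character's AnimInstance through SetAnimationTaskMessage.
; An open door receives NPCClose with the character and the task succeeds immediately, without waiting for completion.
; A playing montage, invalid door or already closed door fails the task.
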(event EventReceiveExecuteAI
  (params (OwnerController :type AI%20Controller%20Object%20Reference) (ControlledPawn :type Pawn%20Object%20Reference))
  (bind _asbp_aicharacter_base_character (Utilities|Casting|CastToBP_AICharacterBase_CHARACTER ControlledPawn))
  (if (not (Class|AnimInstance|IsAnyMontagePlaying (Components|SkeletalMesh|GetAnimInstance (Variables|/Script/Engine.Character|GetMesh _asbp_aicharacter_base_character)))) ; Ensure NPC is not playing any montages
    (Class|AnimationControllerINTERFACE|SetAnimationTask(Message) (Components|SkeletalMesh|GetAnimInstance (Variables|/Script/Engine.Character|GetMesh _asbp_aicharacter_base_character)) self)
    (bind _asbp_door (Utilities|Casting|CastToBP_Door (Class|BTFunctionLibrary|GetBlackboardValueasObject (Variables|Default|GetDoor)))
      (:then
        (if (Variables|/Game/Interactable/Door/BP_Door.BP_Door_C|GetDoorOpen _asbp_door)
          (Default|NPCClose _asbp_door (.AsBP%20AICharacter%20Base%20CHARACTER (Utilities|Casting|CastToBP_AICharacterBase_CHARACTER ControlledPawn)))
          (AI|BehaviorTree|FinishExecute true)
          (else
            (AI|BehaviorTree|FinishExecute false :!label _label))))
      (:CastFailed
        (goto _label)))
    (else
      (AI|BehaviorTree|FinishExecute false))))