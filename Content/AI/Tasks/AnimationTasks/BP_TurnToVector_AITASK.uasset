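; Behavior tree task that turns an AI character toward a Blackboard vector through its animation instance.
; It fails if a montage is playing or the vector is zero, and succeeds immediately if the look-at yaw is zero.
; Otherwise it messages the anim instance, disables controller-desired rotation and snaps control yaw to the target.
; The Finished override restores controller-desired rotation.
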(event EventReceiveExecuteAI
  (params (OwnerController :type AI%20Controller%20Object%20Reference) (ControlledPawn :type Pawn%20Object%20Reference))
  (bind _vector (Variables|Default|GetVector))
  (bind _returnvalue (Class|BTFunctionLibrary|GetBlackboardValueasVector _vector))
  (bind _asbp_aicharacter_base_character (Utilities|Casting|CastToBP_AICharacterBase_CHARACTER ControlledPawn))
  (if (not (Class|AnimInstance|IsAnyMontagePlaying (Components|SkeletalMesh|GetAnimInstance (Variables|/Script/Engine.Character|GetMesh _asbp_aicharacter_base_character)))) ; Ensure NPC is not playing any montages
    (Class|AnimationControllerINTERFACE|SetAnimationTask(Message) (Components|SkeletalMesh|GetAnimInstance (Variables|/Script/Engine.Character|GetMesh _asbp_aicharacter_base_character)) self)
    (if (Math|Vector|NotEqual(Vector) _returnvalue "0, 0, 0" 0.0001) ; If vector is not 0,0,0
      (Utilities|IsValid (Variables|/Script/Engine.Character|GetCharacterMovement _asbp_aicharacter_base_character)
        (:Is%20Valid
          (if (> (Math|Float|Absolute(Float) (.yaw (Math|Rotator|FindLookatRotation (Transformation|GetActorLocation _asbp_aicharacter_base_character) _returnvalue))) 0.0) ; If not already looking at target
            (Class|AnimationControllerINTERFACE|SetTurnto(Message) (Components|SkeletalMesh|GetAnimInstance (Variables|/Script/Engine.Character|GetMesh _asbp_aicharacter_base_character)) _returnvalue)
            (bind _output_get (Variables|Default|SetSavedCharacterMovement (Variables|/Script/Engine.Character|GetCharacterMovement _asbp_aicharacter_base_character)))
            (Variables|/Script/Engine.CharacterMovementComponent|SetbUseControllerDesiredRotation _output_get false) ; Disable controller rotation
            (Pawn|SetControlRotation OwnerController (Math|Rotator|MakeRotator 0.0 0.0 (.yaw (Math|Rotator|FindLookatRotation (Transformation|GetActorLocation _asbp_aicharacter_base_character) _returnvalue)))) ; Reorient controller
            (else
              (AI|BehaviorTree|FinishExecute true))))
        (:Is%20Not%20Valid
          (AI|BehaviorTree|FinishExecute false :!label _label)))
      (else
        (goto _label)))
    (else
      (AI|BehaviorTree|FinishExecute false))))

(fn Finished
  (Variables|/Script/Engine.CharacterMovementComponent|SetbUseControllerDesiredRotation (Variables|Default|GetSavedCharacterMovement) true) ; Enable controller rotation
  (|CallParentFunction))