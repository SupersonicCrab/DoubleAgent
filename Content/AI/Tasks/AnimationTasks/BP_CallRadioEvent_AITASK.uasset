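; Behavior tree task that makes an AI character send a radio event through the level's BP_RadioHub.
; It fails if a montage is playing on the NPC; otherwise it registers itself with the anim instance and passes event, blackboard location, delay and NPC to the hub.
; A timer finishes the task successfully after the delay, allowing time for the voice line; the radio animation is still a TODO.
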(event Custom|PostDelay
  ;[1 1 1] Delaying execution untill voiceline has been spoken
  (AI|BehaviorTree|FinishExecute true))

(event EventReceiveExecuteAI
  (params (OwnerController :type AI%20Controller%20Object%20Reference) (ControlledPawn :type Pawn%20Object%20Reference))
  (bind _delay (Variables|Default|GetDelay))
  ;[1 1 1] Todo: Add radio animation
  (bind _asbp_aicharacter_base_character (Utilities|Casting|CastToBP_AICharacterBase_CHARACTER ControlledPawn))
  (if (not (Class|AnimInstance|IsAnyMontagePlaying (Components|SkeletalMesh|GetAnimInstance (Variables|/Script/Engine.Character|GetMesh _asbp_aicharacter_base_character)))) ; Ensure NPC is not playing any montages
    (Class|AnimationControllerINTERFACE|SetAnimationTask(Message) (Components|SkeletalMesh|GetAnimInstance (Variables|/Script/Engine.Character|GetMesh _asbp_aicharacter_base_character)) self)
    ;[1 1 1] Sending radio event to radio hub
    (bind _returnvalue (Actor|GetActorOfClass "/Game/SecuritySystem/Radio/BP_RadioHub.BP_RadioHub_C"))
    (Default|SendRadioEvent _returnvalue (Utilities|Struct|MakeFRadioEvent (Variables|Default|GetRadioEvent) (Class|BTFunctionLibrary|GetBlackboardValueasVector (Variables|Default|GetLocation)) _delay _asbp_aicharacter_base_character))
    ;[1 1 1] Delaying execution untill voiceline has been spoken
    (Utilities|Time|SetTimerbyEvent (delegate Custom|PostDelay) _delay)
    (else
      (AI|BehaviorTree|FinishExecute false))))