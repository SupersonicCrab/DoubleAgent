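; Behavior tree task that makes a guard fire its pistol at the LastPlayer blackboard target.
; It line-traces along the barrel sockets over the target's distance, damaging a hit player before checking montages.
; Player hits and misses pass the task to the anim instance for shooting, failing if a montage plays; other hits or no target also fail.
; The Finished callback reports a loud noise, decrements blackboard ammo and succeeds.
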(event EventReceiveExecuteAI
  (params (OwnerController :type AI%20Controller%20Object%20Reference) (ControlledPawn :type Pawn%20Object%20Reference))
  (bind _returnvalue (AI|GetBlackboard ControlledPawn))
  (bind _returnvalue_2 (Utilities|Name|MakeLiteralName "LastPlayer"))
  (bind _returnvalue_3 (AI|Components|Blackboard|GetValueasObject _returnvalue _returnvalue_2))
  (Variables|Default|SetSavedPawn ControlledPawn) ; Saving pawn to reference in finished function
  (bind _asbp_guard_character (Utilities|Casting|CastToBP_Guard_CHARACTER ControlledPawn))
  ;[1 1 1] Shoot ray at player
  (Utilities|IsValid _returnvalue_3
    (:Is%20Valid
      (bind _outhit (Collision|LineTraceByChannel (.location (Transformation|GetSocketTransform (Variables|/Game/AI/NPC/Guard/BP_Guard_CHARACTER.BP_Guard_CHARACTER_C|GetPistolHand _asbp_guard_character) "GunBack" "RTS_World")) (+ (* (Math|Vector|GetForwardVector (Math|Rotator|FindLookatRotation (.location (Transformation|GetSocketTransform (Variables|/Game/AI/NPC/Guard/BP_Guard_CHARACTER.BP_Guard_CHARACTER_C|GetPistolHand _asbp_guard_character) "GunBack" "RTS_World")) (.location (Transformation|GetSocketTransform (Variables|/Game/AI/NPC/Guard/BP_Guard_CHARACTER.BP_Guard_CHARACTER_C|GetPistolHand _asbp_guard_character) "GunFront" "RTS_World")))) (Transformation|GetDistanceTo (.AsActor (Utilities|Casting|CastToActor _returnvalue_3)) ControlledPawn)) (.location (Transformation|GetSocketTransform (Variables|/Game/AI/NPC/Guard/BP_Guard_CHARACTER.BP_Guard_CHARACTER_C|GetPistolHand _asbp_guard_character) "GunFront" "RTS_World"))) "TraceTypeQuery2" false 0 "ForDuration"))
      ;[1 1 1] Handling player collision
      (if (.bBlockingHit (Collision|BreakHitResult _outhit))
        (bind _asbp_player_character (Utilities|Casting|CastToBP_Player_CHARACTER (.HitActor (Collision|BreakHitResult _outhit)))
          (:then
            (Default|LoseHealth (Variables|/Game/Player/BP_Player_CHARACTER.BP_Player_CHARACTER_C|GetHealthComponent _asbp_player_character) (Variables|Default|GetDamage))
            ;[1 1 1] Calling shooting animation
            (if (not (Class|AnimInstance|IsAnyMontagePlaying (Components|SkeletalMesh|GetAnimInstance (Variables|/Script/Engine.Character|GetMesh _asbp_guard_character)))) :!label _label ; Ensure NPC is not playing any montages
              (Class|AnimationControllerINTERFACE|SetAnimationTask(Message) (Components|SkeletalMesh|GetAnimInstance (Variables|/Script/Engine.Character|GetMesh _asbp_guard_character)) self)
              (Class|AnimationControllerINTERFACE|Shoot(Message) (Components|SkeletalMesh|GetAnimInstance (Variables|/Script/Engine.Character|GetMesh _asbp_guard_character)))
              (else
                (AI|BehaviorTree|FinishExecute false))))
          (:CastFailed
            (AI|BehaviorTree|FinishExecute false) ; Return false if shot hit anything other then a player
          ))
        (else
          (goto _label))))
    (:Is%20Not%20Valid
      (AI|BehaviorTree|FinishExecute false))))

(fn Finished
  (bind _returnvalue (Utilities|Name|MakeLiteralName "Ammo"))
  (bind _savedpawn (Variables|Default|GetSavedPawn))
  (bind _returnvalue_2 (AI|GetBlackboard _savedpawn))
  (Class|AISenseHearing|ReportNoiseEvent (Transformation|GetWorldLocation (Variables|/Game/AI/NPC/Guard/BP_Guard_CHARACTER.BP_Guard_CHARACTER_C|GetPistolHand (.AsBP%20Guard%20CHARACTER (Utilities|Casting|CastToBP_Guard_CHARACTER _savedpawn)))) 1.0 _savedpawn 0.0 "LoudNoise") ; Making noise at the guns location
  (Class|BlackboardComponent|SetValueasInt _returnvalue_2 _returnvalue (- (Class|BlackboardComponent|GetValueasInt _returnvalue_2 _returnvalue) 1)) ; Decrement ammo
  (AI|BehaviorTree|FinishExecute true))