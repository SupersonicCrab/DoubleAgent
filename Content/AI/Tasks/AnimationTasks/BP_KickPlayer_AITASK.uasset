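; A behavior tree task that makes an AI character turn toward the LastPlayer blackboard target and kick it.
; It fails if the player is invalid or a montage is already playing; otherwise it registers itself with the anim instance and plays a networked kick animation.
; The Finished callback deals health damage and succeeds only if the right-foot socket is within range of the player, failing otherwise.
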(event EventReceiveExecuteAI
  (params (OwnerController :type AI%20Controller%20Object%20Reference) (ControlledPawn :type Pawn%20Object%20Reference))
  (bind _lastplayer (Variables|Default|GetLastPlayer))
  (bind _returnvalue (AI|BehaviorTree|GetBlackboardValueasActor _lastplayer))
  (bind _output_get (Variables|Default|SetPlayer _returnvalue))
  (Utilities|IsValid _output_get
    (:Is%20Valid
      (Transformation|SetActorRotation ControlledPawn (Math|Rotator|MakeRotator 0.0 0.0 (.yaw (Math|Rotator|FindLookatRotation (Transformation|GetActorLocation ControlledPawn) (Transformation|GetActorLocation _returnvalue)))))
      (bind _asbp_aicharacter_base_character (Utilities|Casting|CastToBP_AICharacterBase_CHARACTER ControlledPawn))
      (Variables|Default|SetSavedCharacter _asbp_aicharacter_base_character)
      (if (not (Class|AnimInstance|IsAnyMontagePlaying (Components|SkeletalMesh|GetAnimInstance (Variables|/Script/Engine.Character|GetMesh _asbp_aicharacter_base_character)))) ; Ensure NPC is not playing any montages
        (Class|AnimationControllerINTERFACE|SetAnimationTask(Message) (Components|SkeletalMesh|GetAnimInstance (Variables|/Script/Engine.Character|GetMesh _asbp_aicharacter_base_character)) self)
        (Default|NetPlayAnimation _asbp_aicharacter_base_character "/Game/Animations/Sequences/Standing/Melee/A_Kicking.A_Kicking" 0.25 0.25 0.0)
        (else
          (AI|BehaviorTree|FinishExecute false))))
    (:Is%20Not%20Valid
      (AI|BehaviorTree|FinishExecute false))))

(fn Finished
  (bind _player (Variables|Default|GetPlayer))
  (if (<= (Math|Vector|Distance(Vector) (Transformation|GetSocketLocation (Variables|/Script/Engine.Character|GetMesh (Variables|Default|GetSavedCharacter)) "Foot_R") (Transformation|GetActorLocation _player)) 75.0)
    (Default|LoseHealth (Variables|/Game/Player/BP_Player_CHARACTER.BP_Player_CHARACTER_C|GetHealthComponent (.AsBP%20Player%20CHARACTER (Utilities|Casting|CastToBP_Player_CHARACTER _player))) (Variables|Default|GetDamage) (Variables|Default|GetAttacker%20Name))
    (AI|BehaviorTree|FinishExecute true)
    (else
      (AI|BehaviorTree|FinishExecute false))))