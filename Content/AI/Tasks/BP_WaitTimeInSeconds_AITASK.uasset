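; Behavior tree task that makes an AI wait for a number of seconds read from a float blackboard key.
; On execute it starts a one-shot timer that finishes the task successfully, or succeeds at once when the value is zero.
; An abort clears the timer and finishes the task as failed via FinishExecute rather than FinishAbort.
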(event Custom|WaitFinished
  (AI|BehaviorTree|FinishExecute true))

(event EventReceiveExecuteAI
  (params (OwnerController :type AI%20Controller%20Object%20Reference) (ControlledPawn :type Pawn%20Object%20Reference))
  (bind _timetowaitfloat (Variables|Default|GetTimeToWaitFloat))
  (bind _returnvalue (Class|BTFunctionLibrary|GetBlackboardValueasFloat _timetowaitfloat))
  (if (!= _returnvalue 0.0)
    (bind _returnvalue_2 (Utilities|Time|SetTimerbyEvent (delegate Custom|WaitFinished) _returnvalue))
    (else
      (AI|BehaviorTree|FinishExecute true))))

(event EventReceiveAbortAI
  (params (OwnerController :type AI%20Controller%20Object%20Reference) (ControlledPawn :type Pawn%20Object%20Reference))
  (Utilities|Time|ClearandInvalidateTimerbyHandle (stale EventReceiveExecuteAI _returnvalue_2))
  (AI|BehaviorTree|FinishExecute false))