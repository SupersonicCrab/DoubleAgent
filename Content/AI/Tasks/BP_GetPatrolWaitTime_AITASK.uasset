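; Behavior tree task that sets how long an AI waits at its current patrol point.
; On execute it reads the DesignatedRoute patrol route and LastPatrolPoint index from the pawn's blackboard.
; It copies that path entry's WaitTime into a blackboard float and finishes successfully.
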(event EventReceiveExecuteAI
  (params (OwnerController :type AI%20Controller%20Object%20Reference) (ControlledPawn :type Pawn%20Object%20Reference))
  (bind _returnvalue (AI|GetBlackboard ControlledPawn))
  (Class|BTFunctionLibrary|SetBlackboardValueasFloat (Variables|Default|GetWaitTime) (.WaitTime (Utilities|Struct|BreakFPatrol (Utilities|Array|Get(acopy) (Variables|/Game/AI/Patrol/BP_PatrolRoute.BP_PatrolRoute_C|GetPath (.AsBP%20Patrol%20Route (Utilities|Casting|CastToBP_PatrolRoute (AI|Components|Blackboard|GetValueasObject _returnvalue (Utilities|Name|MakeLiteralName "DesignatedRoute"))))) (Class|BlackboardComponent|GetValueasInt _returnvalue (Utilities|Name|MakeLiteralName "LastPatrolPoint"))))))
  (AI|BehaviorTree|FinishExecute true))