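; Behavior tree task that finds an actor at a location stored in a blackboard vector key.
; It runs a sphere overlap with a configurable radius, object type and class filter around that point.
; The first overlapping actor is written to a blackboard object key, and the task succeeds only if one is found.
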(event EventReceiveExecuteAI
  (params (OwnerController :type AI%20Controller%20Object%20Reference) (ControlledPawn :type Pawn%20Object%20Reference))
  (bind (_outactors _returnvalue) (Collision|SphereOverlapActors (Class|BTFunctionLibrary|GetBlackboardValueasVector (Variables|Default|GetVector)) (Variables|Default|GetRadius) (Utilities|Array|MakeArray (Variables|Default|GetObjectType)) (Variables|Default|GetClassFilter))) ; Overlap at location searching for actor
  (if _returnvalue
    (Class|BTFunctionLibrary|SetBlackboardValueasObject (Variables|Default|GetActor) (Utilities|Array|Get(acopy) _outactors)) ; Set actor if found
  )
  (AI|BehaviorTree|FinishExecute _returnvalue))