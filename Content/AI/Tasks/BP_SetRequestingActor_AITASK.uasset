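; Behavior tree task that lets an AI pawn register itself as the requesting actor on a waiter AI.
; It reads the waiter controller from the pawn's "Waiter" blackboard key, then checks that waiter's own blackboard for an empty RequestingActor and a true HoldingItem.
; If both hold, it writes the pawn into RequestingActor and succeeds, otherwise it fails.
; A failed controller cast leaves the task unfinished.
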(event EventReceiveExecuteAI
  (params (OwnerController :type AI%20Controller%20Object%20Reference) (ControlledPawn :type Pawn%20Object%20Reference))
  (bind _returnvalue (Utilities|Name|MakeLiteralName "RequestingActor"))
  (bind _asbp_waiter_ai_aicontroller (Utilities|Casting|CastToBP_WaiterAI_AICONTROLLER (AI|Components|Blackboard|GetValueasObject (AI|GetBlackboard ControlledPawn) (Utilities|Name|MakeLiteralName "Waiter"))))
  (if (and (== (AI|Components|Blackboard|GetValueasObject (AI|GetBlackboard _asbp_waiter_ai_aicontroller) _returnvalue) 0) (ScalableFloat|GetValueasBool (AI|GetBlackboard _asbp_waiter_ai_aicontroller) (Utilities|Name|MakeLiteralName "HoldingItem")))
    (AI|Components|Blackboard|SetValueasObject (AI|GetBlackboard _asbp_waiter_ai_aicontroller) _returnvalue ControlledPawn)
    (AI|BehaviorTree|FinishExecute true)
    (else
      (AI|BehaviorTree|FinishExecute false))))