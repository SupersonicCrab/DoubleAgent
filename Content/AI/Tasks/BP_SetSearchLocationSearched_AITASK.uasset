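; Behavior tree task that marks a search location as searched for a staff AI.
; It reads the TempObject blackboard key, casts it to SearchLocation and adds it to the StaffAIController's SearchedLocations array if not already there.
; The task finishes successfully for a valid location, including one already recorded, and fails when the object is invalid or not a SearchLocation.
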(event EventReceiveExecuteAI
  (params (OwnerController :type AI%20Controller%20Object%20Reference) (ControlledPawn :type Pawn%20Object%20Reference))
  (bind _returnvalue (AI|GetBlackboard ControlledPawn))
  (bind _returnvalue_2 (Utilities|Name|MakeLiteralName "TempObject"))
  (bind _asstaff_aicontroller (Utilities|Casting|CastToStaffAIController OwnerController))
  (bind _returnvalue_3 (AI|Components|Blackboard|GetValueasObject _returnvalue _returnvalue_2))
  (bind _searchedlocations (Variables|/Script/DoubleAgent.StaffAIController|GetSearchedLocations _asstaff_aicontroller))
  (Utilities|IsValid _returnvalue_3
    (:Is%20Valid
      (bind _assearch_location (Utilities|Casting|CastToSearchLocation _returnvalue_3)
        (:then
          (if (== (Utilities|Array|FindItem _searchedlocations _assearch_location) -1)
            (Utilities|Array|Add _searchedlocations _assearch_location))
          (AI|BehaviorTree|FinishExecute true))
        (:CastFailed
          (AI|BehaviorTree|FinishExecute false :!label _label))))
    (:Is%20Not%20Valid
      (goto _label))))