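; Behavior tree task that finds the average position of characters around the controlled pawn.
; A sphere overlap at the pawn's location gathers BaseCharacter_CHARACTER pawns within SphereRadius, excluding itself, and sums their locations.
; When any are found, it writes the mean to the Location blackboard key and finishes successfully; otherwise the task fails.
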(event EventReceiveExecuteAI
  (params (OwnerController :type AI%20Controller%20Object%20Reference) (ControlledPawn :type Pawn%20Object%20Reference))
  (Variables|Default|SetTemp "0, 0, 0")
  (bind (_outactors _returnvalue) (Collision|SphereOverlapActors (Transformation|GetActorLocation ControlledPawn) (Variables|Default|GetSphere%20Radius) (Utilities|Array|MakeArray "ObjectTypeQuery3") "/Script/DoubleAgent.BaseCharacter_CHARACTER" (Utilities|Array|MakeArray ControlledPawn)))
  (for _array_element _outactors
    (Variables|Default|SetTemp (+ (Variables|Default|GetTemp) (Transformation|GetActorLocation _array_element))))
  (if _returnvalue
    (AI|BehaviorTree|SetBlackboardValueasVector (Variables|Default|GetLocation) (/ (Variables|Default|GetTemp) (Utilities|Array|Length _outactors)))
    (AI|BehaviorTree|FinishExecute true)
    (else
      (AI|BehaviorTree|FinishExecute false))))