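; Behavior tree task that makes an AI pawn vocalize by emitting a noise event for AI hearing.
; On execute, it reports noise at the pawn's location with the controller as instigator and a "Local" tag.
; It prints a long-lasting debug message combining the pawn's name with the VocalStatus blackboard enum, then finishes successfully at once.
; The status only feeds the debug text, not the noise event.
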(event EventReceiveExecuteAI
  (params (OwnerController :type AI%20Controller%20Object%20Reference) (ControlledPawn :type Pawn%20Object%20Reference))
  (Class|AISenseHearing|ReportNoiseEvent (Transformation|GetActorLocation ControlledPawn) 1.0 OwnerController 0.0 "Local")
  (Development|PrintString (Utilities|String|Append (Utilities|String|Append (Utilities|GetDisplayName ControlledPawn) (Utilities|String|MakeLiteralString " Vocalized ")) (Utilities|String|EnumtoString (Utilities|Enum|ByteToEnumEVocalStatus (Class|BlackboardComponent|GetValueasEnum (AI|GetBlackboard OwnerController) (Utilities|Name|MakeLiteralName "VocalStatus"))))) true true "(R=0.000000,G=0.660000,B=1.000000,A=1.000000)" 2e+01)
  (AI|BehaviorTree|FinishExecute true))