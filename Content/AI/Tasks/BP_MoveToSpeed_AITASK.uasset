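; Behavior tree task that moves an AI character to a Blackboard vector at a walk, jog or run speed, unless set to keep its current speed.
; It pre-computes a nav path and calls AI MoveTo on the last point only if that lies near the target, otherwise failing.
; Move completion succeeds only if no montage is playing and the controller is no longer moving; abort stops movement.
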(event EventReceiveAbortAI
  (params (OwnerController :type AI%20Controller%20Object%20Reference) (ControlledPawn :type Pawn%20Object%20Reference))
  (AI|Navigation|StopMovement OwnerController)
  (AI|BehaviorTree|FinishExecute false))

(event EventReceiveExecuteAI
  (params (OwnerController :type AI%20Controller%20Object%20Reference) (ControlledPawn :type Pawn%20Object%20Reference))
  (bind _asbp_aicharacter_base_character (Utilities|Casting|CastToBP_AICharacterBase_CHARACTER ControlledPawn))
  (bind _vector (Variables|Default|GetVector))
  (bind _returnvalue (Class|BTFunctionLibrary|GetBlackboardValueasVector _vector))
  (bind _ascharacter (Utilities|Casting|CastToCharacter ControlledPawn))
  (CallFunction|CalculateSpeed _ascharacter)
  (bind _returnvalue_2 (Class|NavigationSystemV1|FindPathtoLocationSynchronously (Transformation|GetActorLocation ControlledPawn) _returnvalue OwnerController "/Script/AIModule.NavFilter_AIControllerDefault")) ; Calculate path
  (if (!= (Utilities|Array|Length (Variables|/Script/NavigationSystem.NavigationPath|GetPathPoints _returnvalue_2)) 0)
    (if (< (Math|Vector|Distance(Vector) (Utilities|Array|Get(acopy) (Variables|/Script/NavigationSystem.NavigationPath|GetPathPoints _returnvalue_2) (- (Utilities|Array|Length (Variables|/Script/NavigationSystem.NavigationPath|GetPathPoints _returnvalue_2)) 1)) _returnvalue) 5e+02) ; ensuring the distance to destination is greater than 500
      (AI|AIMoveTo OwnerController (Utilities|Array|Get(acopy) (Variables|/Script/NavigationSystem.NavigationPath|GetPathPoints _returnvalue_2) (- (Utilities|Array|Length (Variables|/Script/NavigationSystem.NavigationPath|GetPathPoints _returnvalue_2)) 1)) 0 (Variables|Default|GetTolerance) "Default" "Enable" true false false "Enable"
        (:OnRequestFailed
          (AI|BehaviorTree|FinishExecute false))
        (:OnMoveFinished
          (AI|BehaviorTree|FinishExecute (and (not (Class|AnimInstance|IsAnyMontagePlaying (Components|SkeletalMesh|GetAnimInstance (Variables|/Script/Engine.Character|GetMesh _asbp_aicharacter_base_character)))) (not (Utilities|Enum|Equal(Enum) (Class|AIController|GetMoveStatus (AI|GetAIController _asbp_aicharacter_base_character)) "Moving"))))))
      (else
        (AI|BehaviorTree|FinishExecute false)))
    (else
      (AI|BehaviorTree|FinishExecute false))))

(fn CalculateSpeed
  (params (NPC :type Character%20Object%20Reference))
  (bind _charactermovement (Variables|/Script/Engine.Character|GetCharacterMovement NPC))
  (if (not (Variables|Default|GetbKeepSpeed))
    (switch Utilities|FlowControl|Switch|SwitchonMovementSpeed_ENUM (Variables|Default|GetSpeed)
      (:NewEnumerator0
        (Variables|/Script/Engine.CharacterMovementComponent|SetMaxWalkSpeed _charactermovement (LocalVariables|GetwalkingSpeed)))
      (:NewEnumerator1
        (Variables|/Script/Engine.CharacterMovementComponent|SetMaxWalkSpeed _charactermovement (LocalVariables|GetjoggingSpeed)))
      (:NewEnumerator2
        (Variables|/Script/Engine.CharacterMovementComponent|SetMaxWalkSpeed _charactermovement (LocalVariables|GetrunningSpeed))))))