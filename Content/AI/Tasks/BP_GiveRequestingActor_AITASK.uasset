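; BP_GiveRequestingActor_AITASK is a behavior tree task that lets a waiter AI hand a drink or food to the character requesting it.
; It reads the RequestingActor key from the controlled pawn's blackboard and casts it to the AI character base class.
; The WaiterGive setting chooses whether HasDrink or HasFood is set true on that character's own blackboard, then the task finishes successfully.
; A failed cast stops execution without finishing the task.
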(event EventReceiveExecuteAI
  (params (OwnerController :type AI%20Controller%20Object%20Reference) (ControlledPawn :type Pawn%20Object%20Reference))
  (bind _asbp_aicharacter_base_character (Utilities|Casting|CastToBP_AICharacterBase_CHARACTER (AI|Components|Blackboard|GetValueasObject (AI|GetBlackboard ControlledPawn) (Utilities|Name|MakeLiteralName "RequestingActor"))))
  (switch Utilities|FlowControl|Switch|SwitchonEWaiterGive (Variables|Default|GetWaiterGive)
    (:NewEnumerator0
      (AI|Components|Blackboard|SetValueasBool (AI|GetBlackboard _asbp_aicharacter_base_character) (Utilities|Name|MakeLiteralName "HasDrink") true))
    (:NewEnumerator1
      (AI|Components|Blackboard|SetValueasBool (AI|GetBlackboard _asbp_aicharacter_base_character) (Utilities|Name|MakeLiteralName "HasFood") true)))
  (AI|BehaviorTree|FinishExecute true))