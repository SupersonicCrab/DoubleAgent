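; Behavior tree task that sets the AI's look target for its current patrol point.
; It reads the DesignatedRoute and LastPatrolPoint blackboard values to find that point's Location and LookLocation on the BP_PatrolRoute.
; If the two differ beyond a small tolerance, it writes LookLocation, offset by the route actor's position, into the LookVector key and succeeds.
; Otherwise the task fails, marking the point as having no distinct look direction.
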(event EventReceiveExecuteAI
  (params (OwnerController :type AI%20Controller%20Object%20Reference) (ControlledPawn :type Pawn%20Object%20Reference))
  (bind _returnvalue (AI|GetBlackboard ControlledPawn))
  (bind _returnvalue_2 (Utilities|Name|MakeLiteralName "DesignatedRoute"))
  (bind _returnvalue_3 (Utilities|Name|MakeLiteralName "LastPatrolPoint"))
  (bind _returnvalue_4 (AI|Components|Blackboard|GetValueasObject _returnvalue _returnvalue_2))
  (bind _returnvalue_5 (Class|BlackboardComponent|GetValueasInt _returnvalue _returnvalue_3))
  (bind _asbp_patrol_route (Utilities|Casting|CastToBP_PatrolRoute _returnvalue_4))
  (bind _path (Variables|/Game/AI/Patrol/BP_PatrolRoute.BP_PatrolRoute_C|GetPath _asbp_patrol_route))
  (bind _output (Utilities|Array|Get(acopy) _path _returnvalue_5))
  (bind (_location _looklocation) (Utilities|Struct|BreakFPatrol _output))
  (if (Math|Vector|NotEqual(Vector) _location _looklocation 1e+01)
    (AI|BehaviorTree|SetBlackboardValueasVector (Variables|Default|GetLookVector) (+ _looklocation (Transformation|GetActorLocation _asbp_patrol_route)))
    (AI|BehaviorTree|FinishExecute true)
    (else
      (AI|BehaviorTree|FinishExecute false))))