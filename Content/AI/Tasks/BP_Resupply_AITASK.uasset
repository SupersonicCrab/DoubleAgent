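; Behavior tree task that resupplies an AI guard with its standard kit of gun, radio, ammo pouches, flashlight and keycard.
; A RestoreItem helper adds each item to the pawn's inventory component only if that item class is missing, so partial stacks are not topped up.
; It then switches on the guard's matching holsters through Net holster calls and finishes with success.
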(event EventReceiveExecuteAI
  (params (OwnerController :type AI%20Controller%20Object%20Reference) (ControlledPawn :type Pawn%20Object%20Reference))
  (bind _asbp_aicharacter_base_character (Utilities|Casting|CastToBP_AICharacterBase_CHARACTER ControlledPawn))
  (bind _asbp_guard_character (Utilities|Casting|CastToBP_Guard_CHARACTER _asbp_aicharacter_base_character))
  (bind _inventorycomponent (Variables|/Game/AI/NPC/BP_AICharacterBase_CHARACTER.BP_AICharacterBase_CHARACTER_C|GetInventoryComponent _asbp_aicharacter_base_character))
  (CallFunction|RestoreItem _inventorycomponent "/Game/Inventory/Item/NPCItems/BP_Gun_Item.BP_Gun_Item_C" 1)
  (CallFunction|RestoreItem _inventorycomponent "/Game/Inventory/Item/NPCItems/BP_Radio_Item.BP_Radio_Item_C" 1)
  (CallFunction|RestoreItem _inventorycomponent "/Game/Inventory/Item/NPCItems/BP_AmmoPouch_Item.BP_AmmoPouch_Item_C" 3)
  (CallFunction|RestoreItem _inventorycomponent "/Game/Inventory/Item/NPCItems/BP_Flashlight_Item.BP_Flashlight_Item_C" 1)
  (CallFunction|RestoreItem _inventorycomponent "/Game/Inventory/Item/NPCItems/BP_Keycard_Item.BP_Keycard_Item_C" 1)
  (Default|NetPistolHolster _asbp_guard_character true)
  (Default|NetRadioHolster _asbp_guard_character true)
  (Default|NetAmmoHolster _asbp_guard_character true)
  (Default|NetFlashlightHolster _asbp_guard_character true)
  (Default|NetKeycardHolster _asbp_guard_character true)
  (AI|BehaviorTree|FinishExecute true))

(fn RestoreItem
  (params (Inventory :type BP%20Inventory%20Component%20Object%20Reference) (Item :type BP%20Base%20Item%20Class%20Reference) (Quantity :type Integer))
  (bind _itemfound (Default|CheckItemClass Inventory Item))
  (if (not _itemfound)
    (Default|AddtoInventory Inventory (Utilities|Struct|MakeFSlotStructureNew (Utilities|Struct|MakeFItemStructure "None" "N/a" true 4 0 "NewEnumerator3" Item) Quantity))))