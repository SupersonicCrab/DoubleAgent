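; Tripwire actor for the AI security system that triggers an alarm when something crosses its box trigger while active.
; On BeginPlay it takes its active state from the level's PowerBox_BP.
; Players and guards carrying a tripwire remote in their inventory pass safely; any other overlapping actor sets it off.
; Enable and Disable functions toggle the state and point light, while the alarm currently only prints a message.
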(event OnComponentBeginOverlap(Box)
  (params (OverlappedComponent :type Primitive%20Component%20Object%20Reference) (OtherActor :type Actor%20Object%20Reference) (OtherComp :type Primitive%20Component%20Object%20Reference) (OtherBodyIndex :type Integer) (bFromSweep :type Boolean) (SweepResult :type Hit%20Result%20Structure%20%28by%20ref%29))
  (bind _returnvalue (Utilities|GetClass OtherActor))
  ;[1 1 1] Activate alarm if someone collides with this and does not have a tripwire remote
  (if (Variables|Default|GetactiveTripwire)
    (if (== _returnvalue "/Game/Player/Player_CHARACTER.Player_CHARACTER_C")
      (bind _asplayer_character (Utilities|Casting|CastToPlayer_CHARACTER OtherActor))
      (bind _itemfound (Default|CheckItemClass (Variables|/Game/Player/Player_CHARACTER.Player_CHARACTER_C|GetInventoryComponent _asplayer_character) "/Game/Inventory/Item/Item_TripwireRemote.Item_TripwireRemote_C"))
      (if (not _itemfound)
        (CallFunction|ActivateAlarm))
      (elif (== _returnvalue "/Game/AI/Guard/Guard_CHARACTER.Guard_CHARACTER_C")
        (bind _asguard_character (Utilities|Casting|CastToGuard_CHARACTER OtherActor))
        (bind _itemfound_2 (Default|CheckItemClass (Variables|/Game/AI/AICharacterBase_CHARACTER.AICharacterBase_CHARACTER_C|GetInventoryComponent _asguard_character) "/Game/Inventory/Item/Item_TripwireRemote.Item_TripwireRemote_C"))
        (if (not _itemfound_2)
          (CallFunction|ActivateAlarm))
        (else
          (CallFunction|ActivateAlarm))))))

(event EventBeginPlay
  ;[1 1 1] Get current powerbox settings
  (bind _returnvalue (Actor|GetActorOfClass "/Game/Interactable/PowerBox/PowerBox_BP.PowerBox_BP_C"))
  (bind _output_get (Variables|Default|SetpowerBox _returnvalue))
  (Variables|Default|SetactiveTripwire (Variables|/Game/Interactable/PowerBox/PowerBox_BP.PowerBox_BP_C|GetTripwiresOn _output_get)))

(fn ConstructionScript)

(fn ActivateAlarm
  (Development|PrintString "Alarm activated"))

(fn DisableTripwire
  (Variables|Default|SetactiveTripwire false)
  (Rendering|Components|Light|SetIntensity (Variables|Default|GetPointLight) 0.0))

(fn EnableTripwire
  (Variables|Default|SetactiveTripwire true)
  (Rendering|Components|Light|SetIntensity (Variables|Default|GetPointLight) 1.5e+03))