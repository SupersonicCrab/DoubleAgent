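; RadioHub is the security system's radio relay actor, broadcasting radio events to NPC guards.
; SendRadioEvent finds every AICharacterBase actor tagged "Radio", forwards the event to its AI controller's RadioEventDelay and prints a debug message.
; PowerOn and PowerOff toggle RadioPowerOn, though sending does not check that flag.
; TestAlert and TestEngage fire sample events at the hub's own location with a short delay.
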(event EventBeginPlay)

(event Collision|EventActorBeginOverlap
  (params (OtherActor :type Actor%20Object%20Reference)))

(event EventTick
  (params (DeltaSeconds :type Float%20%28single-precision%29)))

(fn ConstructionScript)

(fn PowerOff
  (Variables|Default|SetRadioPowerOn false))

(fn Poweron
  (Variables|Default|SetRadioPowerOn true))

(fn SendRadioEvent
  (params (RadioEvent :type Radio%20Event%20STRUCT%20Structure))
  (bind (_radioevent _location _delay) (Utilities|Struct|BreakRadioEvent_STRUCT RadioEvent))
  ;[1 1 1] Send radio event to NPCs
  (bind _outactors (Actor|GetAllActorsOfClasswithTag "/Game/AI/AICharacterBase_CHARACTER.AICharacterBase_CHARACTER_C" "Radio"))
  (for _array_element _outactors
    (Default|RadioEventDelay (.AsAIController%20Base%20AICONTROLLER (Utilities|Casting|CastToAIControllerBase_AICONTROLLER (AI|GetAIController (.AsAICharacter%20Base%20CHARACTER (Utilities|Casting|CastToAICharacterBase_CHARACTER _array_element))))) RadioEvent)
    ;[1 1 1] Debug output
    (Development|PrintString (Utilities|String|Append (Utilities|String|EnumtoString _radioevent) " radio event at " (Utilities|String|ToString(Vector) _location) " called with " (Utilities|String|ToString(Float) _delay) " delay") true true "(R=0.000000,G=0.660000,B=1.000000,A=1.000000)" 2e+01)))

(fn TestAlert
  (CallFunction|SendRadioEvent (Utilities|Struct|MakeRadioEvent_STRUCT "NewEnumerator3" (Transformation|GetActorLocation) 0.1)))

(fn TestEngage
  (CallFunction|SendRadioEvent (Utilities|Struct|MakeRadioEvent_STRUCT "NewEnumerator4" (Transformation|GetActorLocation) 0.1)))