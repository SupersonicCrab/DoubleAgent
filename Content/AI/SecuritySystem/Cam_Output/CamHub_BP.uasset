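; Security camera hub actor that routes every Camera_CHARACTER in the level to render targets and powers them by player proximity.
; On BeginPlay it gathers all cameras and assigns each scene capture a render target from TextureTargets by matching array index.
; Player_CHARACTER entering or leaving its Box trigger calls CameraOn or CameraOff on every camera, so captures are toggled only around the hub.
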(event OnComponentBeginOverlap(Box)
  (params (OverlappedComponent :type Primitive%20Component%20Object%20Reference) (OtherActor :type Actor%20Object%20Reference) (OtherComp :type Primitive%20Component%20Object%20Reference) (OtherBodyIndex :type Integer) (bFromSweep :type Boolean) (SweepResult :type Hit%20Result%20Structure%20%28by%20ref%29))
  (if (== (Utilities|GetClass OtherActor) "/Game/Player/Player_CHARACTER.Player_CHARACTER_C")
    (CallFunction|Camerason)))

(event OnComponentEndOverlap(Box)
  (params (OverlappedComponent :type Primitive%20Component%20Object%20Reference) (OtherActor :type Actor%20Object%20Reference) (OtherComp :type Primitive%20Component%20Object%20Reference) (OtherBodyIndex :type Integer))
  (if (== (Utilities|GetClass OtherActor) "/Game/Player/Player_CHARACTER.Player_CHARACTER_C")
    (CallFunction|CamerasOff)))

(event EventBeginPlay
  (bind _outactors (Actor|GetAllActorsOfClass "/Game/AI/SecuritySystem/Camera/Camera_CHARACTER.Camera_CHARACTER_C"))
  (bind _output_get (Variables|Default|SetCameras _outactors))
  (for (_array_element _array_index) _output_get
    (Variables|/Script/Engine.SceneCaptureComponent2D|SetTextureTarget (Variables|/Game/AI/SecuritySystem/Camera/Camera_CHARACTER.Camera_CHARACTER_C|GetSceneCaptureComponent2D (.AsCamera%20CHARACTER (Utilities|Casting|CastToCamera_CHARACTER _array_element))) (Utilities|Array|Get(acopy) (Variables|Default|GetTextureTargets) _array_index))))

(fn ConstructionScript)

(fn Camerason
  (for _array_element (Variables|Default|GetCameras)
    (bind _ascamera_character (Utilities|Casting|CastToCamera_CHARACTER _array_element))
    (Default|Cameraon _ascamera_character)))

(fn CamerasOff
  (for _array_element (Variables|Default|GetCameras)
    (bind _ascamera_character (Utilities|Casting|CastToCamera_CHARACTER _array_element))
    (Default|CameraOff _ascamera_character)))