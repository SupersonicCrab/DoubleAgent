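; BP_CamHub is a security camera hub that switches the level's cameras on and off based on player proximity.
; On BeginPlay it gathers every CameraBase actor and assigns each scene capture a render target from TextureTargets by matching index.
; Its box trigger calls CameraOn on all cameras when an exact PlayerCharacter class actor enters, and CameraOff when it leaves.
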(event OnComponentBeginOverlap(Box)
  (params (OverlappedComponent :type Primitive%20Component%20Object%20Reference) (OtherActor :type Actor%20Object%20Reference) (OtherComp :type Primitive%20Component%20Object%20Reference) (OtherBodyIndex :type Integer) (bFromSweep :type Boolean) (SweepResult :type Hit%20Result%20Structure%20%28by%20ref%29))
  (if (== (Utilities|GetClass OtherActor) "/Game/Player/PlayerCharacter.PlayerCharacter_C")
    (CallFunction|Camerason)))

(event OnComponentEndOverlap(Box)
  (params (OverlappedComponent :type Primitive%20Component%20Object%20Reference) (OtherActor :type Actor%20Object%20Reference) (OtherComp :type Primitive%20Component%20Object%20Reference) (OtherBodyIndex :type Integer))
  (if (== (Utilities|GetClass OtherActor) "/Game/Player/PlayerCharacter.PlayerCharacter_C")
    (CallFunction|CamerasOff)))

(event EventBeginPlay
  (bind _outactors (Actor|GetAllActorsOfClass "/Game/AI/SecuritySystem/Cameras/CameraBase.CameraBase_C"))
  (bind _output_get (Variables|Default|SetCameras _outactors))
  (for (_array_element _array_index) _output_get
    (Variables|/Script/Engine.SceneCaptureComponent2D|SetTextureTarget (Variables|/Game/AI/SecuritySystem/Cameras/CameraBase.CameraBase_C|GetSceneCaptureComponent2D (.AsCamera%20Base (Utilities|Casting|CastToCameraBase _array_element))) (Utilities|Array|Get(acopy) (Variables|Default|GetTextureTargets) _array_index))))

(fn ConstructionScript)

(fn Camerason
  (for _array_element (Variables|Default|GetCameras)
    (bind _ascamera_base (Utilities|Casting|CastToCameraBase _array_element))
    (Default|Cameraon _ascamera_base)))

(fn CamerasOff
  (for _array_element (Variables|Default|GetCameras)
    (bind _ascamera_base (Utilities|Casting|CastToCameraBase _array_element))
    (Default|CameraOff _ascamera_base)))