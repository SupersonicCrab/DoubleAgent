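; BP_SearchLocation is a placeable marker for a spot that can be searched, likely by AI, and it registers itself with the rooms containing it.
; On BeginPlay it runs a small sphere overlap at its position against WorldDynamic objects and casts the results to RoomVolume.
; Each room found is added to its Room array, and the location adds itself to that room's SearchLocations list.
; A Debug flag unhides the SearchSpot component in game.
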(event EventBeginPlay
  (if (Variables|Default|GetbDebug) ; Debug
    (Development|SetHiddeninGame (Variables|Default|GetSearchSpot) false false))
  ;[1 1 1] Room handling
  (bind _outactors (Collision|SphereOverlapActors (Transformation|GetActorLocation) 1e+01 (Utilities|Array|MakeArray "ObjectTypeQuery2") 0)) ; Check if searchlocation is in any rooms
  (for _array_element _outactors
    (bind _asroom_volume (Utilities|Casting|CastToRoomVolume _array_element))
    (Utilities|Array|Add (Variables|Default|GetRoom) _asroom_volume) ; Add to room array
    (Utilities|Array|Add (Variables|/Script/DoubleAgent.RoomVolume|GetsearchLocations _asroom_volume) self)))

(fn ConstructionScript)