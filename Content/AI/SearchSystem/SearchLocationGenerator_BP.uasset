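; Search location generator for the AI search system that populates the level with SearchLocation_BP actors when play begins.
; It runs the GenerateSearchLocation EQS query in single-result mode with itself as querier, spawning an actor at the returned location.
; Each success re-runs the query, forming an asynchronous loop that ends when no location is returned.
; Debug prints report the start and the total time taken.
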(event Custom|OnQueryFinished
  (params (QueryInstance :type Env%20Query%20Instance%20Blueprint%20Wrapper%20Object%20Reference) (QueryStatus :type EEnvQueryStatus%20Enum :default "Processing"))
  (bind (_resultlocations _returnvalue) (AI|EQS|GetQueryResultsasLocations QueryInstance))
  (if _returnvalue
    (Game|SpawnActorfromClass "/Game/AI/SearchSystem/SearchLocation_BP.SearchLocation_BP_C" (Math|Conversions|ToTransform(Vector) (Utilities|Array|Get(acopy) _resultlocations)) "Undefined" 0 0)
    (CallFunction|Generate)
    (else
      (Development|PrintString (Utilities|String|Append "Search location generation completed, took : " (Utilities|String|ToString(Float) (- (Utilities|Time|GetRealTimeSeconds) (Variables|Default|GetinitialTime))) " seconds") true true "(R=0.000000,G=1.000000,B=0.000000,A=1.000000)" 1e+01))))

(event Custom|Generate
  (bind _returnvalue (AI|EQS|RunEQSQuery "/Game/AI/EQS/Queries/GenerateSearchLocation_EQSQUERY.GenerateSearchLocation_EQSQUERY" self "SingleResult"))
  (EventDispatchers|BindEventtoOnQueryFinishedEvent _returnvalue (delegate Custom|OnQueryFinished)))

(event EventBeginPlay
  (CallFunction|Generate)
  (Variables|Default|SetinitialTime (Utilities|Time|GetRealTimeSeconds))
  (Development|PrintString "Search location generation started" true true "(R=1.000000,G=1.000000,B=0.000000,A=1.000000)" 1e+01))

(fn ConstructionScript)