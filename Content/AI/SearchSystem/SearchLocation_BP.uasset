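; Search location actor for guard AI, tracking Searched and Searching states, with debug light colours.
; A guard entering its radius with a different valid TempObject in its Blackboard marks it searched if a visibility trace hits that guard.
; Reset, run on BeginPlay, clears Searched, then marks it again if an overlapping guard with high Detection is visible.
; SetSearched disables radius overlap events in both branches, despite a comment saying clearing re-enables them.
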(event OnComponentBeginOverlap(SearchRadius)
  (params (OverlappedComponent :type Primitive%20Component%20Object%20Reference) (OtherActor :type Actor%20Object%20Reference) (OtherComp :type Primitive%20Component%20Object%20Reference) (OtherBodyIndex :type Integer) (bFromSweep :type Boolean) (SweepResult :type Hit%20Result%20Structure%20%28by%20ref%29))
  (bind _returnvalue (AI|GetBlackboard OtherActor))
  (bind _returnvalue_2 (Utilities|Name|MakeLiteralName "TempObject"))
  (bind _returnvalue_3 (AI|Components|Blackboard|GetValueasObject _returnvalue _returnvalue_2))
  ;[1 1 1] Handle search radius collision
  (if (== (Utilities|GetClass OtherActor) "/Game/AI/NPC/Guard/Guard_CHARACTER.Guard_CHARACTER_C")
    (if (and (Utilities|IsValid _returnvalue_3) (!= _returnvalue_3 self))
      (bind _outhit (Collision|LineTraceByChannel (Transformation|GetActorLocation) (Transformation|GetActorLocation OtherActor) "TraceTypeQuery1" true 0 "None" false))
      (if (== (.HitActor (Collision|BreakHitResult _outhit)) OtherActor)
        (CallFunction|SetSearched true)))))

(event EventBeginPlay
  ;[1 1 1] Setup
  (CallFunction|Reset)
  (if (Variables|Default|GetDebug) ; Debug
    (Development|SetHiddeninGame (Variables|Default|GetSearchSpot) false false)
    (Development|SetHiddeninGame (Variables|Default|GetSearchRadius) false false)))

(fn ConstructionScript)

(fn SetSearched
  (params (Boolean :type Boolean))
  (if Boolean
    (Variables|Default|SetSearched true)
    (Variables|/Script/Engine.PrimitiveComponent|SetbGenerateOverlapEvents (Variables|Default|GetSearchRadius) false) ; Disable overlaps if location is already searched
    (if (Variables|Default|GetDebug)
      (Rendering|Components|Light|SetLightColor (Variables|Default|GetPointLight) "(R=255.000000,G=0.000000,B=0.000000,A=1.000000)" true))
    (else
      (Variables|Default|SetSearched false)
      (Variables|/Script/Engine.PrimitiveComponent|SetbGenerateOverlapEvents (Variables|Default|GetSearchRadius) false) ; Re-enabling overlaps when not searched
      (if (and (Variables|Default|GetDebug) (not (Variables|Default|GetSearching)))
        (Rendering|Components|Light|SetLightColor (Variables|Default|GetPointLight) "(R=0.000000,G=0.000000,B=0.000000,A=1.000000)" true)))))

(fn SetSearching
  (params (Boolean :type Boolean))
  (if Boolean
    ;[1 1 1] Set searching and updating lights if debug
    (Variables|Default|SetSearching true)
    (if (Variables|Default|GetDebug)
      (Rendering|Components|Light|SetLightColor (Variables|Default|GetPointLight) "(R=0.000000,G=255.000000,B=0.000000,A=1.000000)" true))
    (else
      (Variables|Default|SetSearching false)
      (if (and (Variables|Default|GetDebug) (not (Variables|Default|GetSearched)))
        (Rendering|Components|Light|SetLightColor (Variables|Default|GetPointLight) "(R=0.000000,G=0.000000,B=0.000000,A=1.000000)" true)))))

(fn ScanforGuards
  (bind _searchradius (Variables|Default|GetSearchRadius))
  ;[1 1 1] Get all guards in radius
  (bind _outactors (Collision|ComponentOverlapActors _searchradius (Transformation|GetWorldTransform _searchradius) (Utilities|Array|MakeArray "ObjectTypeQuery3") "/Game/AI/NPC/Guard/Guard_CHARACTER.Guard_CHARACTER_C"))
  (bind _array_element (Utilities|Array|ForEachLoopwithBreak _outactors :!label _label)
    (:LoopBody
      ;[1 1 1] Checking if guard is above 90 detection
      (if (>= (Class|BlackboardComponent|GetValueasFloat (AI|GetBlackboard _array_element) (Utilities|Name|MakeLiteralName "Detection")) 9e+01)
        ;[1 1 1] Raycasting to guard to ensure visilibity
        (bind _outhit (Collision|LineTraceByChannel (Transformation|GetActorLocation) (Transformation|GetActorLocation _array_element) "TraceTypeQuery1" true 0 "None" false))
        (if (== (.HitActor (Collision|BreakHitResult _outhit)) _array_element)
          (CallFunction|SetSearched true)
          (goto _label Break))))))

(fn Reset
  ;[1 1 1] Resetting all variables
  (CallFunction|SetSearched false)
  (CallFunction|ScanforGuards))