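; Behavior tree decorator that checks whether a guard's pistol is lined up to hit the player.
; It derives the aim direction from the pistol's GunBack and GunFront sockets and traces the Camera channel along it, reaching past the muzzle by the pawn's distance to the blackboard's LastPlayer.
; It passes only if the hit actor's class is exactly Player_CHARACTER, and leaves debug drawing of the trace on.
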(fn PerformConditionCheckAI
  (params (OwnerController :type AI%20Controller%20Object%20Reference) (ControlledPawn :type Pawn%20Object%20Reference))
  (bind _returnvalue (AI|GetBlackboard ControlledPawn))
  (bind _returnvalue_2 (Utilities|Name|MakeLiteralName "LastPlayer"))
  (bind _returnvalue_3 (AI|Components|Blackboard|GetValueasObject _returnvalue _returnvalue_2))
  (bind _asbp_guard_character (Utilities|Casting|CastToBP_Guard_CHARACTER ControlledPawn))
  (Utilities|IsValid _returnvalue_3
    (:Is%20Valid
      (bind _outhit (Collision|LineTraceByChannel (.location (Transformation|GetSocketTransform (Variables|/Game/AI/NPC/Guard/BP_Guard_CHARACTER.BP_Guard_CHARACTER_C|GetPistolHand _asbp_guard_character) "GunBack" "RTS_World")) (+ (* (Math|Vector|GetForwardVector (Math|Rotator|FindLookatRotation (.location (Transformation|GetSocketTransform (Variables|/Game/AI/NPC/Guard/BP_Guard_CHARACTER.BP_Guard_CHARACTER_C|GetPistolHand _asbp_guard_character) "GunBack" "RTS_World")) (.location (Transformation|GetSocketTransform (Variables|/Game/AI/NPC/Guard/BP_Guard_CHARACTER.BP_Guard_CHARACTER_C|GetPistolHand _asbp_guard_character) "GunFront" "RTS_World")))) (Transformation|GetDistanceTo (.AsActor (Utilities|Casting|CastToActor _returnvalue_3)) ControlledPawn)) (.location (Transformation|GetSocketTransform (Variables|/Game/AI/NPC/Guard/BP_Guard_CHARACTER.BP_Guard_CHARACTER_C|GetPistolHand _asbp_guard_character) "GunFront" "RTS_World"))) "TraceTypeQuery2" false 0 "ForDuration" true "(R=1.000000,G=1.000000,B=0.000000,A=1.000000)"))
      (return (== (Utilities|GetClass (.HitActor (Collision|BreakHitResult _outhit))) "/Game/Player/Player_CHARACTER.Player_CHARACTER_C")))))