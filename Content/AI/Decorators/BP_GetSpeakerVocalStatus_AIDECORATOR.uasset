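; Behavior tree decorator that copies the vocal status of an AI's current speaker into a blackboard key.
; Its condition check reads the Speaker object from the controlled pawn's blackboard and casts it to AICharacterBase_CHARACTER.
; On success it writes the VocalStatus enum from that speaker's blackboard to its own VocalStatus key and passes.
; It fails when the cast fails, so the check doubles as a data sync between two AI blackboards.
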(fn PerformConditionCheckAI
  (params (OwnerController :type AI%20Controller%20Object%20Reference) (ControlledPawn :type Pawn%20Object%20Reference))
  (bind _asaicharacter_base_character (Utilities|Casting|CastToAICharacterBase_CHARACTER (AI|Components|Blackboard|GetValueasObject (AI|GetBlackboard ControlledPawn) (Utilities|Name|MakeLiteralName "Speaker")))
    (:then
      (Class|BTFunctionLibrary|SetBlackboardValueasEnum (Variables|Default|GetVocalStatus) (Class|BlackboardComponent|GetValueasEnum (AI|GetBlackboard (AI|GetAIController _asaicharacter_base_character)) (Utilities|Name|MakeLiteralName "VocalStatus")))
      (return true))
    (:CastFailed
      (return false))))