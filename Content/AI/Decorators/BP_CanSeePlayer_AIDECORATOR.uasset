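; A behavior tree decorator that checks whether an AI character can see the player stored in its LastPlayer blackboard key.
; When that key is valid, it traces on the Camera channel from the AI's head socket to the player's neck_01 socket, with debug drawing on.
; The condition passes only if the hit actor's class is exactly BP_Player_CHARACTER, so it does not confirm that the hit is that specific player.
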(fn PerformConditionCheckAI
  (params (OwnerController :type AI%20Controller%20Object%20Reference) (ControlledPawn :type Pawn%20Object%20Reference))
  (bind _returnvalue (AI|GetBlackboard ControlledPawn))
  (bind _returnvalue_2 (Utilities|Name|MakeLiteralName "LastPlayer"))
  (bind _returnvalue_3 (AI|Components|Blackboard|GetValueasObject _returnvalue _returnvalue_2))
  (Utilities|IsValid _returnvalue_3
    (:Is%20Valid
      (bind _outhit (Collision|LineTraceByChannel (Transformation|GetSocketLocation (Variables|/Script/Engine.Character|GetMesh (.AsCharacter (Utilities|Casting|CastToCharacter ControlledPawn))) "head") (Transformation|GetSocketLocation (Variables|/Script/Engine.Character|GetMesh (.AsCharacter (Utilities|Casting|CastToCharacter _returnvalue_3))) "neck_01") "TraceTypeQuery2" false 0 "ForDuration" true "(R=1.000000,G=1.000000,B=0.000000,A=1.000000)"))
      (return (== (Utilities|GetClass (.HitActor (Collision|BreakHitResult _outhit))) "/Game/Player/BP_Player_CHARACTER.BP_Player_CHARACTER_C")))))