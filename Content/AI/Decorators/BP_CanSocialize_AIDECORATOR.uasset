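; Behavior tree decorator that decides whether an AI pawn can socialize in the room it occupies.
; The condition check scans the RoomVolume actors overlapping the controlled pawn for any flagged CivilianGather.
; It passes when such a volume overlaps at least one BP_Civilian_CHARACTER, without excluding the controlled pawn from that count, and fails otherwise.
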(fn PerformConditionCheckAI
  (params (OwnerController :type AI%20Controller%20Object%20Reference) (ControlledPawn :type Pawn%20Object%20Reference))
  (bind _overlappingactors (Collision|GetOverlappingActors ControlledPawn "/Script/DoubleAgent.RoomVolume" :!class /Script/Engine.Actor))
  (if (!= (Utilities|Array|Length _overlappingactors) 0)
    (for _array_element _overlappingactors
      (if (Variables|/Script/DoubleAgent.RoomVolume|GetbCivilianGather (.AsRoom%20Volume (Utilities|Casting|CastToRoomVolume _array_element)))
        (if (> (Utilities|Array|Length (Collision|GetOverlappingActors _array_element "/Game/AI/NPC/Civilian/BP_Civilian_CHARACTER.BP_Civilian_CHARACTER_C" :!class /Script/Engine.Actor)) 0)
          (return true)))))
  (return false))