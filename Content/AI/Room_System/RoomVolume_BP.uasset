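; Room trigger volume that tracks player safety and alerts AI characters inside when the room's light goes out.
; Players entering the box, or already inside at BeginPlay, get RoomSafe set from the room's PlayerSafe; leaving clears it.
; LightUpdate stores the lit state and, when unlit, NPCUpdate writes the switch to each overlapping AI's LightSwitch blackboard key.
; Overlap events identify the player by class display name rather than by cast.
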(event OnComponentBeginOverlap(Box)
  (params (OverlappedComponent :type Primitive%20Component%20Object%20Reference) (OtherActor :type Actor%20Object%20Reference) (OtherComp :type Primitive%20Component%20Object%20Reference) (OtherBodyIndex :type Integer) (bFromSweep :type Boolean) (SweepResult :type Hit%20Result%20Structure%20%28by%20ref%29))
  (switch string (Utilities|String|LeftChop (Utilities|GetClassDisplayName (Utilities|GetClass OtherActor)) 2)
    (:Player_CHARACTER
      (CallFunction|PlayerEnter OtherActor))))

(event OnComponentEndOverlap(Box)
  (params (OverlappedComponent :type Primitive%20Component%20Object%20Reference) (OtherActor :type Actor%20Object%20Reference) (OtherComp :type Primitive%20Component%20Object%20Reference) (OtherBodyIndex :type Integer))
  (switch string (Utilities|String|LeftChop (Utilities|GetClassDisplayName (Utilities|GetClass OtherActor)) 2)
    (:Player_CHARACTER
      (CallFunction|PlayerExit OtherActor))))

(event EventBeginPlay
  (bind _box (Variables|Default|GetBox))
  (bind _outactors (Collision|ComponentOverlapActors _box (Transformation|GetWorldTransform _box) (Utilities|Array|MakeArray "ObjectTypeQuery3") "/Game/Player/Player_CHARACTER.Player_CHARACTER_C"))
  (for _array_element _outactors
    (CallFunction|PlayerEnter _array_element)))

(fn ConstructionScript)

(fn PlayerEnter
  (params (Player :type Actor%20Object%20Reference))
  (bind _asplayer_character (Utilities|Casting|CastToPlayer_CHARACTER Player))
  (Variables|/Game/Player/Player_CHARACTER.Player_CHARACTER_C|SetRoomSafe _asplayer_character (Variables|Default|GetPlayerSafe)))

(fn PlayerExit
  (params (Player :type Actor%20Object%20Reference))
  (bind _asplayer_character (Utilities|Casting|CastToPlayer_CHARACTER Player))
  (Variables|/Game/Player/Player_CHARACTER.Player_CHARACTER_C|SetRoomSafe _asplayer_character false))

(fn LightUpdate
  (params (RoomLit :type Boolean) (LightSwitch :type Light%20Switch%20Object%20Reference))
  (bind _output_get (Variables|Default|SetRoomLit RoomLit))
  (if (not _output_get)
    (CallFunction|NPCUpdate LightSwitch)))

(fn NPCUpdate
  (params (LightSwitch :type Light%20Switch%20Object%20Reference))
  (bind _box (Variables|Default|GetBox))
  (bind _outactors (Collision|ComponentOverlapActors _box (Transformation|GetWorldTransform _box) (Utilities|Array|MakeArray "ObjectTypeQuery3") "/Game/AI/AICharacterBase_CHARACTER.AICharacterBase_CHARACTER_C"))
  (for _array_element _outactors
    (AI|Components|Blackboard|SetValueasObject (AI|GetBlackboard _array_element) (Utilities|Name|MakeLiteralName "LightSwitch") LightSwitch)))