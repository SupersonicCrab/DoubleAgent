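; Behavior tree service that makes AI guards draw or stow their flashlight depending on whether they are lit.
; Each tick it checks the pawn's inventory for a flashlight item, then reads the character's Visibility value.
; Above zero it puts a visible hand flashlight away and unlocks the item's slot; otherwise it brings the flashlight out and locks that slot.
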(event EventReceiveTickAI
  (params (OwnerController :type AI%20Controller%20Object%20Reference) (ControlledPawn :type Pawn%20Object%20Reference) (DeltaSeconds :type Float%20%28single-precision%29))
  (bind _asbp_aicharacter_base_character (Utilities|Casting|CastToBP_AICharacterBase_CHARACTER ControlledPawn))
  (bind _asbp_guard_character (Utilities|Casting|CastToBP_Guard_CHARACTER _asbp_aicharacter_base_character))
  (bind _inventorycomponent (Variables|/Game/AI/NPC/BP_AICharacterBase_CHARACTER.BP_AICharacterBase_CHARACTER_C|GetInventoryComponent _asbp_aicharacter_base_character))
  (bind _flashlighthand (Variables|/Game/AI/NPC/Guard/BP_Guard_CHARACTER.BP_Guard_CHARACTER_C|GetFlashlightHand _asbp_guard_character))
  (bind _bvisible (Variables|/Script/Engine.SceneComponent|GetbVisible _flashlighthand))
  (bind (_itemfound _foundstructure _indexfound) (Default|CheckItemClass _inventorycomponent "/Game/Inventory/Item/NPCItems/BP_Flashlight_Item.BP_Flashlight_Item_C"))
  (if _itemfound
    (if (> (Variables|/Script/DoubleAgent.BaseCharacter_CHARACTER|GetVisibility _asbp_aicharacter_base_character) 0) ; If character is lit
      (if _bvisible ; If flashlight is out
        (Default|NetSetFlashlightOut _asbp_guard_character false)
        (Default|ItemLockSwitch _inventorycomponent _foundstructure _indexfound false))
      (elif (not _bvisible) ; If flashlight out
        (Default|NetSetFlashlightOut _asbp_guard_character true)
        (Default|ItemLockSwitch _inventorycomponent _foundstructure _indexfound true)))))