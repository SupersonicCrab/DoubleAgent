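; Behavior tree service that acts as a distance-based LOD for AI perception update rates.
; Each tick it finds the distance from the AI controller to the nearest player character.
; It then sets the base AI controller's perception and perception memory FPS to default, half, or 1 using two distance thresholds.
; A true Suspicious blackboard value bypasses the distance tiers and keeps both rates at default.
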(event EventReceiveTickAI
  (params (OwnerController :type AI%20Controller%20Object%20Reference) (ControlledPawn :type Pawn%20Object%20Reference) (DeltaSeconds :type Float%20%28single-precision%29))
  (bind _asbp_aicontroller_base_aicontroller (Utilities|Casting|CastToBP_AIControllerBase_AICONTROLLER OwnerController))
  (bind _defaultperceptionfps (Variables|/Game/AI/NPC/BP_AIControllerBase_AICONTROLLER.BP_AIControllerBase_AICONTROLLER_C|GetDefaultPerceptionFPS _asbp_aicontroller_base_aicontroller))
  (bind _defaultmemoryperceptionfps (Variables|/Game/AI/NPC/BP_AIControllerBase_AICONTROLLER.BP_AIControllerBase_AICONTROLLER_C|GetDefaultMemoryPerceptionFPS _asbp_aicontroller_base_aicontroller))
  (bind _outactors (Actor|GetAllActorsOfClass "/Game/Player/BP_Player_CHARACTER.BP_Player_CHARACTER_C"))
  (Variables|Default|SetminimumDistance 0.0) ; Reset minimum distance
  (for _array_element _outactors
    ;[1 1 1] Get minimum distance of all players
    (if (or (== (Variables|Default|GetminimumDistance) 0.0) (< (Transformation|GetDistanceTo OwnerController _array_element) (Variables|Default|GetminimumDistance)))
      (Variables|Default|SetminimumDistance (Transformation|GetDistanceTo OwnerController _array_element))))
  ;[1 1 1] LOD logic
  (if (ScalableFloat|GetValueasBool (AI|GetBlackboard ControlledPawn) (Utilities|Name|MakeLiteralName "Suspicious"))
    (Variables|/Game/AI/NPC/BP_AIControllerBase_AICONTROLLER.BP_AIControllerBase_AICONTROLLER_C|SetPerceptionFPS _asbp_aicontroller_base_aicontroller (Variables|/Game/AI/NPC/BP_AIControllerBase_AICONTROLLER.BP_AIControllerBase_AICONTROLLER_C|GetDefaultPerceptionFPS _asbp_aicontroller_base_aicontroller)) ; Set perception to default if suspicious
    (Variables|/Game/AI/NPC/BP_AIControllerBase_AICONTROLLER.BP_AIControllerBase_AICONTROLLER_C|SetPerceptionMemoryFPS _asbp_aicontroller_base_aicontroller (Variables|/Game/AI/NPC/BP_AIControllerBase_AICONTROLLER.BP_AIControllerBase_AICONTROLLER_C|GetDefaultMemoryPerceptionFPS _asbp_aicontroller_base_aicontroller)) ; Set perception memory to default if suspicious
    (elif (>= (Variables|Default|GetminimumDistance) (Variables|Default|Get1FPSDistance))
      (Variables|/Game/AI/NPC/BP_AIControllerBase_AICONTROLLER.BP_AIControllerBase_AICONTROLLER_C|SetPerceptionFPS _asbp_aicontroller_base_aicontroller 1.0) ; Set FPS to 1 if equal or above 1FPSDistance
      (Variables|/Game/AI/NPC/BP_AIControllerBase_AICONTROLLER.BP_AIControllerBase_AICONTROLLER_C|SetPerceptionMemoryFPS _asbp_aicontroller_base_aicontroller 1.0) ; Set FPS to 1 if equal or above 1FPSDistance
      (elif (>= (Variables|Default|GetminimumDistance) (Variables|Default|GethalfFPSDistance))
        (Variables|/Game/AI/NPC/BP_AIControllerBase_AICONTROLLER.BP_AIControllerBase_AICONTROLLER_C|SetPerceptionFPS _asbp_aicontroller_base_aicontroller (/ _defaultperceptionfps 2.0)) ; Set FPS to half if equal or above halfFPSDistance
        (Variables|/Game/AI/NPC/BP_AIControllerBase_AICONTROLLER.BP_AIControllerBase_AICONTROLLER_C|SetPerceptionMemoryFPS _asbp_aicontroller_base_aicontroller (/ _defaultmemoryperceptionfps 2.0)) ; Set FPS to half if equal or above halfFPSDistance
        (else
          (Variables|/Game/AI/NPC/BP_AIControllerBase_AICONTROLLER.BP_AIControllerBase_AICONTROLLER_C|SetPerceptionFPS _asbp_aicontroller_base_aicontroller _defaultperceptionfps) ; Set FPS to default if within both distances
          (Variables|/Game/AI/NPC/BP_AIControllerBase_AICONTROLLER.BP_AIControllerBase_AICONTROLLER_C|SetPerceptionMemoryFPS _asbp_aicontroller_base_aicontroller _defaultmemoryperceptionfps) ; Set FPS to default if within both distances
        )))))