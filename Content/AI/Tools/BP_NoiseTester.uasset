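; BP_NoiseTester is an AI debug actor that emits test noise events at its own location for AI hearing.
; GenerateNoise reports a normal-range "Noise" event and GenerateLoudNoise a long-range "LoudNoise" event presented as a gunshot, each with a debug print of the position.
; Ranges come from an FSoundType struct of quiet, normal and loud distances.
; The event graph is empty, so both functions rely on being triggered externally.
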(event EventBeginPlay)

(event Collision|EventActorBeginOverlap
  (params (OtherActor :type Actor%20Object%20Reference)))

(event EventTick
  (params (DeltaSeconds :type Float%20%28single-precision%29)))

(fn ConstructionScript)

(fn GenerateNoise
  (bind _returnvalue (Transformation|GetActorLocation))
  (Class|AISenseHearing|ReportNoiseEvent _returnvalue 1.0 self (.normal (Utilities|Struct|MakeFSoundType 5e+02 1.5e+03 3.5e+03)) "Noise")
  (Development|PrintString (Utilities|String|Append "Made a noise at " (Utilities|String|ToString(Vector) _returnvalue))))

(fn GenerateLoudNoise
  (bind _returnvalue (Transformation|GetActorLocation))
  (Class|AISenseHearing|ReportNoiseEvent _returnvalue 1.0 self (.loud (Utilities|Struct|MakeFSoundType 5e+02 1.5e+03 3.5e+03)) "LoudNoise")
  (Development|PrintString (Utilities|String|Append "Made a gun shot at " (Utilities|String|ToString(Vector) _returnvalue))))