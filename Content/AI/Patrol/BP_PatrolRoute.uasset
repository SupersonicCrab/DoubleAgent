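; Patrol route asset that stores an AI path as points, each with a location, look location and wait time.
; Authoring functions add points, clear the route, or write the Select vector into the indexed point's location or look target.
; DebugLocation and DebugLook mirror Path as flat vector arrays, and SetPathFromDebug copies their edits back.
; BeginPlay empties these debug arrays and resets the selection to save memory, leaving Path intact.
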(event EventBeginPlay
  ;[1 1 1] Clearing arrays, index, and selector to free up memory
  (Utilities|Array|Clear (Variables|HelperFunctions|GetDebugLook))
  (Utilities|Array|Clear (Variables|HelperFunctions|GetDebugLocation))
  (Variables|HelperFunctions|SetPathIndex 0)
  (Variables|HelperFunctions|SetSelect "250.000000, 0, 0"))

(fn ConstructionScript)

(fn SetLocation
  (bind _path (Variables|Default|GetPath))
  (bind _pathindex (Variables|HelperFunctions|GetPathIndex))
  (bind _returnvalue (Utilities|Array|Length _path))
  (bind _output (Utilities|Array|Get(acopy) _path _pathindex))
  (if (and (!= _returnvalue 0) (> _returnvalue (Variables|HelperFunctions|GetPathIndex))) ; If path length is not zero and index is in range
    (Utilities|Array|SetArrayElem _path _pathindex (Utilities|Struct|MakeFPatrol (Variables|HelperFunctions|GetSelect) (.looklocation _output) (.waittime _output)))
    (HelperFunctions|DebugUpdate)))

(fn SetLook
  (bind _path (Variables|Default|GetPath))
  (bind _pathindex (Variables|HelperFunctions|GetPathIndex))
  (bind _returnvalue (Utilities|Array|Length _path))
  (bind _output (Utilities|Array|Get(acopy) _path _pathindex))
  (if (and (!= _returnvalue 0) (> _returnvalue (Variables|HelperFunctions|GetPathIndex))) ; If path length is not zero and index is in range
    (Utilities|Array|SetArrayElem _path _pathindex (Utilities|Struct|MakeFPatrol (.location _output) (Variables|HelperFunctions|GetSelect) (.waittime _output)))
    (HelperFunctions|DebugUpdate)))

(fn DebugUpdate
  (Utilities|Array|Clear (Variables|HelperFunctions|GetDebugLocation))
  (Utilities|Array|Clear (Variables|HelperFunctions|GetDebugLook))
  (for _array_element (Variables|Default|GetPath)
    (Utilities|Array|Add (Variables|HelperFunctions|GetDebugLocation) (.location _array_element))
    (Utilities|Array|Add (Variables|HelperFunctions|GetDebugLook) (.looklocation _array_element))))

(fn AddPath
  (bind _path (Variables|Default|GetPath))
  (bind _select (Variables|HelperFunctions|GetSelect))
  (Utilities|Array|Add _path (Utilities|Struct|MakeFPatrol _select _select 0.5))
  (Variables|HelperFunctions|SetPathIndex (- (Utilities|Array|Length _path) 1))
  (HelperFunctions|DebugUpdate))

(fn Clear
  (Utilities|Array|Clear (Variables|Default|GetPath))
  (Utilities|Array|Clear (Variables|HelperFunctions|GetDebugLocation))
  (Utilities|Array|Clear (Variables|HelperFunctions|GetDebugLook))
  (Variables|HelperFunctions|SetPathIndex 0)
  (Variables|HelperFunctions|SetSelect "250.000000, 0, 0")
  (Utilities|Array|Add :TargetArray (Variables|Default|GetPath))
  (HelperFunctions|DebugUpdate))

(fn SetPathfromDebug
  (bind _path (Variables|Default|GetPath))
  (for (_array_element _array_index) (Variables|HelperFunctions|GetDebugLocation)
    (Utilities|Array|SetArrayElem _path _array_index (Utilities|Struct|MakeFPatrol _array_element (Utilities|Array|Get(acopy) (Variables|HelperFunctions|GetDebugLook) _array_index) (.waittime (Utilities|Array|Get(acopy) _path _array_index))))))