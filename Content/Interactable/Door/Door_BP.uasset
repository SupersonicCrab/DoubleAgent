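; Interactable hinged door that players open and close via Interact, with an overlap text prompt, and that NPCs operate through a nav smart link.
; Dot products against OpenDirection choose the swing side for timeline-driven rotation.
; Walking NPCs snap to interaction points for open-and-close animations; other speeds leave it open, unless a montage is playing.
; Smart-link state blocks conflicting use, while repositioning NavLink toggles the simple link for open doors.
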(event OnComponentBeginOverlap(Collision)
  (params (OverlappedComponent :type Primitive%20Component%20Object%20Reference) (OtherActor :type Actor%20Object%20Reference) (OtherComp :type Primitive%20Component%20Object%20Reference) (OtherBodyIndex :type Integer) (bFromSweep :type Boolean) (SweepResult :type Hit%20Result%20Structure%20%28by%20ref%29))
  ;[1 1 1] LogUI
  (bind _asplayer_character (Utilities|Casting|CastToPlayer_CHARACTER OtherActor))
  (if (Variables|Default|GetdoorOpen)
    (Variables|Default|SetdisplayText "Press [E] to close door")
    (else
      (Variables|Default|SetdisplayText "Press [E] to open door")))
  (bind _logid (Default|AddText (Variables|/Game/Player/Player_CHARACTER.Player_CHARACTER_C|GettextLog _asplayer_character) (Variables|Default|GetdisplayText)))
  (if (not (== _logid 666))
    (Variables|Default|SetlogID _logid)))

(event OnComponentEndOverlap(Collision)
  (params (OverlappedComponent :type Primitive%20Component%20Object%20Reference) (OtherActor :type Actor%20Object%20Reference) (OtherComp :type Primitive%20Component%20Object%20Reference) (OtherBodyIndex :type Integer))
  ;[1 1 1] LogUI
  (bind _asplayer_character (Utilities|Casting|CastToPlayer_CHARACTER OtherActor))
  (Default|RemoveText (Variables|/Game/Player/Player_CHARACTER.Player_CHARACTER_C|GettextLog _asplayer_character) (Variables|Default|GetlogID)))

(event Custom|PlayerClose
  (bind _door (Variables|Default|GetDoor))
  (bind _relativerotation (Variables|/Script/Engine.SceneComponent|GetRelativeRotation _door))
  ;[1 1 1] Player animation
  (if (== (Math|Float|Round (Math|Float|Absolute(Float) (.yaw _relativerotation))) 90) ; If door is completely open
    (if (> (.yaw _relativerotation) 0.0)
      (Variables|Default|SettempFloat 1.0)
      (bind _yaw (Timeline|PlayerCloseAnimation PlayFromStart)
        (:Update
          ;;[1 1 1] Close animation
          (Transformation|SetRelativeRotation (Variables|Default|GetDoor) (Math|Rotator|MakeRotator 0.0 0.0 (* _yaw (Variables|Default|GettempFloat))) false false))
        (:Finished
          (Variables|Default|SetdoorOpen false)
          (Transformation|SetRelativeLocation (Variables|Default|GetNavLink) "0, 0,100.000000" false false) ; Disable simple link
          (Class|NavLinkProxy|SetSmartLinkEnabled true)))
      (else
        (Variables|Default|SettempFloat -1.0)
        (Timeline|PlayerCloseAnimation PlayFromStart)))))

(event Custom|PlayerOpen
  (params (Interactor :type Actor%20Object%20Reference))
  (bind _opendirection (Variables|Default|GetOpenDirection))
  ;[1 1 1] Player animation
  (if (Class|NavLinkProxy|IsSmartLinkEnabled) ; Ensure a NPC is not interacting with door
    (Class|NavLinkProxy|SetSmartLinkEnabled false)
    (if (> (Math|Vector|DotProduct (Math|Vector|GetForwardVector (Math|Rotator|FindLookatRotation (Transformation|GetActorLocation (.AsPlayer%20CHARACTER (Utilities|Casting|CastToPlayer_CHARACTER Interactor))) (Transformation|GetWorldLocation _opendirection))) (Math|Vector|GetForwardVector _opendirection)) 0.0)
      (Variables|Default|SettempFloat 1.0)
      (bind _yaw (Timeline|PlayerOpenAnimation PlayFromStart)
        (:Update
          ;;[1 1 1] Open animation
          (Transformation|SetRelativeRotation (Variables|Default|GetDoor) (Math|Rotator|MakeRotator 0.0 0.0 (* _yaw (Variables|Default|GettempFloat))) false false))
        (:Finished
          (Variables|Default|SetdoorOpen true)
          (Transformation|ResetRelativeTransform (Variables|Default|GetNavLink)) ; Activate simple link
        ))
      (else
        (Variables|Default|SettempFloat -1.0)
        (Timeline|PlayerOpenAnimation PlayFromStart)))))

(event EventBeginPlay
  ;[1 1 1] Setup
  (if (Variables|Default|GetdoorOpen)
    (CallFunction|ForceOpen)))

(event EventSmartLinkReached
  (params (Agent :type Actor%20Object%20Reference) (Destination :type Vector%20%28by%20ref%29 :default "0, 0, 0"))
  (bind _returnvalue (AI|GetAIController Agent))
  (bind _returnvalue_2 (Transformation|GetActorForwardVector Agent))
  (bind _asaicharacter_base_character (Utilities|Casting|CastToAICharacterBase_CHARACTER Agent))
  (bind _opendirection (Variables|Default|GetOpenDirection))
  (bind _returnvalue_3 (Math|Vector|GetForwardVector _opendirection))
  (bind _returnvalue_4 (Math|Vector|DotProduct _returnvalue_2 _returnvalue_3))
  (bind _returnvalue_5 (> _returnvalue_4 0.0))
  (if (Class|NavLinkProxy|IsSmartLinkEnabled)
    (Class|NavLinkProxy|SetSmartLinkEnabled false) ; Disable nav link
    (Transformation|SetActorRotation Agent (Math|Rotator|MakeRotator 0.0 0.0 (.yaw (Math|Rotator|FindLookatRotation (Transformation|GetActorLocation Agent) (Transformation|GetActorLocation)))) true)
    (Class|AIController|ClaimTaskResource _returnvalue "/Script/AIModule.AIResource_Movement") ; Disable NPC movement
    (if (not (Class|AnimInstance|IsAnyMontagePlaying (Components|SkeletalMesh|GetAnimInstance (Variables|/Script/Engine.Character|GetMesh _asaicharacter_base_character)))) ; If NPC is not performing a montage
      (if (== (Variables|/Script/Engine.CharacterMovementComponent|GetMaxWalkSpeed (Variables|/Script/Engine.Character|GetCharacterMovement _asaicharacter_base_character)) 1.3e+02) ; If movement speed is walking
        ;[1 1 1] Open and close animation
        (if _returnvalue_5 ; Figure out what direction NPC is interacting from
          ;;[1 1 1] Outwards
          (Transformation|SetActorTransform Agent (Transformation|GetWorldTransform (Variables|Default|GetInteractionPointOutward)) false true)
          (Class|AnimInstance|PlaySlotAnimationasDynamicMontage (Components|SkeletalMesh|GetAnimInstance (Variables|/Script/Engine.Character|GetMesh (.AsCharacter (Utilities|Casting|CastToCharacter Agent)))) "/Game/Animations/Sequences/Standing/Interaction/OpenDoorOutwards_AS.OpenDoorOutwards_AS" "DefaultSlot" 0.25 0.25 1.0 1 -1.0 0.0)
          (bind _yaw (Timeline|NPCInteractionOutward PlayFromStart)
            (:Update
              (Transformation|SetRelativeRotation (Variables|Default|GetDoor) (Math|Rotator|MakeRotator 0.0 0.0 _yaw) false false))
            (:Finished
              (Class|AIController|UnclaimTaskResource _returnvalue "/Script/AIModule.AIResource_Movement" :!label _label) ; Unlock NPC movement
              (Class|NavLinkProxy|SetSmartLinkEnabled true) ; Renable smartlink usage
            ))
          (else
            ;;[1 1 1] Inwards
            (Transformation|SetActorTransform Agent (Transformation|GetWorldTransform (Variables|Default|GetInteractionPointInward)) false true)
            (Class|AnimInstance|PlaySlotAnimationasDynamicMontage (Components|SkeletalMesh|GetAnimInstance (Variables|/Script/Engine.Character|GetMesh (.AsCharacter (Utilities|Casting|CastToCharacter Agent)))) "/Game/Animations/Sequences/Standing/Interaction/OpenDoorInwards_AS.OpenDoorInwards_AS" "DefaultSlot" 0.25 0.25 1.0 1 -1.0 0.0)
            (bind _yaw_2 (Timeline|NPCInteractionInward PlayFromStart)
              (:Update
                (Transformation|SetRelativeRotation (Variables|Default|GetDoor) (Math|Rotator|MakeRotator 0.0 0.0 _yaw_2) false false))
              (:Finished
                (goto _label)))))
        (else
          ;[1 1 1] Open door
          (if _returnvalue_5
            (Variables|Default|SettempFloat 1.0)
            (bind _yaw_3 (Timeline|NPCOpenAnimation PlayFromStart)
              (:Update
                (Transformation|SetRelativeRotation (Variables|Default|GetDoor) (Math|Rotator|MakeRotator 0.0 0.0 (* _yaw_3 (Variables|Default|GettempFloat))) false false))
              (:Finished
                (Variables|Default|SetdoorOpen true)
                (Transformation|ResetRelativeTransform (Variables|Default|GetNavLink)) ; Activate simple link
                (Class|AIController|UnclaimTaskResource _returnvalue "/Script/AIModule.AIResource_Movement")))
            (else
              (Variables|Default|SettempFloat -1.0)
              (Timeline|NPCOpenAnimation PlayFromStart))))))))

(event EventInteract
  (params (Interactor :type Actor%20Object%20Reference))
  ;[1 1 1] Interact
  (if (Variables|Default|GetdoorOpen)
    (CallFunction|CloseDoor)
    (else
      (CallFunction|OpenDoor Interactor))))

(fn ConstructionScript)

(fn OpenDoor
  (params (Interactor :type Actor%20Object%20Reference))
  (CallFunction|PlayerOpen Interactor))

(fn CloseDoor
  (CallFunction|PlayerClose))

(fn ForceOpen
  (Variables|Default|SetdoorOpen true)
  (Transformation|SetRelativeRotation (Variables|Default|GetDoor) (Math|Rotator|MakeRotator 0.0 0.0 9e+01) false false)
  (Transformation|ResetRelativeTransform (Variables|Default|GetNavLink)) ; Enable simple link
)