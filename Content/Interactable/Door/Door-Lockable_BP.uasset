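; Lockable door Blueprint that opens only when the player carries a guard keycard.
; OpenDoor checks the player character's inventory component for the Item_GuardCard class, then rotates the door 90 degrees and marks it open.
; Without the card it prints a hint message, suppressed when the interaction comes from a bot, although the check always reads the player's inventory.
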(event EventBeginPlay)

(event Collision|EventActorBeginOverlap
  (params (OtherActor :type Actor%20Object%20Reference)))

(event EventTick
  (params (DeltaSeconds :type Float%20%28single-precision%29)))

(event EventOpenDoor
  (params (BotInteraction :type Boolean))
  (bind _asplayer_character (Utilities|Casting|CastToPlayer_CHARACTER (Game|GetPlayerCharacter 0)))
  (bind _itemfound (Default|CheckItemClass (Variables|/Game/Player/Player_CHARACTER.Player_CHARACTER_C|GetInventoryComponent _asplayer_character) "/Game/Inventory/Item/Item_GuardCard.Item_GuardCard_C"))
  (if _itemfound
    (Transformation|AddActorLocalRotation "0,90.000000, 0" false false)
    (Variables|Default|SetDoorOpen true)
    (elif (not BotInteraction)
      (Development|PrintString "You need a keycard to open this door, come back when you have it"))))

(fn ConstructionScript
  (|CallParentFunction))