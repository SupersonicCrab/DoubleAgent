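; Interactable door, likely a nav link proxy, that players open or close through an interaction prompt and NPCs use while navigating.
; Timelines swing it, using a dot product to pick direction from the user's side.
; Walking NPCs snap to an interaction point for a montage as the door opens and closes; others leave it open.
; Open doors swap the smart link for a simple one, which closing moves away.
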(event OnComponentBeginOverlap(Collision)
  (params (OverlappedComponent :type Primitive%20Component%20Object%20Reference) (OtherActor :type Actor%20Object%20Reference) (OtherComp :type Primitive%20Component%20Object%20Reference) (OtherBodyIndex :type Integer) (bFromSweep :type Boolean) (SweepResult :type Hit%20Result%20Structure%20%28by%20ref%29))
  ;[1 1 1] Context Menu
  (bind _asbp_player_character (Utilities|Casting|CastToBP_Player_CHARACTER OtherActor))
  (bind _asbp_spy_player_playercontroller (Utilities|Casting|CastToBP_SpyPlayer_PLAYERCONTROLLER (Pawn|GetController _asbp_player_character)))
  (if (Variables|Default|GetdoorOpen)
    (Variables|Default|SetdisplayText "Close Door")
    (else
      (Variables|Default|SetdisplayText "Open Door")))
  (Default|OverlapBegin (Variables|/Game/Player/BP_SpyPlayer_PLAYERCONTROLLER.BP_SpyPlayer_PLAYERCONTROLLER_C|GetInteractionBox _asbp_spy_player_playercontroller) (Variables|Default|GetdisplayText) true false))

(event OnComponentEndOverlap(Collision)
  (params (OverlappedComponent :type Primitive%20Component%20Object%20Reference) (OtherActor :type Actor%20Object%20Reference) (OtherComp :type Primitive%20Component%20Object%20Reference) (OtherBodyIndex :type Integer))
  ;[1 1 1] Context Menu
  (bind _asbp_player_character (Utilities|Casting|CastToBP_Player_CHARACTER OtherActor))
  (bind _asbp_spy_player_playercontroller (Utilities|Casting|CastToBP_SpyPlayer_PLAYERCONTROLLER (Pawn|GetController _asbp_player_character)))
  (Default|OverlapEnd (Variables|/Game/Player/BP_SpyPlayer_PLAYERCONTROLLER.BP_SpyPlayer_PLAYERCONTROLLER_C|GetInteractionBox _asbp_spy_player_playercontroller) true false))

(event Custom|PlayerClose
  (bind _door (Variables|Default|GetDoor))
  (bind _relativerotation (Variables|/Script/Engine.SceneComponent|GetRelativeRotation _door))
  ;[1 1 1] Player animation
  (if (== (Math|Float|Round (Math|Float|Absolute(Float) (.yaw _relativerotation))) 90) ; If door is completely open
    (if (> (.yaw _relativerotation) 0.0)
      (Variables|Default|SettempFloat 1.0)
      (bind _yaw (Timeline|PlayerCloseAnimation PlayFromStart)
        (:Update
          (Transformation|SetRelativeRotation (Variables|Default|GetDoor) (Math|Rotator|MakeRotator 0.0 0.0 (* _yaw (Variables|Default|GettempFloat))) false false))
        (:Finished
          (Variables|Default|SetdoorOpen false)
          (Transformation|SetRelativeLocation (Variables|Default|GetNavLink) "0, 0,100.000000" false false) ; Disable simple link
          (Class|NavLinkProxy|SetSmartLinkEnabled true)))
      (else
        (Variables|Default|SettempFloat -1.0)
        (Timeline|PlayerCloseAnimation PlayFromStart)))))

(event Custom|PlayerOpen
  (params (Interactor :type Actor%20Object%20Reference))
  (bind _opendirection (Variables|Default|GetOpenDirection))
  ;[1 1 1] Player animation
  (if (Class|NavLinkProxy|IsSmartLinkEnabled) ; Ensure a NPC is not interacting with door
    (Class|NavLinkProxy|SetSmartLinkEnabled false)
    (if (> (Math|Vector|DotProduct (Math|Vector|GetForwardVector (Math|Rotator|FindLookatRotation (Transformation|GetActorLocation (.AsBP%20Player%20CHARACTER (Utilities|Casting|CastToBP_Player_CHARACTER Interactor))) (Transformation|GetWorldLocation _opendirection))) (Math|Vector|GetForwardVector _opendirection)) 0.0)
      (Variables|Default|SettempFloat 1.0)
      (bind _yaw (Timeline|PlayerOpenAnimation PlayFromStart)
        (:Update
          (Transformation|SetRelativeRotation (Variables|Default|GetDoor) (Math|Rotator|MakeRotator 0.0 0.0 (* _yaw (Variables|Default|GettempFloat))) false false))
        (:Finished
          (Variables|Default|SetdoorOpen true)
          (Transformation|ResetRelativeTransform (Variables|Default|GetNavLink)) ; Activate simple link
        ))
      (else
        (Variables|Default|SettempFloat -1.0)
        (Timeline|PlayerOpenAnimation PlayFromStart)))))

(event EventBeginPlay
  ;[1 1 1] Setup
  (if (Variables|Default|GetdoorOpen)
    (CallFunction|ForceOpen)))

(event EventSmartLinkReached
  (params (Agent :type Actor%20Object%20Reference) (Destination :type Vector%20%28by%20ref%29 :default "0, 0, 0"))
  (bind _returnvalue (Transformation|GetActorLocation Agent))
  (bind _returnvalue_2 (Transformation|GetActorLocation))
  (bind _asbp_aicharacter_base_character (Utilities|Casting|CastToBP_AICharacterBase_CHARACTER Agent))
  (bind _opendirection (Variables|Default|GetOpenDirection))
  (bind _returnvalue_3 (Math|Rotator|FindLookatRotation _returnvalue _returnvalue_2))
  (bind _returnvalue_4 (Math|Vector|GetForwardVector _opendirection))
  (bind _mesh (Variables|/Script/Engine.Character|GetMesh _asbp_aicharacter_base_character))
  (bind _returnvalue_5 (Math|Vector|GetForwardVector _returnvalue_3))
  (bind _returnvalue_6 (Components|SkeletalMesh|GetAnimInstance _mesh))
  (bind _returnvalue_7 (Math|Vector|DotProduct _returnvalue_5 _returnvalue_4))
  (bind _returnvalue_8 (> _returnvalue_7 0.0))
  ;[1 1 1] NPC door interaction
  (if (Class|NavLinkProxy|IsSmartLinkEnabled) ; If smart link is enabled
    (Class|AIController|ClaimTaskResource (AI|GetAIController _asbp_aicharacter_base_character) "/Script/AIModule.AIResource_Movement") ; Claim NPC movement
    (if (== (Variables|/Script/Engine.CharacterMovementComponent|GetMaxWalkSpeed (Variables|/Script/Engine.Character|GetCharacterMovement _asbp_aicharacter_base_character)) 1.3e+02) ; Is NPC walking
      (if _returnvalue_8 ; If interaction direction is outward
        (Transformation|SetActorTransform _asbp_aicharacter_base_character (Transformation|GetWorldTransform (Variables|Default|GetInteractionPointOutward)) false true) ; Move NPC to interaction location
        (Class|AnimInstance|PlaySlotAnimationasDynamicMontage _returnvalue_6 "/Game/Animations/Sequences/Standing/Interaction/A_OpenDoorOutwards.A_OpenDoorOutwards" "DefaultSlot" 0.25 0.25 1.0 1 -1.0 0.0) ; Play animation
        (bind _yaw (Timeline|NPCOutwardAnimation PlayFromStart)
          (:Update
            (Transformation|SetRelativeRotation (Variables|Default|GetDoor) (Math|Rotator|MakeRotator 0.0 0.0 _yaw) false false) ; Animate door opening and closing
          )
          (:Finished
            (Class|AIController|UnclaimTaskResource (AI|GetAIController _asbp_aicharacter_base_character) "/Script/AIModule.AIResource_Movement" :!label _label) ; Unclaim NPC movement
          ))
        (else
          (Transformation|SetActorTransform _asbp_aicharacter_base_character (Transformation|GetWorldTransform (Variables|Default|GetInteractionPointInward)) false true) ; Move NPC to interaction location
          (Class|AnimInstance|PlaySlotAnimationasDynamicMontage _returnvalue_6 "/Game/Animations/Sequences/Standing/Interaction/A_OpenDoorInwards.A_OpenDoorInwards" "DefaultSlot" 0.25 0.25 1.0 1 -1.0 0.0) ; Play animation
          (bind _yaw_2 (Timeline|NPCInwardAnimation PlayFromStart)
            (:Update
              (Transformation|SetRelativeRotation (Variables|Default|GetDoor) (Math|Rotator|MakeRotator 0.0 0.0 _yaw_2) false false) ; Animate door opening and closing
            )
            (:Finished
              (goto _label)))))
      (else
        (Class|NavLinkProxy|SetSmartLinkEnabled false)
        (if _returnvalue_8 ; If direction is outward
          (Variables|Default|SettempFloat 1.0)
          (bind _yaw_3 (Timeline|NPCOpenAnimation PlayFromStart)
            (:Update
              (Transformation|SetRelativeRotation (Variables|Default|GetDoor) (Math|Rotator|MakeRotator 0.0 0.0 (* _yaw_3 (Variables|Default|GettempFloat))) false false))
            (:Finished
              (Variables|Default|SetdoorOpen true)
              (Transformation|ResetRelativeTransform (Variables|Default|GetNavLink)) ; Activate simple link
              (Class|AIController|UnclaimTaskResource (AI|GetAIController _asbp_aicharacter_base_character) "/Script/AIModule.AIResource_Movement")))
          (else
            (Variables|Default|SettempFloat -1.0)
            (Timeline|NPCOpenAnimation PlayFromStart)))))))

(event EventInteract
  (params (Interactor :type Actor%20Object%20Reference))
  ;[1 1 1] Interact
  (if (Variables|Default|GetdoorOpen)
    (CallFunction|CloseDoor)
    (else
      (CallFunction|OpenDoor Interactor))))

(fn ConstructionScript)

(fn OpenDoor
  (params (Interactor :type Actor%20Object%20Reference))
  (CallFunction|PlayerOpen Interactor))

(fn CloseDoor
  (CallFunction|PlayerClose))

(fn ForceOpen
  (Variables|Default|SetdoorOpen true)
  (Transformation|SetRelativeRotation (Variables|Default|GetDoor) (Math|Rotator|MakeRotator 0.0 0.0 9e+01) false false)
  (Transformation|ResetRelativeTransform (Variables|Default|GetNavLink)) ; Enable simple link
)