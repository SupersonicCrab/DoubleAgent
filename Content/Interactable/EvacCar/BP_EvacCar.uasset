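; BP_EvacCar is an interactable evacuation car that ends the level, optionally requiring an inventory item.
; Interact runs an item check through the game mode's InventoryServerCheck, then branches on no requirement, item held or item missing.
; Successful branches show a notification, slow time and, after a short delay, call the player's AddWinScreen.
; A missing item only triggers a notification naming it; custom depth stencil drives the highlight outline.
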(event Custom|ItemCheck
  (params (Player :type BP%20Player%20CHARACTER%20Object%20Reference))
  (bind _requireditem (Variables|Default|GetRequiredItem))
  (if (== _requireditem 0)
    (Variables|Default|SetItemCheckLevel 0)
    (else
      (bind _success (Default|InventoryServerCheck (.AsBP%20Spy%20Player%20GAMEMODE (Utilities|Casting|CastToBP_SpyPlayer_GAMEMODE (Game|GetGameMode))) Player _requireditem))
      (if _success
        (Variables|Default|SetItemCheckLevel 1)
        (else
          (Variables|Default|SetItemCheckLevel 2)))))
  (CallFunction|HandlePlayerCollision Player (Variables|Default|GetItemCheckLevel)))

(event Custom|HandlePlayerCollision
  (params (Player :type BP%20Player%20CHARACTER%20Object%20Reference) (ItemCheckLevel :type Integer))
  (bind _requireditem (Variables|Default|GetRequiredItem))
  (bind _itemstructure (Utilities|GetClassDefaults _requireditem))
  (switch int ItemCheckLevel
    (:0
      (Default|GlobalNotificationStart Player "Traveling to new level" "/Game/Art/Textures/UI/Icons/Logos/T_DefaultNeon.T_DefaultNeon")
      (Default|NetRequestSetTimeScale Player 0.5 :!label _label)
      (Utilities|FlowControl|Delay 0.75)
      (Default|AddWinScreen Player))
    (:1
      (Default|GlobalNotificationStart Player "You beat this level" "/Game/Art/Textures/UI/Icons/Logos/T_DefaultNeon.T_DefaultNeon")
      (goto _label))
    (:2
      (Default|GlobalNotificationStart Player (Utilities|Text|ToText(String) (Utilities|String|Append "You need [" (Utilities|String|ToString(Text) (.name _itemstructure)) "] to complete this level")) (.thumbnail _itemstructure)))))

(event Custom|AddWinScreen
  (params (Player :type BP%20Player%20CHARACTER%20Object%20Reference))
  (bind _returnvalue (UserInterface|CreateWidget "/Game/UI/Health/EndScreens/WBP_WinScreen.WBP_WinScreen_C"))
  (UserInterface|Viewport|AddtoViewport _returnvalue 0)
  (Default|NetRequestSetTimeScale Player 0.0)
  (Variables|/Script/Engine.PlayerController|SetbShowMouseCursor (.AsBP%20Spy%20Player%20PLAYERCONTROLLER (Utilities|Casting|CastToBP_SpyPlayer_PLAYERCONTROLLER (Pawn|GetController Player))) true))

(event EventInteract
  (params (Interactor :type Actor%20Object%20Reference))
  (bind _asbp_player_character (Utilities|Casting|CastToBP_Player_CHARACTER Interactor))
  (CallFunction|ItemCheck _asbp_player_character))

(event EventEnableOutline
  (bind _staticmesh (Variables|Default|GetStaticMesh))
  (Rendering|SetRenderCustomDepth _staticmesh true)
  (Rendering|SetCustomDepthStencilValue _staticmesh 253))

(event EventDisableOutline
  (bind _staticmesh (Variables|Default|GetStaticMesh))
  (Rendering|SetCustomDepthStencilValue _staticmesh 0)
  (Rendering|SetRenderCustomDepth _staticmesh false))

(fn ConstructionScript)

(fn GetCenter
  (return (.Origin (Collision|GetComponentBounds (Variables|Default|GetStaticMesh)))))

(fn GetInteractText
  (return "Evac Mission"))