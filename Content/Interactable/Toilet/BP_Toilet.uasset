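; BP_Toilet is an interactable toilet prop that the player can flush.
; Interact plays its FMOD audio component unless it is already playing, so flushes do not overlap.
; Outline events toggle custom depth with a stencil value on the Toilet component for highlighting.
; It also supplies the "Flush toilet" prompt text and the component's bounds origin as its center.
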(event EventBeginPlay)

(event Collision|EventActorBeginOverlap
  (params (OtherActor :type Actor%20Object%20Reference)))

(event EventTick
  (params (DeltaSeconds :type Float%20%28single-precision%29)))

(event EventInteract
  (params (Interactor :type Actor%20Object%20Reference))
  (bind _fmodaudio (Variables|Default|GetFMODAudio))
  (bind _returnvalue (Class|FMODAudioComponent|IsPlaying _fmodaudio))
  (if (not _returnvalue)
    (Class|FMODAudioComponent|Play _fmodaudio)))

(event EventEnableOutline
  (bind _toilet (Variables|Default|GetToilet))
  (Rendering|SetRenderCustomDepth _toilet true)
  (Rendering|SetCustomDepthStencilValue _toilet 253))

(event EventDisableOutline
  (bind _toilet (Variables|Default|GetToilet))
  (Rendering|SetCustomDepthStencilValue _toilet 0)
  (Rendering|SetRenderCustomDepth _toilet false))

(fn ConstructionScript)

(fn GetCenter
  (return (.Origin (Collision|GetComponentBounds (Variables|Default|GetToilet)))))

(fn GetInteractText
  (return "Flush toilet"))