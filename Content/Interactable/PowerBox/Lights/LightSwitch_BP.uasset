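; Interactable wall switch that toggles all HouseLight_BP actors sharing its LightGroup, provided the power is on.
; BeginPlay caches the power state from PowerBox_BP and gathers the group's lights, while box overlaps show and remove the player's prompt.
; Enable and disable functions switch each light and notify the Room of its lit state.
; Disabling with FromPowerBox set preserves the switch's state, letting RestoreLights reapply it later.
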(event OnComponentBeginOverlap(Box)
  (params (OverlappedComponent :type Primitive%20Component%20Object%20Reference) (OtherActor :type Actor%20Object%20Reference) (OtherComp :type Primitive%20Component%20Object%20Reference) (OtherBodyIndex :type Integer) (bFromSweep :type Boolean) (SweepResult :type Hit%20Result%20Structure%20%28by%20ref%29))
  ;[1 1 1] Set interaction text
  (bind _asplayer_character (Utilities|Casting|CastToPlayer_CHARACTER OtherActor))
  (if (Variables|Default|GetLightGroupOn)
    (Variables|Default|SetInteractText "Press [E] to turn lights off")
    (else
      (Variables|Default|SetInteractText "Press [E] to turn lights on")))
  (bind _logid (Default|AddText (Variables|/Game/Player/Player_CHARACTER.Player_CHARACTER_C|GetTextLog _asplayer_character) (Variables|Default|GetInteractText)))
  (if (not (== _logid 666))
    (Variables|Default|SetLogID _logid)))

(event OnComponentEndOverlap(Box)
  (params (OverlappedComponent :type Primitive%20Component%20Object%20Reference) (OtherActor :type Actor%20Object%20Reference) (OtherComp :type Primitive%20Component%20Object%20Reference) (OtherBodyIndex :type Integer))
  ;[1 1 1] Set interaction text
  (bind _asplayer_character (Utilities|Casting|CastToPlayer_CHARACTER OtherActor))
  (Default|RemoveText (Variables|/Game/Player/Player_CHARACTER.Player_CHARACTER_C|GetTextLog _asplayer_character) (Variables|Default|GetLogID)))

(event EventBeginPlay
  ;[1 1 1] Get current power box settings
  (bind _returnvalue (Actor|GetActorOfClass "/Game/Interactable/PowerBox/PowerBox_BP.PowerBox_BP_C"))
  (bind _output_get (Variables|Default|SetPowerBox _returnvalue))
  (Variables|Default|SetPowerOn (Variables|/Game/Interactable/PowerBox/PowerBox_BP.PowerBox_BP_C|GetLightsOn _output_get))
  (bind _outactors (Actor|GetAllActorsOfClass "/Game/Interactable/PowerBox/Lights/HouseLight_BP.HouseLight_BP_C"))
  (for _array_element _outactors
    (if (== (Variables|/Game/Interactable/PowerBox/Lights/HouseLight_BP.HouseLight_BP_C|GetLightGroup _array_element) (Variables|Default|GetLightGroup))
      (Utilities|Array|Add (Variables|Default|GetGroupLights) _array_element))))

(event EventInteract
  (params (Interactor :type Actor%20Object%20Reference))
  ;[1 1 1] Toggle lights on & off
  (if (Variables|Default|GetPowerOn)
    (if (Variables|Default|GetLightGroupOn)
      (CallFunction|DisableLightGroup false)
      (Variables|Default|SetLightGroupOn false)
      (else
        (CallFunction|EnableLightGroup)
        (Variables|Default|SetLightGroupOn true)))
    (else
      (Development|PrintString "Power is off"))))

(fn ConstructionScript)

(fn EnableLightGroup
  (for _array_element (Variables|Default|GetGroupLights)
    (Default|Turnon _array_element)
    (bind _output_get (Variables|Default|SetLightGroupOn true))
    (Default|LightUpdate (Variables|Default|GetRoom) _output_get self)))

(fn DisableLightGroup
  (params (FromPowerBox :type Boolean))
  (for _array_element (Variables|Default|GetGroupLights)
    (Default|TurnOff _array_element)
    (if FromPowerBox
      _
      (else
        (Variables|Default|SetLightGroupOn false)))
    (Default|LightUpdate (Variables|Default|GetRoom) false self)))

(fn RestoreLights
  (if (Variables|Default|GetLightGroupOn)
    (CallFunction|EnableLightGroup)
    (else
      (CallFunction|DisableLightGroup false))))