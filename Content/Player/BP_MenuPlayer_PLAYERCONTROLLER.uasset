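; Player controller for the main menu, which creates the menu widget on BeginPlay and switches to UI-only input with the cursor visible.
; An event shows a loading widget and returns input to game-only.
; Another stores the player's info on the controller.
; RequestGM passes the menu game mode's list of all controllers to the menu to update user images, then prints each stored username.
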(event Custom|ShowLoadingScreen
  (bind _self self)
  (bind _returnvalue (UserInterface|CreateWidget "/Game/UI/Menus/WBP_Loading.WBP_Loading_C" _self))
  (UserInterface|Viewport|AddtoViewport _returnvalue 0)
  (Input|SetInputModeGameOnly _self))

(event Custom|RequestGM
  (bind _returnvalue (Game|GetGameMode))
  (bind _asbp_menu_player_gamemode (Utilities|Casting|CastToBP_MenuPlayer_GAMEMODE _returnvalue))
  (bind _allplayercontrollers (Variables|/Game/Player/BP_MenuPlayer_GAMEMODE.BP_MenuPlayer_GAMEMODE_C|GetAllPlayerControllers _asbp_menu_player_gamemode))
  (Default|UpdateUserImage (Variables|Default|GetMainMenuWB) _allplayercontrollers)
  (for _array_element _allplayercontrollers
    (Development|PrintString (Utilities|String|Append "PC Username: " (.username (Variables|BP_MenuPlayer_PLAYERCONTROLLER_C|GetClientPlayerInfo (.AsBP%20Menu%20Player%20PLAYERCONTROLLER (Utilities|Casting|CastToBP_MenuPlayer_PLAYERCONTROLLER _array_element))))))))

(event Custom|UpdateServerWithInfo
  (params (PlayerInfo :type Player%20Info%20Structure))
  (Variables|Default|SetClientPlayerInfo PlayerInfo))

(event EventBeginPlay
  ;[1 1 1] Setup main menu
  (Variables|Default|SetbShowMouseCursor true)
  (bind _returnvalue (UserInterface|CreateWidget "/Game/UI/Menus/WBP_MainMenu.WBP_MainMenu_C"))
  (bind _output_get (Variables|Default|SetMainMenuWB _returnvalue))
  (UserInterface|Viewport|AddtoViewport _output_get 0)
  (Input|SetInputModeUIOnly 0 _output_get "DoNotLock"))

(fn ConstructionScript)