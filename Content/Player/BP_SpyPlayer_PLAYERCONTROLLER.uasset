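; Player controller for the spy player that builds the HUD on possession, toggles it with H and sets the audio listener to the character's camera.
; It fills the inventory from PlayerInfo equipment and shows a loading screen.
; Dropped items spawn at the pawn, then move to a navmesh point ahead if a trace from there hits the player.
; Tick drives a butler-distance music parameter, but the Music and Butler setup is disconnected.
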(event Custom|ShowLoadingScreen
  ;[1 1 1] Loading screen
  (bind _returnvalue (UserInterface|CreateWidget "/Game/UI/Menus/WBP_Loading.WBP_Loading_C" self))
  (UserInterface|Viewport|AddtoViewport _returnvalue 0))

(event Custom|NetDropItem
  (params (ClassToSpawn :type Actor%20Class%20Reference))
  (bind _returnvalue (Pawn|GetControlledPawn))
  (bind _returnvalue_2 (Transformation|GetActorForwardVector _returnvalue))
  (bind _returnvalue_3 (Transformation|GetActorTransform _returnvalue))
  (bind _returnvalue_4 (* _returnvalue_2 1e+02))
  (bind _returnvalue_5 (+ (.location _returnvalue_3) _returnvalue_4))
  (bind (_projectedlocation _returnvalue_6) (AI|Navigation|ProjectPointtoNavigation _returnvalue_5 0 0 "500.000000,500.000000,500.000000"))
  ;[1 1 1] Drop item from inventory
  (bind _returnvalue_7 (Game|SpawnActorfromClass ClassToSpawn (Math|Transform|MakeTransform (.location _returnvalue_3) "0, 0, 0" "1,1,1") "AdjustIfPossibleButAlwaysSpawn" 0 0)) ; Spawning item near players feet
  (if _returnvalue_6 ; If point on the navmesh was found
    (bind _outhit (Collision|LineTraceByChannel _projectedlocation (.location _returnvalue_3) "TraceTypeQuery1" false 0 "None" false))
    (if (== (.HitActor (Collision|BreakHitResult _outhit)) _returnvalue) ; If point on navmesh can see player
      (bind _boxextent (Collision|GetActorArrayBounds (Utilities|Array|MakeArray _returnvalue_7)))
      (Transformation|SetActorLocation _returnvalue_7 (+ _projectedlocation (Math|Vector|MakeVector 0.0 0.0 (.z _boxextent))) false false) ; Offset item by its own half height
    )))

(event Custom|ClientOnPossess
  (bind _self self)
  ;[1 1 1] Network player setup
  (Viewport|RemoveAllWidgets)
  (Input|SetInputModeGameOnly _self)
  (bind _returnvalue (UserInterface|CreateWidget "/Game/Inventory/InventoryUI/WBP_InventoryHUD.WBP_InventoryHUD_C" _self))
  (bind _output_get (Variables|Default|SetHUDWidget _returnvalue))
  (UserInterface|Viewport|AddtoViewport _output_get 0)
  (bind _returnvalue_2 (UserInterface|CreateWidget "/Game/UI/Health/WBP_HealthBar.WBP_HealthBar_C" _self))
  (bind _output_get_2 (Variables|Default|SetHealth _returnvalue_2))
  (UserInterface|Viewport|AddtoViewport _output_get_2 0)
  (bind _returnvalue_3 (UserInterface|CreateWidget "/Game/UI/ContextMenu/WBP_ContextMenu.WBP_ContextMenu_C" _self))
  (bind _output_get_3 (Variables|Default|SetContexMenu _returnvalue_3))
  (UserInterface|Viewport|AddtoViewport _output_get_3 0)
  (bind _returnvalue_4 (UserInterface|CreateWidget "/Game/UI/ScreenText/WBP_TextLog.WBP_TextLog_C" _self))
  (bind _output_get_4 (Variables|Default|SetTextLog _returnvalue_4))
  (UserInterface|Viewport|AddtoViewport _output_get_4 0)
  (bind _returnvalue_5 (UserInterface|CreateWidget "/Game/UI/ScreenText/WBP_StatsDisplay.WBP_StatsDisplay_C"))
  (bind _output_get_5 (Variables|Default|SetStatsDisplay _returnvalue_5))
  (UserInterface|Viewport|AddtoViewport _output_get_5 0)
  (Development|ExecuteConsoleCommand "p.NetEnableMoveCombining 0" 0))

(event Custom|SetupInventory
  (for _array_element (.PlayerEquipment (Utilities|Struct|BreakSPlayerInfoNew (Variables|Default|GetPlayerInfo)))
    (bind _asbp_player_character (Utilities|Casting|CastToBP_Player_CHARACTER (Pawn|GetControlledPawn)))
    (Default|PrepareInventory (Variables|/Game/Player/BP_Player_CHARACTER.BP_Player_CHARACTER_C|GetInventoryComponent _asbp_player_character))
    (bind _success (Default|AddtoInventory (Variables|/Game/Player/BP_Player_CHARACTER.BP_Player_CHARACTER_C|GetInventoryComponent _asbp_player_character) (Utilities|Struct|MakeFSlotStructure (Utilities|Struct|MakeFItemStructure (.name (.ItemStructure (Utilities|GetClassDefaults (.class (.ItemStructure (Utilities|Struct|BreakFSlotStructure _array_element)))))) (.description (.ItemStructure (Utilities|GetClassDefaults (.class (.ItemStructure (Utilities|Struct|BreakFSlotStructure _array_element)))))) (.stackable (.ItemStructure (Utilities|GetClassDefaults (.class (.ItemStructure (Utilities|Struct|BreakFSlotStructure _array_element)))))) (.maxstacksize (.ItemStructure (Utilities|GetClassDefaults (.class (.ItemStructure (Utilities|Struct|BreakFSlotStructure _array_element)))))) (.thumbnail (.ItemStructure (Utilities|GetClassDefaults (.class (.ItemStructure (Utilities|Struct|BreakFSlotStructure _array_element)))))) (.itemtype (.ItemStructure (Utilities|GetClassDefaults (.class (.ItemStructure (Utilities|Struct|BreakFSlotStructure _array_element)))))) (.class (.ItemStructure (Utilities|GetClassDefaults (.class (.ItemStructure (Utilities|Struct|BreakFSlotStructure _array_element)))))) (.consumable (.ItemStructure (Utilities|GetClassDefaults (.class (.ItemStructure (Utilities|Struct|BreakFSlotStructure _array_element)))))) (.detectionrating (.ItemStructure (Utilities|GetClassDefaults (.class (.ItemStructure (Utilities|Struct|BreakFSlotStructure _array_element)))))) (.locked (.ItemStructure (Utilities|GetClassDefaults (.class (.ItemStructure (Utilities|Struct|BreakFSlotStructure _array_element)))))) false false) (.Quantity (Utilities|Struct|BreakFSlotStructure _array_element)))))
    (Development|PrintText (.name (.ItemStructure (Utilities|GetClassDefaults (.class (.ItemStructure (Utilities|Struct|BreakFSlotStructure _array_element)))))))
    (Development|PrintString (Utilities|String|ToString(Boolean) _success))))

(event EventBeginPlay
  (bind _asbp_player_character (Utilities|Casting|CastToBP_Player_CHARACTER (Pawn|GetControlledPawn)))
  (Class|PlayerController|SetAudioListenerOverride (Variables|/Game/Player/BP_Player_CHARACTER.BP_Player_CHARACTER_C|GetCamera _asbp_player_character) "0, 0, 0" "0, 0, 0"))

(event EventPossess
  (params (PossessedPawn :type Pawn%20Object%20Reference))
  ;[1 1 1] Network player setup
  (CallFunction|ClientonPossess))

(event EventTick
  (params (DeltaSeconds :type Float%20%28single-precision%29))
  (bind _returnvalue (Pawn|GetControlledPawn))
  (bind _butler (Variables|Default|GetButler))
  (bind _butlerrange (Variables|Default|GetButlerRange))
  (bind _returnvalue_2 (Transformation|GetDistanceTo _returnvalue _butler))
  (Utilities|IsValid _returnvalue
    (:Is%20Valid
      (if (< _returnvalue_2 _butlerrange)
        (Class|FMODBlueprintStatics|EventInstanceSetParameter (Variables|Default|GetMusic) "butlerLevel" (/ _returnvalue_2 _butlerrange))
        (else
          (bind _returnvalue_3 (Class|FMODBlueprintStatics|EventInstanceGetParameter (Variables|Default|GetMusic) "butlerLevel"))
          (if (!= _returnvalue_3 0.0)
            (Class|FMODBlueprintStatics|EventInstanceSetParameter (Variables|Default|GetMusic) "butlerLevel" 0.0)))))))

(event Input|KeyboardEvents|H
  (params (Key :type Key%20Structure :default "None"))
  (:Pressed
    (Utilities|FlowControl|FlipFlop
      (:A
        (CallFunction|HideUI))
      (:B
        (CallFunction|UnhideUI)))))

(fn ConstructionScript)

(fn ReplaceInventory
  (Widget|RemovefromParent (Variables|Default|GetExistingInventory))
  (bind _asbp_player_character (Utilities|Casting|CastToBP_Player_CHARACTER (Pawn|GetControlledPawn)))
  (Variables|/Game/Inventory/BP_InventoryComponent.BP_InventoryComponent_C|SetInventoryWindow (Variables|/Game/Player/BP_Player_CHARACTER.BP_Player_CHARACTER_C|GetInventoryComponent _asbp_player_character) 0))

(fn HideUI
  (bind _returnvalue (Pawn|GetControlledPawn))
  (bind _asbp_player_character (Utilities|Casting|CastToBP_Player_CHARACTER _returnvalue))
  (bind _pause (Variables|/Game/Player/BP_Player_CHARACTER.BP_Player_CHARACTER_C|GetPause _asbp_player_character))
  (Widget|SetVisibility (Variables|Default|GetContexMenu) "Hidden")
  (Widget|SetVisibility (Variables|Default|GetTextLog) "Hidden")
  (Widget|SetVisibility (Variables|Default|GetHealth) "Hidden")
  (Widget|SetVisibility (Variables|Default|GetStatsDisplay) "Hidden")
  (Utilities|IsValid _pause
    (:Is%20Valid
      (Widget|SetIsEnabled _pause false)
      (Widget|SetVisibility _pause "Hidden"))))

(fn UnhideUI
  (bind _returnvalue (Pawn|GetControlledPawn))
  (bind _asbp_player_character (Utilities|Casting|CastToBP_Player_CHARACTER _returnvalue))
  (bind _pause (Variables|/Game/Player/BP_Player_CHARACTER.BP_Player_CHARACTER_C|GetPause _asbp_player_character))
  (Widget|SetVisibility (Variables|Default|GetContexMenu) "Visible")
  (Widget|SetVisibility (Variables|Default|GetTextLog) "Visible")
  (Widget|SetVisibility (Variables|Default|GetHealth) "Visible")
  (Widget|SetVisibility (Variables|Default|GetStatsDisplay) "Visible")
  (Utilities|IsValid _pause
    (:Is%20Valid
      (Widget|SetIsEnabled _pause true)
      (Widget|SetVisibility _pause "Visible"))))