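; Game mode for the co-op menu maps that tracks joining player controllers and coordinates the lobby before play.
; When a second player joins on the main menu, it hides and disables the host's invite button and friends list.
; It gathers each controller's player info to redistribute to everyone and checks whether all are ready.
; Launch events show loading screens, then server travel to the item select or showcase map.
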(event Custom|EnterGame
  ;[1 1 1] Launch into the item select map
  (for _array_element (Variables|Default|GetAllPlayerControllers)
    (Default|ShowLoadingScreen (.AsBP%20Menu%20Player%20PLAYERCONTROLLER (Utilities|Casting|CastToBP_MenuPlayer_PLAYERCONTROLLER _array_element))))
  (Development|ExecuteConsoleCommand "servertravel ItemSelect_MAP" 0))

(event Custom|EveryoneUpdate
  (bind _allplayercontrollers (Variables|Default|GetAllPlayerControllers))
  (bind _connectedplayers (Variables|Default|GetConnectedPlayers))
  ;[1 1 1] Everyone Update
  (if (> (Utilities|Array|Length _allplayercontrollers) 0)
    (Utilities|Array|Clear _connectedplayers)
    (for _array_element _allplayercontrollers
      (Utilities|Array|Add _connectedplayers (Variables|/Game/Player/Menu/BP_MenuPlayer_PLAYERCONTROLLER.BP_MenuPlayer_PLAYERCONTROLLER_C|GetPlayerInfo (.AsBP%20Menu%20Player%20PLAYERCONTROLLER (Utilities|Casting|CastToBP_MenuPlayer_PLAYERCONTROLLER _array_element)))))
    (for _array_element_2 _allplayercontrollers
      (Default|AddPlayerInfo (.AsBP%20Menu%20Player%20PLAYERCONTROLLER (Utilities|Casting|CastToBP_MenuPlayer_PLAYERCONTROLLER _array_element_2)) (Variables|Default|GetConnectedPlayers)))))

(event Custom|SwapInventory
  (params (PlayerController :type Player%20Controller%20Object%20Reference) (EquipmentArray :type Array%20of%20Strings) (ChangedStatus :type Boolean)))

(event Custom|LaunchGame
  ;[1 1 1] Launch into the showcase map
  (for _array_element (Variables|Default|GetAllPlayerControllers)
    (Default|ShowLoadingScreen (.AsBP%20Menu%20Player%20PLAYERCONTROLLER (Utilities|Casting|CastToBP_MenuPlayer_PLAYERCONTROLLER _array_element))))
  (Development|ExecuteConsoleCommand "servertravel Showcase_MAP" 0))

(event Custom|ReadyCheck
  ;[1 1 1] Checks to see if everyone is ready
  (bind _array_element (Utilities|Array|ForEachLoopwithBreak (Variables|Default|GetConnectedPlayers) :!label _label)
    (:LoopBody
      (if (Utilities|Enum|Equal(Enum) (.ReadyStatus (Utilities|Struct|BreakSPlayerInfo _array_element)) "Ready")
        (Variables|Default|SetbEveryoneReady true)
        (else
          (Variables|Default|SetbEveryoneReady (Utilities|Enum|Equal(Enum) (.ReadyStatus (Utilities|Struct|BreakSPlayerInfo _array_element)) "Ready"))
          (goto _label Break))))))

(event EventPostLogin
  (params (NewPlayer :type Player%20Controller%20Object%20Reference))
  (bind _allplayercontrollers (Variables|Default|GetAllPlayerControllers))
  (bind _output (Utilities|Array|Get(acopy) _allplayercontrollers))
  (bind _asbp_menu_player_playercontroller (Utilities|Casting|CastToBP_MenuPlayer_PLAYERCONTROLLER _output))
  (bind _mainmenuwb (Variables|/Game/Player/Menu/BP_MenuPlayer_PLAYERCONTROLLER.BP_MenuPlayer_PLAYERCONTROLLER_C|GetMainMenuWB _asbp_menu_player_playercontroller))
  (bind _invitebutton (Variables|/Game/UI/Menus/WBP_MainMenu.WBP_MainMenu_C|GetInviteButton _mainmenuwb))
  (bind _friendslist (Variables|/Game/UI/Menus/WBP_MainMenu.WBP_MainMenu_C|GetFriendsList _mainmenuwb))
  (Utilities|Array|Add _allplayercontrollers NewPlayer)
  (if (> (Utilities|Array|Length _allplayercontrollers) 1)
    (bind _returnvalue (Game|GetCurrentLevelName true))
    (if (Utilities|Enum|Equal(Enum) _returnvalue "MainMenu_MAP")
      (Widget|SetIsEnabled _invitebutton false)
      (Widget|SetVisibility _invitebutton "Hidden")
      (Widget|SetIsEnabled _friendslist false)
      (Widget|SetVisibility _friendslist "Hidden")
      (Development|PrintString "Coop player has joined" true true "(R=1.000000,G=0.000000,B=0.000000,A=1.000000)" 1e+01))))

(fn ConstructionScript)