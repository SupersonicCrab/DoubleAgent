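; Player controller for the menu maps that starts menu music, opens the main menu or item select widget by level name, and destroys the session on EndPlay.
; It builds player info from Steam name, avatar and net ID, tracking ready status and capped equipment.
; On item select it asks the game mode to update everyone, and AddPlayerInfo rebuilds the user list.
; Helpers save player info and options, pushing settings to the game instance.
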(event Custom|ShowLoadingScreen
  ;[1 1 1] Show loading screen
  (bind _returnvalue (UserInterface|CreateWidget "/Game/UI/Menus/WBP_Loading.WBP_Loading_C" self))
  (UserInterface|Viewport|AddtoViewport _returnvalue 0))

(event Custom|NetClientOnPossess
  (bind _returnvalue (Game|GetGameInstance))
  (bind _self self)
  (bind _asbp_spy_game_instance (Utilities|Casting|CastToBP_SpyGameInstance _returnvalue))
  (Variables|Default|SetbShowMouseCursor true)
  (bind _returnvalue_2 (Game|GetCurrentLevelName true))
  (switch string _returnvalue_2 ; Checks which map the player is on. Depending on the map, this switch will open up a different menu
    (:MainMenu_MAP
      (bind _returnvalue_3 (UserInterface|CreateWidget "/Game/UI/Menus/WBP_MainMenu.WBP_MainMenu_C" _self))
      (bind _output_get (Variables|Default|SetMainMenuWB _returnvalue_3))
      (UserInterface|Viewport|AddtoViewport _output_get 0)
      (Input|SetInputModeUIOnly _self _output_get "LockAlways")
      (CallFunction|SetPlayerInfo)
      (bind _settingssave (Default|LoadSettings _asbp_spy_game_instance))
      (Default|UpdateSettings _asbp_spy_game_instance _settingssave))
    (:ItemSelect_MAP
      (bind _returnvalue_4 (UserInterface|CreateWidget "/Game/UI/Menus/ItemSelect/WBP_ItemSelect.WBP_ItemSelect_C" _self))
      (bind _output_get_2 (Variables|Default|SetItemSelectWB _returnvalue_4))
      (UserInterface|Viewport|AddtoViewport _output_get_2 0)
      (Input|SetInputModeUIOnly _self _output_get_2 "LockAlways")
      (CallFunction|SetPlayerInfo)
      (CallFunction|InitialSetup))))

(event Custom|InitialSetup
  ;[1 1 1] Check for save game info and then update the server
  (CallFunction|CallUpdate))

(event Custom|CallUpdate
  ;[1 1 1] Assigns the updated inventory / Tells everyone to update
  (Default|EveryoneUpdate (.AsBP%20Menu%20Player%20GAMEMODE (Utilities|Casting|CastToBP_MenuPlayer_GAMEMODE (Game|GetGameMode)))))

(event Custom|AddPlayerInfo
  (params (ConnectedPlayersInfo :type Array%20of%20S%20Player%20Info%20Structures))
  (bind _itemselectwb (Variables|Default|GetItemSelectWB))
  ;[1 1 1] Updated user list window when called
  (Variables|Default|SetConnectedPlayersInfo ConnectedPlayersInfo)
  (Utilities|IsValid _itemselectwb
    (:Is%20Valid
      (Default|ClearUserList _itemselectwb)
      (for _array_element (Variables|Default|GetConnectedPlayersInfo)
        (Default|UpdatePlayerWindow _itemselectwb _array_element)))))

(event Custom|SetReady
  (params (ReadyStatus :type String))
  (Utilities|Struct|SetmembersinSPlayerInfo (Variables|Default|GetPlayerInfo) ReadyStatus))

(event Custom|AddEquipment
  (params (EquipmentToAdd :type F%20Slot%20Structure%20New%20Structure))
  (bind _playerinfo (Variables|Default|GetPlayerInfo))
  (bind _playerequipment (Utilities|Struct|BreakSPlayerInfo _playerinfo))
  (if (!= (Utilities|Array|Length _playerequipment) 12)
    (Utilities|Array|Add _playerequipment EquipmentToAdd)))

(event EventEndPlay
  (params (EndPlayReason :type EEndPlayReason%20Enum :default "Destroyed"))
  ;[1 1 1] Destroys session if player leaves
  (|DestroySession self))

(event EventPossess
  (params (PossessedPawn :type Pawn%20Object%20Reference))
  (CallFunction|NetClientonPossess))

(event EventBeginPlay
  (bind _returnvalue (Class|FMODBlueprintStatics|FindEventInstances "/Game/FMOD/Events/Menu_Music_Loop.Menu_Music_Loop"))
  (if (== (Utilities|Array|Length _returnvalue) 0)
    (Class|FMODBlueprintStatics|PlayEvent2D "/Game/FMOD/Events/Menu_Music_Loop.Menu_Music_Loop")))

(fn ConstructionScript)

(fn LoadGame
  (bind _returnvalue (SaveGame|DoesSaveGameExist (LocalVariables|GetPlayerInfoSettings)))
  (if _returnvalue
    ;[1 1 1] Load save game into player info
    (Development|PrintString "Loading save")
    (bind _returnvalue_2 (SaveGame|LoadGamefromSlot (LocalVariables|GetPlayerInfoSettings)))
    (bind _asbp_player_save_game (Utilities|Casting|CastToBP_PlayerSaveGame _returnvalue_2))
    (bind _output_get (Variables|Default|SetSaveGameReference _asbp_player_save_game))
    (Variables|Default|SetPlayerInfo (Variables|/Game/Networking/BP_PlayerSaveGame.BP_PlayerSaveGame_C|GetS_PlayerInfo _output_get))
    (else
      ;[1 1 1] If a save game doesn't exist create one
      (Development|PrintString "No save found, creating new save file")
      (bind _returnvalue_3 (SaveGame|CreateSaveGameObject "/Game/Networking/BP_PlayerSaveGame.BP_PlayerSaveGame_C"))
      (Variables|Default|SetSaveGameReference _returnvalue_3)
      (SaveGame|SaveGametoSlot (Variables|Default|GetSaveGameReference) (LocalVariables|GetPlayerInfoSettings)))))

(fn SetPlayerInfo
  (bind _self self)
  (bind _uniquenetid (Class|AdvancedSessionsLibrary|GetUniqueNetID _self))
  (Development|PrintString "Setting player info")
  (bind _returnvalue (Class|AdvancedSteamFriendsLibrary|GetSteamFriendAvatar _uniquenetid "SteamAvatar_Large")
    (:OnSuccess
      (Variables|Default|SetPlayerInfo (Utilities|Struct|MakeSPlayerInfo (Class|AdvancedSessionsLibrary|GetPlayerName _self) _returnvalue _uniquenetid (.currentlevel (Variables|Default|GetPlayerInfo)) "Not Ready" 0)))
    (:AsyncLoading
      (Development|PrintString "Failed to get avatar" :!label _label))
    (:OnFailure
      (goto _label))))

(fn CheckPlayerInfo
  (bind _playerinfo (Variables|Default|GetPlayerInfo))
  (Development|PrintString (Utilities|String|Append "Username: " (.username _playerinfo)))
  (Development|PrintString (Utilities|String|Append "Avatar is valid: " (Utilities|String|ToString(Boolean) (Utilities|IsValid (.avatar _playerinfo)))))
  (Development|PrintString (Utilities|String|Append "Net ID: " (Class|AdvancedSessionsLibrary|UniqueNetIdtoString (.networkid _playerinfo))))
  (Development|PrintString (Utilities|String|Append "Current level:" (Utilities|String|ToString(Integer) (.currentlevel _playerinfo)) " 
       ")))

(fn SaveGame
  (bind _savegamereference (Variables|Default|GetSaveGameReference))
  (bind _returnvalue (SaveGame|DoesSaveGameExist (LocalVariables|GetPlayerInfoSettings)))
  (if _returnvalue
    ;[1 1 1] Load save game into player info
    (Development|PrintString "Saving player info")
    (Variables|/Game/Networking/BP_PlayerSaveGame.BP_PlayerSaveGame_C|SetS_PlayerInfo _savegamereference (Variables|Default|GetPlayerInfo))
    (SaveGame|SaveGametoSlot _savegamereference (LocalVariables|GetPlayerInfoSettings))
    (else
      (Development|PrintString "Tried to save to a save file that doesnt exist"))))

(fn LoadSettings
  (bind _returnvalue (SaveGame|DoesSaveGameExist (LocalVariables|GetOptionsSlot)))
  (if _returnvalue
    (bind _returnvalue_2 (SaveGame|LoadGamefromSlot (LocalVariables|GetOptionsSlot)))
    (bind _asbp_game_settings (Utilities|Casting|CastToBP_GameSettings _returnvalue_2))
    (bind _output_get (Variables|Default|SetOptionsSaveReference _asbp_game_settings))
    (return _output_get)
    (else
      ;[1 1 1] If no options save exists, create one with default settings
      (bind _returnvalue_3 (SaveGame|CreateSaveGameObject "/Game/Player/Settings/BP_GameSettings.BP_GameSettings_C"))
      (bind _output_get_2 (Variables|Default|SetOptionsSaveReference _returnvalue_3))
      (SaveGame|SaveGametoSlot _output_get_2 (LocalVariables|GetOptionsSlot)))))

(fn SaveSettings
  (params (GraphicsSettings :type F%20Graphics%20Settings%20Structure) (AudioSettings :type F%20Audio%20Settings%20Structure) (ControlSettings :type F%20Control%20Settings%20New%20Structure) (GameplaySettings :type F%20Gameplay%20Settings%20Structure) (AccessibilitySettings :type F%20Accessibility%20Settings%20New%20Structure))
  (bind _optionssavereference (Variables|Default|GetOptionsSaveReference))
  (bind _optionssavereference_2 (Variables|Default|GetOptionsSaveReference))
  (bind _returnvalue (SaveGame|DoesSaveGameExist (LocalVariables|GetOptionsSlot)))
  (if _returnvalue
    (Variables|/Game/Player/Settings/BP_GameSettings.BP_GameSettings_C|SetGraphicSettings _optionssavereference_2 GraphicsSettings)
    (Variables|/Game/Player/Settings/BP_GameSettings.BP_GameSettings_C|SetAudioSettings _optionssavereference_2 AudioSettings)
    (Variables|/Game/Player/Settings/BP_GameSettings.BP_GameSettings_C|SetControlSettings _optionssavereference_2 ControlSettings)
    (Variables|/Game/Player/Settings/BP_GameSettings.BP_GameSettings_C|SetGameplaySettings _optionssavereference_2 GameplaySettings)
    (Variables|/Game/Player/Settings/BP_GameSettings.BP_GameSettings_C|SetAccessibilitySettings _optionssavereference_2 AccessibilitySettings)
    (SaveGame|SaveGametoSlot _optionssavereference (LocalVariables|GetOptionsSlot))
    (bind _asbp_spy_game_instance (Utilities|Casting|CastToBP_SpyGameInstance (Game|GetGameInstance)))
    (Default|UpdateSettings _asbp_spy_game_instance _optionssavereference)
    (else
      (Development|PrintString "Somehow the options save slot doesn't exist. Reboot game."))))