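; Multiplayer game mode for a spy game that spawns and possesses a character for each joining player at a PlayerStart.
; On login it restores saved PlayerInfo from the game instance by join order and makes the newest pawn owner of cameras, map-travel actors and the power box.
; It relays notifications and pause changes to all players, and handles restart and map changes through servertravel behind loading screens.
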(event Custom|GlobalNotification
  (params (LogText :type Text) (LogImage :type Texture%202D%20Object%20Reference))
  (for _array_element (Variables|Default|GetAllPlayerControllers)
    (bind _asbp_player_character (Utilities|Casting|CastToBP_Player_CHARACTER (Pawn|GetControlledPawn _array_element)))
    (Default|GlobalNotificationSend _asbp_player_character LogText LogImage)))

(event Custom|Restart
  (for _array_element (Variables|Default|GetAllPlayerControllers)
    (Default|ShowLoadingScreen (.AsBP%20Spy%20Player%20PLAYERCONTROLLER (Utilities|Casting|CastToBP_SpyPlayer_PLAYERCONTROLLER _array_element))))
  (Utilities|Time|SetGlobalTimeDilation 1.0)
  (Utilities|FlowControl|Delay 0.2)
  (bind _returnvalue (Game|GetCurrentLevelName true))
  (Development|ExecuteConsoleCommand (Utilities|String|Append "servertravel " _returnvalue) 0))

(event Custom|GlobalPause
  (params (Pausing :type Boolean))
  (bind _allplayercontrollers (Variables|Default|GetAllPlayerControllers))
  (if Pausing
    (for _array_element _allplayercontrollers
      (Default|NetRecievePause (.AsBP%20Player%20CHARACTER (Utilities|Casting|CastToBP_Player_CHARACTER (Pawn|GetControlledPawn _array_element)))))
    (else
      (for _array_element_2 _allplayercontrollers
        (Default|NetRecieveUnpause (.AsBP%20Player%20CHARACTER (Utilities|Casting|CastToBP_Player_CHARACTER (Pawn|GetControlledPawn _array_element_2))))))))

(event Custom|Travel
  (params (NewMap :type String))
  (for _array_element (Variables|Default|GetAllPlayerControllers)
    (Default|ShowLoadingScreen (.AsBP%20Spy%20Player%20PLAYERCONTROLLER (Utilities|Casting|CastToBP_SpyPlayer_PLAYERCONTROLLER _array_element))))
  (Development|ExecuteConsoleCommand (Utilities|String|Append "servertravel " NewMap) 0))

(event EventPostLogin
  (params (NewPlayer :type Player%20Controller%20Object%20Reference))
  (bind _asbp_spy_player_playercontroller (Utilities|Casting|CastToBP_SpyPlayer_PLAYERCONTROLLER NewPlayer))
  (Utilities|Array|Add (Variables|Default|GetAllPlayerControllers) NewPlayer)
  (bind _returnvalue (Actor|GetActorOfClass "/Script/Engine.PlayerStart"))
  (bind _returnvalue_2 (Game|SpawnActorfromClass "/Game/Player/BP_Player_CHARACTER.BP_Player_CHARACTER_C" (Transformation|GetActorTransform _returnvalue) "Undefined" 0 0))
  (Pawn|Possess NewPlayer _returnvalue_2)
  (Development|PrintString "Spawned player")
  (CallFunction|GiveOwnership NewPlayer)
  (if (!= (Utilities|Array|Length (Variables|/Game/Networking/BP_SpyGameInstance.BP_SpyGameInstance_C|GetPlayerInfo (.AsBP%20Spy%20Game%20Instance (Utilities|Casting|CastToBP_SpyGameInstance (Game|GetGameInstance))))) 0)
    (Variables|/Game/Player/BP_SpyPlayer_PLAYERCONTROLLER.BP_SpyPlayer_PLAYERCONTROLLER_C|SetPlayerInfo _asbp_spy_player_playercontroller (Utilities|Array|Get(acopy) (Variables|/Game/Networking/BP_SpyGameInstance.BP_SpyGameInstance_C|GetPlayerInfo (.AsBP%20Spy%20Game%20Instance (Utilities|Casting|CastToBP_SpyGameInstance (Game|GetGameInstance)))) (- (Utilities|Array|Length (Variables|Default|GetAllPlayerControllers)) 1)))
    (Default|SetupInventory _asbp_spy_player_playercontroller)))

(fn ConstructionScript)

(fn GiveOwnership
  (params (ClientController :type Player%20Controller%20Object%20Reference))
  (bind _returnvalue (Pawn|GetControlledPawn ClientController))
  ;[1 1 1] Give cameras ownership
  (bind _outactors (Actor|GetAllActorsOfClass "/Script/DoubleAgent.Camera"))
  (for _array_element _outactors
    (Actor|SetOwner _array_element _returnvalue))
  ;[1 1 1] Give map travel ownership
  (bind _outactors_2 (Actor|GetAllActorsOfClass "/Game/Maps/Showcase/Blueprints/BP_MapTravel.BP_MapTravel_C"))
  (for _array_element_2 _outactors_2
    (Actor|SetOwner _array_element_2 _returnvalue))
  ;[1 1 1] Give power box ownership
  (bind _returnvalue_2 (Actor|GetActorOfClass "/Script/DoubleAgent.PowerBox"))
  (Utilities|IsValid _returnvalue_2
    (:Is%20Valid
      (Actor|SetOwner _returnvalue_2 _returnvalue))))