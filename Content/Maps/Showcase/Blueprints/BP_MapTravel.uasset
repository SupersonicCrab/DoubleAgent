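; BP_MapTravel is a trigger that moves the game to NewMap when a player overlaps it, optionally requiring an inventory item.
; Overlaps, including one found shortly after BeginPlay, run an item check, commented as client-side because the server lacks client inventories.
; On success it notifies, slows time and calls the game mode's Travel; otherwise it shows the missing item.
; An empty map name disables overlap events.
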(event OnComponentBeginOverlap(Collision)
  (params (OverlappedComponent :type Primitive%20Component%20Object%20Reference) (OtherActor :type Actor%20Object%20Reference) (OtherComp :type Primitive%20Component%20Object%20Reference) (OtherBodyIndex :type Integer) (bFromSweep :type Boolean) (SweepResult :type Hit%20Result%20Structure%20%28by%20ref%29))
  ;[1 1 1] Collision
  (bind _asbp_player_character (Utilities|Casting|CastToBP_Player_CHARACTER OtherActor))
  (CallFunction|ItemCheck _asbp_player_character))

(event Custom|ItemCheck
  (params (Player :type BP%20Player%20CHARACTER%20Object%20Reference))
  (bind _requireditem (Variables|Default|GetRequiredItem))
  ;[1 1 1] Checks the players inventory on the client side - server doesn't have any reference of the clients inventory
  (if (== _requireditem 0)
    (Variables|Default|SetItemCheckLevel 0)
    (else
      (bind _itemfound (Default|CheckItemClass (Variables|/Game/Player/BP_Player_CHARACTER.BP_Player_CHARACTER_C|GetInventoryComponent Player) _requireditem))
      (if _itemfound
        (Variables|Default|SetItemCheckLevel 1)
        (else
          (Variables|Default|SetItemCheckLevel 2)))))
  (CallFunction|HandlePlayerCollision Player (Variables|Default|GetItemCheckLevel)))

(event Custom|HandlePlayerCollision
  (params (Player :type BP%20Player%20CHARACTER%20Object%20Reference) (ItemCheckLevel :type Integer))
  (bind _requireditem (Variables|Default|GetRequiredItem))
  (bind _itemstructure (Utilities|GetClassDefaults _requireditem))
  ;[1 1 1] Handle player collision
  (switch int ItemCheckLevel
    (:0
      (Default|GlobalNotificationStart Player "Traveling to new level")
      (Default|NetRequestSetTimeScale Player 0.5 :!label _label)
      (Utilities|FlowControl|Delay 0.75)
      (Default|Travel (.AsBP%20Spy%20Player%20GAMEMODE (Utilities|Casting|CastToBP_SpyPlayer_GAMEMODE (Game|GetGameMode))) (Variables|Default|GetNewMap)))
    (:1
      (Default|GlobalNotificationStart Player "You beat this level")
      (goto _label))
    (:2
      (Default|GlobalNotificationStart Player (Utilities|Text|ToText(String) (Utilities|String|Append "You need [" (Utilities|String|ToString(Text) (.name _itemstructure)) "] to complete this level")) (.thumbnail _itemstructure)))))

(event EventBeginPlay
  (bind _overlappingactors (Collision|GetOverlappingActors "/Game/Player/BP_Player_CHARACTER.BP_Player_CHARACTER_C" :!class /Script/Engine.Actor))
  ;[1 1 1] Disable travel if no map has been specified
  (if (Utilities|Enum|Equal(Enum) (Variables|Default|GetNewMap) "")
    (Variables|/Script/Engine.PrimitiveComponent|SetbGenerateOverlapEvents (Variables|Default|GetCollision) false))
  ;[1 1 1] Check overlaps
  (Utilities|FlowControl|Delay 0.5)
  (if (> (Utilities|Array|Length _overlappingactors) 0)
    (CallFunction|ItemCheck (.AsBP%20Player%20CHARACTER (Utilities|Casting|CastToBP_Player_CHARACTER (Utilities|Array|Get(acopy) _overlappingactors))))))

(fn ConstructionScript)