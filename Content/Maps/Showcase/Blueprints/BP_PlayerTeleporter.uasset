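; BP_PlayerTeleporter is a showcase map trigger that moves an overlapping player character to a linked EndPoint.
; It copies the EndPoint's TeleportLocation world transform to the character and sets the controller's rotation to match.
; On the server, it then enables every NPC in its RoomNPCs list.
; At BeginPlay it turns off collision overlap events if no EndPoint is assigned.
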(event OnComponentBeginOverlap(Collision)
  (params (OverlappedComponent :type Primitive%20Component%20Object%20Reference) (OtherActor :type Actor%20Object%20Reference) (OtherComp :type Primitive%20Component%20Object%20Reference) (OtherBodyIndex :type Integer) (bFromSweep :type Boolean) (SweepResult :type Hit%20Result%20Structure%20%28by%20ref%29))
  (bind _endpoint (Variables|Default|GetendPoint))
  (bind _teleportlocation (Variables|BP_PlayerTeleporter_C|GetTeleportLocation _endpoint))
  (bind _returnvalue (Transformation|GetWorldTransform _teleportlocation))
  (bind _asbp_player_character (Utilities|Casting|CastToBP_Player_CHARACTER OtherActor))
  (Transformation|SetActorTransform _asbp_player_character _returnvalue false true)
  (Pawn|SetControlRotation (Pawn|GetController _asbp_player_character) (.Rotation (Math|Transform|BreakTransform _returnvalue)))
  (if (Networking|IsServer)
    (for _array_element (Variables|Default|GetRoomNPCs)
      (Default|EnableNPC _array_element))))

(event EventBeginPlay
  ;[1 1 1] Disable overlap if endPoint is not specified
  (Utilities|IsValid (Variables|Default|GetendPoint)
    (:Is%20Not%20Valid
      (Variables|/Script/Engine.PrimitiveComponent|SetbGenerateOverlapEvents (Variables|Default|GetCollision) false))))

(fn ConstructionScript)