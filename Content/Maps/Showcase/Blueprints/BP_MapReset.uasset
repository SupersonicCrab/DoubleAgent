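; BP_MapReset is an exit trigger that reloads the Showcase map when the player reaches it carrying a required win-condition item.
; On collision overlap it checks the player's inventory for the WinConditionItem class and reports to the player controller's text log.
; Without the item, the log shows its name and thumbnail, read from class defaults.
; With it, a completion message and short delay precede Reset, which freezes global time and runs servertravel.
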(event OnComponentBeginOverlap(Collision)
  (params (OverlappedComponent :type Primitive%20Component%20Object%20Reference) (OtherActor :type Actor%20Object%20Reference) (OtherComp :type Primitive%20Component%20Object%20Reference) (OtherBodyIndex :type Integer) (bFromSweep :type Boolean) (SweepResult :type Hit%20Result%20Structure%20%28by%20ref%29))
  (bind _winconditionitem (Variables|Default|GetwinConditionItem))
  (bind _itemstructure (Utilities|GetClassDefaults _winconditionitem))
  (bind _asbp_player_character (Utilities|Casting|CastToBP_Player_CHARACTER OtherActor))
  (bind _itemfound (Default|CheckItemClass (Variables|/Game/Player/BP_Player_CHARACTER.BP_Player_CHARACTER_C|GetInventoryComponent _asbp_player_character) _winconditionitem))
  (if _itemfound
    (bind _asbp_spy_player_playercontroller (Utilities|Casting|CastToBP_SpyPlayer_PLAYERCONTROLLER (Pawn|GetController _asbp_player_character)))
    (Default|DisplayLog (Variables|/Game/Player/BP_SpyPlayer_PLAYERCONTROLLER.BP_SpyPlayer_PLAYERCONTROLLER_C|GetTextLog _asbp_spy_player_playercontroller) "You finished that room!")
    (Utilities|FlowControl|Delay 3.0)
    (CallFunction|Reset)
    (else
      (bind _asbp_spy_player_playercontroller_2 (Utilities|Casting|CastToBP_SpyPlayer_PLAYERCONTROLLER (Pawn|GetController _asbp_player_character)))
      (Default|DisplayLog (Variables|/Game/Player/BP_SpyPlayer_PLAYERCONTROLLER.BP_SpyPlayer_PLAYERCONTROLLER_C|GetTextLog _asbp_spy_player_playercontroller_2) (Utilities|Text|ToText(String) (Utilities|String|Append "Need " (Utilities|String|ToString(Text) (.name _itemstructure)) " to exit")) (.thumbnail _itemstructure)))))

(event Custom|Reset
  (Utilities|Time|SetGlobalTimeDilation 0.0)
  (Development|ExecuteConsoleCommand "servertravel Showcase_MAP" 0))

(fn ConstructionScript)