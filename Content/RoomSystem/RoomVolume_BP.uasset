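; Room volume that tracks whether the player is safe in a room and points NPCs inside at its light switch when unlit.
; Box overlaps set the player's RoomSafe from PlayerSafe on entry or at BeginPlay, and clear it on exit.
; NPCs crossing either way get their LightSwitch blackboard key set if unlit, or cleared if lit and matching this room's switch.
; LightUpdate reapplies that rule to every overlapping NPC.
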(event OnComponentBeginOverlap(Box)
  (params (OverlappedComponent :type Primitive%20Component%20Object%20Reference) (OtherActor :type Actor%20Object%20Reference) (OtherComp :type Primitive%20Component%20Object%20Reference) (OtherBodyIndex :type Integer) (bFromSweep :type Boolean) (SweepResult :type Hit%20Result%20Structure%20%28by%20ref%29))
  (bind _returnvalue (Utilities|GetClass OtherActor))
  (switch string (Utilities|String|LeftChop (Utilities|GetClassDisplayName _returnvalue) 2)
    (:Default
      (if (Utilities|ClassIsChildOf _returnvalue "/Game/AI/NPC/AICharacterBase_CHARACTER.AICharacterBase_CHARACTER_C")
        (CallFunction|NPCUpdate OtherActor)))
    (:Player_CHARACTER
      (CallFunction|PlayerEnter OtherActor))))

(event OnComponentEndOverlap(Box)
  (params (OverlappedComponent :type Primitive%20Component%20Object%20Reference) (OtherActor :type Actor%20Object%20Reference) (OtherComp :type Primitive%20Component%20Object%20Reference) (OtherBodyIndex :type Integer))
  (bind _returnvalue (Utilities|GetClass OtherActor))
  (switch string (Utilities|String|LeftChop (Utilities|GetClassDisplayName _returnvalue) 2)
    (:Default
      (if (Utilities|ClassIsChildOf _returnvalue "/Game/AI/NPC/AICharacterBase_CHARACTER.AICharacterBase_CHARACTER_C")
        (CallFunction|NPCUpdate OtherActor)))
    (:Player_CHARACTER
      (CallFunction|PlayerExit OtherActor))))

(event EventBeginPlay
  (bind _box (Variables|Default|GetBox))
  ;[1 1 1] Setup
  (bind _outactors (Collision|ComponentOverlapActors _box (Transformation|GetWorldTransform _box) (Utilities|Array|MakeArray "ObjectTypeQuery3") "/Game/Player/Player_CHARACTER.Player_CHARACTER_C"))
  (for _array_element _outactors
    (CallFunction|PlayerEnter _array_element)))

(fn ConstructionScript)

(fn PlayerEnter
  (params (Player :type Actor%20Object%20Reference))
  ;[1 1 1] Updating playerSafe variable
  (bind _asplayer_character (Utilities|Casting|CastToPlayer_CHARACTER Player))
  (Variables|/Game/Player/Player_CHARACTER.Player_CHARACTER_C|SetRoomSafe _asplayer_character (Variables|Default|GetPlayerSafe)))

(fn PlayerExit
  (params (Player :type Actor%20Object%20Reference))
  ;[1 1 1] Updating playerSafe variable
  (bind _asplayer_character (Utilities|Casting|CastToPlayer_CHARACTER Player))
  (Variables|/Game/Player/Player_CHARACTER.Player_CHARACTER_C|SetRoomSafe _asplayer_character false))

(fn LightUpdate
  (params (RoomLit :type Boolean))
  ;[1 1 1] Updating lit status
  (Variables|Default|SetRoomLit RoomLit)
  ;[1 1 1] Calling NPCupdate
  (CallFunction|AllNPCUpdate))

(fn AllNPCUpdate
  (bind _returnvalue (Utilities|Name|MakeLiteralName "LightSwitch"))
  (bind _box (Variables|Default|GetBox))
  ;[1 1 1] Getting all NPCs within room
  (bind _outactors (Collision|ComponentOverlapActors _box (Transformation|GetWorldTransform _box) (Utilities|Array|MakeArray "ObjectTypeQuery3") "/Game/AI/NPC/AICharacterBase_CHARACTER.AICharacterBase_CHARACTER_C"))
  (if (Variables|Default|GetRoomLit)
    ;[1 1 1] Ensuring all NPCs dont have self as lightswitch
    (for _array_element _outactors
      (if (Class|BlackboardComponent|IsVectorValueSet (AI|GetBlackboard _array_element) _returnvalue)
        (if (== (AI|Components|Blackboard|GetValueasObject (AI|GetBlackboard _array_element) _returnvalue) (Variables|Default|GetLightSwitch))
          (AI|Components|Blackboard|ClearValue (AI|GetBlackboard _array_element) _returnvalue))))
    (else
      ;[1 1 1] Updating all NPCs with lightswitch value
      (for _array_element_2 _outactors
        (AI|Components|Blackboard|SetValueasObject (AI|GetBlackboard _array_element_2) (Utilities|Name|MakeLiteralName "LightSwitch") (Variables|Default|GetLightSwitch))))))

(fn NPCUpdate
  (params (NPC :type Actor%20Object%20Reference))
  (bind _returnvalue (AI|GetBlackboard NPC))
  (bind _returnvalue_2 (Utilities|Name|MakeLiteralName "LightSwitch"))
  (if (Variables|Default|GetRoomLit)
    ;[1 1 1] Ensuring NPC does not have self as lightswitch
    (if (Class|BlackboardComponent|IsVectorValueSet _returnvalue _returnvalue_2)
      (if (== (AI|Components|Blackboard|GetValueasObject _returnvalue _returnvalue_2) (Variables|Default|GetLightSwitch))
        (AI|Components|Blackboard|ClearValue _returnvalue _returnvalue_2)))
    (else
      ;[1 1 1] Updating NPC with lightswitch value
      (AI|Components|Blackboard|SetValueasObject (AI|GetBlackboard NPC) (Utilities|Name|MakeLiteralName "LightSwitch") (Variables|Default|GetLightSwitch)))))