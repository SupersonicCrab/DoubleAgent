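; BP_Safe is an interactable safe container whose inventory opens only for players carrying the code note item.
; On Interact, it casts the interactor to the player character and checks that character's inventory for BP_CodeNote_Item.
; With the note, it toggles its own inventory component for the interactor; without it, the player controller's text log displays a non-global message that the safe combination is needed.
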(event EventBeginPlay
  (|CallParentFunction) ; This node is disabled and will not be called.\nDrag off pins to build functionality.
)

(event EventInteract
  (params (Interactor :type Actor%20Object%20Reference))
  (bind _asbp_player_character (Utilities|Casting|CastToBP_Player_CHARACTER Interactor))
  (bind _itemfound (Default|CheckItemClass (Variables|/Game/Player/BP_Player_CHARACTER.BP_Player_CHARACTER_C|GetInventoryComponent _asbp_player_character) "/Game/Inventory/Item/BP_CodeNote_item.BP_CodeNote_Item_C"))
  (if _itemfound
    (Default|ToggleInventory (Variables|Default|GetInventoryComponent) Interactor)
    (else
      (bind _asbp_spy_player_playercontroller (Utilities|Casting|CastToBP_SpyPlayer_PLAYERCONTROLLER (Pawn|GetController _asbp_player_character)))
      (Default|DisplayLog (Variables|/Game/Player/BP_SpyPlayer_PLAYERCONTROLLER.BP_SpyPlayer_PLAYERCONTROLLER_C|GetTextLog _asbp_spy_player_playercontroller) false "You need the safe combination" "/Game/Art/Textures/UI/Icons/T_DefaultIcon.T_DefaultIcon"))))

(fn ConstructionScript
  (|CallParentFunction))