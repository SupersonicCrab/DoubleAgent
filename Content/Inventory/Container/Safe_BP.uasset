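; Safe container Blueprint that only opens its inventory when the player carries the required item.
; Its ToggleInventory event checks the player character's InventoryComponent for the Item_CodeNote class, then toggles the safe's own InventoryComponent.
; Without the item it prints a message saying a keycard is needed, although the class checked is a code note.
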(event EventBeginPlay
  (|CallParentFunction) ; This node is disabled and will not be called.\nDrag off pins to build functionality.
)

(event Collision|EventActorBeginOverlap
  (params (OtherActor :type Actor%20Object%20Reference)))

(event EventTick
  (params (DeltaSeconds :type Float%20%28single-precision%29)))

(event EventToggleInventory
  (bind _asplayer_character (Utilities|Casting|CastToPlayer_CHARACTER (Game|GetPlayerCharacter 0)))
  (bind _itemfound (Default|CheckItemClass (Variables|/Game/Player/Player_CHARACTER.Player_CHARACTER_C|GetInventoryComponent _asplayer_character) "/Game/Inventory/Item/Item_CodeNote.Item_CodeNote_C"))
  (if _itemfound
    (Default|ToggleInventory (Variables|Default|GetInventoryComponent))
    (else
      (Development|PrintString "You need the keycard to open this up"))))

(fn ConstructionScript
  (|CallParentFunction))