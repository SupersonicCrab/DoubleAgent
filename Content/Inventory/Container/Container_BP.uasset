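; Container_BP is an interactable world container whose inventory a player character can toggle.
; On BeginPlay it copies its Items array into the InventoryComponent's inventory by index.
; The Interact event forwards to the component's ToggleInventory only for a Player_CHARACTER.
; Box overlap adds an action-plus-name prompt to that player's TextLog, stores the returned ID unless it is 666, and removes it by that ID on exit.
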(event OnComponentBeginOverlap(Box)
  (params (OverlappedComponent :type Primitive%20Component%20Object%20Reference) (OtherActor :type Actor%20Object%20Reference) (OtherComp :type Primitive%20Component%20Object%20Reference) (OtherBodyIndex :type Integer) (bFromSweep :type Boolean) (SweepResult :type Hit%20Result%20Structure%20%28by%20ref%29))
  (bind _asplayer_character (Utilities|Casting|CastToPlayer_CHARACTER OtherActor))
  (bind _logid (Default|AddText (Variables|/Game/Player/Player_CHARACTER.Player_CHARACTER_C|GetTextLog _asplayer_character) (Utilities|String|Append (Variables|Default|GetActionString) (Variables|Default|GetContainerName))))
  (if (not (== _logid 666))
    (Variables|Default|SetLogID _logid)))

(event OnComponentEndOverlap(Box)
  (params (OverlappedComponent :type Primitive%20Component%20Object%20Reference) (OtherActor :type Actor%20Object%20Reference) (OtherComp :type Primitive%20Component%20Object%20Reference) (OtherBodyIndex :type Integer))
  (bind _asplayer_character (Utilities|Casting|CastToPlayer_CHARACTER OtherActor))
  (Default|RemoveText (Variables|/Game/Player/Player_CHARACTER.Player_CHARACTER_C|GetTextLog _asplayer_character) (Variables|Default|GetLogID)))

(event EventInteract
  (params (Interactor :type Actor%20Object%20Reference))
  (Utilities|Casting|CastToPlayer_CHARACTER Interactor)
  (CallFunction|ToggleInventory))

(event EventBeginPlay
  (for (_array_element _array_index) (Variables|Default|GetItems)
    (Utilities|Array|SetArrayElem (Variables|/Game/Inventory/InventoryComponent.InventoryComponent_C|GetInventory (Variables|Default|GetInventoryComponent)) _array_index _array_element)))

(fn ConstructionScript)

(fn ToggleInventory
  (Default|ToggleInventory (Variables|Default|GetInventoryComponent)))