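; BP_Container is an interactable inventory container for the player character.
; On BeginPlay it names its InventoryComponent after the container and copies its Items into the inventory slots; interacting toggles that inventory.
; A Box overlap adds an E-key prompt to the player controller's context menu and removes it on exit.
; NetSetInventory overwrites the inventory, intended for network updates, while the actor's own ToggleInventory function is empty.
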(event OnComponentBeginOverlap(Box)
  (params (OverlappedComponent :type Primitive%20Component%20Object%20Reference) (OtherActor :type Actor%20Object%20Reference) (OtherComp :type Primitive%20Component%20Object%20Reference) (OtherBodyIndex :type Integer) (bFromSweep :type Boolean) (SweepResult :type Hit%20Result%20Structure%20%28by%20ref%29))
  ;[1 1 1] Context menu
  (bind _asbp_player_character (Utilities|Casting|CastToBP_Player_CHARACTER OtherActor))
  (bind _asbp_spy_player_playercontroller (Utilities|Casting|CastToBP_SpyPlayer_PLAYERCONTROLLER (Pawn|GetController _asbp_player_character)))
  (bind _slotref (Default|OverlapBegin (Variables|/Game/Player/BP_SpyPlayer_PLAYERCONTROLLER.BP_SpyPlayer_PLAYERCONTROLLER_C|GetContexMenu _asbp_spy_player_playercontroller) (Utilities|String|Append (Variables|Default|GetActionString) (Variables|Default|GetContainerName)) _asbp_spy_player_playercontroller "/Game/UI/ContextMenu/T_EKey.T_EKey"))
  (Variables|Default|SetSlotRef _slotref))

(event OnComponentEndOverlap(Box)
  (params (OverlappedComponent :type Primitive%20Component%20Object%20Reference) (OtherActor :type Actor%20Object%20Reference) (OtherComp :type Primitive%20Component%20Object%20Reference) (OtherBodyIndex :type Integer))
  ;[1 1 1] Context menu
  (bind _asbp_player_character (Utilities|Casting|CastToBP_Player_CHARACTER OtherActor))
  (bind _asbp_spy_player_playercontroller (Utilities|Casting|CastToBP_SpyPlayer_PLAYERCONTROLLER (Pawn|GetController _asbp_player_character)))
  (Default|OverlapEnd (Variables|/Game/Player/BP_SpyPlayer_PLAYERCONTROLLER.BP_SpyPlayer_PLAYERCONTROLLER_C|GetContexMenu _asbp_spy_player_playercontroller) (Variables|Default|GetSlotRef))
  (Variables|Default|SetSlotRef 0))

(event Custom|NetSetInventory
  (params (NewInventory :type Array%20of%20F%20Slot%20Structure%20Structures))
  ;[1 1 1] Set inventory over network
  (Variables|/Game/Inventory/BP_InventoryComponent.BP_InventoryComponent_C|SetInventory (Variables|Default|GetInventoryComponent) NewInventory))

(event EventInteract
  (params (Interactor :type Actor%20Object%20Reference))
  ;[1 1 1] Interact handling
  (Utilities|Casting|CastToBP_Player_CHARACTER Interactor)
  (Default|ToggleInventory (Variables|Default|GetInventoryComponent) Interactor))

(event EventBeginPlay
  ;[1 1 1] Setup
  (Variables|/Game/Inventory/BP_InventoryComponent.BP_InventoryComponent_C|SetInventoryName (Variables|Default|GetInventoryComponent) (Utilities|Text|ToText(String) (Variables|Default|GetContainerName)))
  (for (_array_element _array_index) (Variables|Default|GetItems)
    (Utilities|Array|SetArrayElem (Variables|/Game/Inventory/BP_InventoryComponent.BP_InventoryComponent_C|GetInventory (Variables|Default|GetInventoryComponent)) _array_index _array_element)))

(fn ConstructionScript)

(fn ToggleInventory
  (params (Interactor :type Actor%20Object%20Reference)))