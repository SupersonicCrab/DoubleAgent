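; Inventory item for a camera hack tool that toggles a camera-hacking HUD when used while equipped.
; UseItem runs the parent logic and an equipped-item check, then returns true.
; UseEquippedItem flips ToolActive, creating or removing the WBP_CameraHack_HUD widget on the player's screen.
; Opening it switches the player controller to Game and UI input with a locked, visible cursor, while closing restores game-only input and hides the cursor.
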(event EventBeginPlay)

(event Collision|EventActorBeginOverlap
  (params (OtherActor :type Actor%20Object%20Reference)))

(event EventTick
  (params (DeltaSeconds :type Float%20%28single-precision%29)))

(fn ConstructionScript
  (|CallParentFunction))

(fn UseItem
  (params (Player :type Character%20Object%20Reference))
  (|CallParentFunction Player)
  (CallFunction|EquippedItemCheck Player)
  (return true))

(fn UseEquippedItem
  (params (Player :type Controller%20Object%20Reference))
  (|CallParentFunction Player)
  (if (LocalVariables|GetbToolActive)
    (LocalVariables|SetbToolActive false)
    (Widget|RemovefromParent (LocalVariables|GetHackToolWidget))
    (LocalVariables|SetHackToolWidget 0)
    (bind _asplayer_controller (Utilities|Casting|CastToPlayerController Player))
    (Input|SetInputModeGameOnly _asplayer_controller)
    (Variables|/Script/Engine.PlayerController|SetbShowMouseCursor _asplayer_controller false)
    (else
      (LocalVariables|SetbToolActive true)
      (bind _asplayer_controller_2 (Utilities|Casting|CastToPlayerController Player))
      (bind _returnvalue (UserInterface|CreateWidget "/Game/SecuritySystem/UI/WBP_CameraHack_HUD.WBP_CameraHack_HUD_C" _asplayer_controller_2))
      (bind _output_get (LocalVariables|SetHackToolWidget _returnvalue))
      (UserInterface|Viewport|AddtoPlayerScreen _output_get)
      (Input|SetInputModeGameandUI _asplayer_controller_2 _output_get "LockAlways" true)
      (Variables|/Script/Engine.PlayerController|SetbShowMouseCursor _asplayer_controller_2 true))))