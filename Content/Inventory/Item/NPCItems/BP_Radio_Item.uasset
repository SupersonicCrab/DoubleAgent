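; Radio inventory item Blueprint that marks the actor carrying it with a "Radio" actor tag.
; OnPickup adds the tag to the given actor if it is absent, and OnRemove removes it if present.
; The event graph holds only disabled stub events, and the construction script just calls the parent.
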(event EventBeginPlay)

(event Collision|EventActorBeginOverlap
  (params (OtherActor :type Actor%20Object%20Reference)))

(event EventTick
  (params (DeltaSeconds :type Float%20%28single-precision%29)))

(fn ConstructionScript
  (|CallParentFunction))

(fn OnPickup
  (params (Actor :type Actor%20Object%20Reference))
  (bind _tags (Variables|/Script/Engine.Actor|GetTags Actor))
  (if (== (Utilities|Array|FindItem _tags "Radio") -1) ; if tag was not found
    (Utilities|Array|Add _tags "Radio")))

(fn OnRemove
  (params (Actor :type Actor%20Object%20Reference))
  (bind _tags (Variables|/Script/Engine.Actor|GetTags Actor))
  (if (!= (Utilities|Array|FindItem _tags "Radio") -1) ; If item was found
    (Utilities|Array|RemoveItem _tags "Radio")))