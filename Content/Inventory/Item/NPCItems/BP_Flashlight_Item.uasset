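; Flashlight inventory item that the player equips, holds in hand and switches on and off.
; Using it from the inventory runs the inherited equipped-item check.
; When held, it sets the player's flashlight-out flag and snaps to a hand socket on the player mesh; removal clears the flag.
; Using the equipped item toggles the spot light's visibility and updates the on/off prompt text.
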(event EventBeginPlay
  (|CallParentFunction) ; This node is disabled and will not be called.\nDrag off pins to build functionality.
)

(event Collision|EventActorBeginOverlap
  (params (OtherActor :type Actor%20Object%20Reference)))

(event EventTick
  (params (DeltaSeconds :type Float%20%28single-precision%29)))

(fn ConstructionScript
  (|CallParentFunction))

(fn UseItem
  (params (Player :type Character%20Object%20Reference) (ItemIndex :type Integer))
  (CallFunction|EquippedItemCheck Player ItemIndex)
  (return true))

(fn EquippedItemCheck
  (params (Player :type Character%20Object%20Reference) (Index :type Integer))
  (|CallParentFunction Player Index))

(fn OnHeld
  (|CallParentFunction)
  (Default|SetFlashLightOut (.AsBP%20Player%20CHARACTER (Utilities|Casting|CastToBP_Player_CHARACTER (Actor|GetParentActor))) true)
  (Transformation|AttachComponentToComponent (Variables|/Script/Engine.Character|GetMesh (.AsPlayer%20Character (Utilities|Casting|CastToPlayer_Character (Actor|GetParentActor)))) "HoldHandSocket2" "SnapToTarget" "SnapToTarget" "SnapToTarget" true))

(fn OnRemove
  (params (Actor :type Actor%20Object%20Reference))
  (|CallParentFunction Actor)
  (Default|SetFlashLightOut (.AsBP%20Player%20CHARACTER (Utilities|Casting|CastToBP_Player_CHARACTER (Actor|GetParentActor))) false))

(fn UseEquippedItem
  (params (Player :type Controller%20Object%20Reference))
  (bind _spotlight (Variables|Default|GetSpotLight))
  (|CallParentFunction Player)
  (if (Variables|/Script/Engine.SceneComponent|GetbVisible (Variables|Default|GetSpotLight))
    (Rendering|SetVisibility _spotlight false false)
    (Variables|Default|SetPrimaryText "Turn flashlight on")
    (else
      (Rendering|SetVisibility _spotlight true false)
      (Variables|Default|SetPrimaryText "Turn flashlight off"))))