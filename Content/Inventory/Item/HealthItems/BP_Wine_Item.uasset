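; Wine health item Blueprint that heals the player at a cost of altered vision and play rate when used.
; Its UseItem override casts to BP_Player_CHARACTER, triggers a vision change, applies a timed play-rate reduction and adds a small amount of health through HealthComponent.
; It then returns the result of the parent UseItem, while the event graph holds only disabled default events.
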(event EventBeginPlay
  (|CallParentFunction) ; This node is disabled and will not be called.\nDrag off pins to build functionality.
)

(event Collision|EventActorBeginOverlap
  (params (OtherActor :type Actor%20Object%20Reference)))

(event EventTick
  (params (DeltaSeconds :type Float%20%28single-precision%29)))

(fn ConstructionScript
  (|CallParentFunction))

(fn UseItem
  (params (Player :type Character%20Object%20Reference) (ItemIndex :type Integer))
  (bind _asbp_player_character (Utilities|Casting|CastToBP_Player_CHARACTER Player))
  (Default|VisionChange _asbp_player_character 3)
  (Default|ChangePlayRate _asbp_player_character 0.8 3e+01)
  (Default|GainHealth (Variables|/Game/Player/BP_Player_CHARACTER.BP_Player_CHARACTER_C|GetHealthComponent _asbp_player_character) 1e+01)
  (bind _success (|CallParentFunction Player ItemIndex))
  (return _success))