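; Equippable spotter glasses item that sits on the player's head and lets them mark AI enemies with outlines.
; Using it fires a forward line trace that toggles the hit enemy in a capped tracked list, replacing the oldest when full, and logs the result.
; Outline changes route through the player's ServerUpdateOutlines.
; The tracked list is copied to the player on unequip so it can be restored on re-equip.
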(event Custom|ServerMarkUpdate
  (params (Player :type BP%20AI%20Character%20Base%20CHARACTER%20Object%20Reference) (EnableOutline :type Boolean))
  (if EnableOutline
    (Default|EnableOutline Player)
    (else
      (Default|DisableOutline Player))))

(event EventBeginPlay
  (|CallParentFunction) ; This node is disabled and will not be called.\nDrag off pins to build functionality.
)

(event Collision|EventActorBeginOverlap
  (params (OtherActor :type Actor%20Object%20Reference)))

(event EventTick
  (params (DeltaSeconds :type Float%20%28single-precision%29)))

(fn ConstructionScript
  (|CallParentFunction))

(fn UseItem
  (params (Player :type Character%20Object%20Reference) (ItemIndex :type Integer))
  (bind _asbp_player_character (Utilities|Casting|CastToBP_Player_CHARACTER Player)
    (:then
      (if (.equipped (.itemstructure (Utilities|Array|Get(acopy) (Variables|/Game/Inventory/BP_InventoryComponent.BP_InventoryComponent_C|GetInventory (Variables|/Game/Player/BP_Player_CHARACTER.BP_Player_CHARACTER_C|GetInventoryComponent _asbp_player_character)) ItemIndex))) ; Is the item currently equipped?
        (Variables|/Game/Player/BP_Player_CHARACTER.BP_Player_CHARACTER_C|SetTrackedEnemies _asbp_player_character (Variables|BP_SpotterGlasses_Item_C|GetTrackedEnemies (.AsBP%20Spotter%20Glasses%20Item (Utilities|Casting|CastToBP_SpotterGlasses_Item (Variables|/Script/Engine.ChildActorComponent|GetChildActor (Variables|/Game/Player/BP_Player_CHARACTER.BP_Player_CHARACTER_C|GetEquippedItem _asbp_player_character)))))) ; Save the equipped enemies on the player to be used when the glasses are put back on
      ))
    (:CastFailed
      _))
  (CallFunction|EquippedItemCheck Player ItemIndex)
  (if (.bSuccess (Utilities|Casting|CastToBP_SpotterGlasses_Item (Variables|/Script/Engine.ChildActorComponent|GetChildActor (Variables|/Game/Player/BP_Player_CHARACTER.BP_Player_CHARACTER_C|GetEquippedItem _asbp_player_character))))
    (Variables|BP_SpotterGlasses_Item_C|SetTrackedEnemies (.AsBP%20Spotter%20Glasses%20Item (Utilities|Casting|CastToBP_SpotterGlasses_Item (Variables|/Script/Engine.ChildActorComponent|GetChildActor (Variables|/Game/Player/BP_Player_CHARACTER.BP_Player_CHARACTER_C|GetEquippedItem _asbp_player_character)))) (Variables|/Game/Player/BP_Player_CHARACTER.BP_Player_CHARACTER_C|GetTrackedEnemies _asbp_player_character)))
  (bind _success (|CallParentFunction Player ItemIndex))
  (return _success))

(fn UseEquippedItem
  (params (Player :type Controller%20Object%20Reference))
  (bind _returnvalue (Actor|GetParentActor))
  (bind _asbp_player_character (Utilities|Casting|CastToBP_Player_CHARACTER _returnvalue))
  (bind _returnvalue_2 (Pawn|GetController _asbp_player_character))
  (bind _asbp_spy_player_playercontroller (Utilities|Casting|CastToBP_SpyPlayer_PLAYERCONTROLLER _returnvalue_2))
  (bind _textlog (Variables|/Game/Player/BP_SpyPlayer_PLAYERCONTROLLER.BP_SpyPlayer_PLAYERCONTROLLER_C|GetTextLog _asbp_spy_player_playercontroller))
  (|CallParentFunction Player)
  (bind (_outhit _returnvalue_3) (Collision|LineTraceByChannel (Transformation|GetActorLocation) (* (Transformation|GetActorForwardVector) 1e+08) "TraceTypeQuery1" false (Utilities|Array|MakeArray (Actor|GetParentActor)) "None"))
  (if _returnvalue_3
    (bind _asbp_aicharacter_base_character (Utilities|Casting|CastToBP_AICharacterBase_CHARACTER (.HitActor (Collision|BreakHitResult _outhit)))
      (:then
        (bind _displaytext (CallFunction|MarkEnemy _asbp_aicharacter_base_character))
        (Default|DisplayLog _textlog false _displaytext "/Game/Art/Textures/UI/Icons/Logos/T_DefaultIcon.T_DefaultIcon"))
      (:CastFailed
        (Default|DisplayLog _textlog false "Not a markable enemy" "/Game/Art/Textures/UI/Icons/Logos/T_DefaultIcon.T_DefaultIcon")))
    (else
      (Default|DisplayLog _textlog false "Nothing was hit" "/Game/Art/Textures/UI/Icons/Logos/T_DefaultIcon.T_DefaultIcon"))))

(fn MarkEnemy
  (params (EnemyHit :type BP%20AI%20Character%20Base%20CHARACTER%20Object%20Reference))
  (bind (_array_element _array_index) (Utilities|Array|ForEachLoopwithBreak (Variables|Default|GetTrackedEnemies) :!label _label)
    (:LoopBody
      (if (== _array_element EnemyHit) ; Is the hit enemy already being tracked?
        (LocalVariables|SetTrackedIndex _array_index)
        (LocalVariables|SetTracked true)
        (goto _label Break)))
    (:Completed
      (if (LocalVariables|GetTracked) ; Was the hit enemy already being tracked?
        (Default|ServerUpdateOutlines (.AsBP%20Player%20CHARACTER (Utilities|Casting|CastToBP_Player_CHARACTER (Game|GetPlayerCharacter 0))) EnemyHit false)
        (Utilities|Array|RemoveItem (Variables|Default|GetTrackedEnemies) EnemyHit) ; Remove enemy from tracked list
        (LocalVariables|SetDisplayMessage "Unmarked Enemy")
        (elif (== (Utilities|Array|Length (Variables|Default|GetTrackedEnemies)) (Variables|Default|GetTrackLimit)) ; Is the player already tracking the maximum number of enemies
          (CallFunction|TrackUpdate EnemyHit)
          (LocalVariables|SetDisplayMessage "5 Trackers reached, replacing first tracker")
          (else
            (Utilities|Array|Add (Variables|Default|GetTrackedEnemies) EnemyHit) ; Add enemy to tracked list
            (Default|ServerUpdateOutlines (.AsBP%20Player%20CHARACTER (Utilities|Casting|CastToBP_Player_CHARACTER (Game|GetPlayerCharacter 0))) EnemyHit true)
            (LocalVariables|SetDisplayMessage "Enemy Marked"))))
      (return (LocalVariables|GetDisplayMessage)))))

(fn OnHeld
  (|CallParentFunction)
  (Transformation|AttachComponentToComponent (Variables|/Script/Engine.Character|GetMesh (.AsPlayer%20Character (Utilities|Casting|CastToPlayer_Character (Actor|GetParentActor)))) "head" "SnapToTarget" "SnapToTarget" "SnapToTarget" true)
  (Transformation|SetActorRelativeTransform (Math|Transform|MakeTransform "6.000000,8.000000,-0.500000" "180.000000,-90.000000,90.000000" "1.300000,1.300000,1.300000") false true) ; Positioning tool relative to head
)

(fn TrackUpdate
  (params (HitEnemy :type BP%20AI%20Character%20Base%20CHARACTER%20Object%20Reference))
  (bind _returnvalue (Components|GetOwner))
  (bind _trackedenemies (Variables|Default|GetTrackedEnemies))
  (bind _asbp_player_character (Utilities|Casting|CastToBP_Player_CHARACTER _returnvalue))
  (Default|ServerUpdateOutlines _asbp_player_character (Utilities|Array|Get(acopy) _trackedenemies) false)
  (Utilities|Array|RemoveIndex _trackedenemies)
  (Utilities|Array|Add _trackedenemies HitEnemy)
  (Default|ServerUpdateOutlines _asbp_player_character HitEnemy true))