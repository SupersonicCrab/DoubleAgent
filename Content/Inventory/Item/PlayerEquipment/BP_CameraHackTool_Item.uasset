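; Equippable inventory item for a camera hack tool that opens a camera hacking HUD when used.
; Selecting it runs the parent item logic and an equipped-item check.
; Using it while equipped creates the HUD widget, switches to UI-only input with a visible cursor, and sets the hack tool state on the player character.
; When held, it snaps to a hand socket on the character mesh with an adjusted relative transform.
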(event Collision|EventActorBeginOverlap
  (params (OtherActor :type Actor%20Object%20Reference)))

(event EventTick
  (params (DeltaSeconds :type Float%20%28single-precision%29)))

(fn ConstructionScript
  (|CallParentFunction))

(fn UseItem
  (params (Player :type Character%20Object%20Reference) (ItemIndex :type Integer))
  (|CallParentFunction Player ItemIndex)
  (CallFunction|EquippedItemCheck Player ItemIndex)
  (return true))

(fn UseEquippedItem
  (params (Player :type Controller%20Object%20Reference))
  (|CallParentFunction Player)
  (bind _asplayer_controller (Utilities|Casting|CastToPlayerController Player))
  (bind _returnvalue (UserInterface|CreateWidget "/Game/UI/Equipment/WBP_CameraHack_HUD.WBP_CameraHack_HUD_C" _asplayer_controller))
  (bind _output_get (Variables|Default|SetHackToolWidget _returnvalue))
  (UserInterface|Viewport|AddtoViewport _output_get 0)
  (Input|SetInputModeUIOnly _asplayer_controller _output_get "DoNotLock")
  (Variables|/Script/Engine.PlayerController|SetbShowMouseCursor _asplayer_controller true)
  (Default|SetHacktool (.AsBP%20Player%20CHARACTER (Utilities|Casting|CastToBP_Player_CHARACTER (Pawn|GetControlledPawn Player))) true))

(fn OnHeld
  (|CallParentFunction)
  (Transformation|AttachComponentToComponent (Variables|/Script/Engine.Character|GetMesh (.AsPlayer%20Character (Utilities|Casting|CastToPlayer_Character (Actor|GetParentActor)))) "HoldHandSocket2" "SnapToTarget" "SnapToTarget" "SnapToTarget" true)
  (Transformation|SetActorRelativeTransform (Math|Transform|MakeTransform "14.000000,-12.000000,0.000000" "190.000000,45.000000,0.000000" "1,1,1") false true) ; Positioning tool relative to hand
)