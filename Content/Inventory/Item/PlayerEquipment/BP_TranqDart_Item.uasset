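; Tranquilizer dart item that, when spawned as fired, launches as a physics projectile along the owner's controller aim and knocks out AI characters it hits.
; BeginPlay orients the mesh toward a point ahead of the owner and sets a fast linear velocity.
; On hit, a standing NPC is disabled, movement-locked, animated as knocked out and the dart destroys itself.
; Players and doors just stop the dart, while other surfaces also freeze it in place.
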(event OnComponentHit(StaticMesh)
  (params (HitComponent :type Primitive%20Component%20Object%20Reference) (OtherActor :type Actor%20Object%20Reference) (OtherComp :type Primitive%20Component%20Object%20Reference) (NormalImpulse :type Vector :default "0, 0, 0") (Hit :type Hit%20Result%20Structure%20%28by%20ref%29))
  (bind _staticmesh (Variables|Default|GetStaticMesh))
  (if (Variables|Default|GetbFired)
    (bind _asbp_aicharacter_base_character (Utilities|Casting|CastToBP_AICharacterBase_CHARACTER OtherActor)
      (:then
        (if (not (Variables|/Game/AI/NPC/BP_AICharacterBase_CHARACTER.BP_AICharacterBase_CHARACTER_C|GetbDowned _asbp_aicharacter_base_character))
          (CallFunction|KnockoutNPC _asbp_aicharacter_base_character)))
      (:CastFailed
        (Utilities|Casting|CastToBP_Player_CHARACTER OtherActor
          (:then
            (Physics|SetPhysicsLinearVelocity (Variables|Default|GetStaticMesh) "0, 0, 0" false "None" :!label _label)
            (Variables|Default|SetbFired false))
          (:CastFailed
            (Utilities|Casting|CastToBP_Door OtherActor
              (:then
                (goto _label))
              (:CastFailed
                (Physics|SetPhysicsLinearVelocity _staticmesh "0, 0, 0" false "None")
                (Physics|SetEnableGravity _staticmesh false)
                (Physics|SetSimulatePhysics _staticmesh false)
                (Variables|Default|SetbFired false)))))))))

(event Custom|KnockoutNPC
  (params (NPC :type BP%20AI%20Character%20Base%20CHARACTER%20Object%20Reference))
  (bind _charactermovement (Variables|/Script/Engine.Character|GetCharacterMovement NPC))
  (Class|AICharacterBaseCHARACTER|DisableNPC NPC)
  (Default|NetDownedHitbox NPC)
  (Variables|/Script/Engine.CharacterMovementComponent|SetbUseControllerDesiredRotation _charactermovement false)
  (Components|Movement|StopMovementImmediately _charactermovement)
  (Class|AIController|ClaimTaskResource (AI|GetAIController NPC) "/Script/AIModule.AIResource_Movement") ; Locking NPC movement
  (Variables|/Script/DoubleAgent.AICharacterBase_CHARACTER|SetbTranquilized NPC true)
  (Class|BaseCharacterCHARACTER|StopSpeaking NPC)
  (Default|NetPlayAnimation NPC "/Game/Animations/Sequences/Standing/A_KnockedOut.A_KnockedOut" 0.25 0.0 0.0)
  (Actor|DestroyActor))

(event EventBeginPlay
  (bind _returnvalue (Transformation|GetActorLocation))
  (bind _returnvalue_2 (Components|GetOwner))
  (bind _staticmesh (Variables|Default|GetStaticMesh))
  (bind _controllerforward (Variables|Default|GetControllerForward))
  (bind _returnvalue_3 (Transformation|GetActorLocation _returnvalue_2))
  (bind _returnvalue_4 (* _controllerforward 1e+03))
  (bind _returnvalue_5 (+ _returnvalue_4 _returnvalue_3))
  (bind _returnvalue_6 (Math|Rotator|FindLookatRotation _returnvalue _returnvalue_5))
  (|CallParentFunction)
  (if (Variables|Default|GetbFired)
    (Transformation|SetActorRotation (Math|Rotator|MakeRotator (.roll _returnvalue_6) (+ (.pitch _returnvalue_6) -9e+01) (.yaw _returnvalue_6)) true)
    (Physics|SetSimulatePhysics _staticmesh true)
    (Class|PrimitiveComponent|SetAllPhysicsLinearVelocity _staticmesh (* (Math|Vector|GetForwardVector (Math|Rotator|FindLookatRotation _returnvalue _returnvalue_5)) 7e+03) false)))

(fn ConstructionScript
  (|CallParentFunction))