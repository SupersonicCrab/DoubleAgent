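; Equippable vision glasses item that switches the player's vision mode and snaps to the head socket when held.
; Use toggles mode 1 and alt-use toggles mode 2, each overriding the other, with 0 as off.
; Each use passes the mode to the player character's VisionChange.
; Using the item while already equipped resets the character's vision to 0 before the parent equip check runs.
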(event EventBeginPlay
  (|CallParentFunction) ; This node is disabled and will not be called.\nDrag off pins to build functionality.
)

(event Collision|EventActorBeginOverlap
  (params (OtherActor :type Actor%20Object%20Reference)))

(event EventTick
  (params (DeltaSeconds :type Float%20%28single-precision%29)))

(fn ConstructionScript
  (|CallParentFunction))

(fn UseItem
  (params (Player :type Character%20Object%20Reference) (ItemIndex :type Integer))
  (bind _success (|CallParentFunction 0 0))
  (CallFunction|EquippedItemCheck Player)
  (return _success))

(fn UseEquippedItem
  (params (Player :type Controller%20Object%20Reference))
  (|CallParentFunction Player)
  (switch int (Variables|Default|GetVision)
    (:0
      (Variables|Default|SetVision 1 :!label _label)
      (Variables|Default|SetbActive true))
    (:1
      (Variables|Default|SetVision 0)
      (Variables|Default|SetbActive false))
    (:2
      (goto _label)))
  (bind _asbp_player_character (Utilities|Casting|CastToBP_Player_CHARACTER (Pawn|GetControlledPawn Player)))
  (Default|VisionChange _asbp_player_character (Variables|Default|GetVision)))

(fn AltUseEquippedItem
  (params (Player :type Controller%20Object%20Reference))
  (|CallParentFunction Player)
  (switch int (Variables|Default|GetVision)
    (:0
      (Variables|Default|SetVision 2 :!label _label)
      (Variables|Default|SetbActive true))
    (:1
      (goto _label))
    (:2
      (Variables|Default|SetVision 0)
      (Variables|Default|SetbActive false)))
  (bind _asbp_player_character (Utilities|Casting|CastToBP_Player_CHARACTER (Pawn|GetControlledPawn Player)))
  (Default|VisionChange _asbp_player_character (Variables|Default|GetVision)))

(fn OnHeld
  (|CallParentFunction)
  (Transformation|AttachComponentToComponent (Variables|/Script/Engine.Character|GetMesh (.AsPlayer%20Character (Utilities|Casting|CastToPlayer_Character (Actor|GetParentActor)))) "head" "SnapToTarget" "SnapToTarget" "SnapToTarget" true)
  (Transformation|SetActorRelativeTransform (Math|Transform|MakeTransform "6.000000,8.000000,-0.500000" "180.000000,-90.000000,90.000000" "1.300000,1.300000,1.300000") false true) ; Positioning tool relative to head
)

(fn EquippedItemCheck
  (params (Player :type Character%20Object%20Reference) (Index :type Integer))
  (bind _asbp_player_character (Utilities|Casting|CastToBP_Player_CHARACTER Player))
  (bind _output_get (LocalVariables|SetPlayerCast _asbp_player_character))
  (if (.equipped (.itemstructure (Utilities|Array|Get(acopy) (Variables|/Game/Inventory/BP_InventoryComponent.BP_InventoryComponent_C|GetInventory (Variables|/Game/Player/BP_Player_CHARACTER.BP_Player_CHARACTER_C|GetInventoryComponent _output_get)) Index)))
    (Default|VisionChange (LocalVariables|GetPlayerCast)))
  (|CallParentFunction Player Index))