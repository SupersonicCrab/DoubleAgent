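; Inventory item for vision glasses that are worn on the player's head and switch between vision modes.
; Using the item runs the equip check, and holding it snaps it to the mesh's head socket with a fitted offset.
; Primary and alternate use each toggle their own mode, replacing the other if active.
; Each change passes the new Vision value to BP_Player_CHARACTER's VisionChange, which applies it.
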(event EventBeginPlay
  (|CallParentFunction) ; This node is disabled and will not be called.\nDrag off pins to build functionality.
)

(event Collision|EventActorBeginOverlap
  (params (OtherActor :type Actor%20Object%20Reference)))

(event EventTick
  (params (DeltaSeconds :type Float%20%28single-precision%29)))

(fn ConstructionScript
  (|CallParentFunction))

(fn UseItem
  (params (Player :type Character%20Object%20Reference))
  (bind _success (|CallParentFunction 0))
  (CallFunction|EquippedItemCheck Player)
  (return _success))

(fn UseEquippedItem
  (params (Player :type Controller%20Object%20Reference))
  (|CallParentFunction Player)
  (switch int (Variables|Default|GetVision)
    (:0
      (Variables|Default|SetVision 1 :!label _label))
    (:1
      (Variables|Default|SetVision 0))
    (:2
      (goto _label)))
  (bind _asbp_player_character (Utilities|Casting|CastToBP_Player_CHARACTER (Pawn|GetControlledPawn Player)))
  (Default|VisionChange _asbp_player_character (Variables|Default|GetVision)))

(fn AltUseEquippedItem
  (params (Player :type Controller%20Object%20Reference))
  (|CallParentFunction Player)
  (switch int (Variables|Default|GetVision)
    (:0
      (Variables|Default|SetVision 2 :!label _label))
    (:1
      (goto _label))
    (:2
      (Variables|Default|SetVision 0)))
  (bind _asbp_player_character (Utilities|Casting|CastToBP_Player_CHARACTER (Pawn|GetControlledPawn Player)))
  (Default|VisionChange _asbp_player_character (Variables|Default|GetVision)))

(fn OnHeld
  (|CallParentFunction)
  (Transformation|AttachComponentToComponent (Variables|/Script/Engine.Character|GetMesh (.AsPlayer%20Character (Utilities|Casting|CastToPlayer_Character (Actor|GetParentActor)))) "head" "SnapToTarget" "SnapToTarget" "SnapToTarget" true)
  (Transformation|SetActorRelativeTransform (Math|Transform|MakeTransform "6.000000,8.000000,-0.500000" "180.000000,-90.000000,90.000000" "1.350000,1.300000,1") false true) ; Positioning tool relative to head
)