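; Tranquilizer gun inventory item that the player holds, aims and fires.
; Alt use toggles aiming by switching the character's view and weapon aim state.
; Use fires a dart through the player character only while aiming with a tranq dart item in the inventory, otherwise logging the reason to the player's text log.
; Being held applies a fixed relative transform to position the gun.
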(event EventBeginPlay
  (|CallParentFunction) ; This node is disabled and will not be called.\nDrag off pins to build functionality.
)

(event Collision|EventActorBeginOverlap
  (params (OtherActor :type Actor%20Object%20Reference)))

(event EventTick
  (params (DeltaSeconds :type Float%20%28single-precision%29)))

(fn ConstructionScript
  (|CallParentFunction))

(fn UseItem
  (params (Player :type Character%20Object%20Reference) (ItemIndex :type Integer))
  (CallFunction|EquippedItemCheck Player)
  (bind _success (|CallParentFunction 0 0))
  (return _success))

(fn UseEquippedItem
  (params (Player :type Controller%20Object%20Reference))
  (bind _returnvalue (Pawn|GetControlledPawn Player))
  (bind _asbp_spy_player_playercontroller (Utilities|Casting|CastToBP_SpyPlayer_PLAYERCONTROLLER Player))
  (bind _asbp_player_character (Utilities|Casting|CastToBP_Player_CHARACTER _returnvalue))
  (bind _textlog (Variables|/Game/Player/BP_SpyPlayer_PLAYERCONTROLLER.BP_SpyPlayer_PLAYERCONTROLLER_C|GetTextLog _asbp_spy_player_playercontroller))
  (|CallParentFunction Player)
  (bind _itemfound (Default|CheckItemClass (Variables|/Game/Player/BP_Player_CHARACTER.BP_Player_CHARACTER_C|GetInventoryComponent _asbp_player_character) "/Game/Inventory/Item/BP_TranqDart_Item.BP_TranqDart_Item_C"))
  (if _itemfound
    (if (Variables|Default|GetbAiming)
      (Default|FireTranqDart _asbp_player_character)
      (else
        (Default|DisplayLog _textlog false "Can't fire without aiming" "/Game/Art/Textures/UI/Icons/T_DefaultNeon.T_DefaultNeon")))
    (else
      (Default|DisplayLog _textlog false "No Tranq Darts" "/Game/Art/Textures/UI/Icons/T_DefaultNeon.T_DefaultNeon"))))

(fn OnHeld
  (|CallParentFunction)
  (Transformation|SetActorRelativeTransform (Math|Transform|MakeTransform "-4.000000,-1.500000,4.000000" "10.000000,90.000000,10.000000" "1,1,1") false false))

(fn AltUseEquippedItem
  (params (Player :type Controller%20Object%20Reference))
  (bind _returnvalue (Pawn|GetControlledPawn Player))
  (bind _asbp_player_character (Utilities|Casting|CastToBP_Player_CHARACTER _returnvalue))
  (|CallParentFunction Player)
  (if (not (Variables|Default|GetbAiming))
    (Default|SwitchView _asbp_player_character)
    (Default|SetWeaponAim _asbp_player_character true)
    (Variables|Default|SetbAiming true)
    (else
      (Default|SwitchView _asbp_player_character)
      (Default|SetWeaponAim _asbp_player_character false)
      (Variables|Default|SetbAiming false))))