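; Base inventory item that serves as a world pickup, added to the interactor's inventory and then destroyed, and as a player's held item.
; As a child actor, server BeginPlay disables physics, collision and sight stimulus, then attaches it to the hand socket after a delay workaround.
; OnHeld flags illegal equipment by item type.
; It also provides equip toggling, custom-depth outlines and stub use/pickup hooks; overlap prompt logic is disconnected.
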(event OnComponentBeginOverlap(Collision)
  (params (OverlappedComponent :type Primitive%20Component%20Object%20Reference) (OtherActor :type Actor%20Object%20Reference) (OtherComp :type Primitive%20Component%20Object%20Reference) (OtherBodyIndex :type Integer) (bFromSweep :type Boolean) (SweepResult :type Hit%20Result%20Structure%20%28by%20ref%29))
  ;[1 1 1] Context overlap
)

(event OnComponentEndOverlap(Collision)
  (params (OverlappedComponent :type Primitive%20Component%20Object%20Reference) (OtherActor :type Actor%20Object%20Reference) (OtherComp :type Primitive%20Component%20Object%20Reference) (OtherBodyIndex :type Integer))
  ;[1 1 1] Context overlap
)

(event Custom|NetSetChild
  (bind _staticmesh (Variables|Default|GetStaticMesh))
  ;[1 1 1] Child actor handling
  (Physics|SetSimulatePhysics _staticmesh false)
  (Collision|SetCollisionEnabled _staticmesh "NoCollision")
  (Collision|SetCollisionEnabled (Variables|Default|GetCollision) "NoCollision")
  (Class|AIPerceptionStimuliSourceComponent|UnregisterfromSense (Variables|Default|GetAIPerceptionStimuliSource) "/Script/AIModule.AISense_Sight")
  (Utilities|FlowControl|Delay 0.01) ; Unreal wont let me attach to the hand properly unless I use a delay
  (Transformation|AttachComponentToComponent (Variables|/Script/Engine.Character|GetMesh (.AsPlayer%20Character (Utilities|Casting|CastToPlayer_Character (Actor|GetParentActor)))) "HoldHandSocket" "SnapToTarget" "SnapToTarget" "SnapToTarget" true)
  (CallFunction|OnHeld))

(event EventBeginPlay
  (if (and (Class|Actor|IsChildActor) (Networking|IsServer))
    (CallFunction|NetSetChild)))

(event EventDisableOutline
  (bind _staticmesh (Variables|Default|GetStaticMesh))
  (Rendering|SetCustomDepthStencilValue _staticmesh 0)
  (Rendering|SetRenderCustomDepth _staticmesh false))

(event EventEnableOutline
  (bind _staticmesh (Variables|Default|GetStaticMesh))
  (Rendering|SetRenderCustomDepth _staticmesh true)
  (Rendering|SetCustomDepthStencilValue _staticmesh 253))

(event EventInteract
  (params (Interactor :type Actor%20Object%20Reference))
  ;[1 1 1] Interaction
  (bind _success (Default|AddtoInventory (Actor|GetComponentbyClass Interactor "/Game/Inventory/BP_InventoryComponent.BP_InventoryComponent_C") (Utilities|Struct|MakeFSlotStructure (Variables|Default|GetItemStructure) 1)))
  (if _success
    (Actor|DestroyActor)))

(fn ConstructionScript)

(fn UseItem
  (params (Player :type Character%20Object%20Reference) (ItemIndex :type Integer))
  (return true))

(fn EquippedItemCheck
  (params (Player :type Character%20Object%20Reference) (Index :type Integer))
  (bind _asbp_player_character (Utilities|Casting|CastToBP_Player_CHARACTER Player))
  (bind _output_get (LocalVariables|SetPlayerCast _asbp_player_character))
  (if (.equipped (.itemstructure (Utilities|Array|Get(acopy) (Variables|/Game/Inventory/BP_InventoryComponent.BP_InventoryComponent_C|GetInventory (Variables|/Game/Player/BP_Player_CHARACTER.BP_Player_CHARACTER_C|GetInventoryComponent _output_get)) Index)))
    (Default|SetEquippedItem (LocalVariables|GetPlayerCast) "/Game/Inventory/Item/BP_Empty.BP_Empty_C")
    (Default|UpdateContextSlots (LocalVariables|GetPlayerCast))
    (else
      (Default|SetEquippedItem (LocalVariables|GetPlayerCast) (.Class (Utilities|Struct|BreakFItemStructure (Variables|Default|GetItemStructure))))
      (Default|UpdateContextSlots (LocalVariables|GetPlayerCast) (Variables|Default|GetPrimaryText) (Variables|Default|GetAlternateText)))))

(fn OnPickup
  (params (Actor :type Actor%20Object%20Reference)))

(fn OnRemove
  (params (Actor :type Actor%20Object%20Reference)))

(fn UseEquippedItem
  (params (Player :type Controller%20Object%20Reference)))

(fn OnHeld
  (bind _returnvalue (Actor|GetParentActor))
  (bind _itemstructure (Variables|Default|GetItemStructure))
  (bind _asbp_player_character (Utilities|Casting|CastToBP_Player_CHARACTER _returnvalue))
  (if (>= (.itemtype _itemstructure) (Utilities|Enum|LiteralenumEItemType "NewEnumerator4"))
    (Variables|/Script/DoubleAgent.Player_Character|SetbIllegalEquipment _asbp_player_character true)
    (bind _asbp_spy_player_playercontroller (Utilities|Casting|CastToBP_SpyPlayer_PLAYERCONTROLLER (Pawn|GetController _asbp_player_character)))
    (Utilities|IsValid (Variables|/Game/Player/BP_SpyPlayer_PLAYERCONTROLLER.BP_SpyPlayer_PLAYERCONTROLLER_C|GetTextLog _asbp_spy_player_playercontroller)
      (:Is%20Valid
        (Default|DisplayLog (Variables|/Game/Player/BP_SpyPlayer_PLAYERCONTROLLER.BP_SpyPlayer_PLAYERCONTROLLER_C|GetTextLog _asbp_spy_player_playercontroller) false "You are using illegal equipment" (.thumbnail _itemstructure))))
    (else
      (Variables|/Script/DoubleAgent.Player_Character|SetbIllegalEquipment _asbp_player_character false))))

(fn AltUseEquippedItem
  (params (Player :type Controller%20Object%20Reference)))

(fn GetCenter
  (return (.Origin (Collision|GetComponentBounds (Variables|Default|GetStaticMesh)))))

(fn GetInteractText
  (return (Utilities|String|Append (Utilities|String|MakeLiteralString "Pickup ") (Utilities|String|ToString(Text) (.name (Variables|Default|GetItemStructure))))))