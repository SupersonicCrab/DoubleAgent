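; Slot-based inventory component for a spy game, with stacking, slot locking and a toggleable inventory window on the player's HUD.
; PrepareInventory, run at BeginPlay and on each window opening, fills slots from item class defaults, briefly spawns items to fire OnPickup and snapshots the contents.
; Adding items fills partial stacks, recursing on overflow, then updates the player's summed detection rating and refreshes slots.
; CheckInventory compares against the snapshot to report the highest-priority changed item type.
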(event EventBeginPlay
  (CallFunction|PrepareInventory))

(fn ToggleInventory
  (params (Interactor :type Actor%20Object%20Reference))
  (bind _asbp_player_character (Utilities|Casting|CastToBP_Player_CHARACTER Interactor))
  (bind _asbp_spy_player_playercontroller (Utilities|Casting|CastToBP_SpyPlayer_PLAYERCONTROLLER (Pawn|GetController _asbp_player_character)))
  (Variables|Default|SetInteractorPC _asbp_spy_player_playercontroller)
  (Variables|Widgets|GetInventoryWindow ; Checks to see if there is already a window
    (:then
      ;[1 1 1] Removes the inventory from the GUI
      (Variables|Default|SetInventoryPosition (Variables|/Game/Inventory/InventoryUI/WBP_InventoryWindow.WBP_InventoryWindow_C|GetsavedPosition (Variables|Widgets|GetInventoryWindow)))
      (Widget|RemovefromParent (Variables|Widgets|GetInventoryWindow))
      (Variables|Widgets|SetInventoryWindow 0)
      (Input|SetInputModeGameOnly (Variables|Default|GetInteractorPC))
      (Variables|/Script/Engine.PlayerController|SetbShowMouseCursor (Variables|Default|GetInteractorPC) false)
      (bind _asbp_spy_player_playercontroller_2 (Utilities|Casting|CastToBP_SpyPlayer_PLAYERCONTROLLER (Variables|Default|GetInteractorPC)))
      (Variables|/Game/Player/BP_SpyPlayer_PLAYERCONTROLLER.BP_SpyPlayer_PLAYERCONTROLLER_C|SetExistingInventory _asbp_spy_player_playercontroller_2 0))
    (:else
      ;[1 1 1] Creates the inventory on the GUI
      (bind _asbp_spy_player_playercontroller_3 (Utilities|Casting|CastToBP_SpyPlayer_PLAYERCONTROLLER (Variables|Default|GetInteractorPC)))
      (if (!= (Variables|/Game/Player/BP_SpyPlayer_PLAYERCONTROLLER.BP_SpyPlayer_PLAYERCONTROLLER_C|GetExistingInventory _asbp_spy_player_playercontroller_3) 0) ; Does an inventory exist that's not tied to this component?
        (Default|ReplaceInventory _asbp_spy_player_playercontroller_3))
      (CallFunction|PrepareInventory)
      (bind _returnvalue (UserInterface|CreateWidget "/Game/Inventory/InventoryUI/WBP_InventoryWindow.WBP_InventoryWindow_C" 0 self (Variables|Default|GetInventoryPosition)))
      (bind _output_get (Variables|Widgets|SetInventoryWindow _returnvalue))
      (bind _asbp_spy_player_playercontroller_4 (Utilities|Casting|CastToBP_SpyPlayer_PLAYERCONTROLLER (Variables|Default|GetInteractorPC)))
      (bind _output_get_2 (Variables|/Game/Player/BP_SpyPlayer_PLAYERCONTROLLER.BP_SpyPlayer_PLAYERCONTROLLER_C|SetExistingInventory _asbp_spy_player_playercontroller_4 _output_get))
      (bind _returnvalue_2 (Class|CanvasPanel|AddChildtoCanvas (Variables|/Game/Inventory/InventoryUI/WBP_InventoryHUD.WBP_InventoryHUD_C|GetHUDCanvas (Variables|/Game/Player/BP_SpyPlayer_PLAYERCONTROLLER.BP_SpyPlayer_PLAYERCONTROLLER_C|GetHUDWidget _asbp_spy_player_playercontroller_4)) _output_get_2))
      (Class|CanvasPanelSlot|SetAutoSize _returnvalue_2 true)
      (Class|CanvasPanelSlot|SetPosition _returnvalue_2 (Variables|Default|GetInventoryPosition))
      (Input|SetInputModeGameandUI (Variables|Default|GetInteractorPC) 0 "LockAlways" true)
      (Variables|/Script/Engine.PlayerController|SetbShowMouseCursor (Variables|Default|GetInteractorPC) true))))

(fn AddtoInventory
  (params (ContentToAdd :type F%20Slot%20Structure%20Structure))
  (bind _inventorywindow (Variables|Widgets|GetInventoryWindow))
  (if (.stackable (.itemstructure ContentToAdd))
    (bind _stackindex (Utilities|HasPartialStack ContentToAdd)
      (:True
        (bind _success (CallFunction|AddtoStack ContentToAdd _stackindex))
        (LocalVariables|SetIsSuccessful _success))
      (:False
        (bind _success_2 (CallFunction|CreateStack ContentToAdd :!label _label))
        (LocalVariables|SetIsSuccessful _success_2)))
    (else
      (goto _label)))
  (CallFunction|GetTotalDetection)
  (Utilities|IsValid _inventorywindow
    (:Is%20Valid
      (for _array_element (Variables|/Game/Inventory/InventoryUI/WBP_InventoryWindow.WBP_InventoryWindow_C|GetinventorySlots _inventorywindow)
        (Default|RefreshSlot _array_element)
        (return (LocalVariables|GetIsSuccessful))))
    (:Is%20Not%20Valid
      (return (LocalVariables|GetIsSuccessful)))))

(fn PrepareInventory
  (Utilities|Array|Resize (Variables|Default|GetInventory) (Variables|Default|GetSlotCount))
  (for (_array_element _array_index) (Variables|Default|GetInventory)
    (if (!= (.Class (Utilities|Struct|BreakFItemStructure (.itemstructure _array_element))) 0)
      (Utilities|Array|SetArrayElem (Variables|Default|GetInventory) _array_index (Utilities|Struct|MakeFSlotStructure (.ItemStructure (Utilities|GetClassDefaults (.Class (Utilities|Struct|BreakFItemStructure (.itemstructure _array_element))))) (.quantity _array_element)))
      (bind _returnvalue (Game|SpawnActorfromClass (.Class (Utilities|Struct|BreakFItemStructure (.itemstructure _array_element))) (Math|Transform|MakeTransform "0, 0, 0") "Undefined" 0 0))
      (Default|OnPickup _returnvalue (Components|GetOwner))
      (Actor|DestroyActor _returnvalue)))
  (Variables|Default|SetOriginalInventory (Variables|Default|GetInventory)))

(fn CreateStack
  (params (ContentToAdd :type F%20Slot%20Structure%20Structure))
  (bind _inventory (Variables|Default|GetInventory))
  (bind (_array_element _array_index) (Utilities|Array|ForEachLoopwithBreak _inventory)
    (:LoopBody
      (if (<= (.Quantity (Utilities|Struct|BreakFSlotStructure _array_element)) 0) ; Check if there is an open slot
        (Utilities|Array|SetArrayElem _inventory _array_index ContentToAdd)
        (return true)))
    (:Completed
      (return false))))

(fn AddtoStack
  (params (SlotStructure :type F%20Slot%20Structure%20Structure) (SlotIndex :type Integer))
  (bind _inventory (Variables|Default|GetInventory))
  (bind _inventory_2 (Variables|Default|GetInventory))
  (bind _maxstacksize (Utilities|Struct|BreakFItemStructure (.itemstructure SlotStructure)))
  (bind _output (Utilities|Array|Get(acopy) _inventory SlotIndex))
  (bind _output_2 (Utilities|Array|Get(acopy) _inventory_2 SlotIndex))
  (bind _output_get (LocalVariables|SetCurrentQuantity (.quantity _output)))
  (if (> (+ _output_get (.Quantity (Utilities|Struct|BreakFSlotStructure SlotStructure))) (.maxstacksize (.itemstructure _output)))
    (Utilities|Array|SetArrayElem (Variables|Default|GetInventory) SlotIndex (Utilities|Struct|MakeFSlotStructure "(Name_7_313F0C1D422501D154A1FE9DB9F66E8F=NSLOCTEXT(\"[346FABB54D6CDFECF44F7B958AABD72B]\", \"D8D9C25F429DE0A8B71171B7C31453AE\", \"None\"),Description_9_4AD2F53549AD42913C4538A8D8BB6D19=NSLOCTEXT(\"[346FABB54D6CDFECF44F7B958AABD72B]\", \"55CCEB5D412A009EBBB5FB8F5DC7FF83\", \"N/a\"),Stackable_1_A9AE80A8469B17882D1758AEA799573E=True,MaxStackSize_4_7659C8E0481061CF0C75FFAD93E33772=4,Thumbnail_12_6F2306714B2F36A3EB2C71A5E1EC76D2=None,ItemType_29_551AF96C44B0A98E9433D9AD3C823ED5=NewEnumerator0,Class_21_73043DED4FF903F8CBE504864018F7B7=None,Consumable_23_9BFE81FE4D8A1167E817C69A28A319E2=False,DetectionRating_26_EB01ECDB47EAEC6EEA75D48566E78861=0.000000,Locked_28_0B8A2B4045125F33B4D575A9F314A4BA=False)" _maxstacksize))
    (CallFunction|AddtoInventory (Utilities|Struct|MakeFSlotStructure (.itemstructure SlotStructure) (- (.quantity SlotStructure) (- _maxstacksize (LocalVariables|GetCurrentQuantity)))))
    (else
      (Utilities|Array|SetArrayElem _inventory_2 SlotIndex (Utilities|Struct|MakeFSlotStructure (.itemstructure _output_2) (+ (.quantity _output_2) (.quantity SlotStructure))))))
  (return true))

(fn CheckItemType
  (params (ItemType :type EItemType%20Enum :default "NewEnumerator0"))
  (bind _array_element (Utilities|Array|ForEachLoopwithBreak (Variables|Default|GetInventory) :!label _label)
    (:LoopBody
      (if (== (.itemtype (.itemstructure _array_element)) ItemType)
        (LocalVariables|SetFound false)
        (goto _label Break)))
    (:Completed
      (return (LocalVariables|GetFound)))))

(fn GetTotalDetection
  (Variables|Default|SetTotalDetection 0.0)
  (for _array_element (Variables|Default|GetInventory)
    (Variables|Default|SetTotalDetection (+ (Variables|Default|GetTotalDetection) (.detectionrating (.itemstructure _array_element)))))
  (bind _asbp_player_character (Utilities|Casting|CastToBP_Player_CHARACTER (Game|GetPlayerCharacter 0)))
  (bind _output_get (Variables|/Game/Player/BP_Player_CHARACTER.BP_Player_CHARACTER_C|SetDetectionRating _asbp_player_character (Variables|Default|GetTotalDetection)))
  (return _output_get))

(fn CheckInventory
  (bind _originalinventory (Variables|Default|GetOriginalInventory))
  (if (Utilities|Array|Identical _originalinventory (Variables|Default|GetInventory)) ; If the inventory is the exact same as how it started
    (return "NewEnumerator3")
    (else
      (for (_array_element _array_index) _originalinventory
        (if (not (Utilities|Enum|Equal(Enum) (.name (.itemstructure _array_element)) (.name (.itemstructure (Utilities|Array|Get(acopy) (Variables|Default|GetInventory) _array_index))))) ; Checks each slot to see if the item is still there
          (if (< (LocalVariables|GetItemPriority) (.itemtype (.itemstructure _array_element)))
            (LocalVariables|SetItemPriority (.itemtype (.itemstructure _array_element))))))
      (return (LocalVariables|GetItemPriority)))))

(fn CheckItemClass
  (params (ItemClass :type BP%20Base%20Item%20Class%20Reference))
  (bind _array_element (Utilities|Array|ForEachLoopwithBreak (Variables|Default|GetInventory) :!label _label)
    (:LoopBody
      (if (== (.class (.itemstructure _array_element)) ItemClass)
        (LocalVariables|SetFound true)
        (goto _label Break)))
    (:Completed
      (return (LocalVariables|GetFound)))))

(fn ItemLockSwitch
  (params (ItemToLock :type F%20Slot%20Structure%20Structure) (SlotToLock :type Integer) (Lock :type Boolean))
  (bind (_itemstructure _quantity) (Utilities|Struct|BreakFSlotStructure ItemToLock))
  (Utilities|Array|SetArrayElem (Variables|Default|GetInventory) SlotToLock (Utilities|Struct|MakeFSlotStructure (Utilities|Struct|MakeFItemStructure (.name _itemstructure) (.description _itemstructure) (.stackable _itemstructure) (.maxstacksize _itemstructure) (.thumbnail _itemstructure) (.itemtype _itemstructure) (.class _itemstructure) (.consumable _itemstructure) (.detectionrating _itemstructure) Lock) _quantity)))