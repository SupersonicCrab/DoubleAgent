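; Interactable power box that switches the level's lights, cameras, tripwires, landlines and radios on or off.
; Overlapping its box shows an interact prompt in the player's text log; interacting opens PowerBox_HUD with mouse-only UI input.
; Per-system functions call every light switch, tripwire and landline actor, or the camera and radio hubs, and track state flags.
; CutPower sets a flag that blocks TurnAllPowerOn from restoring everything.
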(event OnComponentBeginOverlap(Box)
  (params (OverlappedComponent :type Primitive%20Component%20Object%20Reference) (OtherActor :type Actor%20Object%20Reference) (OtherComp :type Primitive%20Component%20Object%20Reference) (OtherBodyIndex :type Integer) (bFromSweep :type Boolean) (SweepResult :type Hit%20Result%20Structure%20%28by%20ref%29))
  ;[1 1 1] Display & remove text when player enters/leaves interaction box
  (bind _asplayer_character (Utilities|Casting|CastToPlayer_CHARACTER OtherActor))
  (bind _logid (Default|AddText (Variables|/Game/Player/Player_CHARACTER.Player_CHARACTER_C|GetTextLog _asplayer_character) "Press [E] to open the power box"))
  (if (not (== _logid 666))
    (Variables|Default|SetLogID _logid)))

(event OnComponentEndOverlap(Box)
  (params (OverlappedComponent :type Primitive%20Component%20Object%20Reference) (OtherActor :type Actor%20Object%20Reference) (OtherComp :type Primitive%20Component%20Object%20Reference) (OtherBodyIndex :type Integer))
  ;[1 1 1] Display & remove text when player enters/leaves interaction box
  (bind _asplayer_character (Utilities|Casting|CastToPlayer_CHARACTER OtherActor))
  (Default|RemoveText (Variables|/Game/Player/Player_CHARACTER.Player_CHARACTER_C|GetTextLog _asplayer_character) (Variables|Default|GetLogID)))

(event EventBeginPlay
  ;[1 1 1] Setup
  (bind _returnvalue (Actor|GetActorOfClass "/Game/AI/SecuritySystem/Cam_Output/CamHub_BP.CamHub_BP_C"))
  (Variables|Default|SetCameraHub _returnvalue))

(event EventInteract
  (params (Interactor :type Actor%20Object%20Reference))
  (bind _returnvalue (Game|GetPlayerController 0))
  ;[1 1 1] Interact
  (Utilities|Casting|CastToPlayer_CHARACTER Interactor)
  (bind _returnvalue_2 (UserInterface|CreateWidget "/Game/UI/PowerBox/PowerBox_HUD.PowerBox_HUD_C" _returnvalue))
  (UserInterface|Viewport|AddtoViewport _returnvalue_2 0)
  (Variables|/Script/Engine.PlayerController|SetbShowMouseCursor _returnvalue true)
  (Input|SetInputModeUIOnly _returnvalue _returnvalue_2 "LockAlways"))

(fn ConstructionScript)

(fn TurnLightson
  (Variables|Default|SetLightsOn true)
  (bind _outactors (Actor|GetAllActorsOfClass "/Game/PowerSystem/Lights/LightSwitch_BP.LightSwitch_BP_C"))
  (for _array_element _outactors
    (Variables|/Game/PowerSystem/Lights/LightSwitch_BP.LightSwitch_BP_C|SetPowerOn _array_element true)
    (Default|RestoreLights _array_element)))

(fn TurnLightsOff
  (Variables|Default|SetLightsOn false)
  (bind _outactors (Actor|GetAllActorsOfClass "/Game/PowerSystem/Lights/LightSwitch_BP.LightSwitch_BP_C"))
  (for _array_element _outactors
    (Default|DisableLightGroup _array_element true)
    (Variables|/Game/PowerSystem/Lights/LightSwitch_BP.LightSwitch_BP_C|SetPowerOn _array_element false)))

(fn TurnCamerasOff
  (Variables|Default|SetCamerasOn false)
  (Default|PowerDisabled (Variables|Default|GetCameraHub)))

(fn TurnCamerason
  (Variables|Default|SetCamerasOn true)
  (Default|PowerEnabled (Variables|Default|GetCameraHub)))

(fn TurnTripwiresOff
  (bind _outactors (Actor|GetAllActorsOfClass "/Game/AI/SecuritySystem/Tripwires/Tripwire_BP.Tripwire_BP_C"))
  (for _array_element _outactors
    (Default|DisableTripwire _array_element)
    (Variables|Default|SetTripwiresOn false)))

(fn TurnTripwireson
  (bind _outactors (Actor|GetAllActorsOfClass "/Game/AI/SecuritySystem/Tripwires/Tripwire_BP.Tripwire_BP_C"))
  (for _array_element _outactors
    (Default|EnableTripwire _array_element)
    (Variables|Default|SetTripwiresOn true)))

(fn TurnLandlineson
  (bind _outactors (Actor|GetAllActorsOfClass "/Game/AI/SecuritySystem/Landlines/Landline_BP.Landline_BP_C"))
  (for _array_element _outactors
    (Default|EnableLandline _array_element)
    (Variables|Default|SetLandlinesOn true)))

(fn TurnLandlinesOff
  (bind _outactors (Actor|GetAllActorsOfClass "/Game/AI/SecuritySystem/Landlines/Landline_BP.Landline_BP_C"))
  (for _array_element _outactors
    (Default|DisableLandline _array_element)
    (Variables|Default|SetLandlinesOn false)))

(fn CutPower
  (Variables|Default|SetPowerCut true))

(fn TurnRadioson
  (bind _returnvalue (Actor|GetActorOfClass "/Game/AI/SecuritySystem/Radio/RadioHub_BP.RadioHub_BP_C"))
  (Default|Poweron _returnvalue)
  (Variables|Default|SetRadiosOn true))

(fn TurnRadiosOff
  (bind _returnvalue (Actor|GetActorOfClass "/Game/AI/SecuritySystem/Radio/RadioHub_BP.RadioHub_BP_C"))
  (Default|PowerOff _returnvalue)
  (Variables|Default|SetRadiosOn false))

(fn TurnAllPoweron
  (if (Variables|Default|GetPowerCut)
    (return false)
    (else
      (CallFunction|TurnLightson)
      (CallFunction|TurnCamerason)
      (CallFunction|TurnLandlineson)
      (CallFunction|TurnTripwireson)
      (CallFunction|TurnRadioson)
      (bind _output_get (Variables|Default|SetLightsOn true))
      (bind _output_get_2 (Variables|Default|SetLandlinesOn _output_get))
      (bind _output_get_3 (Variables|Default|SetRadiosOn _output_get_2))
      (bind _output_get_4 (Variables|Default|SetCamerasOn _output_get_3))
      (bind _output_get_5 (Variables|Default|SetTripwiresOn _output_get_4))
      (return _output_get_5))))