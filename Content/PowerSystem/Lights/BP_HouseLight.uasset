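; BP_HouseLight is a switchable house point light tied to a Room, with TurnOn and TurnOff toggling its visibility.
; On BeginPlay, its collision sphere is sized to the light's attenuation radius.
; When an AI character enters the sphere while outside the Room and RoomLit is false, CheckNPC runs a debug-drawn Camera-channel line trace.
; If that trace hits the character directly, it passes the NPC to Room.UpdateNPC.
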(event OnComponentBeginOverlap(Collision)
  (params (OverlappedComponent :type Primitive%20Component%20Object%20Reference) (OtherActor :type Actor%20Object%20Reference) (OtherComp :type Primitive%20Component%20Object%20Reference) (OtherBodyIndex :type Integer) (bFromSweep :type Boolean) (SweepResult :type Hit%20Result%20Structure%20%28by%20ref%29))
  (bind _room (Variables|Default|GetRoom))
  (if (Math|Boolean|ANDBoolean (Utilities|ClassIsChildOf (Utilities|GetClass OtherActor) "/Game/AI/NPC/BP_AICharacterBase_CHARACTER.BP_AICharacterBase_CHARACTER_C") (not (Collision|IsOverlappingActor _room OtherActor :!class /Script/Engine.Actor)) (not (Variables|/Script/ProjectSpy.RoomVolume|GetbRoomLit _room)))
    (CallFunction|CheckNPC OtherActor)))

(event EventBeginPlay
  (Components|Sphere|SetSphereRadius (Variables|Default|GetCollision) (Variables|/Script/Engine.LocalLightComponent|GetAttenuationRadius (Variables|Default|GetPointLight)) true))

(fn ConstructionScript)

(fn TurnOff
  (Rendering|SetVisibility (Variables|Default|GetPointLight) false false))

(fn Turnon
  (Rendering|SetVisibility (Variables|Default|GetPointLight) true false))

(fn CheckNPC
  (params (NPC :type Actor%20Object%20Reference))
  (bind _outhit (Collision|LineTraceByChannel (Transformation|GetActorLocation) (Transformation|GetActorLocation NPC) "TraceTypeQuery2" false 0 "ForDuration"))
  (if (== (.HitActor (Collision|BreakHitResult _outhit)) NPC)
    (Class|RoomVolume|UpdateNPC (Variables|Default|GetRoom) NPC)))