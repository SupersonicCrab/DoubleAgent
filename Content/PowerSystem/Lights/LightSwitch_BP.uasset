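; Interactable light switch that toggles all house lights sharing its LightGroup, provided the power box has power.
; On BeginPlay it registers with its Room, reads the power state and gathers matching lights, while box overlap shows an on/off prompt.
; Toggling updates the Room and has lights re-check overlapping AI characters, skipping those inside the room bounds when switching on.
; Power box shutoffs preserve the switch state so RestoreLights can reapply it.
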(event OnComponentBeginOverlap(Box)
  (params (OverlappedComponent :type Primitive%20Component%20Object%20Reference) (OtherActor :type Actor%20Object%20Reference) (OtherComp :type Primitive%20Component%20Object%20Reference) (OtherBodyIndex :type Integer) (bFromSweep :type Boolean) (SweepResult :type Hit%20Result%20Structure%20%28by%20ref%29))
  ;[1 1 1] Set interaction text
  (bind _asplayer_character (Utilities|Casting|CastToPlayer_CHARACTER OtherActor))
  (if (Variables|Default|GetLightGroupOn)
    (Variables|Default|SetInteractText "Press [E] to turn lights off")
    (else
      (Variables|Default|SetInteractText "Press [E] to turn lights on")))
  (bind _logid (Default|AddText (Variables|/Game/Player/Player_CHARACTER.Player_CHARACTER_C|GettextLog _asplayer_character) (Variables|Default|GetInteractText)))
  (if (not (== _logid 666))
    (Variables|Default|SetLogID _logid)))

(event OnComponentEndOverlap(Box)
  (params (OverlappedComponent :type Primitive%20Component%20Object%20Reference) (OtherActor :type Actor%20Object%20Reference) (OtherComp :type Primitive%20Component%20Object%20Reference) (OtherBodyIndex :type Integer))
  ;[1 1 1] Set interaction text
  (bind _asplayer_character (Utilities|Casting|CastToPlayer_CHARACTER OtherActor))
  (Default|RemoveText (Variables|/Game/Player/Player_CHARACTER.Player_CHARACTER_C|GettextLog _asplayer_character) (Variables|Default|GetLogID)))

(event EventBeginPlay
  ;[1 1 1] Setup
  (Variables|/Game/RoomSystem/RoomVolume_BP.RoomVolume_BP_C|SetlightSwitch (Variables|Default|GetRoom) self)
  (bind _returnvalue (Actor|GetActorOfClass "/Game/PowerSystem/PowerBox_BP.PowerBox_BP_C"))
  (bind _output_get (Variables|Default|SetPowerBox _returnvalue))
  (Variables|Default|SetPowerOn (Variables|/Game/PowerSystem/PowerBox_BP.PowerBox_BP_C|GetLightsOn _output_get))
  (bind _outactors (Actor|GetAllActorsOfClass "/Game/PowerSystem/Lights/HouseLight_BP.HouseLight_BP_C"))
  (for _array_element _outactors
    (if (== (Variables|/Game/PowerSystem/Lights/HouseLight_BP.HouseLight_BP_C|GetLightGroup _array_element) (Variables|Default|GetLightGroup))
      (Utilities|Array|Add (Variables|Default|GetGroupLights) _array_element)
      (Variables|/Game/PowerSystem/Lights/HouseLight_BP.HouseLight_BP_C|SetRoom _array_element (Variables|Default|GetRoom)))))

(event EventInteract
  (params (Interactor :type Actor%20Object%20Reference))
  ;[1 1 1] Toggle lights on & off
  (if (Variables|Default|GetPowerOn)
    (if (Variables|Default|GetLightGroupOn)
      (CallFunction|DisableLightGroup false)
      (Variables|Default|SetLightGroupOn false)
      (else
        (CallFunction|EnableLightGroup)
        (Variables|Default|SetLightGroupOn true)))
    (else
      (Development|PrintString "Power is off"))))

(fn ConstructionScript)

(fn EnableLightGroup
  (bind _room (Variables|Default|GetRoom))
  (for _array_element (Variables|Default|GetGroupLights)
    (Default|Turnon _array_element))
  (bind _output_get (Variables|Default|SetLightGroupOn true))
  (Default|LightUpdate _room _output_get)
  (for _array_element_2 (Variables|Default|GetGroupLights)
    (for _array_element_3 (Collision|GetOverlappingActors (Variables|/Game/PowerSystem/Lights/HouseLight_BP.HouseLight_BP_C|GetCollision _array_element_2) "/Game/AI/NPC/AICharacterBase_CHARACTER.AICharacterBase_CHARACTER_C" :!class /Script/Engine.PrimitiveComponent)
      (if (not (Collision|IsOverlappingActor (Variables|/Game/RoomSystem/RoomVolume_BP.RoomVolume_BP_C|GetRoomBoundingBox _room) _array_element_3 :!class /Script/Engine.PrimitiveComponent))
        (Default|CheckNPC _array_element_2 _array_element_3)))))

(fn DisableLightGroup
  (params (FromPowerBox :type Boolean))
  (for _array_element (Variables|Default|GetGroupLights)
    (Default|TurnOff _array_element))
  (if FromPowerBox
    _
    (else
      (Variables|Default|SetLightGroupOn false)))
  (Default|LightUpdate (Variables|Default|GetRoom) false)
  (for _array_element_2 (Variables|Default|GetGroupLights)
    (for _array_element_3 (Collision|GetOverlappingActors (Variables|/Game/PowerSystem/Lights/HouseLight_BP.HouseLight_BP_C|GetCollision _array_element_2) "/Game/AI/NPC/AICharacterBase_CHARACTER.AICharacterBase_CHARACTER_C" :!class /Script/Engine.PrimitiveComponent)
      (Default|CheckNPC _array_element_2 _array_element_3))))

(fn RestoreLights
  (if (Variables|Default|GetLightGroupOn)
    (CallFunction|EnableLightGroup)
    (else
      (CallFunction|DisableLightGroup false))))