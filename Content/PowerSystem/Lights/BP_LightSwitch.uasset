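; BP_LightSwitch is an interactable switch that toggles a group of house lights in a room while power is on.
; On BeginPlay it registers with its Room, reads the BP_PowerBox state and gathers BP_HouseLights sharing its LightGroup.
; Box overlap shows or removes the player's prompt.
; Toggling updates the Room and has lights recheck overlapping NPCs; power-box shutoffs can preserve switch state for RestoreLights.
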(event OnComponentBeginOverlap(Box)
  (params (OverlappedComponent :type Primitive%20Component%20Object%20Reference) (OtherActor :type Actor%20Object%20Reference) (OtherComp :type Primitive%20Component%20Object%20Reference) (OtherBodyIndex :type Integer) (bFromSweep :type Boolean) (SweepResult :type Hit%20Result%20Structure%20%28by%20ref%29))
  ;[1 1 1] Set interaction text
  (bind _asbp_player_character (Utilities|Casting|CastToBP_Player_CHARACTER OtherActor))
  (if (Variables|Default|GetbLightGroupOn)
    (Variables|Default|SetInteractText "Press [E] to turn lights off")
    (else
      (Variables|Default|SetInteractText "Press [E] to turn lights on")))
  (bind _logid (Default|AddText (Variables|/Game/Player/BP_Player_CHARACTER.BP_Player_CHARACTER_C|GetTextLog _asbp_player_character) (Variables|Default|GetInteractText)))
  (if (not (== _logid 666))
    (Variables|Default|SetLogID _logid)))

(event OnComponentEndOverlap(Box)
  (params (OverlappedComponent :type Primitive%20Component%20Object%20Reference) (OtherActor :type Actor%20Object%20Reference) (OtherComp :type Primitive%20Component%20Object%20Reference) (OtherBodyIndex :type Integer))
  ;[1 1 1] Set interaction text
  (bind _asbp_player_character (Utilities|Casting|CastToBP_Player_CHARACTER OtherActor))
  (Default|RemoveText (Variables|/Game/Player/BP_Player_CHARACTER.BP_Player_CHARACTER_C|GetTextLog _asbp_player_character) (Variables|Default|GetLogID)))

(event EventBeginPlay
  ;[1 1 1] Setup
  (Variables|/Script/ProjectSpy.RoomVolume_BP_CPP|SetlightSwitch (Variables|Default|GetRoom) self)
  (bind _returnvalue (Actor|GetActorOfClass "/Game/PowerSystem/BP_PowerBox.BP_PowerBox_C"))
  (bind _output_get (Variables|Default|SetPowerBox _returnvalue))
  (Variables|Default|SetbPowerOn (Variables|/Game/PowerSystem/BP_PowerBox.BP_PowerBox_C|GetbLightsOn _output_get))
  (bind _outactors (Actor|GetAllActorsOfClass "/Game/PowerSystem/Lights/BP_HouseLight.BP_HouseLight_C"))
  (for _array_element _outactors
    (if (== (Variables|/Game/PowerSystem/Lights/BP_HouseLight.BP_HouseLight_C|GetLightGroup _array_element) (Variables|Default|GetLightGroup))
      (Utilities|Array|Add (Variables|Default|GetGroupLights) _array_element)
      (Variables|/Game/PowerSystem/Lights/BP_HouseLight.BP_HouseLight_C|SetRoom _array_element (Variables|Default|GetRoom)))))

(event EventInteract
  (params (Interactor :type Actor%20Object%20Reference))
  ;[1 1 1] Toggle lights on & off
  (if (Variables|Default|GetbPowerOn)
    (if (Variables|Default|GetbLightGroupOn)
      (CallFunction|DisableLightGroup false)
      (Variables|Default|SetbLightGroupOn false)
      (else
        (CallFunction|EnableLightGroup)
        (Variables|Default|SetbLightGroupOn true)))
    (else
      (Development|PrintString "Power is off"))))

(fn ConstructionScript)

(fn EnableLightGroup
  (bind _room (Variables|Default|GetRoom))
  (for _array_element (Variables|Default|GetGroupLights)
    (Default|Turnon _array_element))
  (bind _output_get (Variables|Default|SetbLightGroupOn true))
  (Class|RoomVolumeBPCPP|UpdateLight _room _output_get)
  (for _array_element_2 (Variables|Default|GetGroupLights)
    (for _array_element_3 (Collision|GetOverlappingActors (Variables|/Game/PowerSystem/Lights/BP_HouseLight.BP_HouseLight_C|GetCollision _array_element_2) "/Game/AI/NPC/BP_AICharacterBase_CHARACTER.BP_AICharacterBase_CHARACTER_C" :!class /Script/Engine.PrimitiveComponent)
      (if (Collision|IsOverlappingActor _room _array_element_3 :!class /Script/Engine.Actor)
        (Default|CheckNPC _array_element_2 _array_element_3)))))

(fn DisableLightGroup
  (params (FromPowerBox :type Boolean))
  (for _array_element (Variables|Default|GetGroupLights)
    (Default|TurnOff _array_element))
  (if FromPowerBox
    _
    (else
      (Variables|Default|SetbLightGroupOn false)))
  (Class|RoomVolumeBPCPP|UpdateLight (Variables|Default|GetRoom) false)
  (for _array_element_2 (Variables|Default|GetGroupLights)
    (for _array_element_3 (Collision|GetOverlappingActors (Variables|/Game/PowerSystem/Lights/BP_HouseLight.BP_HouseLight_C|GetCollision _array_element_2) "/Game/AI/NPC/BP_AICharacterBase_CHARACTER.BP_AICharacterBase_CHARACTER_C" :!class /Script/Engine.PrimitiveComponent)
      (Default|CheckNPC _array_element_2 _array_element_3))))

(fn RestoreLights
  (if (Variables|Default|GetbLightGroupOn)
    (CallFunction|EnableLightGroup)
    (else
      (CallFunction|DisableLightGroup false))))