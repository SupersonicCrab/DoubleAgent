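; BP_PowerBox is an interactable power box that opens the WBP_PowerBox widget for the local player, switching to cursor and UI-only input.
; A player entering its collision triggers PerformIllegalAction and plays the DoorOpen timeline; leaving clears IllegalAction and reverses it, unless already playing.
; Custom depth stencil on box and door provides the outline, and getters supply prompt text and center.
; Older context-menu prompt logic remains disconnected.
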(event OnComponentBeginOverlap(Collision)
  (params (OverlappedComponent :type Primitive%20Component%20Object%20Reference) (OtherActor :type Actor%20Object%20Reference) (OtherComp :type Primitive%20Component%20Object%20Reference) (OtherBodyIndex :type Integer) (bFromSweep :type Boolean) (SweepResult :type Hit%20Result%20Structure%20%28by%20ref%29))
  (bind _dooropen (Variables|Default|GetDoorOpen))
  ;[1 1 1] Display & remove text when player enters/leaves interaction box
  (bind _asbp_player_character (Utilities|Casting|CastToBP_Player_CHARACTER OtherActor))
  (Class|PlayerCharacter|PerformIllegalAction _asbp_player_character 0.0)
  (if (not (Audio|Components|Audio|IsPlaying _dooropen))
    (Components|Timeline|PlayfromStart _dooropen)))

(event OnComponentEndOverlap(Collision)
  (params (OverlappedComponent :type Primitive%20Component%20Object%20Reference) (OtherActor :type Actor%20Object%20Reference) (OtherComp :type Primitive%20Component%20Object%20Reference) (OtherBodyIndex :type Integer))
  (bind _dooropen (Variables|Default|GetDoorOpen))
  ;[1 1 1] Display & remove text when player enters/leaves interaction box
  (bind _asbp_player_character (Utilities|Casting|CastToBP_Player_CHARACTER OtherActor))
  (Variables|/Script/DoubleAgent.Player_Character|SetbIllegalAction _asbp_player_character false)
  (if (not (Audio|Components|Audio|IsPlaying _dooropen))
    (Components|Timeline|ReversefromEnd _dooropen)))

(event EventDisableOutline
  (bind _staticmesh (Variables|Components|GetStaticMesh))
  (bind _door (Variables|Default|GetDoor))
  (Rendering|SetRenderCustomDepth _staticmesh false)
  (Rendering|SetRenderCustomDepth _door false)
  (Rendering|SetCustomDepthStencilValue _staticmesh 0)
  (Rendering|SetCustomDepthStencilValue _door 0))

(event EventEnableOutline
  (bind _staticmesh (Variables|Components|GetStaticMesh))
  (bind _door (Variables|Default|GetDoor))
  (Rendering|SetRenderCustomDepth _staticmesh true)
  (Rendering|SetRenderCustomDepth _door true)
  (Rendering|SetCustomDepthStencilValue _staticmesh 254)
  (Rendering|SetCustomDepthStencilValue _door 254))

(event EventInteract
  (params (Interactor :type Actor%20Object%20Reference))
  ;[1 1 1] Interact
  (bind _asbp_player_character (Utilities|Casting|CastToBP_Player_CHARACTER Interactor))
  (bind _asplayer_controller (Utilities|Casting|CastToPlayerController (Pawn|GetController _asbp_player_character)))
  (if (Pawn|IsLocalController _asplayer_controller)
    (bind _returnvalue (UserInterface|CreateWidget "/Game/UI/PowerBox/WBP_PowerBox.WBP_PowerBox_C" _asplayer_controller))
    (UserInterface|Viewport|AddtoViewport _returnvalue 0)
    (Variables|/Script/Engine.PlayerController|SetbShowMouseCursor _asplayer_controller true)
    (Input|SetInputModeUIOnly _asplayer_controller _returnvalue "LockAlways")))

(fn ConstructionScript)

(fn GetCenter
  (return (.Origin (Collision|GetComponentBounds (Variables|Components|GetStaticMesh)))))

(fn GetInteractText
  (return "Open power box"))