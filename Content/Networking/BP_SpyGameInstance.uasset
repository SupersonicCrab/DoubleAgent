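; Game instance for the spy game that runs two-player online sessions and owns the player's options.
; Hosts an advanced session and, on an accepted invite, joins it and client-travels to the current level name.
; Settings load from and save to an options slot, with defaults built at Init.
; UpdateSettings pushes each category into console commands, VCA volumes, remapped inputs, the player character and colorblind correction.
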(event Custom|StorePlayerInfo
  (params (PlayerInfo :type Array%20of%20S%20Player%20Info%20Structures))
  (Variables|Default|SetPlayerInfo PlayerInfo))

(event Custom|UpdateSettings
  (params (SettingsSave :type BP%20Game%20Settings%20Object%20Reference))
  ;[1 1 1] Update the settings for each of the settings categories
  (CallFunction|UpdateGraphicSettings (Variables|/Game/Player/Settings/BP_GameSettings.BP_GameSettings_C|GetGraphicSettings SettingsSave))
  (CallFunction|UpdateAudioSettings (Variables|/Game/Player/Settings/BP_GameSettings.BP_GameSettings_C|GetAudioSettings SettingsSave))
  (CallFunction|UpdateControlSettings (Variables|/Game/Player/Settings/BP_GameSettings.BP_GameSettings_C|GetControlSettings SettingsSave))
  (CallFunction|UpdateGameplaySettings (Variables|/Game/Player/Settings/BP_GameSettings.BP_GameSettings_C|GetGameplaySettings SettingsSave))
  (CallFunction|UpdateAccessibilitySettings (Variables|/Game/Player/Settings/BP_GameSettings.BP_GameSettings_C|GetAccessibilitySettings SettingsSave)))

(event Custom|TravelClient
  ;[1 1 1] Move client to session
  (bind _returnvalue (Game|GetCurrentLevelName true))
  (Development|ExecuteConsoleCommand (Utilities|String|Append "clienttravel " _returnvalue) 0)
  (Development|PrintString "Traveled client"))

(event Custom|HostGame
  (params (PlayerHost :type Player%20Controller%20Object%20Reference))
  ;[1 1 1] Host game
  (bind _output_get (Variables|Default|SetHostController PlayerHost))
  (|AdvancedSession 0 _output_get 2 0 false true false true true true false false false
    (:OnSuccess
      (Development|PrintString "Session created successfully")
      (Development|ExecuteConsoleCommand "NetProfile Enable" 0))
    (:OnFailure
      (Development|PrintString "Failed to create session"))))

(event EventInit
  (|CallParentFunction)
  (bind _returnvalue (SaveGame|CreateSaveGameObject "/Game/Player/Settings/BP_GameSettings.BP_GameSettings_C"))
  (Variables|Default|SetDefaultSettings _returnvalue)
  (Variables|/Game/Player/Settings/BP_GameSettings.BP_GameSettings_C|SetGameplaySettings (Variables|Default|GetDefaultSettings) (Utilities|Struct|MakeFGameplaySettingsNew true false false false true false))
  (Variables|/Game/Player/Settings/BP_GameSettings.BP_GameSettings_C|SetAudioSettings (Variables|Default|GetDefaultSettings) (Utilities|Struct|MakeFAudioSettingsNew 1.0 1.0 1.0 0.4 1.0 false false))
  (Variables|/Game/Player/Settings/BP_GameSettings.BP_GameSettings_C|SetGraphicSettings (Variables|Default|GetDefaultSettings) (Utilities|Struct|MakeFGraphicsSettingsNew 100 0.5 2 1 1 1 1 1))
  (Variables|/Game/Player/Settings/BP_GameSettings.BP_GameSettings_C|SetControlSettings (Variables|Default|GetDefaultSettings) (Utilities|Struct|MakeFControlSettings "F" "E" "LeftControl" "W" "S" "A" "D" "LeftAlt" "Tab" "LeftMouseButton" "RightMouseButton" "LeftMouseButton" "RightMouseButton" "H" "C" "G" "X" "B" 2.5)))

(event EventOnSessionInviteAccepted
  (params (LocalPlayerNum :type Integer) (PersonInvited :type BP%20Unique%20Net%20Id%20Structure) (SessionToJoin :type Blueprint%20Session%20Result%20Structure%20%28by%20ref%29))
  (bind _returnvalue (Game|GetPlayerController 0))
  ;[1 1 1] Join game
  (Development|PrintString "Accepted invite")
  (Variables|Default|SetJoinedSession SessionToJoin)
  (|DestroySession _returnvalue
    (:OnSuccess
      _)
    (:OnFailure
      _))
  (|JoinSession _returnvalue SessionToJoin
    (:OnSuccess
      (Development|PrintString "Joined session")
      (bind _returnvalue_2 (Game|GetCurrentLevelName true))
      (Development|ExecuteConsoleCommand (Utilities|String|Append "clienttravel  " _returnvalue_2) 0)
      (Development|ExecuteConsoleCommand "p.NetEnableMoveCombining 0" 0))
    (:OnFailure
      (Development|PrintString "Joining failed"))))

(fn UpdateGraphicSettings
  (params (NewSettings :type F%20Graphics%20Settings%20New%20Structure))
  (bind (_resolutionscale _viewdistance _antialiasing _postprocessing _shadowquality _texturequality _effectsquality _foliagequality) (Utilities|Struct|BreakFGraphicsSettingsNew NewSettings))
  (Development|ExecuteConsoleCommand (Utilities|String|Append "r.ScreenPercentage " (Utilities|String|ToString(Integer) _resolutionscale)) 0)
  (Development|ExecuteConsoleCommand (Utilities|String|Append "r.ViewDistanceScale " (Utilities|String|ToString(Float) _viewdistance)) 0)
  (Development|ExecuteConsoleCommand (Utilities|String|Append "r.PostProcessAAQuality " (Utilities|String|ToString(Integer) _antialiasing)) 0)
  (Development|ExecuteConsoleCommand (Utilities|String|Append "r.PostProcessQuality " (Utilities|String|ToString(Integer) _postprocessing)) 0)
  (Development|ExecuteConsoleCommand (Utilities|String|Append "sg.ShadowQuality " (Utilities|String|ToString(Integer) _shadowquality)) 0)
  (Development|ExecuteConsoleCommand (Utilities|String|Append "sg.TextureQuality " (Utilities|String|ToString(Integer) _texturequality)) 0)
  (Development|ExecuteConsoleCommand (Utilities|String|Append "sg.EffectsQuality " (Utilities|String|ToString(Integer) _effectsquality)) 0)
  (Development|ExecuteConsoleCommand (Utilities|String|Append "FoliageQuality " (Utilities|String|ToString(Integer) _foliagequality)) 0))

(fn UpdateAudioSettings
  (params (NewSettings :type F%20Audio%20Settings%20New%20Structure))
  (bind (_effectsvolume _voicevolume _uivolume _musicvolume _mastervolume _censormode _subtitlesenabled) (Utilities|Struct|BreakFAudioSettingsNew NewSettings))
  (Class|SpyGameInstance|UpdateVCA _effectsvolume 1)
  (Class|SpyGameInstance|UpdateVCA _musicvolume 2)
  (Class|SpyGameInstance|UpdateVCA _uivolume 3)
  (Class|SpyGameInstance|UpdateVCA _voicevolume 4)
  (Class|SpyGameInstance|UpdateVCA _mastervolume 5)
  (Class|SpyGameInstance|UpdateVCas)
  (Variables|Default|SetbCensorMode _censormode)
  (Variables|Default|SetbSubtitlesEnabled _subtitlesenabled)
  (bind _asbp_spy_player_playercontroller (Utilities|Casting|CastToBP_SpyPlayer_PLAYERCONTROLLER (Game|GetPlayerController 0)))
  (Default|UpdateSubtitleDisplay _asbp_spy_player_playercontroller (Variables|Default|GetbSubtitlesEnabled)))

(fn UpdateControlSettings
  (params (NewSettings :type F%20Control%20Settings%20Structure))
  (bind (_takedown _interact _crouch _forward _backward _leftstrafe _rightstrafe _walk _openinventory _useequippeditem _useequippeditemsecondary _itemequip _itemdrop _togglehud _cameraswitch _godmode _objectives _hideplayer _mousesensitivity) (Utilities|Struct|BreakFControlSettings NewSettings))
  (bind _returnvalue (Game|GetPlayerController 0))
  (CallFunction|UpdateInput "Takedown" "Action" _takedown 0.0 false)
  (CallFunction|UpdateInput "Interact" "Action" _interact 0.0 false)
  (CallFunction|UpdateInput "Crouch" "Action" _crouch 0.0 false)
  (CallFunction|UpdateInput "MoveForward" "Axis" _forward 1.0 false)
  (CallFunction|UpdateInput "MoveForward" "Axis" _backward -1.0 true)
  (CallFunction|UpdateInput "MoveRight" "Axis" _leftstrafe -1.0 false)
  (CallFunction|UpdateInput "MoveRight" "Axis" _rightstrafe 1.0 true)
  (CallFunction|UpdateInput "Walk" "Action" _walk 1.0 false)
  (CallFunction|UpdateInput "Inventory" "Action" _openinventory 1.0 false)
  (CallFunction|UpdateInput "Primary Use Item" "Action" _useequippeditem 1.0 false)
  (CallFunction|UpdateInput "Alternate Use Item" "Action" _useequippeditemsecondary 1.0 false)
  (CallFunction|UpdateInput "ItemEquip" "Action" _itemequip 1.0 false)
  (CallFunction|UpdateInput "ItemDrop" "Action" _itemdrop 1.0 false)
  (CallFunction|UpdateInput "CameraSwitch" "Action" _cameraswitch 1.0 false)
  (CallFunction|UpdateInput "ToggleHUD" "Action" _togglehud 1.0 false)
  (CallFunction|UpdateInput "HideToNPC" "Action" _hideplayer 1.0 false)
  (CallFunction|UpdateInput "GodModeToggle" "Action" _godmode 1.0 false)
  (CallFunction|UpdateInput "Objectives" "Action" _objectives 1.0 false)
  (Variables|/Script/Engine.PlayerController|SetInputPitchScale _returnvalue (* -1 _mousesensitivity))
  (Variables|/Script/Engine.PlayerController|SetInputYawScale _returnvalue _mousesensitivity))

(fn UpdateGameplaySettings
  (params (NewSettings :type F%20Gameplay%20Settings%20New%20Structure))
  (bind (_togglewalk _togglerun _togglecrouch _cheatsenabled _toggleaim _autoequip) (Utilities|Struct|BreakFGameplaySettingsNew NewSettings))
  (bind _returnvalue (Game|Player|GetPlayerPawn 0))
  (Utilities|IsValid _returnvalue
    (:Is%20Valid
      (bind _asbp_player_character (Utilities|Casting|CastToBP_Player_CHARACTER _returnvalue))
      (Variables|/Game/Player/BP_Player_CHARACTER.BP_Player_CHARACTER_C|SetGameplaySettings _asbp_player_character (Utilities|Struct|MakeFGameplaySettingsNew _togglewalk _togglerun _togglecrouch _cheatsenabled _toggleaim _autoequip)))))

(fn UpdateAccessibilitySettings
  (params (NewSettings :type F%20Accessibility%20Settings%20New%20Structure))
  (bind (_captioningenabled _outlineinteractableitems _colorblindtype _colorblindseverity _hearingimpairedsoundassist _staffoutline _regularoutline) (Utilities|Struct|BreakFAccessibilitySettingsNew NewSettings))
  (switch int _colorblindtype
    (:Default
      (LocalVariables|SetType "NormalVision" :!label _label))
    (:0
      (goto _label))
    (:1
      (LocalVariables|SetType "Deuteranope"))
    (:2
      (LocalVariables|SetType "Protanope"))
    (:3
      (LocalVariables|SetType "Tritanope")))
  (Class|WidgetBlueprintLibrary|SetColorVisionDeficiencyType (LocalVariables|GetType) _colorblindseverity true)
  (bind _asbp_player_character (Utilities|Casting|CastToBP_Player_CHARACTER (Game|Player|GetPlayerPawn 0)))
  (Default|SetupOutline _asbp_player_character _outlineinteractableitems _staffoutline _regularoutline))

(fn UpdateInput
  (params (InputName :type Name) (AxisOrAction :type String) (Key :type Key%20Structure :default "None") (Scale :type Float%20%28single-precision%29) (SecondAxis :type Boolean))
  (bind _returnvalue (Class|InputSettings|GetInputSettings))
  (bind _outmappings (Class|InputSettings|GetActionMappingbyName _returnvalue InputName))
  (switch string AxisOrAction
    (:Axis
      (if SecondAxis ; If true, this is the second axis so  do not remove any axis mappings
        _
        (else
          (Class|InputSettings|RemoveAxisMapping _returnvalue (Utilities|Array|Get(acopy) (Class|InputSettings|GetAxisMappingbyName _returnvalue InputName)) true)))
      (Class|InputSettings|AddAxisMapping _returnvalue (Utilities|Struct|MakeInputAxisKeyMapping InputName Scale Key) true))
    (:Action
      (if (Utilities|Array|IsValidIndex _outmappings)
        (Class|InputSettings|RemoveActionMapping _returnvalue (Utilities|Array|Get(acopy) _outmappings) true)
        (Class|InputSettings|AddActionMapping _returnvalue (Utilities|Struct|MakeInputActionKeyMapping InputName false false false false Key) true)))))

(fn LoadSettings
  (bind _returnvalue (SaveGame|DoesSaveGameExist (LocalVariables|GetOptionsSlot)))
  (if _returnvalue
    (bind _returnvalue_2 (SaveGame|LoadGamefromSlot (LocalVariables|GetOptionsSlot)))
    (bind _asbp_game_settings (Utilities|Casting|CastToBP_GameSettings _returnvalue_2))
    (Variables|Default|SetOptionsSaveReference _asbp_game_settings)
    (else
      ;[1 1 1] If no options save exists, create one with default settings
      (bind _returnvalue_3 (SaveGame|CreateSaveGameObject "/Game/Player/Settings/BP_GameSettings.BP_GameSettings_C"))
      (bind _output_get (Variables|Default|SetOptionsSaveReference _returnvalue_3))
      (SaveGame|SaveGametoSlot _output_get (LocalVariables|GetOptionsSlot))))
  (return (Variables|Default|GetOptionsSaveReference)))

(fn SaveSettings
  (params (GraphicsSettings :type F%20Graphics%20Settings%20New%20Structure) (AudioSettings :type F%20Audio%20Settings%20New%20Structure) (ControlSettings :type F%20Control%20Settings%20Structure) (GameplaySettings :type F%20Gameplay%20Settings%20New%20Structure) (AccessibilitySettings :type F%20Accessibility%20Settings%20New%20Structure))
  (bind _returnvalue (SaveGame|DoesSaveGameExist (LocalVariables|GetOptionsSlot)))
  (if _returnvalue
    _
    (else
      ;[1 1 1] If no options save exists, create one and apply settings
      (bind _returnvalue_2 (SaveGame|CreateSaveGameObject "/Game/Player/Settings/BP_GameSettings.BP_GameSettings_C"))
      (Variables|Default|SetOptionsSaveReference _returnvalue_2)))
  (Variables|/Game/Player/Settings/BP_GameSettings.BP_GameSettings_C|SetGraphicSettings (Variables|Default|GetOptionsSaveReference) GraphicsSettings)
  (Variables|/Game/Player/Settings/BP_GameSettings.BP_GameSettings_C|SetAudioSettings (Variables|Default|GetOptionsSaveReference) AudioSettings)
  (Variables|/Game/Player/Settings/BP_GameSettings.BP_GameSettings_C|SetControlSettings (Variables|Default|GetOptionsSaveReference) ControlSettings)
  (Variables|/Game/Player/Settings/BP_GameSettings.BP_GameSettings_C|SetGameplaySettings (Variables|Default|GetOptionsSaveReference) GameplaySettings)
  (Variables|/Game/Player/Settings/BP_GameSettings.BP_GameSettings_C|SetAccessibilitySettings (Variables|Default|GetOptionsSaveReference) AccessibilitySettings)
  (SaveGame|SaveGametoSlot (Variables|Default|GetOptionsSaveReference) (LocalVariables|GetOptionsSlot))
  (CallFunction|UpdateSettings (Variables|Default|GetOptionsSaveReference)))

(fn SetDefaults
  (CallFunction|UpdateSettings (Variables|Default|GetDefaultSettings)))

(fn SetInfo
  (bind _returnvalue (Game|GetPlayerController 0))
  (bind _uniquenetid (Class|AdvancedSessionsLibrary|GetUniqueNetID _returnvalue))
  (Class|AdvancedSteamFriendsLibrary|GetSteamFriendAvatar _uniquenetid "SteamAvatar_Large"
    (:OnSuccess
      _)
    (:AsyncLoading
      _)
    (:OnFailure
      (Development|PrintString "Failed to get info for some reason")
      (return "")))
  (return (Utilities|Struct|MakeSPlayerInfo (Class|AdvancedSessionsLibrary|GetPlayerName _returnvalue) 0 _uniquenetid 0 "Not Ready" 0)))