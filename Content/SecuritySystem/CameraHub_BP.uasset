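; Security camera hub that controls every Camera_BP in the level as part of the security system.
; On BeginPlay it gathers the cameras and pairs each by index with a render target for an initial scene capture.
; Player overlap turns live capture on while powered and off on exit.
; Power and perception functions fan out to all cameras, with perception also linking the operator NPC's AI controller.
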(event OnComponentBeginOverlap(PlayerCollision)
  (params (OverlappedComponent :type Primitive%20Component%20Object%20Reference) (OtherActor :type Actor%20Object%20Reference) (OtherComp :type Primitive%20Component%20Object%20Reference) (OtherBodyIndex :type Integer) (bFromSweep :type Boolean) (SweepResult :type Hit%20Result%20Structure%20%28by%20ref%29))
  ;[1 1 1] Player collision handling
  (if (== (Utilities|GetClass OtherActor) "/Game/Player/Player_CHARACTER.Player_CHARACTER_C")
    (if (Variables|Default|GetpowerOn)
      (SceneCapture|EnableCapture))))

(event OnComponentEndOverlap(PlayerCollision)
  (params (OverlappedComponent :type Primitive%20Component%20Object%20Reference) (OtherActor :type Actor%20Object%20Reference) (OtherComp :type Primitive%20Component%20Object%20Reference) (OtherBodyIndex :type Integer))
  ;[1 1 1] Player collision handling
  (if (== (Utilities|GetClass OtherActor) "/Game/Player/Player_CHARACTER.Player_CHARACTER_C")
    (SceneCapture|DisableCapture)))

(event EventBeginPlay
  ;[1 1 1] Setup
  (bind _outactors (Actor|GetAllActorsOfClass "/Game/SecuritySystem/Camera_BP.Camera_BP_C"))
  (bind _output_get (Variables|Default|Setcameras _outactors))
  (for (_array_element _array_index) _output_get
    (Variables|/Script/Engine.SceneCaptureComponent2D|SetTextureTarget (Variables|/Game/SecuritySystem/Camera_BP.Camera_BP_C|GetSceneCaptureComponent2D (.AsCamera%20BP (Utilities|Casting|CastToCamera_BP _array_element))) (Utilities|Array|Get(acopy) (Variables|Default|GettextureTargets) _array_index))
    (Rendering|SceneCapture|CaptureScene (Variables|/Game/SecuritySystem/Camera_BP.Camera_BP_C|GetSceneCaptureComponent2D (.AsCamera%20BP (Utilities|Casting|CastToCamera_BP _array_element))) :!class /Script/Engine.SceneCaptureComponent2D)))

(fn ConstructionScript)

(fn EnableCapture
  (for _array_element (Variables|Default|Getcameras)
    (bind _ascamera_bp (Utilities|Casting|CastToCamera_BP _array_element))
    (Default|EnableCapture _ascamera_bp)))

(fn DisableCapture
  (for _array_element (Variables|Default|Getcameras)
    (bind _ascamera_bp (Utilities|Casting|CastToCamera_BP _array_element))
    (Default|DisableCapture _ascamera_bp)))

(fn PowerEnabled
  (for _array_element (Variables|Default|Getcameras)
    (bind _ascamera_bp (Utilities|Casting|CastToCamera_BP _array_element))
    (Variables|/Game/SecuritySystem/Camera_BP.Camera_BP_C|SetpowerOn _ascamera_bp true))
  (Variables|Default|SetpowerOn true))

(fn PowerDisabled
  (for _array_element (Variables|Default|Getcameras)
    (bind _ascamera_bp (Utilities|Casting|CastToCamera_BP _array_element))
    (Variables|/Game/SecuritySystem/Camera_BP.Camera_BP_C|SetpowerOn _ascamera_bp false))
  (Variables|Default|SetpowerOn false))

(fn EnablePerception
  (for _array_element (Variables|Default|Getcameras)
    (Default|EnablePerception (.AsCamera%20BP (Utilities|Casting|CastToCamera_BP _array_element)))
    (Variables|/Game/SecuritySystem/Camera_BP.Camera_BP_C|SetoperatorAI (.AsCamera%20BP (Utilities|Casting|CastToCamera_BP _array_element)) (.AsAIController%20Base%20AICONTROLLER (Utilities|Casting|CastToAIControllerBase_AICONTROLLER (AI|GetAIController (Variables|Default|GetoperatorNPC)))))))

(fn DisablePerception
  (for _array_element (Variables|Default|Getcameras)
    (Default|DisablePerception (.AsCamera%20BP (Utilities|Casting|CastToCamera_BP _array_element)))
    (Variables|/Game/SecuritySystem/Camera_BP.Camera_BP_C|SetoperatorAI (.AsCamera%20BP (Utilities|Casting|CastToCamera_BP _array_element)) 0)))