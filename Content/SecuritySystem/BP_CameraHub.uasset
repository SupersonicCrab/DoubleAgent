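; Security camera hub that links every BP_Camera in the level to monitor render targets and relays power state to them.
; On BeginPlay it assigns each camera's scene capture a texture target by index.
; Player overlap with a powered hub turns capture on, and leaving turns it off.
; EnablePerception hands cameras the operator NPC's AI controller; that NPC leaving clears its blackboard camera flags and disables perception.
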(event OnComponentBeginOverlap(Collision)
  (params (OverlappedComponent :type Primitive%20Component%20Object%20Reference) (OtherActor :type Actor%20Object%20Reference) (OtherComp :type Primitive%20Component%20Object%20Reference) (OtherBodyIndex :type Integer) (bFromSweep :type Boolean) (SweepResult :type Hit%20Result%20Structure%20%28by%20ref%29))
  ;[1 1 1] Collision handling
  (if (== (Utilities|GetClass OtherActor) "/Game/Player/BP_Player_CHARACTER.BP_Player_CHARACTER_C")
    (if (Variables|Default|GetbPowerOn)
      (SceneCapture|EnableCapture) ; Player enters camera hub
    )))

(event OnComponentEndOverlap(Collision)
  (params (OverlappedComponent :type Primitive%20Component%20Object%20Reference) (OtherActor :type Actor%20Object%20Reference) (OtherComp :type Primitive%20Component%20Object%20Reference) (OtherBodyIndex :type Integer))
  (bind _returnvalue (Utilities|GetClass OtherActor))
  (bind _returnvalue_2 (AI|GetBlackboard OtherActor))
  ;[1 1 1] Collision handling
  (if (== _returnvalue "/Game/Player/BP_Player_CHARACTER.BP_Player_CHARACTER_C")
    (SceneCapture|DisableCapture) ; Player leaves camera hub
    (else
      ;;[1 1 1] Operator NPC leaves camera hub
      (if (and (Utilities|ClassIsChildOf _returnvalue "/Game/AI/NPC/BP_AICharacterBase_CHARACTER.BP_AICharacterBase_CHARACTER_C") (== OtherActor (Variables|Default|GetOperatorNPC)))
        (AI|Components|Blackboard|SetValueasBool _returnvalue_2 (Utilities|Name|MakeLiteralName "CamerasActive") false)
        (AI|Components|Blackboard|SetValueasBool _returnvalue_2 (Utilities|Name|MakeLiteralName "UsingCameras") false)
        (Variables|Default|SetOperatorNPC 0)
        (PerceptionSystem|DisablePerception)))))

(event EventBeginPlay
  ;[1 1 1] Setup
  (bind _outactors (Actor|GetAllActorsOfClass "/Game/SecuritySystem/BP_Camera.BP_Camera_C"))
  (bind _output_get (Variables|Default|SetCameras _outactors))
  (for (_array_element _array_index) _output_get
    (Variables|/Script/Engine.SceneCaptureComponent2D|SetTextureTarget (Variables|/Game/SecuritySystem/BP_Camera.BP_Camera_C|GetSceneCaptureComponent2D (.AsBP%20Camera (Utilities|Casting|CastToBP_Camera _array_element))) (Utilities|Array|Get(acopy) (Variables|Default|GetTextureTargets) _array_index))))

(fn ConstructionScript)

(fn EnableCapture
  (for _array_element (Variables|Default|GetCameras)
    (bind _asbp_camera (Utilities|Casting|CastToBP_Camera _array_element))
    (Default|EnableCapture _asbp_camera)))

(fn DisableCapture
  (for _array_element (Variables|Default|GetCameras)
    (bind _asbp_camera (Utilities|Casting|CastToBP_Camera _array_element))
    (Default|DisableCapture _asbp_camera)))

(fn PowerEnabled
  (for _array_element (Variables|Default|GetCameras)
    (bind _asbp_camera (Utilities|Casting|CastToBP_Camera _array_element))
    (Variables|/Game/SecuritySystem/BP_Camera.BP_Camera_C|SetbPowerOn _asbp_camera true))
  (Variables|Default|SetbPowerOn true))

(fn PowerDisabled
  (for _array_element (Variables|Default|GetCameras)
    (bind _asbp_camera (Utilities|Casting|CastToBP_Camera _array_element))
    (Variables|/Game/SecuritySystem/BP_Camera.BP_Camera_C|SetbPowerOn _asbp_camera false))
  (Variables|Default|SetbPowerOn false))

(fn EnablePerception
  (Variables|Default|SetbDisplayOn true)
  (for _array_element (Variables|Default|GetCameras)
    (Variables|/Game/SecuritySystem/BP_Camera.BP_Camera_C|SetOperatorAI (.AsBP%20Camera (Utilities|Casting|CastToBP_Camera _array_element)) (.AsBP%20AIController%20Base%20AICONTROLLER (Utilities|Casting|CastToBP_AIControllerBase_AICONTROLLER (AI|GetAIController (Variables|Default|GetOperatorNPC)))))
    (Default|EnablePerception (.AsBP%20Camera (Utilities|Casting|CastToBP_Camera _array_element)))))

(fn DisablePerception
  (for _array_element (Variables|Default|GetCameras)
    (Default|DisablePerception (.AsBP%20Camera (Utilities|Casting|CastToBP_Camera _array_element)))
    (Variables|/Game/SecuritySystem/BP_Camera.BP_Camera_C|SetOperatorAI (.AsBP%20Camera (Utilities|Casting|CastToBP_Camera _array_element)) 0))
  (Variables|Default|SetOperatorNPC 0))