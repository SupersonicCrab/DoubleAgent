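; Landline phone in the security system that a player can interact with to disable, provided they have a toolbox.
; Interact passes the player's controller to ServerItemCheck, which asks the game mode for an inventory check on player index 0's character, not the interactor.
; Success clears Functional, while failure shows a non-global log message on that controller.
; Outline events toggle custom depth stencil on the static mesh for highlighting.
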(event Custom|ServerItemCheck
  (params (Controller :type BP%20Spy%20Player%20PLAYERCONTROLLER%20Object%20Reference))
  (bind _success (Default|InventoryServerCheck (.AsBP%20Spy%20Player%20GAMEMODE (Utilities|Casting|CastToBP_SpyPlayer_GAMEMODE (Game|GetGameMode))) (.AsBP%20Player%20CHARACTER (Utilities|Casting|CastToBP_Player_CHARACTER (Game|GetPlayerCharacter 0))) "/Game/Inventory/Item/PlayerEquipment/BP_Toolbox_Item.BP_Toolbox_Item_C"))
  (if _success
    (Variables|Default|SetbFunctional false)
    (else
      (Default|DisplayLog (Variables|/Game/Player/BP_SpyPlayer_PLAYERCONTROLLER.BP_SpyPlayer_PLAYERCONTROLLER_C|GetTextLog Controller) false "Need toolbox to disable" "/Game/Art/Textures/UI/Icons/Logos/T_DefaultNeon.T_DefaultNeon"))))

(event EventInteract
  (params (Interactor :type Actor%20Object%20Reference))
  (bind _asbp_player_character (Utilities|Casting|CastToBP_Player_CHARACTER Interactor))
  (bind _asbp_spy_player_playercontroller (Utilities|Casting|CastToBP_SpyPlayer_PLAYERCONTROLLER (Pawn|GetController _asbp_player_character)))
  (CallFunction|ServerItemCheck _asbp_spy_player_playercontroller))

(event EventEnableOutline
  (bind _staticmesh (Variables|Default|GetStaticMesh))
  (Rendering|SetRenderCustomDepth _staticmesh true)
  (Rendering|SetCustomDepthStencilValue _staticmesh 253))

(event EventDisableOutline
  (bind _staticmesh (Variables|Default|GetStaticMesh))
  (Rendering|SetCustomDepthStencilValue _staticmesh 0)
  (Rendering|SetRenderCustomDepth _staticmesh false))

(fn ConstructionScript)

(fn GetCenter
  (return (.Origin (Collision|GetComponentBounds (Variables|Default|GetStaticMesh)))))

(fn GetInteractText
  (return "Disable landline"))