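; Security camera actor that pans in stepped increments within yaw limits, renders a feed and spots targets for an operator AI.
; Scene capture and sight perception each run on self-rescheduling timers at their own FPS; perception forwards sensed actors to OperatorAI.
; Perception updates also flag search locations as camera-visible.
; Tick eases yaw toward the target at constant speed and updates debug text, including the operator's blackboard Detection value.
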(event OnTargetPerceptionUpdated(AIPerception)
  (params (Actor :type Actor%20Object%20Reference) (Stimulus :type AI%20Stimulus%20Structure))
  ;[1 1 1] Mark search location as visible to camera
  (bind _asbp_search_location (Utilities|Casting|CastToBP_SearchLocation Actor))
  (Variables|/Game/AI/SearchSystem/BP_SearchLocation.BP_SearchLocation_C|SetbVisibleToCamera _asbp_search_location true))

(event EventBeginPlay
  (bind _returnvalue (Transformation|GetActorRotation))
  (bind _rotationlimit (Variables|Rotate|GetrotationLimit))
  ;[1 1 1] Rotation setup
  (Variables|Rotate|SetrightRotateLimit (Math|Conversions|ToFloat(Integer) (Math|Float|Round (+ (.yaw _returnvalue) _rotationlimit))))
  (Variables|Rotate|SetleftRotateLimit (Math|Conversions|ToFloat(Integer) (Math|Float|Round (+ (.yaw _returnvalue) (* -1 _rotationlimit)))))
  (Variables|Rotate|SetrotateTarget (Math|Conversions|ToFloat(Integer) (Math|Float|Round (.yaw _returnvalue)))))

(event EventTick
  (params (DeltaSeconds :type Float%20%28single-precision%29))
  ;[1 1 1] Tick
  (Rotation|RotationTick DeltaSeconds)
  (CallFunction|DetectionDisplayTick))

(fn ConstructionScript)

(fn EnableCapture
  (Variables|SceneCapture|SetupdatingCapture true)
  (SceneCapture|CaptureTick))

(fn DisableCapture
  (Variables|SceneCapture|SetupdatingCapture false))

(fn CaptureTick
  (if (and (Variables|SceneCapture|GetupdatingCapture) (Variables|Default|GetpowerOn))
    (Rendering|SceneCapture|CaptureScene (Variables|Default|GetSceneCaptureComponent2D) :!class /Script/Engine.SceneCaptureComponent2D)
    (Utilities|Time|SetTimerbyFunctionName 0 "CaptureTick" (/ 1.0 (Variables|SceneCapture|GetcaptureFPS))) ; Recursively call capture function based on capture fps
  ))

(fn RotateLeft
  (if (>= (Math|Conversions|ToFloat(Integer) (Math|Float|Round (- (Variables|Rotate|GetrotateTarget) 3e+01))) (Variables|Rotate|GetleftRotateLimit))
    (Variables|Rotate|SetrotateTarget (Math|Conversions|ToFloat(Integer) (Math|Float|Round (- (Variables|Rotate|GetrotateTarget) 3e+01))))))

(fn RotateRight
  (if (<= (Math|Conversions|ToFloat(Integer) (Math|Float|Round (+ (Variables|Rotate|GetrotateTarget) 3e+01))) (Variables|Rotate|GetrightRotateLimit))
    (Variables|Rotate|SetrotateTarget (Math|Conversions|ToFloat(Integer) (Math|Float|Round (+ (Variables|Rotate|GetrotateTarget) 3e+01))))))

(fn EnablePerception
  (Variables|Perception|SetupdatingPerception true)
  (Class|AIPerceptionComponent|SetSenseEnabled (Variables|Default|GetAIPerception) "/Script/AIModule.AISense_Sight" true)
  (PerceptionSystem|PerceptionTick))

(fn DisablePerception
  (Variables|Perception|SetupdatingPerception false)
  (Class|AIPerceptionComponent|SetSenseEnabled (Variables|Default|GetAIPerception) "/Script/AIModule.AISense_Sight" false))

(fn PerceptionTick
  (if (and (Variables|Perception|GetupdatingPerception) (Utilities|IsValid (Variables|Perception|GetoperatorAI)))
    ;[1 1 1] Call operatorNPC sight tick
    (bind _array_element (Utilities|Array|ForEachLoopwithBreak (Class|AIPerceptionComponent|GetCurrentlyPerceivedActors (Variables|Default|GetAIPerception) "/Script/AIModule.AISense_Sight"))
      (:LoopBody
        (bind _info (Class|AIPerceptionComponent|GetActorsPerception (Variables|Default|GetAIPerception) _array_element))
        (if (Utilities|Struct|BreakAIStimulus (Utilities|Array|Get(acopy) (.lastsensedstimuli _info)))
          (Default|HandleSightTick (Variables|Perception|GetoperatorAI) (.target _info) (Utilities|Struct|BreakAIStimulus (Utilities|Array|Get(acopy) (.lastsensedstimuli _info))) self)))
      (:Completed
        ;[1 1 1] Call function recursively based on perception fps
        (Utilities|Time|SetTimerbyFunctionName 0 "PerceptionTick" (/ 1.0 (Variables|Perception|GetperceptionFPS)))))))

(fn RotationTick
  (params (InputPin :type Float%20%28single-precision%29))
  (bind _returnvalue (Transformation|GetActorRotation))
  (bind _rotatetarget (Variables|Rotate|GetrotateTarget))
  (bind _returnvalue_2 (Math|Float|Round (.yaw _returnvalue)))
  (bind _returnvalue_3 (Math|Conversions|ToFloat(Integer) _returnvalue_2))
  (if (!= _returnvalue_3 _rotatetarget) ; If current rotation is not the same as rotate target
    ;[1 1 1] Left rotation
    (if (> _returnvalue_3 _rotatetarget) ; If current rotation is less than rotate target
      (Transformation|AddActorLocalRotation (* (Math|Rotator|MakeRotator 0.0 0.0 (* (Variables|Rotate|GetrotationSpeed) -1.0)) InputPin) false false)
      (else
        ;[1 1 1] Right rotation
        (if (< _returnvalue_3 _rotatetarget) ; if current rotation is greater then rotate target
          (Transformation|AddActorLocalRotation (* (Math|Rotator|MakeRotator 0.0 0.0 (* (Variables|Rotate|GetrotationSpeed) 1.0)) InputPin) false false))))))

(fn DetectionDisplayTick
  (bind _returnvalue (Game|GetPlayerCharacter 0))
  (Utilities|IsValid _returnvalue
    (:Is%20Valid
      (Transformation|SetWorldRotation (Variables|Default|GetDebugName) (Math|Rotator|FindLookatRotation (Transformation|GetWorldLocation (Variables|Default|GetDebugName)) (Transformation|GetWorldLocation (Variables|/Game/Player/Player_CHARACTER.Player_CHARACTER_C|GetThirdPersonCamera (.AsPlayer%20CHARACTER (Utilities|Casting|CastToPlayer_CHARACTER _returnvalue))))) false false) ; Look at player camera
    )
    (:Is%20Not%20Valid
      _))
  (Utilities|IsValid (Variables|Perception|GetoperatorAI)
    (:Is%20Valid
      (Rendering|Components|TextRender|SetText (Variables|Default|GetDebugDetection) (Utilities|Text|MakeLiteralText (Utilities|Text|ToText(Integer) (Math|Float|Round (Class|BlackboardComponent|GetValueasFloat (AI|GetBlackboard (Variables|Perception|GetoperatorAI)) (Utilities|Name|MakeLiteralName "Detection")))))) ; Update detection
    )))