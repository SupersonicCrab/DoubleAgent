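; RadioHub_BP is the security system's radio hub, broadcasting radio events to NPCs tagged Radio.
; It records the radio NPCs at BeginPlay, but each send looks them up again and calls RadioEventDelay on their AI controllers.
; Each send prints a debug message and sets an in-use flag that a timer clears after the event's delay.
; Power on/off only toggles a flag; test functions fire sample events.
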(event EventBeginPlay
  ;[1 1 1] Save all NPCs with radios
  (bind _outactors (Actor|GetAllActorsOfClasswithTag "/Game/AI/NPC/AICharacterBase_CHARACTER.AICharacterBase_CHARACTER_C" "Radio"))
  (for _array_element _outactors
    (Utilities|Array|Add (Variables|Default|GetinitialRadioNPCs) (.AsAICharacter%20Base%20CHARACTER (Utilities|Casting|CastToAICharacterBase_CHARACTER _array_element)))))

(fn ConstructionScript)

(fn PowerOff
  (Variables|Default|SetradioPowerOn false))

(fn Poweron
  (Variables|Default|SetradioPowerOn true))

(fn SendRadioEvent
  (params (RadioEvent :type Radio%20Event%20STRUCT%20Structure))
  (bind (_radioevent _location _delay _npc) (Utilities|Struct|BreakRadioEvent_STRUCT RadioEvent))
  ;[1 1 1] Send radio event to NPCs
  (bind _outactors (Actor|GetAllActorsOfClasswithTag "/Game/AI/NPC/AICharacterBase_CHARACTER.AICharacterBase_CHARACTER_C" "Radio"))
  (for _array_element _outactors
    (Default|RadioEventDelay (.AsAIController%20Base%20AICONTROLLER (Utilities|Casting|CastToAIControllerBase_AICONTROLLER (AI|GetAIController (.AsAICharacter%20Base%20CHARACTER (Utilities|Casting|CastToAICharacterBase_CHARACTER _array_element))))) RadioEvent))
  ;[1 1 1] Debug output for radio event
  (Development|PrintString (Utilities|String|Append (Utilities|String|EnumtoString _radioevent) " radio event at " (Utilities|String|ToString(Vector) _location) " by " (Utilities|GetDisplayName _npc) " with a " (Utilities|String|ToString(Float) _delay) " second delay") true true "(R=0.000000,G=0.660000,B=1.000000,A=1.000000)" 2e+01)
  ;[1 1 1] Lock radio for voice line duration
  (Variables|Default|SetradioInUse true)
  (Utilities|Time|SetTimerbyFunctionName 0 "FinishRadioEvent" _delay))

(fn FinishRadioEvent
  (Variables|Default|SetradioInUse false))

(fn TestAlert
  (CallFunction|SendRadioEvent (Utilities|Struct|MakeRadioEvent_STRUCT "NewEnumerator3" (+ (Transformation|GetActorLocation) "0, 0,150.000000") 0.1 0)))

(fn TestEngage
  (CallFunction|SendRadioEvent (Utilities|Struct|MakeRadioEvent_STRUCT "NewEnumerator4" (+ (Transformation|GetActorLocation) "0, 0,150.000000") 0.1 0)))

(fn TestCheckinCall
  (CallFunction|SendRadioEvent (Utilities|Struct|MakeRadioEvent_STRUCT "NewEnumerator1" "0.000000,0.000000,0.000000" 1.0 0)))