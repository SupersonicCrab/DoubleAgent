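; Radio hub actor for the security system that relays radio events to AI NPCs tagged "Radio".
; BeginPlay records the initial radio NPCs, while each send re-queries tagged characters and calls RadioEventDelay on their AI controllers.
; Sending prints debug details and flags the radio as in use until a timer matching the event's delay clears it.
; Power toggles only set a flag, and test functions fire sample alert, engage and check-in events.
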(event EventBeginPlay
  ;[1 1 1] Save all NPCs with radios
  (bind _outactors (Actor|GetAllActorsOfClasswithTag "/Game/AI/NPC/BP_AICharacterBase_CHARACTER.BP_AICharacterBase_CHARACTER_C" "Radio"))
  (for _array_element _outactors
    (Utilities|Array|Add (Variables|Default|GetInitialRadioNPCs) (.AsBP%20AICharacter%20Base%20CHARACTER (Utilities|Casting|CastToBP_AICharacterBase_CHARACTER _array_element)))))

(fn ConstructionScript)

(fn PowerOff
  (Variables|Default|SetbRadioPowerOn false))

(fn Poweron
  (Variables|Default|SetbRadioPowerOn true))

(fn SendRadioEvent
  (params (RadioEvent :type F%20Radio%20Event%20Structure))
  (bind (_radioevent _location _delay _npc) (Utilities|Struct|BreakFRadioEvent RadioEvent))
  ;[1 1 1] Send radio event to NPCs
  (bind _outactors (Actor|GetAllActorsOfClasswithTag "/Game/AI/NPC/BP_AICharacterBase_CHARACTER.BP_AICharacterBase_CHARACTER_C" "Radio"))
  (for _array_element _outactors
    (Default|RadioEventDelay (.AsBP%20AIController%20Base%20AICONTROLLER (Utilities|Casting|CastToBP_AIControllerBase_AICONTROLLER (AI|GetAIController (.AsBP%20AICharacter%20Base%20CHARACTER (Utilities|Casting|CastToBP_AICharacterBase_CHARACTER _array_element)))))))
  ;[1 1 1] Debug output for radio event
  (Development|PrintString (Utilities|String|Append (Utilities|String|EnumtoString _radioevent) " radio event at " (Utilities|String|ToString(Vector) _location) " by " (Utilities|GetDisplayName _npc) " with a " (Utilities|String|ToString(Float) _delay) " second delay") true true "(R=0.000000,G=0.660000,B=1.000000,A=1.000000)" 2e+01)
  ;[1 1 1] Lock radio for voice line duration
  (Variables|Default|SetbRadioInUse true)
  (Utilities|Time|SetTimerbyFunctionName 0 "FinishRadioEvent" _delay))

(fn FinishRadioEvent
  (Variables|Default|SetbRadioInUse false))

(fn TestAlert
  (CallFunction|SendRadioEvent (Utilities|Struct|MakeFRadioEvent "NewEnumerator3" (+ (Transformation|GetActorLocation) "0, 0,150.000000") 0.1 0)))

(fn TestEngage
  (CallFunction|SendRadioEvent (Utilities|Struct|MakeFRadioEvent "NewEnumerator4" (+ (Transformation|GetActorLocation) "0, 0,150.000000") 0.1 0)))

(fn TestCheckinCall
  (CallFunction|SendRadioEvent (Utilities|Struct|MakeFRadioEvent "NewEnumerator1" "0.000000,0.000000,0.000000" 1.0 0)))