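; Networked security camera that sweeps between yaw limits or steps on manual request, and serves as remote eyes for an operator NPC.
; Self-rescheduling timers drive scene capture and forward sight perception from the lens to the operator AI.
; Manual rotation stops the sweep; after the operator's reaction delay, it resumes and the operator's detection is raised to a minimum.
; Seen search locations and their rooms are flagged camera-visible, and operator detection feeds a debug display.
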(event OnPerceptionUpdated(AIPerception)
  (params (UpdatedActors :type Array%20of%20Actor%20Object%20References))
  ;[1 1 1] Update operatingNPC perception
  (if (and (Variables|Perception|GetbUpdatingPerception) (Utilities|IsValid (Variables|Perception|GetOperatorAI)))
    (for _array_element UpdatedActors
      (bind _info (Class|AIPerceptionComponent|GetActorsPerception (Variables|Default|GetAIPerception) _array_element))
      (Default|HandleSightUpdate (Variables|Perception|GetOperatorAI) (.target _info) (Utilities|Struct|BreakAIStimulus (Utilities|Array|Get(acopy) (.lastsensedstimuli _info)))))))

(event OnTargetPerceptionUpdated(AIPerception)
  (params (Actor :type Actor%20Object%20Reference) (Stimulus :type AI%20Stimulus%20Structure))
  ;[1 1 1] Mark search location and/or room as visible to camera
  (bind _asbp_search_location (Utilities|Casting|CastToBP_SearchLocation Actor))
  (Variables|/Game/AI/BP_SearchLocation.BP_SearchLocation_C|SetbVisibleToCamera _asbp_search_location true)
  (if (!= (Utilities|Array|Length (Variables|/Game/AI/BP_SearchLocation.BP_SearchLocation_C|GetRoom _asbp_search_location)) 0)
    (for _array_element (Variables|/Game/AI/BP_SearchLocation.BP_SearchLocation_C|GetRoom _asbp_search_location)
      (for _array_element_2 (Variables|/Script/DoubleAgent.RoomVolume|GetsearchLocations _array_element)
        (Variables|/Game/AI/BP_SearchLocation.BP_SearchLocation_C|SetbVisibleToCamera (.AsBP%20Search%20Location (Utilities|Casting|CastToBP_SearchLocation _array_element_2)) true)))))

(event Custom|NetRequestRotateRight
  ;[1 1 1] Network functions
  (CallFunction|NetRotateRight))

(event Custom|NetRotateRight
  ;[1 1 1] Network functions
  (Rotation|RotateRight))

(event Custom|NetRequestRotateLeft
  ;[1 1 1] Network functions
  (CallFunction|NetRotateLeft))

(event Custom|NetRotateLeft
  ;[1 1 1] Network functions
  (Rotation|RotateLeft))

(event EventBeginPlay
  ;[1 1 1] Setup
  (Variables|Rotate|SetbAutoRotate (Variables|Rotate|GetbAutoRotateDefault))
  (Variables|Rotate|SetAutoRotateDelay (+ (Variables|Rotate|GetAutoRotateDelay) (Math|Random|RandomFloatinRange 0.5 1e+01))))

(event EventTick
  (params (DeltaSeconds :type Float%20%28single-precision%29))
  ;[1 1 1] Debug update
  (Rotation|RotationTick DeltaSeconds)
  (CallFunction|DebugDisplayUpdate)
  (CallFunction|DetectionUpdate))

(fn ConstructionScript)

(fn EnableCapture
  (Variables|SceneCapture|SetbUpdatingCapture true)
  (SceneCapture|CaptureTick))

(fn DisableCapture
  (Variables|SceneCapture|SetbUpdatingCapture false))

(fn CaptureTick
  (if (and (Variables|SceneCapture|GetbUpdatingCapture) (Variables|Default|GetbPowerOn))
    (Rendering|SceneCapture|CaptureScene (Variables|Default|GetSceneCaptureComponent2D) :!class /Script/Engine.SceneCaptureComponent2D)
    (Utilities|Time|SetTimerbyFunctionName 0 "CaptureTick" (/ 1.0 (Variables|SceneCapture|GetCaptureFPS))) ; Recursively call capture function based on capture fps
  ))

(fn RotateLeft
  (bind _leftyawlimit (Variables|Rotate|GetLeftYawLimit))
  (bind _rotateamount (Variables|Rotate|GetRotateAmount))
  (bind _camerapivot (Variables|Default|GetCameraPivot))
  (bind _relativerotation (Variables|/Script/Engine.SceneComponent|GetRelativeRotation _camerapivot))
  (bind _returnvalue (/ (.yaw _relativerotation) _rotateamount))
  (bind _returnvalue_2 (Math|Float|Round _returnvalue))
  (bind _returnvalue_3 (Math|Conversions|ToFloat(Integer) _returnvalue_2))
  (bind _returnvalue_4 (+ _returnvalue_3 -1.0))
  (bind _returnvalue_5 (* _returnvalue_4 _rotateamount))
  (if (>= _returnvalue_5 _leftyawlimit) ; If rotation is within limit
    (Variables|Rotate|SetTargetYaw _returnvalue_5)
    (else
      (Variables|Rotate|SetTargetYaw _leftyawlimit)))
  (Rotation|DisableAutoRotate))

(fn RotateRight
  (bind _rightyawlimit (Variables|Rotate|GetRightYawLimit))
  (bind _rotateamount (Variables|Rotate|GetRotateAmount))
  (bind _camerapivot (Variables|Default|GetCameraPivot))
  (bind _relativerotation (Variables|/Script/Engine.SceneComponent|GetRelativeRotation _camerapivot))
  (bind _returnvalue (/ (.yaw _relativerotation) _rotateamount))
  (bind _returnvalue_2 (Math|Float|Round _returnvalue))
  (bind _returnvalue_3 (Math|Conversions|ToFloat(Integer) _returnvalue_2))
  (bind _returnvalue_4 (+ _returnvalue_3 1.0))
  (bind _returnvalue_5 (* _returnvalue_4 _rotateamount))
  (if (<= _returnvalue_5 _rightyawlimit) ; If rotation is within limit
    (Variables|Rotate|SetTargetYaw _returnvalue_5)
    (else
      (Variables|Rotate|SetTargetYaw _rightyawlimit)))
  (Rotation|DisableAutoRotate))

(fn EnablePerception
  (Variables|Perception|SetbUpdatingPerception true)
  (Class|AIPerceptionComponent|SetSenseEnabled (Variables|Default|GetAIPerception) "/Script/AIModule.AISense_Sight" true)
  (PerceptionSystem|PerceptionTick))

(fn DisablePerception
  (Variables|Perception|SetbUpdatingPerception false)
  (Class|AIPerceptionComponent|SetSenseEnabled (Variables|Default|GetAIPerception) "/Script/AIModule.AISense_Sight" false))

(fn PerceptionTick
  (if (and (Variables|Perception|GetbUpdatingPerception) (Utilities|IsValid (Variables|Perception|GetOperatorAI)))
    ;[1 1 1] Call operatorNPC sight tick
    (bind _array_element (Utilities|Array|ForEachLoopwithBreak (Class|AIPerceptionComponent|GetCurrentlyPerceivedActors (Variables|Default|GetAIPerception) "/Script/AIModule.AISense_Sight"))
      (:LoopBody
        (bind _info (Class|AIPerceptionComponent|GetActorsPerception (Variables|Default|GetAIPerception) _array_element))
        (if (Utilities|Struct|BreakAIStimulus (Utilities|Array|Get(acopy) (.lastsensedstimuli _info)))
          (Default|HandleSightTick (Variables|Perception|GetOperatorAI) (.target _info) (Utilities|Struct|BreakAIStimulus (Utilities|Array|Get(acopy) (.lastsensedstimuli _info))) self)))
      (:Completed
        ;[1 1 1] Call function recursively based on perception fps
        (Utilities|Time|SetTimerbyFunctionName 0 "PerceptionTick" (/ 1.0 (Variables|Perception|GetPerceptionFPS)))))))

(fn RotationTick
  (params (DeltaTime :type Float%20%28single-precision%29))
  (bind _camerapivot (Variables|Default|GetCameraPivot))
  (bind _relativerotation (Variables|/Script/Engine.SceneComponent|GetRelativeRotation _camerapivot))
  (bind _returnvalue (Math|Float|Round (.yaw _relativerotation)))
  (bind _returnvalue_2 (Math|Conversions|ToFloat(Integer) _returnvalue))
  (LocalVariables|SetCurrentYaw _returnvalue_2)
  (if (!= _returnvalue_2 (Variables|Rotate|GetTargetYaw)) ; If current rotation is not the same as rotate target
    ;[1 1 1] Speed handling
    (if (Variables|Rotate|GetbAutoRotate)
      (Variables|Rotate|SetCurrentRotationSpeed (/ (Variables|Rotate|GetRotationSpeed) 2.0)) ; Half rotation speed if rotating automatically
      (else
        (Variables|Rotate|SetCurrentRotationSpeed (Variables|Rotate|GetRotationSpeed))))
    ;[1 1 1] Left rotation
    (if (> (LocalVariables|GetCurrentYaw) (Variables|Rotate|GetTargetYaw)) ; If current rotation is less than rotate target
      (Transformation|AddRelativeRotation (Variables|Default|GetCameraPivot) (* (Math|Rotator|MakeRotator 0.0 0.0 (* (Variables|Rotate|GetCurrentRotationSpeed) -1.0)) DeltaTime) false false)
      (else
        ;[1 1 1] Right rotation
        (if (< (LocalVariables|GetCurrentYaw) (Variables|Rotate|GetTargetYaw)) ; if current rotation is greater then rotate target
          (Transformation|AddRelativeRotation (Variables|Default|GetCameraPivot) (* (Math|Rotator|MakeRotator 0.0 0.0 (* (Variables|Rotate|GetCurrentRotationSpeed) 1.0)) DeltaTime) false false))))
    (else
      ;[1 1 1] Auto rotate handling
      (if (and (Variables|Rotate|GetbAutoRotate) (not (Class|KismetSystemLibrary|IsTimerActive 0 "HandleAutoRotate"))) ; If auto rotate is set and not already counting down
        (Utilities|Time|SetTimerbyFunctionName 0 "HandleAutoRotate" (Variables|Rotate|GetAutoRotateDelay))))))

(fn OperatorReaction
  (bind _returnvalue (Utilities|Name|MakeLiteralName "Detection"))
  (bind _operatorai (Variables|Perception|GetOperatorAI))
  (bind _returnvalue_2 (AI|GetBlackboard _operatorai))
  (Variables|Rotate|SetbAutoRotate true)
  (if (< (Class|BlackboardComponent|GetValueasFloat _returnvalue_2 _returnvalue) 4e+01)
    (AI|Components|Blackboard|SetValueasFloat _returnvalue_2 _returnvalue 4e+01)))

(fn DetectionDisplayTick)

(fn SetTargetRotation
  (bind _output_get (Variables|Rotate|SetTargetYaw (Math|Conversions|ToFloat(Integer) (Math|Float|Round (.yaw (Variables|/Script/Engine.SceneComponent|GetRelativeRotation (Variables|Default|GetCameraPivot)))))))
  (if (and (== (Variables|Rotate|GetRightYawLimit) 0.0) (== (Variables|Rotate|GetLeftYawLimit) 0.0))
    (Variables|Rotate|SetRightYawLimit _output_get)
    (Variables|Rotate|SetLeftYawLimit _output_get)))

(fn GetPerceptionLocationRotation
  (bind _scenecapturecomponent2d (Variables|Default|GetSceneCaptureComponent2D))
  ;[1 1 1] Override perception to lens location and rotation
  (return (Transformation|GetWorldLocation _scenecapturecomponent2d) (Transformation|GetWorldRotation _scenecapturecomponent2d)))

(fn HandleAutoRotate
  (LocalVariables|SetCurrentYaw (Math|Conversions|ToFloat(Integer) (Math|Float|Round (.yaw (Variables|/Script/Engine.SceneComponent|GetRelativeRotation (Variables|Default|GetCameraPivot))))))
  (if (!= (LocalVariables|GetCurrentYaw) (Variables|Rotate|GetRightYawLimit)) ; If current yaw is not eqaul to right limit
    (Variables|Rotate|SetTargetYaw (Variables|Rotate|GetRightYawLimit))
    (elif (!= (LocalVariables|GetCurrentYaw) (Variables|Rotate|GetLeftYawLimit)) ; If current yaw not eqaul to left limit
      (Variables|Rotate|SetTargetYaw (Variables|Rotate|GetLeftYawLimit)))))

(fn GetCenterLocation
  (return (Transformation|GetWorldLocation (Variables|Default|GetCamera))))

(fn DisableAutoRotate
  (bind _operatorai (Variables|Perception|GetOperatorAI))
  (if (Networking|IsServer)
    (if (Variables|Rotate|GetbAutoRotate)
      (Variables|Rotate|SetbAutoRotate false)
      (Utilities|IsValid _operatorai
        (:Is%20Valid
          (Utilities|Time|SetTimerbyFunctionName 0 "OperatorReaction" (Variables|/Game/AI/NPC/BP_AIControllerBase_AICONTROLLER.BP_AIControllerBase_AICONTROLLER_C|GetOperatorReactionDelay _operatorai)))))))

(fn DebugDisplayUpdate
  (bind _returnvalue (Game|GetPlayerCharacter 0))
  (Utilities|IsValid _returnvalue
    (:Is%20Valid
      (Transformation|SetWorldRotation (Variables|Default|GetDebugName) (Math|Rotator|FindLookatRotation (Transformation|GetWorldLocation (Variables|Default|GetDebugName)) (Transformation|GetWorldLocation (Variables|/Game/Player/BP_Player_CHARACTER.BP_Player_CHARACTER_C|GetCamera (.AsBP%20Player%20CHARACTER (Utilities|Casting|CastToBP_Player_CHARACTER _returnvalue))))) false false) ; Look at player camera
    )))

(fn OnRepNetDetection
  (Rendering|Components|TextRender|SetText (Variables|Default|GetDebugDetection) (Utilities|Text|ToText(Integer) (Variables|Default|GetNetDetection))))

(fn DetectionUpdate
  (if (Networking|IsServer)
    (Utilities|IsValid (Variables|Perception|GetOperatorAI)
      (:Is%20Valid
        (Variables|Default|SetNetDetection (Math|Float|Round (Class|BlackboardComponent|GetValueasFloat (AI|GetBlackboard (Variables|Perception|GetOperatorAI)) (Utilities|Name|MakeLiteralName "Detection"))))))))