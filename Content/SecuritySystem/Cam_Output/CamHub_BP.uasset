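; CamHub_BP is the security camera hub that manages every Camera_BP in the level and its render-target feed.
; On BeginPlay it gathers the cameras, assigns each a render target by array index, and captures an initial frame.
; A trigger box enables camera updates when the player enters while powered and disables them on exit.
; PowerEnabled and PowerDisabled propagate the power state to the hub and all cameras.
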(event OnComponentBeginOverlap(Box)
  (params (OverlappedComponent :type Primitive%20Component%20Object%20Reference) (OtherActor :type Actor%20Object%20Reference) (OtherComp :type Primitive%20Component%20Object%20Reference) (OtherBodyIndex :type Integer) (bFromSweep :type Boolean) (SweepResult :type Hit%20Result%20Structure%20%28by%20ref%29))
  (if (== (Utilities|GetClass OtherActor) "/Game/Player/Player_CHARACTER.Player_CHARACTER_C")
    (if (Variables|Default|GetPowerOn)
      (CallFunction|Camerason))))

(event OnComponentEndOverlap(Box)
  (params (OverlappedComponent :type Primitive%20Component%20Object%20Reference) (OtherActor :type Actor%20Object%20Reference) (OtherComp :type Primitive%20Component%20Object%20Reference) (OtherBodyIndex :type Integer))
  (if (== (Utilities|GetClass OtherActor) "/Game/Player/Player_CHARACTER.Player_CHARACTER_C")
    (CallFunction|CamerasOff)))

(event EventBeginPlay
  (bind _outactors (Actor|GetAllActorsOfClass "/Game/SecuritySystem/Camera/Camera_BP.Camera_BP_C"))
  (bind _output_get (Variables|Default|SetCameras _outactors))
  (for (_array_element _array_index) _output_get
    (Variables|/Script/Engine.SceneCaptureComponent2D|SetTextureTarget (Variables|/Game/SecuritySystem/Camera/Camera_BP.Camera_BP_C|GetSceneCaptureComponent2D (.AsCamera%20BP (Utilities|Casting|CastToCamera_BP _array_element))) (Utilities|Array|Get(acopy) (Variables|Default|GetTextureTargets) _array_index))
    (Rendering|SceneCapture|CaptureScene (Variables|/Game/SecuritySystem/Camera/Camera_BP.Camera_BP_C|GetSceneCaptureComponent2D (.AsCamera%20BP (Utilities|Casting|CastToCamera_BP _array_element))) :!class /Script/Engine.SceneCaptureComponent2D)))

(fn ConstructionScript)

(fn Camerason
  (for _array_element (Variables|Default|GetCameras)
    (bind _ascamera_bp (Utilities|Casting|CastToCamera_BP _array_element))
    (Default|EnableUpdate _ascamera_bp)))

(fn CamerasOff
  (for _array_element (Variables|Default|GetCameras)
    (bind _ascamera_bp (Utilities|Casting|CastToCamera_BP _array_element))
    (Default|DisableUpdate _ascamera_bp)))

(fn PowerEnabled
  (for _array_element (Variables|Default|GetCameras)
    (bind _ascamera_bp (Utilities|Casting|CastToCamera_BP _array_element))
    (Variables|/Game/SecuritySystem/Camera/Camera_BP.Camera_BP_C|SetPowerOn _ascamera_bp true))
  (Variables|Default|SetPowerOn true))

(fn PowerDisabled
  (for _array_element (Variables|Default|GetCameras)
    (bind _ascamera_bp (Utilities|Casting|CastToCamera_BP _array_element))
    (Variables|/Game/SecuritySystem/Camera/Camera_BP.Camera_BP_C|SetPowerOn _ascamera_bp false))
  (Variables|Default|SetPowerOn false))