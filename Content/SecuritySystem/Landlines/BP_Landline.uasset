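; BP_Landline is an interactable security-system landline that a player can sabotage if carrying a toolbox.
; On interact, it checks the player's InventoryComponent for the toolbox item class, then either calls DisableLandline or shows a non-global text-log message saying a toolbox is needed.
; It also supplies the interaction prompt and uses the static mesh's bounds origin as its center.
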(event EventInteract
  (params (Interactor :type Actor%20Object%20Reference))
  (bind _asbp_player_character (Utilities|Casting|CastToBP_Player_CHARACTER Interactor))
  (bind _itemfound (Default|CheckItemClass (Variables|/Game/Player/BP_Player_CHARACTER.BP_Player_CHARACTER_C|GetInventoryComponent _asbp_player_character) "/Game/Inventory/Item/PlayerEquipment/BP_Toolbox_Item.BP_Toolbox_Item_C"))
  (if _itemfound
    (Class|Landline|DisableLandline)
    (else
      (Default|DisplayLog (Variables|/Game/Player/BP_SpyPlayer_PLAYERCONTROLLER.BP_SpyPlayer_PLAYERCONTROLLER_C|GetTextLog (.AsBP%20Spy%20Player%20PLAYERCONTROLLER (Utilities|Casting|CastToBP_SpyPlayer_PLAYERCONTROLLER (Pawn|GetController _asbp_player_character)))) false "Toolbox needed to sabotage" "/Game/Art/Textures/UI/Icons/Logos/T_DefaultNeon.T_DefaultNeon"))))

(fn ConstructionScript)

(fn GetCenter
  (return (.Origin (Collision|GetComponentBounds (Variables|Default|GetStaticMesh)))))

(fn GetInteractText
  (return "Disable landline"))