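; BP_Spawnpoint is a guard spawn point in the security system that spawns a BP_Guard_CHARACTER when SpawnGuard is called.
; SpawnGuard projects the actor's location onto the navmesh and spawns the guard there, facing the spawn point's direction.
; It then writes the new guard's blackboard, starting it with high Detection and BackupAvailable set to false.
; The event graph and construction script are empty.
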(event EventBeginPlay)

(event Collision|EventActorBeginOverlap
  (params (OtherActor :type Actor%20Object%20Reference)))

(event EventTick
  (params (DeltaSeconds :type Float%20%28single-precision%29)))

(fn ConstructionScript)

(fn SpawnGuard
  (bind _self self)
  (bind _returnvalue (Transformation|GetActorTransform _self))
  (bind (_location _rotation) (Math|Transform|BreakTransform _returnvalue))
  ;[1 1 1] Spawn guard with spawnpoints direction
  (bind _returnvalue_2 (Game|SpawnActorfromClass "/Game/AI/NPC/Guard/BP_Guard_CHARACTER.BP_Guard_CHARACTER_C" (Math|Transform|MakeTransform (.ProjectedLocation (AI|Navigation|ProjectPointtoNavigation _location 0 0 "100.000000,100.000000,100.000000")) _rotation) "Undefined" 0 0 0))
  ;[1 1 1] Set guards detection to 90
  (AI|Components|Blackboard|SetValueasFloat (AI|GetBlackboard _returnvalue_2) (Utilities|Name|MakeLiteralName "Detection") 9e+01)
  (AI|Components|Blackboard|SetValueasBool (AI|GetBlackboard _returnvalue_2) (Utilities|Name|MakeLiteralName "BackupAvailable") false))