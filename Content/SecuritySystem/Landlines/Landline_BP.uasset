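; Landline actor in the security system that can call in guard backup and can be disabled by player interaction.
; Interacting with it clears its LandlineEnabled flag, and EnableLandline sets it again.
; CallBackup, when the landline is enabled, spawns a guard at every Spawnpoint_BP in the level, then disables every landline, so one call uses up all of them.
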(event EventInteract
  (params (Interactor :type Actor%20Object%20Reference))
  (CallFunction|DisableLandline))

(fn ConstructionScript)

(fn DisableLandline
  (Variables|Default|SetLandlineEnabled false))

(fn EnableLandline
  (Variables|Default|SetLandlineEnabled true))

(fn CallBackup
  (if (Variables|Default|GetLandlineEnabled)
    ;[1 1 1] Get all spawnpoints
    (bind _outactors (Actor|GetAllActorsOfClass "/Game/SecuritySystem/Landlines/Spawnpoint_BP.Spawnpoint_BP_C"))
    (for _array_element _outactors
      ;[1 1 1] Spawn a guard in each spawnpoint
      (Default|SpawnGuard _array_element))
    ;[1 1 1] Get all landlines
    (bind _outactors_2 (Actor|GetAllActorsOfClass "Landline_BP_C"))
    (for _array_element_2 _outactors_2
      ;[1 1 1] Disable all landlines
      (CallFunction|DisableLandline _array_element_2))))