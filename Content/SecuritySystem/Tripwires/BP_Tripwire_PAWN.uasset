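; Security tripwire pawn that raises an alarm when the player or an AI character crosses it without a tripwire remote item.
; On BeginPlay it finds the level's power box and copies its tripwire state, toggling the light, beam visibility and collision overlap events.
; Overlaps check the character's inventory component for the remote; a failed check prints a message and emits a tagged MakeNoise with the tripwire as instigator.
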(event OnComponentBeginOverlap(Collision)
  (params (OverlappedComponent :type Primitive%20Component%20Object%20Reference) (OtherActor :type Actor%20Object%20Reference) (OtherComp :type Primitive%20Component%20Object%20Reference) (OtherBodyIndex :type Integer) (bFromSweep :type Boolean) (SweepResult :type Hit%20Result%20Structure%20%28by%20ref%29))
  (bind _returnvalue (Utilities|GetClass OtherActor))
  ;[1 1 1] Handle player and NPC collision
  (if (== _returnvalue "/Game/Player/BP_Player_CHARACTER.BP_Player_CHARACTER_C")
    (bind _itemfound (Default|CheckItemClass (Variables|/Game/Player/BP_Player_CHARACTER.BP_Player_CHARACTER_C|GetInventoryComponent (.AsBP%20Player%20CHARACTER (Utilities|Casting|CastToBP_Player_CHARACTER OtherActor))) "/Game/Inventory/Item/BP_TripwireRemote_Item.BP_TripwireRemote_Item_C"))
    (if (not _itemfound)
      (CallFunction|ActivateAlarm))
    (elif (Utilities|ClassIsChildOf _returnvalue "/Game/AI/NPC/BP_AICharacterBase_CHARACTER.BP_AICharacterBase_CHARACTER_C")
      (bind _itemfound_2 (Default|CheckItemClass (Variables|/Game/AI/NPC/BP_AICharacterBase_CHARACTER.BP_AICharacterBase_CHARACTER_C|GetInventoryComponent (.AsBP%20AICharacter%20Base%20CHARACTER (Utilities|Casting|CastToBP_AICharacterBase_CHARACTER OtherActor))) "/Game/Inventory/Item/BP_TripwireRemote_Item.BP_TripwireRemote_Item_C"))
      (if (not _itemfound_2)
        (CallFunction|ActivateAlarm)))))

(event EventBeginPlay
  ;[1 1 1] Setup
  (bind _returnvalue (Actor|GetActorOfClass "/Game/PowerSystem/BP_PowerBox.BP_PowerBox_C"))
  (bind _output_get (Variables|Default|SetpowerBox _returnvalue))
  (if (Variables|/Game/PowerSystem/BP_PowerBox.BP_PowerBox_C|GetbTripwiresOn _output_get)
    (CallFunction|EnableTripwire)
    (else
      (CallFunction|DisableTripwire))))

(fn ConstructionScript)

(fn ActivateAlarm
  (Development|PrintString "Tripwire has been tripped")
  (Class|Actor|MakeNoise 1.0 self (Transformation|GetActorLocation) 0.0 "Noise"))

(fn DisableTripwire
  (Variables|Default|SetactiveTripwire false)
  (Rendering|Components|Light|SetIntensity (Variables|Default|GetPointLight) 0.0)
  (Variables|/Script/Engine.PrimitiveComponent|SetbGenerateOverlapEvents (Variables|Default|GetCollision) false)
  (Rendering|SetVisibility (Variables|Default|GetTripwire) false false))

(fn EnableTripwire
  (Variables|Default|SetactiveTripwire true)
  (Rendering|Components|Light|SetIntensity (Variables|Default|GetPointLight) 1.5e+03)
  (Variables|/Script/Engine.PrimitiveComponent|SetbGenerateOverlapEvents (Variables|Default|GetCollision) true)
  (Rendering|SetVisibility (Variables|Default|GetTripwire) true false))