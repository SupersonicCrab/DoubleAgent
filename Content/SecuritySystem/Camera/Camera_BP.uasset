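; Security camera actor for the security system that can pan in steps and render its view through a scene capture component.
; RotateLeft and RotateRight move a rounded yaw target in fixed increments within limits set around the starting yaw, and Tick turns the actor toward it.
; EnableUpdate starts a self-rescheduling timer that captures the scene at the FPS rate while updating is enabled and power is on.
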(event EventBeginPlay
  (bind _returnvalue (Transformation|GetActorRotation))
  ;[1 1 1] Rotation setup
  (Variables|Rotate|SetRightRotateLimit (Math|Conversions|ToFloat(Integer) (Math|Float|Round (+ (.yaw _returnvalue) 9e+01))))
  (Variables|Rotate|SetLeftRotateLimit (Math|Conversions|ToFloat(Integer) (Math|Float|Round (+ (.yaw _returnvalue) -9e+01))))
  (Variables|Rotate|SetRotateTarget (Math|Conversions|ToFloat(Integer) (Math|Float|Round (.yaw _returnvalue)))))

(event EventTick
  (params (DeltaSeconds :type Float%20%28single-precision%29))
  (bind _returnvalue (Transformation|GetActorRotation))
  (bind _rotatetarget (Variables|Rotate|GetRotateTarget))
  (bind _returnvalue_2 (Math|Float|Round (.yaw _returnvalue)))
  (bind _returnvalue_3 (Math|Conversions|ToFloat(Integer) _returnvalue_2))
  ;[1 1 1] Rotation tick
  (if (!= _returnvalue_3 _rotatetarget) ; If current rotation is not the same as rotate target
    ;[1 1 1] Left rotation
    (if (> _returnvalue_3 _rotatetarget)
      (Transformation|AddActorLocalRotation (* (Math|Rotator|MakeRotator 0.0 0.0 (* (Variables|Rotate|GetRotationSpeed) -1.0)) DeltaSeconds) false false)
      (else
        ;[1 1 1] Right rotation
        (if (< _returnvalue_3 _rotatetarget)
          (Transformation|AddActorLocalRotation (* (Math|Rotator|MakeRotator 0.0 0.0 (* (Variables|Rotate|GetRotationSpeed) 1.0)) DeltaSeconds) false false))))))

(fn ConstructionScript)

(fn EnableUpdate
  (Variables|SceneCapture|SetUpdating true)
  (SceneCapture|Update))

(fn DisableUpdate
  (Variables|SceneCapture|SetUpdating false))

(fn Update
  (if (and (Variables|SceneCapture|GetUpdating) (Variables|Default|GetPowerOn))
    (Rendering|SceneCapture|CaptureScene (Variables|Default|GetSceneCaptureComponent2D) :!class /Script/Engine.SceneCaptureComponent2D)
    (Utilities|Time|SetTimerbyFunctionName 0 "Update" (/ 1.0 (Variables|SceneCapture|GetFPS)))))

(fn RotateLeft
  (if (>= (Math|Conversions|ToFloat(Integer) (Math|Float|Round (- (Variables|Rotate|GetRotateTarget) 3e+01))) (Variables|Rotate|GetLeftRotateLimit))
    (Variables|Rotate|SetRotateTarget (Math|Conversions|ToFloat(Integer) (Math|Float|Round (- (Variables|Rotate|GetRotateTarget) 3e+01))))))

(fn RotateRight
  (if (<= (Math|Conversions|ToFloat(Integer) (Math|Float|Round (+ (Variables|Rotate|GetRotateTarget) 3e+01))) (Variables|Rotate|GetRightRotateLimit))
    (Variables|Rotate|SetRotateTarget (Math|Conversions|ToFloat(Integer) (Math|Float|Round (+ (Variables|Rotate|GetRotateTarget) 3e+01))))))