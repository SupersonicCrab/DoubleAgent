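; Light probe editor utility that refreshes probes through a light controller and validates point lights for replacement by LightProbes.
; The construction script starts a looping update timer; updates, also attempted on Tick, require PauseOnPlay, which BeginPlay clears.
; Replacement skips inverse-squared or shadow-casting lights, checks a 256-probe cap and clears its list.
; The property-copy and destroy steps are disconnected, so no light is actually converted.
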(event Custom|Update%20Lights
  (bind _light_controller_reference (Variables|Default|GetLight%20Controller%20Reference))
  (if (Variables|Default|GetPause%20On%20Play)
    (if (Utilities|IsValid _light_controller_reference)
      (Default|UpdateLightProbes _light_controller_reference))))

(event EventBeginPlay
  (Variables|Default|SetPause%20On%20Play false))

(event EventTick
  (params (DeltaSeconds :type Float%20%28single-precision%29))
  (bind _light_controller_reference (Variables|Default|GetLight%20Controller%20Reference))
  (if (Variables|Default|GetPause%20On%20Play)
    (if (Utilities|IsValid _light_controller_reference)
      (Default|UpdateLightProbes _light_controller_reference))))

(fn ConstructionScript
  (Utilities|Time|SetTimerbyFunctionName self "Update Lights" (Variables|Default|GetLight%20Probes%20Update%20Time) true)
  (if (Variables|Default|GetReplace%20Point%20Lights)
    (Variables|Default|SetReplace%20Point%20Lights false)
    (bind _outactors (Actor|GetAllActorsOfClass "/Game/LightProbes/Blueprints/LightProbe.LightProbe_C"))
    (Math|Integer|CompareInt (Utilities|Array|Length _outactors) 256
      (:>
        (Development|PrintString "Already Too many Light Probes" :!label _label))
      (:==
        (goto _label))
      (:<
        (Variables|Default|SetNum%20Light%20Probes (Utilities|Array|Length _outactors))
        (for _array_element (Variables|Default|GetPoint%20Lights%20to%20Replace)
          (if (Variables|/Script/Engine.PointLightComponent|GetbUseInverseSquaredFalloff (Variables|/Script/Engine.PointLight|GetPointLightComponent _array_element))
            (Development|PrintString (Utilities|String|Append (Utilities|GetDisplayName _array_element) " Skipped, only supported on lights with \"Use Inverse Squared Falloff\" Disabled"))
            (elif (Variables|/Script/Engine.LightComponentBase|GetCastDynamicShadows (Variables|/Script/Engine.PointLight|GetPointLightComponent _array_element))
              (if (Variables|/Script/Engine.LightComponentBase|GetCastShadows (Variables|/Script/Engine.PointLight|GetPointLightComponent _array_element))
                (Development|PrintString (Utilities|String|Append (Utilities|GetDisplayName _array_element) " Skipped, only lights without \"Cast Dynamic Shadows\" enabled get replaced"))
                (else
                  (bind _output_get (Variables|Default|SetNum%20Light%20Probes (+ (Variables|Default|GetNum%20Light%20Probes) 1) :!label _label_2))
                  (Math|Integer|CompareInt _output_get 256
                    (:>
                      _)
                    (:==
                      _))
                  (Development|PrintString "Too Many Light Probes, Conversion Cancelled")))
              (else
                (goto _label_2)))))
        (Utilities|Array|Clear (Variables|Default|GetPoint%20Lights%20to%20Replace))))))