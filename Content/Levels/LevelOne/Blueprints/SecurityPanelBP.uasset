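; A level security keypad panel that lets the player open a password entry screen when standing near it.
; Its trigger box enables input and shows an "E to Enter Password" prompt through FirstPersonHUD, then disables input and clears the prompt on exit.
; Pressing E creates the Password_Screen widget with a reference back to the panel and switches to UI-only input with a visible cursor.
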(event OnComponentBeginOverlap(TriggerBox)
  (params (OverlappedComponent :type Primitive%20Component%20Object%20Reference) (OtherActor :type Actor%20Object%20Reference) (OtherComp :type Primitive%20Component%20Object%20Reference) (OtherBodyIndex :type Integer) (bFromSweep :type Boolean) (SweepResult :type Hit%20Result%20Structure%20%28by%20ref%29))
  (bind _returnvalue (Game|GetPlayerController 0))
  (Input|EnableInput _returnvalue)
  (Variables|Default|SetInsertCode "E to Enter Password")
  (bind _asfirst_person_hud (Utilities|Casting|CastToFirstPersonHUD (HUD|GetHUD _returnvalue)))
  (Default|DrawTexttoHUD _asfirst_person_hud true (Variables|Default|GetInsertCode)))

(event OnComponentEndOverlap(TriggerBox)
  (params (OverlappedComponent :type Primitive%20Component%20Object%20Reference) (OtherActor :type Actor%20Object%20Reference) (OtherComp :type Primitive%20Component%20Object%20Reference) (OtherBodyIndex :type Integer))
  (Input|DisableInput 0)
  (Variables|Default|SetInsertCode "")
  (bind _asfirst_person_hud (Utilities|Casting|CastToFirstPersonHUD (HUD|GetHUD (Game|GetPlayerController 0))))
  (Default|DrawTexttoHUD _asfirst_person_hud true (Variables|Default|GetInsertCode)))

(event Custom|UseKeypad
  (bind _returnvalue (Game|GetPlayerController 0))
  (bind _returnvalue_2 (UserInterface|CreateWidget "/Game/Levels/LevelOne/UI/Password_Screen.Password_Screen_C"))
  (Variables|/Game/Levels/LevelOne/UI/Password_Screen.Password_Screen_C|SetSecurityPanelBP _returnvalue_2 self)
  (UserInterface|Viewport|AddtoViewport _returnvalue_2 0)
  (Input|SetInputModeUIOnly _returnvalue _returnvalue_2 "DoNotLock")
  (Variables|/Script/Engine.PlayerController|SetbShowMouseCursor _returnvalue true))

(event Input|KeyboardEvents|E
  (params (Key :type Key%20Structure :default "None"))
  (:Pressed
    (CallFunction|UseKeypad)))

(fn ConstructionScript)