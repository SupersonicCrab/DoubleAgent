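; MapReset_ACTOR is a level exit trigger that restarts the level when the player carries the required item.
; On overlap by Player_CHARACTER, it asks the player's InventoryComponent whether it holds the WinConditionItem class.
; A match runs the RestartLevel console command; otherwise it prints a message naming the needed item, read from that class's default ItemStructure.
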(event OnComponentBeginOverlap(Collision)
  (params (OverlappedComponent :type Primitive%20Component%20Object%20Reference) (OtherActor :type Actor%20Object%20Reference) (OtherComp :type Primitive%20Component%20Object%20Reference) (OtherBodyIndex :type Integer) (bFromSweep :type Boolean) (SweepResult :type Hit%20Result%20Structure%20%28by%20ref%29))
  (bind _asplayer_character (Utilities|Casting|CastToPlayer_CHARACTER OtherActor))
  (bind _itemfound (Default|CheckItemClass (Variables|/Game/Player/Player_CHARACTER.Player_CHARACTER_C|GetInventoryComponent _asplayer_character) (Variables|Default|GetwinConditionItem)))
  (if _itemfound
    (Development|ExecuteConsoleCommand "RestartLevel" 0)
    (else
      (Development|PrintString (Utilities|String|Append "You need " (Utilities|String|ToString(Text) (.name (.ItemStructure (Utilities|GetClassDefaults (Variables|Default|GetwinConditionItem))))) " to leave")))))

(fn ConstructionScript)