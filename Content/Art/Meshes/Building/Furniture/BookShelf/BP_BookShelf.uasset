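; Bookshelf furniture Blueprint that randomizes its shelf meshes whenever the construction script runs.
; RefreshShelves assigns each child of the primary bookshelf a random mesh from a working copy of ShelfVariations, removing each pick to avoid repeats.
; The Double flag enables the secondary bookshelf's visibility and collision and fills its children from the remaining meshes; otherwise that component is hidden without collision, without propagating visibility to its children.
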(fn ConstructionScript
  (CallFunction|RefreshShelves))

(fn RefreshShelves
  (bind _secondarybookshelf (Variables|Default|GetSecondaryBookshelf))
  (LocalVariables|SetTempVariations (Variables|Default|GetShelfVariations))
  (for _array_element (Components|GetChildrenComponents (Variables|Default|GetPrimaryBookshelf) false)
    (Components|StaticMesh|SetStaticMesh (.AsStatic%20Mesh%20Component (Utilities|Casting|CastToStaticMeshComponent _array_element)) (Utilities|Array|Get(acopy) (LocalVariables|GetTempVariations) (Math|Random|RandomIntegerinRange 0 (- (Utilities|Array|Length (LocalVariables|GetTempVariations)) 1))))
    (Utilities|Array|RemoveItem (LocalVariables|GetTempVariations) (Variables|/Script/Engine.StaticMeshComponent|GetStaticMesh (.AsStatic%20Mesh%20Component (Utilities|Casting|CastToStaticMeshComponent _array_element)))))
  (if (Variables|Default|GetbDouble)
    (Collision|SetCollisionEnabled _secondarybookshelf "QueryAndPhysics")
    (Rendering|SetVisibility _secondarybookshelf true true)
    (for _array_element_2 (Components|GetChildrenComponents _secondarybookshelf false)
      (Components|StaticMesh|SetStaticMesh (.AsStatic%20Mesh%20Component (Utilities|Casting|CastToStaticMeshComponent _array_element_2)) (Utilities|Array|Get(acopy) (LocalVariables|GetTempVariations) (Math|Random|RandomIntegerinRange 0 (- (Utilities|Array|Length (LocalVariables|GetTempVariations)) 1))))
      (Utilities|Array|RemoveItem (LocalVariables|GetTempVariations) (Variables|/Script/Engine.StaticMeshComponent|GetStaticMesh (.AsStatic%20Mesh%20Component (Utilities|Casting|CastToStaticMeshComponent _array_element_2)))))
    (else
      (Collision|SetCollisionEnabled _secondarybookshelf "NoCollision")
      (Rendering|SetVisibility _secondarybookshelf false false))))