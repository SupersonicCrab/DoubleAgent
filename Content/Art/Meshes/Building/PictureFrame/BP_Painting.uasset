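; Decorative framed painting actor that randomly becomes either a landscape or a portrait picture.
; The construction script calls Refresh, which flips a random bool and hides the unused frame along with its child components.
; It then applies a random material from the matching orientation's array to the remaining painting.
; The pick is unseeded, so it can change whenever construction reruns.
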(event Custom|Refresh
  (bind _landscapepaintings (Variables|Default|GetLandscapePaintings))
  (bind _portraitpaintings (Variables|Default|GetPortraitPaintings))
  (if (Math|Random|RandomBool) ; If true, landscape paintings
    (Rendering|SetVisibility (Variables|Default|GetPortraitFrame) false true)
    (Rendering|Material|SetMaterial (Variables|Default|GetLandscapePainting) 0 (Utilities|Array|Get(acopy) _landscapepaintings (Math|Random|RandomIntegerinRange 0 (- (Utilities|Array|Length _landscapepaintings) 1))))
    (else
      (Rendering|SetVisibility (Variables|Default|GetLandscapeFrame) false true)
      (Rendering|Material|SetMaterial (Variables|Default|GetPortraitPainting) 0 (Utilities|Array|Get(acopy) _portraitpaintings (Math|Random|RandomIntegerinRange 0 (- (Utilities|Array|Length _portraitpaintings) 1)))))))

(event EventBeginPlay)

(event Collision|EventActorBeginOverlap
  (params (OtherActor :type Actor%20Object%20Reference)))

(event EventTick
  (params (DeltaSeconds :type Float%20%28single-precision%29)))

(fn ConstructionScript
  (CallFunction|Refresh))