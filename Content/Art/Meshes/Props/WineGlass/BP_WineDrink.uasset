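; BP_WineDrink is a wine glass prop with fake liquid that has configurable colour and fill level.
; The construction script creates a dynamic material, setting its colour and slice height and raising a Plane component to match the fill.
; While recently rendered with simulation enabled, Tick tilts the Plane through UpdateLiquid's velocity-driven facing, otherwise resetting its orientation.
; The Plane's up vector feeds the material's FakeNormalDirection every tick, faking the liquid surface.
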(event Custom|UpdateLiquidWithVelocity
  (bind _maxangle (Variables|Default|GetmaxAngle))
  (bind (_planerotator _lastvelocityout _ppfacingout _facing _stopelapsedtime _moveelapsedtime) (Class|LiquidActor|UpdateLiquid (Variables|Default|GetInitialize) (Variables|Default|GetVelocityFalloff) (Variables|Default|GetfacingScale) (Variables|Default|GetvelocitySpeed) (Variables|Default|GetminVelocity) (Variables|Default|GetPlane) (Utilities|Time|GetWorldDeltaSeconds)))
  (bind _output_get (Variables|Default|SetFacing (Math|Vector|ClampVectorSize _facing -1.0 1.0)))
  (Transformation|SetWorldRotation (Variables|Default|GetPlane) (Math|Rotator|MakeRotator (* (.x _output_get) _maxangle) (* (.y _output_get) _maxangle) 9e+01) false false)
  (Variables|Default|SetMoveTime _moveelapsedtime)
  (if (Variables|Default|GetInitialize)
    (Variables|Default|SetInitialize false)))

(event EventBeginPlay)

(event Collision|EventActorBeginOverlap
  (params (OtherActor :type Actor%20Object%20Reference)))

(event EventTick
  (params (DeltaSeconds :type Float%20%28single-precision%29))
  (bind _plane (Variables|Default|GetPlane))
  (bind _returnvalue (Transformation|GetWorldLocation _plane))
  (bind _returnvalue_2 (Math|Vector|GetUpVector _plane))
  (bind _returnvalue_3 (Math|Vector|Normalize _returnvalue_2))
  (bind (_x _y _z) (Math|Vector|BreakVector _returnvalue_3))
  (if (and (Class|Actor|WasRecentlyRendered 0.2) (Variables|Default|GetSimulateLiquidPhysics))
    (CallFunction|UpdateLiquidwithVelocity)
    (else
      (Transformation|SetWorldRotation _plane (Math|Rotator|FindLookatRotation _returnvalue (+ _returnvalue "10.000000, 0,0.000000")) false false)))
  (Rendering|Material|SetVectorParameterValue (Variables|Default|GetLiquidMaterial) "FakeNormalDirection" (Math|Conversions|ToLinearColor(Vector) (Math|Vector|MakeVector _x _y (Math|Float|Absolute(Float) _z))) :!class /Script/Engine.MaterialInstanceDynamic))

(fn ConstructionScript
  (bind _returnvalue (Rendering|Material|CreateDynamicMaterialInstance (Variables|Default|GetSM_WineGlassLiquid) 0 (Rendering|Material|GetMaterial (Variables|Default|GetSM_WineGlassLiquid) 0) "None" :!class /Script/Engine.PrimitiveComponent))
  (Variables|Default|SetLiquidMaterial _returnvalue)
  (Rendering|Material|SetVectorParameterValue (Variables|Default|GetLiquidMaterial) "Liquid Color" (Variables|Default|GetLiquidColor) :!class /Script/Engine.MaterialInstanceDynamic)
  (Transformation|SetRelativeLocation (Variables|Default|GetPlane) (Math|Vector|MakeVector 0.0 0.0 (Math|Float|Lerp 0.0 9.0 (Variables|Default|GetFilledAmount))) false false)
  (Rendering|Material|SetScalarParameterValue (Variables|Default|GetLiquidMaterial) "SliceHeight" (Variables|Default|GetFilledAmount) :!class /Script/Engine.MaterialInstanceDynamic))

(fn Slowmotion
  (Utilities|Time|SetGlobalTimeDilation 0.1))

(fn SimLiquidwithVelocity
  (params (DeltaTime :type Float%20%28single-precision%29)))