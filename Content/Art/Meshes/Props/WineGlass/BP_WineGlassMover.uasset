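; Wine glass prop actor that shuttles back and forth in the horizontal plane between its spawn location and an X/Y offset from it.
; While MOVE is on, Tick lerps from the current location toward the active endpoint using a growing time alpha, so motion accelerates rather than staying linear.
; Coming within the ReverseSpeed tolerance of either endpoint flips GoToEnd and resets the timer, which accumulates even while MOVE is off.
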(event EventBeginPlay
  (bind _output_get (Variables|Default|SetStartLoc (Transformation|GetActorLocation)))
  (Variables|Default|SetEndLoc (+ _output_get (Math|Vector|MakeVector (Variables|Default|GetRangeX) (Variables|Default|GetRangeY) 0.0))))

(event Collision|EventActorBeginOverlap
  (params (OtherActor :type Actor%20Object%20Reference)))

(event EventTick
  (params (DeltaSeconds :type Float%20%28single-precision%29))
  (bind _returnvalue (Transformation|GetActorLocation))
  (bind _reversespeed (Variables|Default|GetReverseSpeed))
  (Variables|Default|SetTime (+ (* DeltaSeconds (Variables|Default|GetInterp%20Speed)) (Variables|Default|GetTime)))
  (if (Variables|Default|GetMOVE)
    (Transformation|SetActorLocation (Math|Vector|Lerp(Vector) (Transformation|GetActorLocation) (Math|Vector|SelectVector (Variables|Default|GetEndLoc) (Variables|Default|GetStartLoc) (Variables|Default|GetGoToEnd)) (Variables|Default|GetTime)) false false)
    (if (Math|Vector|Equal(Vector) _returnvalue (Variables|Default|GetEndLoc) _reversespeed)
      (Variables|Default|SetGoToEnd false)
      (Variables|Default|SetTime 0.0)
      (elif (Math|Vector|Equal(Vector) _returnvalue (Variables|Default|GetStartLoc) _reversespeed)
        (Variables|Default|SetGoToEnd true)
        (Variables|Default|SetTime 0.0)))))

(fn ConstructionScript)