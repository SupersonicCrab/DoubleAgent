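; BP_WineBottle is a wine bottle prop that shows a randomly chosen label material.
; One second after BeginPlay, the server picks a rare Crab material at 1% odds, otherwise one of three regular variants at random.
; A multicast event applies the chosen material to the mesh's first slot so connected clients show the same bottle.
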(event Custom|RefreshServer
  (if (Math|Random|RandomBoolwithWeight 0.01)
    (CallFunction|MulticastRefresh "/Game/Art/Meshes/Props/WineBottle/Materials/MI_WineBottle_Crab.MI_WineBottle_Crab")
    (else
      (switch int (Math|Random|RandomIntegerinRange 0 2)
        (:0
          (CallFunction|MulticastRefresh "/Game/Art/Meshes/Props/WineBottle/Materials/MI_WineBottle_Cockade.MI_WineBottle_Cockade"))
        (:1
          (CallFunction|MulticastRefresh "/Game/Art/Meshes/Props/WineBottle/Materials/MI_WineBottle_NeonGrape.MI_WineBottle_NeonGrape"))
        (:2
          (CallFunction|MulticastRefresh "/Game/Art/Meshes/Props/WineBottle/Materials/MI_WineBottle_SilkVine.MI_WineBottle_SilkVine"))))))

(event Custom|MulticastRefresh
  (params (Material :type Material%20Instance%20Object%20Reference))
  (Rendering|Material|SetMaterial (Variables|Default|GetMesh) 0 Material))

(event EventBeginPlay
  (if (Networking|IsServer)
    (Utilities|FlowControl|Delay 1.0)
    (CallFunction|RefreshServer)))

(fn ConstructionScript)