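; Actor that shows a randomly chosen static mesh from its Variants array, giving placed models visual variety.
; The construction script calls RefreshStart, which rolls a random index through ServerRefresh and passes it to MulticastRefresh to set the mesh.
; The server-to-multicast naming suggests one shared pick for all clients, and the separate Refresh function is an empty stub.
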(event Custom|ServerRefresh
  (CallFunction|MulticastRefresh (Math|Random|RandomIntegerinRange 0 (- (Utilities|Array|Length (Variables|Default|GetVariants)) 1))))

(event Custom|MulticastRefresh
  (params (Index :type Integer))
  (Components|StaticMesh|SetStaticMesh (Variables|Default|GetStaticMesh) (Utilities|Array|Get(acopy) (Variables|Default|GetVariants) Index)))

(event Custom|RefreshStart
  (CallFunction|ServerRefresh))

(event EventBeginPlay)

(event Collision|EventActorBeginOverlap
  (params (OtherActor :type Actor%20Object%20Reference)))

(event EventTick
  (params (DeltaSeconds :type Float%20%28single-precision%29)))

(fn ConstructionScript
  (CallFunction|RefreshStart))

(fn Refresh
  (params (Index :type Integer)))