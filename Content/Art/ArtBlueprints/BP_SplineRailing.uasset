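; Procedural railing actor that builds rails, posts and end caps along an editable spline in the construction script.
; Each spline segment gets a spline mesh rail raised by RailingHeight.
; AddPosts spaces PostFrequency intervals evenly by distance, placing yaw-only, height-scaled HISM instances from PostMeshes, with an accent mesh swapped in periodically via AccentPost.
; AddCaps instances a cap at both spline ends, turning the last one 180 degrees.
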(event EventBeginPlay)

(event Collision|EventActorBeginOverlap
  (params (OtherActor :type Actor%20Object%20Reference)))

(event EventTick
  (params (DeltaSeconds :type Float%20%28single-precision%29)))

(fn ConstructionScript
  (bind _spline (Variables|Default|GetSpline))
  (bind _railingheight (Variables|Default|GetRailingHeight))
  (Utilities|Array|Clear (Variables|Default|GetSplineMeshComponents))
  (Utilities|Array|Clear (Variables|Default|GetHISMs))
  (for _index (range 0 (- (Spline|GetNumberOfSplinePoints (Variables|Default|GetSpline)) 2))
    (bind _returnvalue (AddComponent|AddSplineMeshComponent false))
    (Utilities|Array|Add (Variables|Default|GetSplineMeshComponents) _returnvalue)
    (SplineMesh|SetStartandEnd _returnvalue (Math|Vector|MakeVector (.x (Spline|GetLocationatSplinePoint _spline _index "Local")) (.y (Spline|GetLocationatSplinePoint _spline _index "Local")) (+ (.z (Spline|GetLocationatSplinePoint _spline _index "Local")) _railingheight)) (Spline|GetTangentatSplinePoint _spline _index "Local") (Math|Vector|MakeVector (.x (Spline|GetLocationatSplinePoint _spline (+ _index 1) "Local")) (.y (Spline|GetLocationatSplinePoint _spline (+ _index 1) "Local")) (+ _railingheight (.z (Spline|GetLocationatSplinePoint _spline (+ _index 1) "Local")))) (Spline|GetArriveTangentatSplinePoint _spline (+ _index 1) "Local") true :!class /Script/Engine.SplineMeshComponent))
  (CallFunction|AddPosts)
  (CallFunction|AddCaps))

(fn AddPosts
  (for _array_element (Variables|Default|GetPostMeshes)
    (bind _returnvalue (AddComponent|AddHierarchicalInstancedStaticMeshComponent false))
    (Utilities|Array|Add (Variables|Default|GetHISMs) _returnvalue)
    (Components|StaticMesh|SetStaticMesh _returnvalue _array_element))
  (for _index (range 0 (Variables|Default|GetPostFrequency))
    (Components|InstancedStaticMesh|AddInstance (Utilities|Array|Get(acopy) (Variables|Default|GetHISMs) (Math|Integer|SelectInt 1 0 (== (LocalVariables|GetPostIteration) (Variables|Default|GetAccentPost)))) (Math|Transform|MakeTransform (Math|Vector|MakeVector (.x (.Location (Math|Transform|BreakTransform (Spline|GetTransformatDistanceAlongSpline (Variables|Default|GetSpline) (* _index (/ (Spline|GetSplineLength (Variables|Default|GetSpline)) (Math|Conversions|ToFloat(Integer) (Variables|Default|GetPostFrequency)))) "Local" false)))) (.y (.Location (Math|Transform|BreakTransform (Spline|GetTransformatDistanceAlongSpline (Variables|Default|GetSpline) (* _index (/ (Spline|GetSplineLength (Variables|Default|GetSpline)) (Math|Conversions|ToFloat(Integer) (Variables|Default|GetPostFrequency)))) "Local" false)))) (+ (.z (.Location (Math|Transform|BreakTransform (Spline|GetTransformatDistanceAlongSpline (Variables|Default|GetSpline) (* _index (/ (Spline|GetSplineLength (Variables|Default|GetSpline)) (Math|Conversions|ToFloat(Integer) (Variables|Default|GetPostFrequency)))) "Local" false)))) (Variables|Default|GetRailingHeight))) (Math|Rotator|MakeRotator 0.0 0.0 (.yaw (.Rotation (Math|Transform|BreakTransform (Spline|GetTransformatDistanceAlongSpline (Variables|Default|GetSpline) (* _index (/ (Spline|GetSplineLength (Variables|Default|GetSpline)) (Math|Conversions|ToFloat(Integer) (Variables|Default|GetPostFrequency)))) "Local" false))))) (Math|Vector|MakeVector (.x (.Scale (Math|Transform|BreakTransform (Spline|GetTransformatDistanceAlongSpline (Variables|Default|GetSpline) (* _index (/ (Spline|GetSplineLength (Variables|Default|GetSpline)) (Math|Conversions|ToFloat(Integer) (Variables|Default|GetPostFrequency)))) "Local" false)))) (.y (.Scale (Math|Transform|BreakTransform (Spline|GetTransformatDistanceAlongSpline (Variables|Default|GetSpline) (* _index (/ (Spline|GetSplineLength (Variables|Default|GetSpline)) (Math|Conversions|ToFloat(Integer) (Variables|Default|GetPostFrequency)))) "Local" false)))) (/ (Variables|Default|GetRailingHeight) 1e+02))))
    (if (== (LocalVariables|GetPostIteration) (Variables|Default|GetAccentPost))
      (LocalVariables|SetPostIteration 0)
      (else
        (Math|Integer|IncrementInt (LocalVariables|GetPostIteration))))))

(fn AddCaps
  (bind _spline (Variables|Default|GetSpline))
  (bind _spline_2 (Variables|Default|GetSpline))
  (bind _spline_3 (Variables|Default|GetSpline))
  (bind _returnvalue (Spline|GetTransformatSplinePoint _spline_2 0 "Local" false))
  (bind _returnvalue_2 (Spline|GetNumberOfSplinePoints _spline_3))
  (bind (_location _rotation _scale) (Math|Transform|BreakTransform _returnvalue))
  (bind _returnvalue_3 (- _returnvalue_2 1))
  (bind _returnvalue_4 (Spline|GetTransformatSplinePoint _spline _returnvalue_3 "Local" false))
  (bind (_location_2 _rotation_2 _scale_2) (Math|Transform|BreakTransform _returnvalue_4))
  (bind _returnvalue_5 (AddComponent|AddHierarchicalInstancedStaticMeshComponent false))
  (Components|InstancedStaticMesh|AddInstance _returnvalue_5 (Math|Transform|MakeTransform (Math|Vector|MakeVector (.x _location) (.y _location) (+ (.z _location) (Variables|Default|GetRailingHeight))) _rotation _scale))
  (Components|InstancedStaticMesh|AddInstance _returnvalue_5 (Math|Transform|MakeTransform (Math|Vector|MakeVector (.x _location_2) (.y _location_2) (+ (.z _location_2) (Variables|Default|GetRailingHeight))) (Math|Rotator|MakeRotator (.roll _rotation_2) (.pitch _rotation_2) (+ (.yaw _rotation_2) 1.8e+02)) _scale_2)))